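; Player component that manages a global slow-motion effect whose duration can be extended through SlowTimeAddDuration.
; Adding time clamps the remaining total, scales all of it by SlowTimeAmount for additions above a small threshold, then applies that global time dilation.
; A millisecond-interval looping timer counts the duration down and restores normal speed at zero.
; An unconnected lerp-based dilation fragment never runs.
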(event Custom|Slow%20Time%20Add%20Duration
  (params (Duration%20To%20Add :type Float%20%28double-precision%29))
  (bind _output_get (Variables|Default|SetCurrent%20Slow%20Time%20Duration (Math|Float|Clamp(Float) (+ (Variables|Default|GetCurrent%20Slow%20Time%20Duration) Duration%20To%20Add) 0.0 3.0)))
  (if (> Duration%20To%20Add 0.01)
    (Variables|Default|SetCurrent%20Slow%20Time%20Duration (* _output_get (Variables|Default|GetSlow%20Time%20Amount))))
  (CallFunction|SlowTimeStart))

(event Custom|Slow%20Time%20Start
  (if (not (Utilities|Time|IsValidTimerHandle (Variables|Default|GetSlow%20Time%20Counter%20Timer%20Handle)))
    (bind _returnvalue (Utilities|Time|SetTimerbyEvent (delegate Custom|Slow%20Time%20Counter) 0.001 true))
    (Variables|Default|SetSlow%20Time%20Counter%20Timer%20Handle _returnvalue)
    (Utilities|Time|SetGlobalTimeDilation (Variables|Default|GetSlow%20Time%20Amount))))

(event Custom|Slow%20Time%20Counter
  (bind _output_get (Variables|Default|SetCurrent%20Slow%20Time%20Duration (Math|Float|Clamp(Float) (- (Variables|Default|GetCurrent%20Slow%20Time%20Duration) 0.001) 0.0 3.0)))
  (if (== _output_get 0.0)
    (CallFunction|StopSlowTime)))

(event Custom|Stop%20Slow%20Time
  (Utilities|Time|ClearandInvalidateTimerbyHandle (Variables|Default|GetSlow%20Time%20Counter%20Timer%20Handle))
  (Utilities|Time|SetGlobalTimeDilation 1.0))