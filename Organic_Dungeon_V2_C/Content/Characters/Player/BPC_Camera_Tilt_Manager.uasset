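; Player character component that rolls the camera through control rotation for strafing, sliding and wall-running.
; After a short BeginPlay delay it caches camera and controller, then Tick interpolates roll from local sideways velocity, clamped to a small angle.
; Tick tilt pauses during slides or wall runs (read from BPC_Slide and BPC_WallRunning) and near vertical pitch.
; Separate events each apply one interpolation step for slide in/out and left/right wall-run tilt.
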(event Custom|Into%20Sliding%20Camera%20Tilt
  (bind _owner_s_controller (Variables|Default|GetOwner's%20Controller))
  (bind _sliding_camera_tilt_amount (Variables|Default|GetSliding%20Camera%20Tilt%20Amount))
  (bind _returnvalue (Pawn|GetControlRotation _owner_s_controller :!class /Script/Engine.Controller))
  (Pawn|SetControlRotation _owner_s_controller (Math|Rotator|MakeRotator (Math|Float|Clamp(Float) (Math|Interpolation|FInterpTo (.roll (Transformation|GetWorldRotation (Variables|Default|GetOwner's%20Camera))) _sliding_camera_tilt_amount (Utilities|Time|GetWorldDeltaSeconds) 5.0) (* _sliding_camera_tilt_amount -1.0) (Variables|Default|GetSliding%20Camera%20Tilt%20Amount)) (.pitch _returnvalue) (.yaw _returnvalue))))

(event Custom|Out%20Sliding%20Camera%20Tilt
  (bind _owner_s_controller (Variables|Default|GetOwner's%20Controller))
  (bind _returnvalue (Pawn|GetControlRotation _owner_s_controller :!class /Script/Engine.Controller))
  (Pawn|SetControlRotation _owner_s_controller (Math|Rotator|MakeRotator (Math|Interpolation|FInterpTo (.roll (Transformation|GetWorldRotation (Variables|Default|GetOwner's%20Camera))) 0.0 (Utilities|Time|GetWorldDeltaSeconds) 5.0) (.pitch _returnvalue) (.yaw _returnvalue))))

(event Custom|Wallrunning%20Right%20Camera%20Tilt
  (bind _owner_s_controller (Variables|Default|GetOwner's%20Controller))
  (bind _returnvalue (Pawn|GetControlRotation _owner_s_controller :!class /Script/Engine.Controller))
  (Pawn|SetControlRotation (Variables|Default|GetOwner's%20Controller) (Math|Rotator|MakeRotator (Math|Interpolation|FInterpTo (.roll (Transformation|GetWorldRotation (Variables|Default|GetOwner's%20Camera))) (* (Variables|Default|GetWallrunning%20Camera%20Tilt%20Amount) -1.0) (Utilities|Time|GetWorldDeltaSeconds) 5.0) (.pitch _returnvalue) (.yaw _returnvalue))))

(event Custom|Wallrunning%20Left%20Camera%20Tilt
  (bind _owner_s_controller (Variables|Default|GetOwner's%20Controller))
  (bind _returnvalue (Pawn|GetControlRotation _owner_s_controller :!class /Script/Engine.Controller))
  (Pawn|SetControlRotation (Variables|Default|GetOwner's%20Controller) (Math|Rotator|MakeRotator (Math|Interpolation|FInterpTo (.roll (Transformation|GetWorldRotation (Variables|Default|GetOwner's%20Camera))) (Variables|Default|GetWallrunning%20Camera%20Tilt%20Amount) (Utilities|Time|GetWorldDeltaSeconds) 5.0) (.pitch _returnvalue) (.yaw _returnvalue))))

(event EventBeginPlay
  (Utilities|FlowControl|Delay 0.2)
  (Variables|Default|SetOwner's%20Camera (Actor|GetComponentbyClass (Components|GetOwner) "/Script/Engine.CameraComponent"))
  (bind _ascharacter (Utilities|Casting|CastToCharacter (Components|GetOwner)))
  (Variables|Default|SetOwner's%20Controller (Pawn|GetController _ascharacter))
  (Components|Tick|SetComponentTickEnabled true))

(event EventTick
  (params (DeltaSeconds :type Float%20%28single-precision%29))
  (bind _returnvalue (Components|GetOwner))
  (bind _returnvalue_2 (Utilities|Time|GetWorldDeltaSeconds))
  (bind _returnvalue_3 (Components|GetOwner))
  (bind _owner_s_camera (Variables|Default|GetOwner's%20Camera))
  (bind _owner_s_controller (Variables|Default|GetOwner's%20Controller))
  (bind _owner_s_controller_2 (Variables|Default|GetOwner's%20Controller))
  (bind _returnvalue_4 (Transformation|GetVelocity _returnvalue))
  (bind _returnvalue_5 (Transformation|GetActorRotation _returnvalue))
  (bind _returnvalue_6 (Pawn|GetControlRotation _owner_s_controller :!class /Script/Engine.Controller))
  (bind _returnvalue_7 (Pawn|GetControlRotation _owner_s_controller_2 :!class /Script/Engine.Controller))
  (bind _returnvalue_8 (Actor|GetComponentbyClass _returnvalue_3 "/Game/Movement/Sliding/BPC_Slide.BPC_Slide_C"))
  (bind _returnvalue_9 (Transformation|GetWorldRotation _owner_s_camera))
  (bind _returnvalue_10 (Math|Vector|UnrotateVector _returnvalue_4 _returnvalue_5))
  (bind _returnvalue_11 (/ (.y _returnvalue_10) 1e+03))
  (bind _returnvalue_12 (* _returnvalue_11 4.0))
  (bind _returnvalue_13 (Math|Interpolation|FInterpTo (.roll _returnvalue_9) _returnvalue_12 _returnvalue_2 5.0))
  (if (Math|Boolean|ANDBoolean (not (Math|Boolean|ORBoolean (Variables|/Game/Movement/Sliding/BPC_Slide.BPC_Slide_C|GetSliding _returnvalue_8) (Variables|/Game/Movement/Sliding/BPC_Slide.BPC_Slide_C|GetStarting_Sliding _returnvalue_8) (Variables|/Game/Movement/Sliding/BPC_Slide.BPC_Slide_C|GetStopping_Sliding _returnvalue_8) (Variables|/Game/Movement/Wall-Running/BPC_Wall-Running.BPC_Wall-Running_C|GetWall-Running (Actor|GetComponentbyClass _returnvalue_3 "/Game/Movement/Wall-Running/BPC_Wall-Running.BPC_Wall-Running_C")))) (not (Math|Float|NearlyEqual(Float) (.roll _returnvalue_9) _returnvalue_13 0.002)) (not (or (and (>= (.pitch _returnvalue_6) 85.0) (<= (.pitch _returnvalue_6) 255.0)) (and (<= (.pitch _returnvalue_6) 275.0) (>= (.pitch _returnvalue_6) 255.0)))))
    (Pawn|SetControlRotation _owner_s_controller_2 (Math|Rotator|MakeRotator (Math|Float|Clamp(Float) _returnvalue_13 -4.0 4.0) (.pitch _returnvalue_7) (.yaw _returnvalue_7)))))