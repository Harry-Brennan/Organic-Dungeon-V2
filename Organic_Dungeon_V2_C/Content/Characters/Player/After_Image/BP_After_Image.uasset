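; BP_After_Image is a player after-image effect that shows a fading, tinted snapshot of a skeletal mesh's pose.
; On Activate, after a delay, it shows its poseable mesh and copies the pose from the source skeletal component.
; It applies a dynamic after-image material with the set colour to two material slots.
; A timeline scaled by fade time drives the fade amount, then hides the mesh via Deactivate for possible reuse.
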(event Custom|Activate
  (bind _after_image_mesh (Variables|Default|GetAfter%20Image%20Mesh))
  (Utilities|FlowControl|Delay (Variables|Default|GetAfter%20Image%20Delay))
  (Rendering|SetVisibility (Variables|Default|GetAfter%20Image%20Mesh) true false)
  (bind _after_image_skeletal_mesh (Variables|Default|GetAfter%20Image%20Skeletal%20Mesh)
    (:then
      (Class|PoseableMeshComponent|CopyPosefromSkeletalComponent (Variables|Default|GetAfter%20Image%20Mesh) _after_image_skeletal_mesh)
      (bind _returnvalue (Rendering|Material|CreateDynamicMaterialInstance (Variables|Default|GetAfter%20Image%20Mesh) 0 "/Game/Assets/Materials/After_Image/M_After_Image.M_After_Image" "None" :!class /Script/Engine.PrimitiveComponent))
      (bind _output_get (Variables|Default|SetAfter%20Image%20Mat _returnvalue))
      (Rendering|Material|SetMaterial _after_image_mesh 0 _output_get)
      (Rendering|Material|SetMaterial _after_image_mesh 1 _output_get)
      (Rendering|Material|SetVectorParameterValue (Variables|Default|GetAfter%20Image%20Mat) "After Image Colour" (Variables|Default|GetAfter%20Image%20Colour) :!class /Script/Engine.MaterialInstanceDynamic)
      (Components|Timeline|SetPlayRate (Variables|Default|GetFade%20Timeline) (/ 1.0 (Variables|Default|GetFade%20Time)))
      (bind _alpha (Timeline|Fade%20Timeline PlayFromStart)
        (:Update
          (Rendering|Material|SetScalarParameterValue (Variables|Default|GetAfter%20Image%20Mat) "Fade Amount" _alpha :!class /Script/Engine.MaterialInstanceDynamic))
        (:Finished
          (CallFunction|Deactivate))))
    (:else)))

(event Custom|Deactivate
  (Rendering|SetVisibility (Variables|Default|GetAfter%20Image%20Mesh) false false))

(fn ConstructionScript)