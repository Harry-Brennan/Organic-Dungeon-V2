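; Player component that leaves after-image trails of the owner's skeletal mesh whenever global time dilation differs from 1.
; BeginPlay pre-spawns a pool of BP_After_Image actors, caches the owner's mesh after a short delay, then enables Tick.
; Tick starts or clears a looping timer based on time dilation.
; Each timer firing reuses the next pooled actor round-robin, passing it the mesh, fade, delay and colour, matching its transform and activating it.
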(event Custom|Activate%20After%20Image
  (if (not (Utilities|Time|IsValidTimerHandle (Variables|Timer|GetAfter%20Image%20Loop%20Timer)))
    (bind _returnvalue (Utilities|Time|SetTimerbyEvent (delegate Custom|After%20Image%20Loop) (Variables|AfterImageDetails|GetAfter%20Image%20Frequency) true))
    (Variables|Timer|SetAfter%20Image%20Loop%20Timer _returnvalue)
    (Variables|Check|SetAfter%20Image%20Active true)))

(event Custom|Deactivate%20After%20Image
  (Utilities|Time|ClearandInvalidateTimerbyHandle (Variables|Timer|GetAfter%20Image%20Loop%20Timer))
  (Variables|Check|SetAfter%20Image%20Active false))

(event Custom|After%20Image%20Loop
  (bind _owner_skeletal_mesh (Variables|Default|GetOwner%20Skeletal%20Mesh))
  (Variables|ObjectPool|SetCurrent%20After%20Image (Utilities|Array|Get(acopy) (Variables|ObjectPool|GetAfter%20Image%20Pool) (Variables|ObjectPool|GetCurrent%20Pool%20Index)))
  (Variables|/Game/Characters/Player/After_Image/BP_After_Image.BP_After_Image_C|SetAfter%20Image%20Skeletal%20Mesh (Variables|ObjectPool|GetCurrent%20After%20Image) (Variables|Default|GetOwner%20Skeletal%20Mesh))
  (Variables|/Game/Characters/Player/After_Image/BP_After_Image.BP_After_Image_C|SetFade%20Time (Variables|ObjectPool|GetCurrent%20After%20Image) (Variables|AfterImageDetails|GetAfter%20Image%20Fade%20Time))
  (Variables|/Game/Characters/Player/After_Image/BP_After_Image.BP_After_Image_C|SetAfter%20Image%20Delay (Variables|ObjectPool|GetCurrent%20After%20Image) (Variables|AfterImageDetails|GetAfter%20Image%20Delay))
  (Variables|/Game/Characters/Player/After_Image/BP_After_Image.BP_After_Image_C|SetAfter%20Image%20Colour (Variables|ObjectPool|GetCurrent%20After%20Image) (Variables|AfterImageDetails|GetAfter%20Image%20Colour))
  (Transformation|SetActorLocationAndRotation (Variables|ObjectPool|GetCurrent%20After%20Image) (Transformation|GetWorldLocation _owner_skeletal_mesh) (Transformation|GetWorldRotation _owner_skeletal_mesh))
  (Default|Activate (Variables|ObjectPool|GetCurrent%20After%20Image))
  (bind _result (Math|Integer|IncrementInt (Variables|ObjectPool|GetCurrent%20Pool%20Index))
    (:%20%20
      (if (>= _result (Variables|ObjectPool|GetAfter%20Image%20Pool%20Max))
        (Variables|ObjectPool|SetCurrent%20Pool%20Index 0))
      (Development|PrintString (Utilities|String|ToString(Integer) (Variables|ObjectPool|GetCurrent%20Pool%20Index))))))

(event EventTick
  (params (DeltaSeconds :type Float%20%28single-precision%29))
  (if (!= (Class|GameplayStatics|GetGlobalTimeDilation) 1.0)
    (CallFunction|ActivateAfterImage)
    (else
      (CallFunction|DeactivateAfterImage))))

(event EventBeginPlay
  (Utilities|Array|Clear (Variables|ObjectPool|GetAfter%20Image%20Pool))
  (Variables|ObjectPool|SetCurrent%20Pool%20Index 0)
  (for _index (range 1 (Variables|ObjectPool|GetAfter%20Image%20Pool%20Max))
    (bind _returnvalue (Game|SpawnActorfromClass "/Game/Characters/Player/After_Image/BP_After_Image.BP_After_Image_C" (Math|Transform|MakeTransform "0, 0, 0" "0, 0, 0" "1.000000,1.000000,1.000000") "Undefined" "MultiplyWithRoot" 0 0 0.0 0.0 "(R=0.000000,G=0.000000,B=0.000000,A=0.000000)" 0))
    (Utilities|Array|Add (Variables|ObjectPool|GetAfter%20Image%20Pool) _returnvalue))
  (Utilities|FlowControl|Delay 0.2)
  (Variables|Default|SetOwner%20Skeletal%20Mesh (Actor|GetComponentbyClass (Components|GetOwner) "/Script/Engine.SkeletalMeshComponent"))
  (Components|Tick|SetComponentTickEnabled true))