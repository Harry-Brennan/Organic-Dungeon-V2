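; Player component for a blood grapple that pulls the player or the target, or swings from surfaces.
; Input sets Grappled; the Grapple event box-traces from the camera and attaches blade actors in hand and at the hit (nearest bone on skeletal meshes).
; GrapplePull branches on collision type to launch either side; enemies are always pulled, as the size check is stubbed.
; Holding swing on world surfaces applies force toward the hit each Tick.
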(event Custom|Stop%20Swing
  (bind _current_blood_grapple (Variables|Grapple|GetCurrent%20Blood%20Grapple))
  (bind _grapple_in_hand (Variables|Grapple|GetGrapple%20In%20Hand))
  (Development|PrintString "Stop Swinging")
  (Variables|Checks|SetSwinging false)
  (Utilities|Time|ClearandInvalidateTimerbyHandle (Variables|Grapple|GetGrapple%20Cooldown%20Timer))
  (Variables|Checks|SetGrapple%20Cooldown false)
  (Variables|/Script/Engine.CharacterMovementComponent|SetGravityScale (Actor|GetComponentbyClass (Components|GetOwner) "/Script/Engine.CharacterMovementComponent") 1.75)
  (Utilities|IsValid _current_blood_grapple
    (:Is%20Valid
      (Actor|SetLifeSpan _current_blood_grapple 4.0))
    (:Is%20Not%20Valid
      _))
  (Utilities|IsValid _grapple_in_hand
    (:Is%20Valid
      (Actor|DestroyActor _grapple_in_hand))
    (:Is%20Not%20Valid
      _))
  (Default|UnhideAllWeaponsWhilstGrappling (Actor|GetComponentbyClass (Components|GetOwner) "/Game/Weapons/Actor_Components/BPC_Weaponry.BPC_Weaponry_C")))

(event Custom|Start%20Swing
  (if (Variables|Checks|GetCan%20Swing)
    (Development|PrintString "Start Swinging")
    (Variables|Checks|SetSwinging true)
    (Utilities|Time|ClearandInvalidateTimerbyHandle (Variables|Grapple|GetGrapple%20Cooldown%20Timer))
    (Variables|Checks|SetGrapple%20Cooldown false)))

(event Custom|Grapple
  (bind _returnvalue (Components|GetOwner))
  (bind _returnvalue_2 (Components|GetOwner))
  (bind _returnvalue_3 (Game|GetPlayerCameraManager 0))
  (bind _returnvalue_4 (Camera|GetCameraLocation _returnvalue_3))
  (Variables|Checks|SetGrappled false)
  (Development|PrintString "Grapple")
  (CallFunction|SetupGrappleinHand)
  (Variables|Checks|SetGrapple%20Cooldown true)
  (bind _returnvalue_5 (Utilities|Time|SetTimerbyFunctionName 0 "Grapple Cooldown Func" (Variables|Grapple|GetGrapple%20Cooldown%20Duration)))
  (Variables|Grapple|SetGrapple%20Cooldown%20Timer _returnvalue_5)
  (bind (_outhit _returnvalue_6) (Class|KismetSystemLibrary|BoxTraceSingleforObjects _returnvalue_4 (+ _returnvalue_4 (* (Math|Vector|GetForwardVector (Pawn|GetControlRotation (Game|GetPlayerController 0) :!class /Script/Engine.Controller)) 2.5e+03)) "0.000000,10.000000,10.000000" (Pawn|GetControlRotation (Game|GetPlayerController 0) :!class /Script/Engine.Controller) (Utilities|Array|MakeArray "ObjectTypeQuery10" "ObjectTypeQuery9" "ObjectTypeQuery12" "ObjectTypeQuery14" "ObjectTypeQuery1" "ObjectTypeQuery2" "ObjectTypeQuery4" "ObjectTypeQuery7") false (Utilities|Array|MakeArray _returnvalue_2 (Variables|/Game/Weapons/Actor_Components/BPC_Weaponry.BPC_Weaponry_C|GetEquipped_Weapon (Actor|GetComponentbyClass _returnvalue_2 "/Game/Weapons/Actor_Components/BPC_Weaponry.BPC_Weaponry_C"))) "None" true))
  (if _returnvalue_6
    (Variables|Checks|SetGrapple%20Pull? true)
    (bind _output_get (Variables|Grapple|SetGrappled%20Actor (.HitActor (Collision|BreakHitResult _outhit))))
    (Variables|Grapple|SetGrappled%20Component (.HitComponent (Collision|BreakHitResult _outhit)))
    (Variables|Grapple|SetHit%20Location (.Location (Collision|BreakHitResult _outhit)))
    (Utilities|IsValid (Actor|GetComponentbyClass _output_get "/Script/Engine.SkeletalMeshComponent")
      (:Is%20Valid
        (bind _returnvalue_7 (Game|SpawnActorfromClass "/Game/Characters/Player/Grappling/BP_Blood_Grapple_Blade.BP_Blood_Grapple_Blade_C" (Math|Transform|MakeTransform (.BoneLocation (Class|SkinnedMeshComponent|FindClosestBoneK2 (Actor|GetComponentbyClass _output_get "/Script/Engine.SkeletalMeshComponent") (.ImpactPoint (Collision|BreakHitResult _outhit)) 1.0)) (Math|Rotator|FindLookatRotation (.Location (Collision|BreakHitResult _outhit)) (Transformation|GetActorLocation (Components|GetOwner))) "1.000000,1.000000,1.000000") "Undefined" "MultiplyWithRoot" _returnvalue 0))
        (Variables|Grapple|SetCurrent%20Blood%20Grapple _returnvalue_7)
        (Transformation|AttachComponentToComponent (Variables|Grapple|GetCurrent%20Blood%20Grapple) (Actor|GetComponentbyClass _output_get "/Script/Engine.SkeletalMeshComponent") (.ReturnValue (Class|SkinnedMeshComponent|FindClosestBoneK2 (Actor|GetComponentbyClass _output_get "/Script/Engine.SkeletalMeshComponent") (.ImpactPoint (Collision|BreakHitResult _outhit)) 1.0)) "KeepWorld" "KeepWorld" "KeepWorld" true))
      (:Is%20Not%20Valid
        (bind _returnvalue_8 (Game|SpawnActorfromClass "/Game/Characters/Player/Grappling/BP_Blood_Grapple_Blade.BP_Blood_Grapple_Blade_C" (Math|Transform|MakeTransform (.Location (Collision|BreakHitResult _outhit)) (Math|Rotator|FindLookatRotation (.Location (Collision|BreakHitResult _outhit)) (Transformation|GetActorLocation (Components|GetOwner))) "1.000000,1.000000,1.000000") "Undefined" "MultiplyWithRoot" _returnvalue 0))
        (Variables|Grapple|SetCurrent%20Blood%20Grapple _returnvalue_8)
        (Transformation|AttachActorToActor (Variables|Grapple|GetCurrent%20Blood%20Grapple) (Variables|Grapple|GetGrappled%20Actor) "None" "KeepWorld" "KeepWorld" "KeepWorld" true)))
    (else
      (Variables|Checks|SetCan%20Swing false)
      (Variables|Checks|SetGrappled false))))

(event Custom|Grapple%20To%20Stationary
  (bind _grapple_in_hand (Variables|Grapple|GetGrapple%20In%20Hand))
  (bind _grapple_to_force (Variables|Grapple|GetGrapple%20To%20Force))
  ;[1 1 1] Pull player towards grapple hook
  (Development|PrintString "Grapple Hook")
  (bind _ascharacter (Utilities|Casting|CastToCharacter (Components|GetOwner)))
  (Character|LaunchCharacter _ascharacter (+ (* (Math|Vector|GetForwardVector (Math|Rotator|FindLookatRotation (Transformation|GetActorLocation (Components|GetOwner)) (Variables|Grapple|GetHit%20Location))) _grapple_to_force) (* (Transformation|GetActorUpVector (Components|GetOwner)) (/ _grapple_to_force 2.0))) true true)
  (Variables|Checks|SetGrapple%20Pull? false)
  (Actor|SetLifeSpan (Variables|Grapple|GetCurrent%20Blood%20Grapple) 4.0)
  (Default|UnhideAllWeaponsWhilstGrappling (Actor|GetComponentbyClass (Components|GetOwner) "/Game/Weapons/Actor_Components/BPC_Weaponry.BPC_Weaponry_C"))
  (Utilities|IsValid _grapple_in_hand
    (:Is%20Valid
      (Actor|DestroyActor _grapple_in_hand))))

(event Custom|Grapple%20Pull%20Small
  (bind _grapple_in_hand (Variables|Grapple|GetGrapple%20In%20Hand))
  ;[1 1 1] Pull hit actor towards player and up a bit
  (Development|PrintString "Grapple Pull Small")
  (bind _ascharacter (Utilities|Casting|CastToCharacter (Variables|Grapple|GetGrappled%20Actor))
    (:then
      (Character|LaunchCharacter _ascharacter (+ (* (Transformation|GetActorUpVector (Variables|Grapple|GetGrappled%20Actor)) (Variables|Grapple|GetGrapple%20Pull%20Force)) (* (Math|Vector|GetForwardVector (Math|Rotator|FindLookatRotation (Transformation|GetActorLocation (Variables|Grapple|GetGrappled%20Actor)) (Transformation|GetActorLocation (Components|GetOwner)))) (/ (Variables|Grapple|GetGrapple%20Pull%20Force) 2.0))) true true))
    (:CastFailed
      (Physics|AddImpulse (Variables|Grapple|GetGrappled%20Component) (+ (* (Math|Vector|GetUpVector (Variables|Grapple|GetGrappled%20Component)) (Variables|Grapple|GetGrapple%20To%20Force)) (* (Math|Vector|GetForwardVector (Math|Rotator|FindLookatRotation (Transformation|GetWorldLocation (Variables|Grapple|GetGrappled%20Component)) (Transformation|GetActorLocation (Components|GetOwner)))) (Variables|Grapple|GetGrapple%20To%20Force))) "None" true)))
  (Variables|Checks|SetGrapple%20Pull? false)
  (Actor|SetLifeSpan (Variables|Grapple|GetCurrent%20Blood%20Grapple) 4.0)
  (Default|UnhideAllWeaponsWhilstGrappling (Actor|GetComponentbyClass (Components|GetOwner) "/Game/Weapons/Actor_Components/BPC_Weaponry.BPC_Weaponry_C"))
  (Utilities|IsValid _grapple_in_hand
    (:Is%20Valid
      (Actor|DestroyActor _grapple_in_hand))))

(event Custom|Grapple%20To%20Moving
  (bind _grapple_in_hand (Variables|Grapple|GetGrapple%20In%20Hand))
  (bind _grapple_to_force (Variables|Grapple|GetGrapple%20To%20Force))
  ;[1 1 1] Pull player towards hit actor
  (Development|PrintString "Grapple Pull Big")
  (bind _ascharacter (Utilities|Casting|CastToCharacter (Components|GetOwner)))
  (Character|LaunchCharacter _ascharacter (+ (* (Math|Vector|GetForwardVector (Math|Rotator|FindLookatRotation (Transformation|GetActorLocation (Components|GetOwner)) (Variables|Grapple|GetHit%20Location))) _grapple_to_force) (* (Transformation|GetActorUpVector (Components|GetOwner)) (/ _grapple_to_force 2.0))) true true)
  (Variables|Checks|SetGrapple%20Pull? false)
  (Actor|SetLifeSpan (Variables|Grapple|GetCurrent%20Blood%20Grapple) 4.0)
  (Default|UnhideAllWeaponsWhilstGrappling (Actor|GetComponentbyClass (Components|GetOwner) "/Game/Weapons/Actor_Components/BPC_Weaponry.BPC_Weaponry_C"))
  (Utilities|IsValid _grapple_in_hand
    (:Is%20Valid
      (Actor|DestroyActor _grapple_in_hand))))

(event Custom|Grapple%20Pull
  (Utilities|IsValid (Variables|Grapple|GetGrappled%20Actor)
    (:Is%20Valid
      (switch Utilities|FlowControl|Switch|SwitchonECollisionChannel (Collision|GetCollisionObjectType (.HitComponent (Collision|BreakHitResult (stale Custom|Grapple _outhit))))
        (:ECC_WorldStatic
          (Variables|Checks|SetCan%20Swing true :!label _label)
          (Utilities|FlowControl|Delay 0.15)
          (if (Variables|Checks|GetSwinging)
            (Variables|Checks|SetGrapple%20Pull? false)
            (else
              (CallFunction|GrappletoStationary))))
        (:ECC_WorldDynamic
          (goto _label))
        (:ECC_PhysicsBody
          (CallFunction|GrapplePullSmall :!label _label_2)
          (Variables|Checks|SetCan%20Swing false))
        (:ECC_GameTraceChannel1
          (goto _label))
        (:ECC_GameTraceChannel3
          (goto _label_2))
        (:ECC_GameTraceChannel4
          ;[1 1 1] Determine if enemy is big or small
          (if false
            (CallFunction|GrappletoMoving)
            (Variables|Checks|SetCan%20Swing false)
            (else
              (CallFunction|GrapplePullSmall)
              (Variables|Checks|SetCan%20Swing false))))
        (:ECC_GameTraceChannel6
          (CallFunction|GrappletoMoving)
          (Variables|Checks|SetCan%20Swing false))
        (:ECC_GameTraceChannel8
          (CallFunction|GrappletoStationary)
          (Variables|Checks|SetCan%20Swing false))))))

(event Input|EnhancedActionEvents|EnhancedInputActionIA_Grapple
  (params (ActionValue :type Boolean) (ElapsedSeconds :type Float%20%28double-precision%29) (TriggeredSeconds :type Float%20%28double-precision%29) (InputAction :type Input%20Action%20Object%20Reference :default "/Game/Characters/Player/Input/Actions/Grappling/IA_Grapple.IA_Grapple"))
  (:Triggered
    (if (Variables|Checks|GetCan%20Grapple)
      (Variables|Checks|SetGrappled true))))

(event Input|EnhancedActionEvents|EnhancedInputActionIA_Swing
  (params (ActionValue :type Boolean) (ElapsedSeconds :type Float%20%28double-precision%29) (TriggeredSeconds :type Float%20%28double-precision%29) (InputAction :type Input%20Action%20Object%20Reference :default "/Game/Characters/Player/Input/Actions/Grappling/IA_Swing.IA_Swing"))
  (:Triggered
    (if (Variables|Checks|GetCan%20Swing)
      (Utilities|FlowControl|DoOnce false :!label _label
        (:Completed
          (CallFunction|StartSwing)))))
  (:Completed
    (Variables|Checks|SetCan%20Swing false)
    (if (Variables|Checks|GetSwinging)
      (Utilities|FlowControl|Sequence
        (:then_0
          (goto _label Reset))
        (:then_1
          (CallFunction|StopSwing))))))

(event EventTick
  (params (DeltaSeconds :type Float%20%28single-precision%29))
  (bind _returnvalue (Components|GetOwner))
  (Variables|Checks|SetCan%20Grapple (not (Math|Boolean|ORBoolean (Variables|Checks|GetGrapple%20Cooldown) (Variables|/Game/Weapons/Actor_Components/BPC_Attack_Handler.BPC_Attack_Handler_C|GetAttacking (Actor|GetComponentbyClass _returnvalue "/Game/Weapons/Actor_Components/BPC_Attack_Handler.BPC_Attack_Handler_C")) (Variables|/Game/Weapons/Actor_Components/BPC_Aim.BPC_Aim_C|GetAiming? (Actor|GetComponentbyClass _returnvalue "/Game/Weapons/Actor_Components/BPC_Aim.BPC_Aim_C")) (Variables|Checks|GetGrapple%20Pull?) (Variables|Checks|GetGrappled) (Variables|Checks|GetSwinging))))
  (if (Variables|Checks|GetSwinging)
    (CallFunction|SwingForce)))

(fn GrappleCooldownFunc
  (Variables|Checks|SetGrapple%20Cooldown false))

(fn SwingForce
  (Physics|AddForce (Actor|GetComponentbyClass (Components|GetOwner) "/Script/Engine.CharacterMovementComponent") (* (Math|Vector|Normalize (- (Variables|Grapple|GetHit%20Location) (Transformation|GetActorLocation (Components|GetOwner)))) (* (Variables|Grapple|GetGrapple%20Pull%20Force) 5e+02))))

(fn SetupGrappleinHand
  (bind _returnvalue (Components|GetOwner))
  (bind _returnvalue_2 (Actor|GetComponentbyClass _returnvalue "/Game/Weapons/Actor_Components/BPC_Weaponry.BPC_Weaponry_C"))
  (Default|HideWeaponsWhilstGrappling _returnvalue_2 (Variables|/Game/Weapons/Actor_Components/BPC_Weaponry.BPC_Weaponry_C|GetEquipped_Weapon _returnvalue_2))
  (bind _returnvalue_3 (Game|SpawnActorfromClass "/Game/Characters/Player/Grappling/BP_Blood_Grapple_Blade.BP_Blood_Grapple_Blade_C" (Math|Transform|MakeTransform "0, 0, 0" "90.000000,0.000000,0.000000" "0.500000,0.500000,0.500000") "Undefined" "MultiplyWithRoot" (Components|GetOwner) 0))
  (bind _output_get (Variables|Grapple|SetGrapple%20In%20Hand _returnvalue_3))
  (Transformation|AttachComponentToComponent _output_get (Actor|GetComponentbyClass (Components|GetOwner) "/Script/Engine.SkeletalMeshComponent") "Grappling_Socket_R" "SnapToTarget" "SnapToTarget" "KeepWorld" true))