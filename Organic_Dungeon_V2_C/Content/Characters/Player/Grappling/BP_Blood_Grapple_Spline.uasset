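; Blood grapple actor that visually extrudes a chain of instanced meshes along a spline.
; The construction script tiles the mesh along the spline, spaced by its bounds plus an offset.
; On BeginPlay, a delayed loop sized by distance to HitActor, or a maximum-range aim point, appends points and instances along the spline's last direction.
; It destroys itself when the loop completes or after overlapping HitActor stops extrusion.
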(event OnComponentBeginOverlap(InstancedStaticMesh)
  (params (OverlappedComponent :type Primitive%20Component%20Object%20Reference) (OtherActor :type Actor%20Object%20Reference) (OtherComp :type Primitive%20Component%20Object%20Reference) (OtherBodyIndex :type Integer) (bFromSweep :type Boolean) (SweepResult :type Hit%20Result%20Structure%20%28by%20ref%29))
  (if (== OtherActor (Variables|Default|GetHit%20Actor))
    (Variables|Default|SetShould%20Extrude false)))

(event Custom|Test
  (bind _hit_actor (Variables|Default|GetHit%20Actor))
  (bind _spline (Variables|Default|GetSpline))
  (bind _hit_actor_2 (Variables|Default|GetHit%20Actor))
  (bind _spacing (Variables|Default|GetSpacing))
  (bind _returnvalue (Spline|GetNumberOfSplinePoints _spline))
  (bind _returnvalue_2 (- _returnvalue 1))
  (bind _returnvalue_3 (Spline|GetLocationatSplinePoint _spline _returnvalue_2 "World"))
  (bind _returnvalue_4 (Spline|GetRotationatSplinePoint _spline _returnvalue_2 "World"))
  (bind _returnvalue_5 (Math|Vector|GetForwardVector _returnvalue_4))
  (bind _returnvalue_6 (* _returnvalue_5 _spacing))
  (bind _returnvalue_7 (+ _returnvalue_3 _returnvalue_6))
  (if (Utilities|IsValid _hit_actor)
    (Variables|Default|SetEnd%20Target%20Location (Transformation|GetActorLocation _hit_actor))
    (else
      (Variables|Default|SetEnd%20Target%20Location (+ (Transformation|GetActorLocation) (* (Math|Vector|GetForwardVector (Pawn|GetControlRotation (Game|GetPlayerController 0) :!class /Script/Engine.Controller)) (Variables|Default|GetMax%20Length%20Extrusion))))))
  (Development|PrintString (Utilities|String|ToString(Integer) (Math|Float|Floor (/ (Math|Vector|Distance(Vector) (Transformation|GetActorLocation (Components|GetOwner)) (Variables|Default|GetEnd%20Target%20Location)) (Variables|Default|GetSpacing)))))
  (Utilities|ForLoopwithDelay 1 (Math|Float|Floor (/ (Math|Vector|Distance(Vector) (Transformation|GetActorLocation (Components|GetOwner)) (Variables|Default|GetEnd%20Target%20Location)) (Variables|Default|GetSpacing))) 0.01
    (:Loop%20Body
      (if (Variables|Default|GetShould%20Extrude)
        (if (Utilities|IsValid _hit_actor_2)
          (Variables|Default|SetEnd%20Target%20Location (Transformation|GetActorLocation _hit_actor_2))
          (else
            (Variables|Default|SetEnd%20Target%20Location (+ (Transformation|GetActorLocation) (* (Math|Vector|GetForwardVector (Pawn|GetControlRotation (Game|GetPlayerController 0) :!class /Script/Engine.Controller)) (Variables|Default|GetMax%20Length%20Extrusion))))))
        (Spline|AddSplinePoint (Variables|Default|GetSpline) _returnvalue_7 "World" true)
        (Components|InstancedStaticMesh|AddInstance (Variables|Default|GetInstancedStaticMesh) (Math|Transform|MakeTransform _returnvalue_7 (Spline|GetRotationatSplinePoint (Variables|Default|GetSpline) (- (Spline|GetNumberOfSplinePoints (Variables|Default|GetSpline)) 1) "World") "1.000000,1.000000,1.000000") true)
        (else
          (Components|InstancedStaticMesh|ClearInstances (Variables|Default|GetInstancedStaticMesh) :!label _label)
          (Actor|DestroyActor))))
    (:Completed
      (goto _label))))

(event EventBeginPlay
  (CallFunction|Test))

(fn ConstructionScript
  (bind _blood_grapple_sm (Variables|Default|GetBlood%20Grapple%20SM))
  (bind _returnvalue (StaticMesh|GetBoundingBox _blood_grapple_sm))
  (bind (_min _max) (Utilities|Struct|BreakBox _returnvalue))
  (Components|StaticMesh|SetStaticMesh (Variables|Default|GetInstancedStaticMesh) (Variables|Default|GetBlood%20Grapple%20SM))
  (bind _output_get (Variables|Default|SetSpacing (+ (.X (Class|KismetMathLibrary|BreakVector3f (- _max _min))) (Variables|Default|GetOffset))))
  (bind _output_get_2 (Variables|Default|SetNumber%20Of%20Instances (Math|Float|Floor (/ (Spline|GetSplineLength (Variables|Default|GetSpline)) _output_get))))
  (for _index (range 0 _output_get_2)
    (Components|InstancedStaticMesh|AddInstance (Variables|Default|GetInstancedStaticMesh) (Math|Transform|MakeTransform (CallFunction|GetLocationatIndex _index) (Math|Rotator|MakeRotfromX (- (CallFunction|GetLocationatIndex (+ _index 1)) (CallFunction|GetLocationatIndex _index)))) false)))

(fn GetLocationatIndex
  (params (A :type Integer))
  (return (Spline|GetLocationatDistanceAlongSpline (Variables|Default|GetSpline) (* A (Variables|Default|GetSpacing)) "Local")))