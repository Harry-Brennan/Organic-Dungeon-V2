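; Blood grapple cable actor for the player that animates its cable extending when spawned.
; A timeline on BeginPlay lerps the cable's EndLocation from zero along local X, re-measuring length each update to HitActor or a max-range point along control rotation.
; It flags ReachedMaxExtrusion at zero remaining distance and destroys itself when the timeline finishes if ShouldExtrude is false.
; Each update prints the remaining distance for debugging.
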(event EventBeginPlay
  (bind _hit_actor (Variables|Default|GetHit%20Actor))
  (bind _alpha (Timeline|Lerping%20Cable%20Length PlayFromStart)
    (:Update
      (Development|PrintString (Utilities|String|ToString(Float) (Math|Vector|Distance(Vector) (Variables|/Script/CableComponent.CableComponent|GetEndLocation (Variables|Default|GetCable)) (Variables|Default|GetEnd%20Target%20Location))))
      (if (<= (Math|Vector|Distance(Vector) (Variables|/Script/CableComponent.CableComponent|GetEndLocation (Variables|Default|GetCable)) (Variables|Default|GetEnd%20Target%20Location)) 0.0)
        (Variables|Default|SetReached%20Max%20Extrusion true)
        (else
          (if (Utilities|IsValid _hit_actor)
            (Variables|Default|SetEnd%20Target%20Location (Math|Vector|MakeVector (Math|Vector|Distance(Vector) (Variables|/Script/CableComponent.CableComponent|GetEndLocation (Variables|Default|GetCable)) (Transformation|GetActorLocation _hit_actor)) 0.0 0.0))
            (else
              (Variables|Default|SetEnd%20Target%20Location (Math|Vector|MakeVector (Math|Vector|Distance(Vector) (Variables|/Script/CableComponent.CableComponent|GetEndLocation (Variables|Default|GetCable)) (+ (Transformation|GetActorLocation (Components|GetOwner)) (* (Math|Vector|GetForwardVector (Pawn|GetControlRotation (Game|GetPlayerController 0) :!class /Script/Engine.Controller)) (Variables|Default|GetMax%20Length%20Extrusion)))) 0.0 0.0))))
          (Variables|/Script/CableComponent.CableComponent|SetEndLocation (Variables|Default|GetCable) (Math|Vector|Lerp(Vector) "0, 0, 0" (Variables|Default|GetEnd%20Target%20Location) _alpha)))))
    (:Finished
      (if (not (Variables|Default|GetShould%20Extrude))
        (Actor|DestroyActor)))))

(fn ConstructionScript)