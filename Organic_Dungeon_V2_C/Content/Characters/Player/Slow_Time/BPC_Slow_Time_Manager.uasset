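; Player component that manages slow motion requested by multiple sources, each stored in a map with its lowest amount.
; The slowest entry drives global time dilation and pitch, and removing the last restores normal time, with start, loop and end audio.
; Tick eases a camera post-process material toward matching blur and radial colour.
; During those transitions, health below 75% overrides the radial amount and darkens the edge to red.
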(event Custom|Remove%20Slow%20Time%20Enemy%20Kill%20Specific
  (Utilities|Map|Remove (Variables|Default|GetSlow%20Time%20Activator%20-%20Amount) "NewEnumerator4")
  (if (Utilities|Map|IsEmpty (Variables|Default|GetSlow%20Time%20Activator%20-%20Amount))
    (CallFunction|DeactivateSlowTime)
    (else
      (CallFunction|ActivateSlowTime))))

(event Custom|Remove%20Slow%20Time%20Explode%20Specific
  (Utilities|Map|Remove (Variables|Default|GetSlow%20Time%20Activator%20-%20Amount) "NewEnumerator6")
  (if (Utilities|Map|IsEmpty (Variables|Default|GetSlow%20Time%20Activator%20-%20Amount))
    (CallFunction|DeactivateSlowTime)
    (else
      (CallFunction|ActivateSlowTime))))

(event Custom|Add%20Slow%20Time
  (params (Amount :type Float%20%28double-precision%29) (Activation%20Source :type Enum_Slow_Time_Activators%20Enum :default "Enum_Slow_Time_Activators_MAX"))
  (bind _slow_time_activator___amount (Variables|Default|GetSlow%20Time%20Activator%20-%20Amount))
  (if (Utilities|Map|Contains _slow_time_activator___amount Activation%20Source)
    (if (< Amount (.Value (Utilities|Map|Find _slow_time_activator___amount Activation%20Source)))
      (Utilities|Map|Add (Variables|Default|GetSlow%20Time%20Activator%20-%20Amount) Activation%20Source Amount))
    (else
      (Utilities|Map|Add _slow_time_activator___amount Activation%20Source Amount)))
  (CallFunction|ActivateSlowTime))

(event Custom|Activate%20Slow%20Time
  (if (== (Class|GameplayStatics|GetGlobalTimeDilation) 1.0)
    (Audio|PlaySound2D "/Game/VFX_SFX/Slow_Time/Slow_Time_Start.Slow_Time_Start" 1.0 1.0 0.0 0 0)
    (Components|Activation|Activate (Variables|Default|GetSlow%20Time%20Continuous%20Audio%20Component) false))
  (Variables|Default|SetSlowest%20Time 1.0)
  (bind _values (Utilities|Map|Values (Variables|Default|GetSlow%20Time%20Activator%20-%20Amount)))
  (for _array_element _values
    (if (< _array_element (Variables|Default|GetSlowest%20Time))
      (Variables|Default|SetSlowest%20Time _array_element)))
  (Utilities|Time|SetGlobalTimeDilation (Variables|Default|GetSlowest%20Time))
  (Class|GameplayStatics|SetGlobalPitchModulation (Variables|Default|GetSlowest%20Time) 0.0)
  (Variables|Default|SetBlur%20Amount (Math|Float|Clamp(Float) (* (- 1.0 (Variables|Default|GetSlowest%20Time)) 3.5) 0.0 1.5))
  (Variables|Default|SetBlur%20Effectiveness (* (- 1.0 (Variables|Default|GetSlowest%20Time)) 3.0))
  (Variables|Default|SetRadial%20Colour%20Value (Math|Float|Clamp(Float) (- 1.0 (/ (- 1.0 (Variables|Default|GetSlowest%20Time)) 1.5)) 0.65)))

(event Custom|Remove%20Slow%20Time
  (params (Activator :type Enum_Slow_Time_Activators%20Enum :default "Enum_Slow_Time_Activators_MAX"))
  (Utilities|Map|Remove (Variables|Default|GetSlow%20Time%20Activator%20-%20Amount) Activator)
  (if (Utilities|Map|IsEmpty (Variables|Default|GetSlow%20Time%20Activator%20-%20Amount))
    (CallFunction|DeactivateSlowTime)
    (else
      (CallFunction|ActivateSlowTime))))

(event Custom|Deactivate%20Slow%20Time
  (Utilities|Time|SetGlobalTimeDilation 1.0)
  (Class|GameplayStatics|SetGlobalPitchModulation 1.0 0.0)
  (Variables|Default|SetBlur%20Amount 0.0)
  (Variables|Default|SetBlur%20Effectiveness 0.0)
  (Variables|Default|SetRadial%20Colour%20Value 1.0)
  (Audio|PlaySound2D "/Game/VFX_SFX/Slow_Time/SC_Slow_Time_End.SC_Slow_Time_End" 1.0 1.0 0.0 0 0)
  (Components|Activation|Deactivate (Variables|Default|GetSlow%20Time%20Continuous%20Audio%20Component)))

(event EventBeginPlay
  (Utilities|FlowControl|Delay 0.2)
  (Variables|Default|SetPlayer%20Camera (Actor|GetComponentbyClass (Components|GetOwner) "/Script/Engine.CameraComponent"))
  (Variables|Default|SetSlow%20Time%20Continuous%20Audio%20Component (Utilities|Array|Get(acopy) (Actor|GetComponentsbyTag (Components|GetOwner) "/Script/Engine.AudioComponent" "Slow Time Continous Audio")))
  (bind _returnvalue (Rendering|Material|CreateDynamicMaterialInstance "/Game/Assets/Materials/Camera_Masks/M_Camera_Blur_Colour_Mask.M_Camera_Blur_Colour_Mask" "None" "None" :!class /Script/Engine.KismetMaterialLibrary))
  (bind _output_get (Variables|Default|SetCamera%20Blur%20Mask%20MI _returnvalue))
  (Utilities|Struct|SetmembersinPostProcessSettings (Variables|/Script/Engine.CameraComponent|GetPostProcessSettings (Variables|Default|GetPlayer%20Camera)) (Utilities|Struct|MakeWeightedBlendables (Utilities|Array|MakeArray (Utilities|Struct|MakeWeightedBlendable 1.0 _output_get))))
  (Rendering|Material|SetScalarParameterValue (Variables|Default|GetCamera%20Blur%20Mask%20MI) "Blur Amount" 0.0 :!class /Script/Engine.MaterialInstanceDynamic)
  (Rendering|Material|SetScalarParameterValue (Variables|Default|GetCamera%20Blur%20Mask%20MI) "Blur Effectiveness" 0.0 :!class /Script/Engine.MaterialInstanceDynamic)
  (Rendering|Material|SetScalarParameterValue (Variables|Default|GetCamera%20Blur%20Mask%20MI) "Radial Colour Amount" 1.0 :!class /Script/Engine.MaterialInstanceDynamic)
  (Components|Tick|SetComponentTickEnabled true))

(event EventTick
  (params (DeltaSeconds :type Float%20%28single-precision%29))
  (bind _returnvalue (Rendering|Material|GetScalarParameterValue (Variables|Default|GetCamera%20Blur%20Mask%20MI) "Blur Amount" :!class /Script/Engine.MaterialInstanceDynamic))
  (bind _returnvalue_2 (Rendering|Material|GetScalarParameterValue (Variables|Default|GetCamera%20Blur%20Mask%20MI) "Blur Effectiveness" :!class /Script/Engine.MaterialInstanceDynamic))
  (if (not (and (== _returnvalue (Variables|Default|GetBlur%20Amount)) (== _returnvalue_2 (Variables|Default|GetBlur%20Effectiveness))))
    (Utilities|ChangeBlurAmountandEffectiveness (Variables|Default|GetBlur%20Amount) (Variables|Default|GetBlur%20Effectiveness) (+ (* (- 1.0 (Class|GameplayStatics|GetGlobalTimeDilation)) 1e+01) 2.0) (Variables|Default|GetRadial%20Colour%20Value))))