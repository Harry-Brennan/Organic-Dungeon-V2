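; Player HUD component that creates WBP_HUD on BeginPlay and relays gameplay events to it.
; Events forward weapon icon swaps, HUD shake, crosshair animations and movement ability use or reset.
; Crosshair updates read the equipped weapon's melee, heavy or ranged texture from BPC_Weaponry.
; An available-action prompt chain polling sibling components is disconnected, leaving the delay-enabled Tick empty.
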(event Custom|Swap_Weapon_Icons
  (params (Next? :type Boolean))
  ;[1 1 1] Changing the weapon icons using the widget HUD
  (Default|UpdateEquippedWeaponUI (Variables|Default|GetHUD_Ref) Next?))

(event Custom|Update_Crosshair
  (params (Aiming :type Boolean) (Melee? :type Boolean) (Heavy? :type Boolean))
  (bind _returnvalue (Components|GetOwner))
  (bind _returnvalue_2 (Actor|GetComponentbyClass _returnvalue "/Game/Weapons/Actor_Components/BPC_Weaponry.BPC_Weaponry_C"))
  (bind _equipped_weapon (Variables|/Game/Weapons/Actor_Components/BPC_Weaponry.BPC_Weaponry_C|GetEquipped_Weapon _returnvalue_2))
  ;[1 1 1] Updates the crosshair
  (if Melee?
    (bind _melee_info (Class|BPIMeleeWeapon|GetMeleeInfo(Message) _equipped_weapon))
    (Default|UpdateCrosshairVisibility (Variables|Default|GetHUD_Ref) Aiming (select Heavy? (Utilities|Struct|BreakStruct_Heavy_Attack_Info (.HeavyAttackInfo (Utilities|Struct|BreakStruct_Melee_Weapon _melee_info))) (.Crosshair (Utilities|Struct|BreakStruct_Melee_Weapon _melee_info))))
    (else
      (bind _ranged_info (Class|BPIRangedWeapon|GetRangedInfo(Message) _equipped_weapon))
      (Default|UpdateCrosshairVisibility (Variables|Default|GetHUD_Ref) Aiming (Utilities|Struct|BreakStruct_Ranged_Weapon _ranged_info)))))

(event Custom|Play_Hit_Crosshair_Anim
  ;[1 1 1] Plays the fire animation in the crosshair widget
  (Default|PlayFireAnim (Variables|/Game/UI/WBP_HUD.WBP_HUD_C|GetWBP_Crosshair (Variables|Default|GetHUD_Ref))))

(event Custom|Play%20Grapple%20Crosshair%20Anim
  ;[1 1 1] Plays the grapple animation in the crosshair widget in the hud widget
  (Default|PlayGrappleAnim (Variables|/Game/UI/WBP_HUD.WBP_HUD_C|GetWBP_Crosshair (Variables|Default|GetHUD_Ref))))

(event Custom|Play%20HUD%20Shake
  (Default|PlayHUDShakeAnim (Variables|Default|GetHUD_Ref)))

(event Custom|Use%20Movement%20Ability
  (params (Movement%20Ability :type Enum_Movement_Abilities%20Enum :default "NewEnumerator0"))
  (Default|UseMovementAbility (Variables|Default|GetHUD_Ref) Movement%20Ability))

(event Custom|Forcibly%20Reset%20Movement%20Ability
  (params (Movement%20Ability :type Enum_Movement_Abilities%20Enum :default "NewEnumerator0"))
  (Default|ForciblyResetMovementAbility (Variables|Default|GetHUD_Ref) Movement%20Ability))

(event EventTick
  (params (DeltaSeconds :type Float%20%28single-precision%29)))

(event EventBeginPlay
  ;[1 1 1] Create the HUD widget and add to viewport and then set tick enabled after spawning in the player
  (bind _returnvalue (UserInterface|CreateWidget "/Game/UI/WBP_HUD.WBP_HUD_C"))
  (UserInterface|Viewport|AddtoViewport _returnvalue 0)
  (Variables|Default|SetHUD_Ref _returnvalue)
  (Utilities|FlowControl|Delay 0.2)
  (Components|Tick|SetComponentTickEnabled true))