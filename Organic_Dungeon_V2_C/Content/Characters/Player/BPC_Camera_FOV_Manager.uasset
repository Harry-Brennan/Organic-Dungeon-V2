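; BPC_Camera_FOV_Manager is a player component that widens the owner's camera field of view as movement speed increases.
; On BeginPlay it caches the owner's camera and character movement components and stores the original FOV.
; Each tick it interpolates the FOV toward a target scaled by velocity magnitude relative to a max speed, clamped between the original FOV and that plus a maximum addition.
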(event EventTick
  (params (DeltaSeconds :type Float%20%28single-precision%29))
  (bind _original_fov (Variables|Default|GetOriginal%20FOV))
  ;[1 1 1] Finterp the FOV of the players camera based on their velocity with some max velocity speeds and max fov additions affecting how much the velocity will change
  (Camera|SetFieldOfView (Variables|Default|GetCamera) (Math|Float|Clamp(Float) (Math|Interpolation|FInterpTo (Variables|/Script/Engine.CameraComponent|GetFieldOfView (Variables|Default|GetCamera)) (+ (Variables|Default|GetOriginal%20FOV) (* (Variables|Default|GetMax_FOV_Addition) (/ (Math|Vector|VectorLength (Variables|/Script/Engine.MovementComponent|GetVelocity (Variables|Default|GetCharacter%20Movement))) (Variables|Default|GetMax_Vel_Speed)))) (Utilities|Time|GetWorldDeltaSeconds) (Variables|Default|GetInterp_Speed)) _original_fov (+ _original_fov (Variables|Default|GetMax_FOV_Addition)))))

(event EventBeginPlay
  ;[1 1 1] Get players camera and character movement component and then also get the FOV before making any changes to it to store it as the original FOV.
  (Variables|Default|SetCamera (Actor|GetComponentbyClass (Components|GetOwner) "/Script/Engine.CameraComponent"))
  (Variables|Default|SetCharacter%20Movement (Actor|GetComponentbyClass (Components|GetOwner) "/Script/Engine.CharacterMovementComponent"))
  (Variables|Default|SetOriginal%20FOV (Variables|/Script/Engine.CameraComponent|GetFieldOfView (Variables|Default|GetCamera))))