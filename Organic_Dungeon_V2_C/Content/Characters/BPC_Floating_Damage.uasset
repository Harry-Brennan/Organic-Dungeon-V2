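; Component that shows floating damage numbers by spawning one pooled Niagara system per character of the damage value.
; MakeFloatingNumber sets each system's digit texture, offsets it along local Y, and faces it by player control yaw.
; Each number gets a shared random roll and colour, with scale and spacing growing with damage within clamped limits.
; DetermineDamageIsFloat checks for non-zero decimals, and the DamageFloat flag decides whether the fractional part is drawn.
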(fn MakeFloatingNumber
  (params (Location :type Vector) (Damage_Amount :type Float%20%28double-precision%29) (Damage_Float :type Boolean))
  (bind _returnvalue (Utilities|String|ToString(Float) Damage_Amount))
  (bind _returnvalue_2 (/ Damage_Amount 35.0))
  (bind _returnvalue_3 (Math|Float|Clamp(Float) _returnvalue_2 0.5 2.5))
  (bind _returnvalue_4 (Utilities|String|GetCharacterArrayfromString _returnvalue))
  ;[1 1 1] Loop through setting the digits of the damage with some random variation to rotation
  (LocalVariables|SetRandom_Roll (Math|Random|RandomFloatinRange -25.0 25.0))
  (LocalVariables|SetRandom_Colour (Utilities|Struct|MakeLinearColor (Math|Random|RandomFloat) (Math|Random|RandomFloat) (Math|Random|RandomFloat) 0.5))
  (if Damage_Float
    (for _array_element (Utilities|String|GetCharacterArrayfromString _returnvalue)
      (bind _returnvalue_5 (Niagara|SpawnSystematLocation "/Game/VFX_SFX/Niagara/Damage_Niumber/NS_Floating_Numbers_FX.NS_Floating_Numbers_FX" Location (Math|Rotator|MakeRotator (LocalVariables|GetRandom_Roll) 1.8e+02 (.yaw (Pawn|GetControlRotation (Game|GetPlayerController 0) :!class /Script/Engine.Controller))) (Math|Vector|MakeVector _returnvalue_3 (Math|Float|Clamp(Float) _returnvalue_2 0.5 2.5) (Math|Float|Clamp(Float) _returnvalue_2 0.5 2.5)) true true "AutoRelease"))
      (LocalVariables|SetDigit_System _returnvalue_5)
      (Transformation|AddLocalOffset (LocalVariables|GetDigit_System) (Math|Vector|MakeVector 0.0 (LocalVariables|GetText_Offset) 0.0) false false)
      (Niagara|SetNiagaraVariable(LinearColor) (LocalVariables|GetDigit_System) "user.Damage_Colour" (LocalVariables|GetRandom_Colour))
      (LocalVariables|SetText_Offset (+ (LocalVariables|GetText_Offset) (* 3e+01 _returnvalue_3)))
      ;[1 1 1] Set the digit of the niagara system
      (switch string (Utilities|String|SelectString _array_element (Utilities|Array|Get(acopy) _returnvalue_4 (stale _index)) Damage_Float)
        (:0
          (Niagara|SetTextureObject (LocalVariables|GetDigit_System) "user.Digit" "/Game/VFX_SFX/Niagara/Damage_Niumber/Digits/0.0"))
        (:1
          (Niagara|SetTextureObject (LocalVariables|GetDigit_System) "user.Digit" "/Game/VFX_SFX/Niagara/Damage_Niumber/Digits/1.1"))
        (:2
          (Niagara|SetTextureObject (LocalVariables|GetDigit_System) "user.Digit" "/Game/VFX_SFX/Niagara/Damage_Niumber/Digits/2.2"))
        (:3
          (Niagara|SetTextureObject (LocalVariables|GetDigit_System) "user.Digit" "/Game/VFX_SFX/Niagara/Damage_Niumber/Digits/3.3"))
        (:4
          (Niagara|SetTextureObject (LocalVariables|GetDigit_System) "user.Digit" "/Game/VFX_SFX/Niagara/Damage_Niumber/Digits/4.4"))
        (:5
          (Niagara|SetTextureObject (LocalVariables|GetDigit_System) "user.Digit" "/Game/VFX_SFX/Niagara/Damage_Niumber/Digits/5.5"))
        (:6
          (Niagara|SetTextureObject (LocalVariables|GetDigit_System) "user.Digit" "/Game/VFX_SFX/Niagara/Damage_Niumber/Digits/6.6"))
        (:7
          (Niagara|SetTextureObject (LocalVariables|GetDigit_System) "user.Digit" "/Game/VFX_SFX/Niagara/Damage_Niumber/Digits/7.7"))
        (:8
          (Niagara|SetTextureObject (LocalVariables|GetDigit_System) "user.Digit" "/Game/VFX_SFX/Niagara/Damage_Niumber/Digits/8.8"))
        (:9
          (Niagara|SetTextureObject (LocalVariables|GetDigit_System) "user.Digit" "/Game/VFX_SFX/Niagara/Damage_Niumber/Digits/9.9"))
        (:.
          (Niagara|SetTextureObject (LocalVariables|GetDigit_System) "user.Digit" "/Game/VFX_SFX/Niagara/Damage_Niumber/Digits/_._"))))
    (else
      (for _index (range 0 (- (Utilities|Array|FindItem _returnvalue_4 ".") 1))
        (bind _returnvalue_6 (Niagara|SpawnSystematLocation "/Game/VFX_SFX/Niagara/Damage_Niumber/NS_Floating_Numbers_FX.NS_Floating_Numbers_FX" Location (Math|Rotator|MakeRotator (LocalVariables|GetRandom_Roll) 1.8e+02 (.yaw (Pawn|GetControlRotation (Game|GetPlayerController 0) :!class /Script/Engine.Controller))) (Math|Vector|MakeVector _returnvalue_3 (Math|Float|Clamp(Float) _returnvalue_2 0.5 2.5) (Math|Float|Clamp(Float) _returnvalue_2 0.5 2.5)) true true "AutoRelease"))
        (LocalVariables|SetDigit_System _returnvalue_6)
        (Transformation|AddLocalOffset (LocalVariables|GetDigit_System) (Math|Vector|MakeVector 0.0 (LocalVariables|GetText_Offset) 0.0) false false)
        (Niagara|SetNiagaraVariable(LinearColor) (LocalVariables|GetDigit_System) "user.Damage_Colour" (LocalVariables|GetRandom_Colour))
        (LocalVariables|SetText_Offset (+ (LocalVariables|GetText_Offset) (* 3e+01 _returnvalue_3)))
        (switch string (Utilities|String|SelectString _array_element (Utilities|Array|Get(acopy) _returnvalue_4 _index) Damage_Float)
          (:0
            (Niagara|SetTextureObject (LocalVariables|GetDigit_System) "user.Digit" "/Game/VFX_SFX/Niagara/Damage_Niumber/Digits/0.0"))
          (:1
            (Niagara|SetTextureObject (LocalVariables|GetDigit_System) "user.Digit" "/Game/VFX_SFX/Niagara/Damage_Niumber/Digits/1.1"))
          (:2
            (Niagara|SetTextureObject (LocalVariables|GetDigit_System) "user.Digit" "/Game/VFX_SFX/Niagara/Damage_Niumber/Digits/2.2"))
          (:3
            (Niagara|SetTextureObject (LocalVariables|GetDigit_System) "user.Digit" "/Game/VFX_SFX/Niagara/Damage_Niumber/Digits/3.3"))
          (:4
            (Niagara|SetTextureObject (LocalVariables|GetDigit_System) "user.Digit" "/Game/VFX_SFX/Niagara/Damage_Niumber/Digits/4.4"))
          (:5
            (Niagara|SetTextureObject (LocalVariables|GetDigit_System) "user.Digit" "/Game/VFX_SFX/Niagara/Damage_Niumber/Digits/5.5"))
          (:6
            (Niagara|SetTextureObject (LocalVariables|GetDigit_System) "user.Digit" "/Game/VFX_SFX/Niagara/Damage_Niumber/Digits/6.6"))
          (:7
            (Niagara|SetTextureObject (LocalVariables|GetDigit_System) "user.Digit" "/Game/VFX_SFX/Niagara/Damage_Niumber/Digits/7.7"))
          (:8
            (Niagara|SetTextureObject (LocalVariables|GetDigit_System) "user.Digit" "/Game/VFX_SFX/Niagara/Damage_Niumber/Digits/8.8"))
          (:9
            (Niagara|SetTextureObject (LocalVariables|GetDigit_System) "user.Digit" "/Game/VFX_SFX/Niagara/Damage_Niumber/Digits/9.9"))
          (:.
            (Niagara|SetTextureObject (LocalVariables|GetDigit_System) "user.Digit" "/Game/VFX_SFX/Niagara/Damage_Niumber/Digits/_._")))))))

(fn DetermineDamageIsFloat
  (params (Damage :type Float%20%28double-precision%29))
  (bind _returnvalue (Utilities|String|ToString(Float) Damage))
  (bind _returnvalue_2 (Utilities|String|GetCharacterArrayfromString _returnvalue))
  ;[1 1 1] Just determine if the damage is a float or not
  (LocalVariables|SetDamage_Float false)
  (bind _index (Utilities|FlowControl|ForLoopwithBreak (+ (Utilities|Array|FindItem _returnvalue_2 ".") 1) (- (Utilities|Array|Length _returnvalue_2) 1) :!label _label)
    (:LoopBody
      (if (Utilities|Enum|NotEqual(Enum) (Utilities|Array|Get(acopy) _returnvalue_2 _index) "0")
        (LocalVariables|SetDamage_Float true)
        (goto _label Break)))
    (:Completed
      (return (LocalVariables|GetDamage_Float)))))