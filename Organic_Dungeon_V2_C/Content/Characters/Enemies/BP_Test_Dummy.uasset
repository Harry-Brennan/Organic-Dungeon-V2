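; Test dummy enemy character whose stats and movement are configured from its EnemyInfo characteristics.
; The construction script applies only the first matching Tanky, Squishy, Slow or Fast data-table preset, then builds HealthInfo and selects flying or walking movement with matching gravity.
; Events set weapons, timeline-lerp walk or fly speed and temporarily switch gravity.
; Getters expose its info structs and component state, including aim, slide, melee and weaponry.
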(event EventSetStartingWeaponsIndex
  (params (Starting_Weapons :type Struct%20Spawnable%20Weapon%20Structure) (Index :type Integer))
  (Utilities|Array|SetArrayElem (Variables|StartingWeaponry|GetStarting_Weapons) Index Starting_Weapons))

(event EventSetStarterWeapon
  (params (Starting_Weapon :type Struct%20Spawnable%20Weapon%20Structure))
  (Variables|StartingWeaponry|SetStarter_Weapon Starting_Weapon))

(event EventUpdateNormalWalkingSpeed
  (params (New_Walk_Speed :type Float%20%28double-precision%29))
  (Variables|Movement|SetSprinting_Info (Utilities|Struct|MakeStruct_Sprinting_Info New_Walk_Speed (.sprinting_max_speed (Variables|Movement|GetSprinting_Info)) (.sprint_startup_speed (Variables|Movement|GetSprinting_Info)) (.sprint_stopping_speed (Variables|Movement|GetSprinting_Info)))))

(event EventToggleGravity
  (params (Starting%20Gravity :type Float%20%28double-precision%29) (Ending%20Gravity :type Float%20%28double-precision%29) (Time%20Between :type Float%20%28double-precision%29))
  (Variables|/Script/Engine.CharacterMovementComponent|SetGravityScale (Variables|Character|GetCharacterMovement) Starting%20Gravity)
  (Utilities|FlowControl|Delay Time%20Between)
  (Variables|/Script/Engine.CharacterMovementComponent|SetGravityScale (Variables|Character|GetCharacterMovement) Ending%20Gravity))

(event EventLerpMovementSpeed
  (params (Starting%20Speed :type Float%20%28double-precision%29) (New%20Speed :type Float%20%28double-precision%29) (Time :type Float%20%28double-precision%29))
  (bind _charactermovement (Variables|Character|GetCharacterMovement))
  (Components|Timeline|SetPlayRate (Variables|Default|GetLerp%20Movement%20Speed) (/ 1.0 Time))
  (bind _alpha (Timeline|Lerp%20Movement%20Speed PlayFromStart)
    (:Update
      (if (Utilities|Array|ContainsItem (Utilities|Struct|BreakStruct_Enemy_Info (Variables|EnemyInfo|GetEnemy%20Info)) "NewEnumerator2")
        (Variables|/Script/Engine.CharacterMovementComponent|SetMaxWalkSpeed _charactermovement (Math|Float|Lerp Starting%20Speed New%20Speed _alpha))
        (else
          (Variables|/Script/Engine.CharacterMovementComponent|SetMaxFlySpeed _charactermovement (Math|Float|Lerp Starting%20Speed New%20Speed _alpha))))
      (Variables|Movement|SetLerping%20Movement%20Speed true))
    (:Finished
      (Variables|Movement|SetLerping%20Movement%20Speed false))))

(fn ConstructionScript
  (bind _charactermovement (Variables|Character|GetCharacterMovement))
  (Default|UpdatingWeapons (Variables|Default|GetBPC_Starting_Weapons))
  (if (Utilities|Array|ContainsItem (Utilities|Struct|BreakStruct_Enemy_Info (Variables|EnemyInfo|GetEnemy%20Info)) "NewEnumerator6")
    (bind _returnvalue (Utilities|GetDataTableRow "/Game/Characters/Enemies/AI/Structs_Data_Tables/Characteristic_Data/Health/DT_Enemy_Health_Characteristics.DT_Enemy_Health_Characteristics" "Tanky")
      (:then
        (Variables|EnemyInfo|SetEnemy%20Info (Utilities|Struct|MakeStruct_Enemy_Info (Utilities|Struct|BreakStruct_Enemy_Health_Characteristics _returnvalue) (.SightInfo (Utilities|Struct|BreakStruct_Enemy_Info (Variables|EnemyInfo|GetEnemy%20Info))) (.HearingInfo (Utilities|Struct|BreakStruct_Enemy_Info (Variables|EnemyInfo|GetEnemy%20Info))) (.LoseAwarenessTime (Utilities|Struct|BreakStruct_Enemy_Info (Variables|EnemyInfo|GetEnemy%20Info))) (.Should_Patrol (Utilities|Struct|BreakStruct_Enemy_Info (Variables|EnemyInfo|GetEnemy%20Info))) (.Patrol_Info (Utilities|Struct|BreakStruct_Enemy_Info (Variables|EnemyInfo|GetEnemy%20Info))) (.ChasingInfo (Utilities|Struct|BreakStruct_Enemy_Info (Variables|EnemyInfo|GetEnemy%20Info))) (.Characteristics (Utilities|Struct|BreakStruct_Enemy_Info (Variables|EnemyInfo|GetEnemy%20Info))) (.Melee_Info (Utilities|Struct|BreakStruct_Enemy_Info (Variables|EnemyInfo|GetEnemy%20Info))) (.Ranged_Info (Utilities|Struct|BreakStruct_Enemy_Info (Variables|EnemyInfo|GetEnemy%20Info))) (.Ground_Info (Utilities|Struct|BreakStruct_Enemy_Info (Variables|EnemyInfo|GetEnemy%20Info))) (.Flying_Info (Utilities|Struct|BreakStruct_Enemy_Info (Variables|EnemyInfo|GetEnemy%20Info))) (.DashLeapInfo (Utilities|Struct|BreakStruct_Enemy_Info (Variables|EnemyInfo|GetEnemy%20Info))) (.ExplodingInfo (Utilities|Struct|BreakStruct_Enemy_Info (Variables|EnemyInfo|GetEnemy%20Info))) (.Multi-BodiedInfo (Utilities|Struct|BreakStruct_Enemy_Info (Variables|EnemyInfo|GetEnemy%20Info))) (.ShotEnemyInfo (Utilities|Struct|BreakStruct_Enemy_Info (Variables|EnemyInfo|GetEnemy%20Info)))))))
    (elif (Utilities|Array|ContainsItem (Utilities|Struct|BreakStruct_Enemy_Info (Variables|EnemyInfo|GetEnemy%20Info)) "NewEnumerator7")
      (bind _returnvalue_2 (Utilities|GetDataTableRow "/Game/Characters/Enemies/AI/Structs_Data_Tables/Characteristic_Data/Health/DT_Enemy_Health_Characteristics.DT_Enemy_Health_Characteristics" "Squishy")
        (:then
          (Variables|EnemyInfo|SetEnemy%20Info (Utilities|Struct|MakeStruct_Enemy_Info (Utilities|Struct|BreakStruct_Enemy_Health_Characteristics _returnvalue_2) (.SightInfo (Utilities|Struct|BreakStruct_Enemy_Info (Variables|EnemyInfo|GetEnemy%20Info))) (.HearingInfo (Utilities|Struct|BreakStruct_Enemy_Info (Variables|EnemyInfo|GetEnemy%20Info))) (.LoseAwarenessTime (Utilities|Struct|BreakStruct_Enemy_Info (Variables|EnemyInfo|GetEnemy%20Info))) (.Should_Patrol (Utilities|Struct|BreakStruct_Enemy_Info (Variables|EnemyInfo|GetEnemy%20Info))) (.Patrol_Info (Utilities|Struct|BreakStruct_Enemy_Info (Variables|EnemyInfo|GetEnemy%20Info))) (.ChasingInfo (Utilities|Struct|BreakStruct_Enemy_Info (Variables|EnemyInfo|GetEnemy%20Info))) (.Characteristics (Utilities|Struct|BreakStruct_Enemy_Info (Variables|EnemyInfo|GetEnemy%20Info))) (.Melee_Info (Utilities|Struct|BreakStruct_Enemy_Info (Variables|EnemyInfo|GetEnemy%20Info))) (.Ranged_Info (Utilities|Struct|BreakStruct_Enemy_Info (Variables|EnemyInfo|GetEnemy%20Info))) (.Ground_Info (Utilities|Struct|BreakStruct_Enemy_Info (Variables|EnemyInfo|GetEnemy%20Info))) (.Flying_Info (Utilities|Struct|BreakStruct_Enemy_Info (Variables|EnemyInfo|GetEnemy%20Info))) (.DashLeapInfo (Utilities|Struct|BreakStruct_Enemy_Info (Variables|EnemyInfo|GetEnemy%20Info))) (.ExplodingInfo (Utilities|Struct|BreakStruct_Enemy_Info (Variables|EnemyInfo|GetEnemy%20Info))) (.Multi-BodiedInfo (Utilities|Struct|BreakStruct_Enemy_Info (Variables|EnemyInfo|GetEnemy%20Info))) (.ShotEnemyInfo (Utilities|Struct|BreakStruct_Enemy_Info (Variables|EnemyInfo|GetEnemy%20Info)))))))
      (elif (Utilities|Array|ContainsItem (Utilities|Struct|BreakStruct_Enemy_Info (Variables|EnemyInfo|GetEnemy%20Info)) "NewEnumerator8")
        (bind _returnvalue_3 (Utilities|GetDataTableRow "/Game/Characters/Enemies/AI/Structs_Data_Tables/Characteristic_Data/Speed/DT_Enemy_Speed_Characteristics.DT_Enemy_Speed_Characteristics" "Slow")
          (:then
            (Variables|EnemyInfo|SetEnemy%20Info (Utilities|Struct|MakeStruct_Enemy_Info (.HealthInfo (Utilities|Struct|BreakStruct_Enemy_Info (Variables|EnemyInfo|GetEnemy%20Info))) (.SightInfo (Utilities|Struct|BreakStruct_Enemy_Info (Variables|EnemyInfo|GetEnemy%20Info))) (.HearingInfo (Utilities|Struct|BreakStruct_Enemy_Info (Variables|EnemyInfo|GetEnemy%20Info))) (.LoseAwarenessTime (Utilities|Struct|BreakStruct_Enemy_Info (Variables|EnemyInfo|GetEnemy%20Info))) (.Should_Patrol (Utilities|Struct|BreakStruct_Enemy_Info (Variables|EnemyInfo|GetEnemy%20Info))) (.PatrolData (Utilities|Struct|BreakStruct_Enemy_Speed_Characteristics _returnvalue_3)) (.ChaseData (Utilities|Struct|BreakStruct_Enemy_Speed_Characteristics _returnvalue_3)) (.Characteristics (Utilities|Struct|BreakStruct_Enemy_Info (Variables|EnemyInfo|GetEnemy%20Info))) (.Melee_Info (Utilities|Struct|BreakStruct_Enemy_Info (Variables|EnemyInfo|GetEnemy%20Info))) (.Ranged_Info (Utilities|Struct|BreakStruct_Enemy_Info (Variables|EnemyInfo|GetEnemy%20Info))) (.Ground_Info (Utilities|Struct|BreakStruct_Enemy_Info (Variables|EnemyInfo|GetEnemy%20Info))) (.Flying_Info (Utilities|Struct|BreakStruct_Enemy_Info (Variables|EnemyInfo|GetEnemy%20Info))) (.DashLeapInfo (Utilities|Struct|BreakStruct_Enemy_Info (Variables|EnemyInfo|GetEnemy%20Info))) (.ExplodingInfo (Utilities|Struct|BreakStruct_Enemy_Info (Variables|EnemyInfo|GetEnemy%20Info))) (.Multi-BodiedInfo (Utilities|Struct|BreakStruct_Enemy_Info (Variables|EnemyInfo|GetEnemy%20Info))) (.ShotEnemyInfo (Utilities|Struct|BreakStruct_Enemy_Info (Variables|EnemyInfo|GetEnemy%20Info)))))))
        (elif (Utilities|Array|ContainsItem (Utilities|Struct|BreakStruct_Enemy_Info (Variables|EnemyInfo|GetEnemy%20Info)) "NewEnumerator9")
          (bind _returnvalue_4 (Utilities|GetDataTableRow "/Game/Characters/Enemies/AI/Structs_Data_Tables/Characteristic_Data/Speed/DT_Enemy_Speed_Characteristics.DT_Enemy_Speed_Characteristics" "Fast")
            (:then
              (Variables|EnemyInfo|SetEnemy%20Info (Utilities|Struct|MakeStruct_Enemy_Info (.HealthInfo (Utilities|Struct|BreakStruct_Enemy_Info (Variables|EnemyInfo|GetEnemy%20Info))) (.SightInfo (Utilities|Struct|BreakStruct_Enemy_Info (Variables|EnemyInfo|GetEnemy%20Info))) (.HearingInfo (Utilities|Struct|BreakStruct_Enemy_Info (Variables|EnemyInfo|GetEnemy%20Info))) (.LoseAwarenessTime (Utilities|Struct|BreakStruct_Enemy_Info (Variables|EnemyInfo|GetEnemy%20Info))) (.Should_Patrol (Utilities|Struct|BreakStruct_Enemy_Info (Variables|EnemyInfo|GetEnemy%20Info))) (.PatrolData (Utilities|Struct|BreakStruct_Enemy_Speed_Characteristics _returnvalue_4)) (.ChaseData (Utilities|Struct|BreakStruct_Enemy_Speed_Characteristics _returnvalue_4)) (.Characteristics (Utilities|Struct|BreakStruct_Enemy_Info (Variables|EnemyInfo|GetEnemy%20Info))) (.Melee_Info (Utilities|Struct|BreakStruct_Enemy_Info (Variables|EnemyInfo|GetEnemy%20Info))) (.Ranged_Info (Utilities|Struct|BreakStruct_Enemy_Info (Variables|EnemyInfo|GetEnemy%20Info))) (.Ground_Info (Utilities|Struct|BreakStruct_Enemy_Info (Variables|EnemyInfo|GetEnemy%20Info))) (.Flying_Info (Utilities|Struct|BreakStruct_Enemy_Info (Variables|EnemyInfo|GetEnemy%20Info))) (.DashLeapInfo (Utilities|Struct|BreakStruct_Enemy_Info (Variables|EnemyInfo|GetEnemy%20Info))) (.ExplodingInfo (Utilities|Struct|BreakStruct_Enemy_Info (Variables|EnemyInfo|GetEnemy%20Info))) (.Multi-BodiedInfo (Utilities|Struct|BreakStruct_Enemy_Info (Variables|EnemyInfo|GetEnemy%20Info))) (.ShotEnemyInfo (Utilities|Struct|BreakStruct_Enemy_Info (Variables|EnemyInfo|GetEnemy%20Info)))))))))))
  (Variables|Health|SetHealth_Info (Utilities|Struct|MakeStruct_Health_Info (.Starting_Health (Utilities|Struct|BreakStruct_Health_Info (Utilities|Struct|BreakStruct_Enemy_Info (Variables|EnemyInfo|GetEnemy%20Info)))) (.Max_Health (Utilities|Struct|BreakStruct_Health_Info (Utilities|Struct|BreakStruct_Enemy_Info (Variables|EnemyInfo|GetEnemy%20Info)))) (.One_Shot_Protection (Utilities|Struct|BreakStruct_Health_Info (Utilities|Struct|BreakStruct_Enemy_Info (Variables|EnemyInfo|GetEnemy%20Info)))) (.One_Shot_Protection_Info (Utilities|Struct|BreakStruct_Health_Info (Utilities|Struct|BreakStruct_Enemy_Info (Variables|EnemyInfo|GetEnemy%20Info)))) (select (Utilities|Array|ContainsItem (Utilities|Struct|BreakStruct_Enemy_Info (Variables|EnemyInfo|GetEnemy%20Info)) "NewEnumerator10") "NewEnumerator2" (.Death_Type (Utilities|Struct|BreakStruct_Health_Info (Utilities|Struct|BreakStruct_Enemy_Info (Variables|EnemyInfo|GetEnemy%20Info))))) (.ExplodeInfo (Utilities|Struct|BreakStruct_Health_Info (Utilities|Struct|BreakStruct_Enemy_Info (Variables|EnemyInfo|GetEnemy%20Info))))))
  (if (Utilities|Array|ContainsItem (Utilities|Struct|BreakStruct_Enemy_Info (Variables|EnemyInfo|GetEnemy%20Info)) "NewEnumerator3")
    (Variables|/Script/Engine.CharacterMovementComponent|SetDefaultLandMovementMode _charactermovement "MOVE_Flying")
    (Variables|/Script/Engine.CharacterMovementComponent|SetGravityScale _charactermovement 0.0)
    (bind _returnvalue_5 (AddComponent|AddBPCFlyingGravityAuto-Toggler))
    (else
      (Variables|/Script/Engine.CharacterMovementComponent|SetDefaultLandMovementMode _charactermovement "MOVE_Walking")
      (Variables|/Script/Engine.CharacterMovementComponent|SetGravityScale _charactermovement 1.75)
      (Utilities|IsValid _returnvalue_5
        (:Is%20Valid
          (Components|DestroyComponent _returnvalue_5))))))

(fn GetAiming
  (return (Variables|/Game/Weapons/Actor_Components/BPC_Aim.BPC_Aim_C|GetAiming? (Variables|Default|GetBPC_Aim))))

(fn GetCapsuleComponent
  (return (Variables|Collision|GetCapsuleComponent)))

(fn GetCharacteristics
  (return (.Characteristics (Utilities|Struct|BreakStruct_Enemy_Info (Variables|EnemyInfo|GetEnemy%20Info)))))

(fn GetChasingInfo
  (return (.ChasingInfo (Utilities|Struct|BreakStruct_Enemy_Info (Variables|EnemyInfo|GetEnemy%20Info)))))

(fn GetCurrentComboIndex
  (return (Variables|/Game/Weapons/Actor_Components/BPC_Melee_Attack.BPC_Melee_Attack_C|GetCombo_Count (Variables|Default|GetBPC_Melee_Attack))))

(fn GetEnemyInfo
  (return (Variables|EnemyInfo|GetEnemy%20Info)))

(fn GetHasStarterWeapon
  (return (Variables|StartingWeaponry|GetHas_Starter_Weapon)))

(fn GetHealthInfo
  (return (Variables|Health|GetHealth_Info)))

(fn GetHealthWidget
  (return 0))

(fn GetHitbox
  (return (Variables|Collision|GetCapsuleComponent)))

(fn GetLerpingMovementSpeed
  (return (Variables|Movement|GetLerping%20Movement%20Speed)))

(fn GetMeleeAttacking
  (bind _basics (Class|BPIWeapon|GetBasicInfo(Message) (Variables|/Game/Weapons/Actor_Components/BPC_Weaponry.BPC_Weaponry_C|GetEquipped_Weapon (Variables|Default|GetBPC_Weaponry))))
  (return (and (not (.ranged _basics)) (Variables|/Game/Weapons/Actor_Components/BPC_Attack_Handler.BPC_Attack_Handler_C|GetAttacking (Variables|Default|GetBPC_Attack_Handler)))))

(fn GetMeleeWeaponName
  (bind _basics (Class|BPIWeapon|GetBasicInfo(Message) (Variables|/Game/Weapons/Actor_Components/BPC_Weaponry.BPC_Weaponry_C|GetEquipped_Weapon (Variables|Default|GetBPC_Weaponry))))
  (return (.name _basics)))

(fn GetMesh
  (return (Variables|Character|GetMesh)))

(fn GetPatrolInfo
  (return (.Patrol_Info (Utilities|Struct|BreakStruct_Enemy_Info (Variables|EnemyInfo|GetEnemy%20Info)))))

(fn GetSliding
  (return (Variables|/Game/Movement/Sliding/BPC_Slide.BPC_Slide_C|GetSliding (Variables|Default|GetBPC_Slide))))

(fn GetSlidingInfo
  (return (Variables|Movement|GetSliding_Info)))

(fn GetSprintInfo
  (return (Variables|Movement|GetSprinting_Info)))

(fn GetStarterWeapon
  (return (Variables|StartingWeaponry|GetStarter_Weapon)))

(fn GetStartingWeapons
  (return (Variables|StartingWeaponry|GetStarting_Weapons)))

(fn GetUnarmedAttackInfo
  (return ""))

(fn GetWall-RunInfo
  (return (Variables|Movement|GetWall-Running_Info)))

(fn GetWeaponName
  (bind _basics (Class|BPIWeapon|GetBasicInfo(Message) (Variables|/Game/Weapons/Actor_Components/BPC_Weaponry.BPC_Weaponry_C|GetEquipped_Weapon (Variables|Default|GetBPC_Weaponry))))
  (return (.name _basics)))