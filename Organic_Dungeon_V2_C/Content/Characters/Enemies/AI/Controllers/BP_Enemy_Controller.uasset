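; AI controller for enemies that runs the main enemy behavior tree and tracks whether the pawn senses a player.
; On BeginPlay it caches the pawn's enemy info, fetching it again after a short delay.
; Perception updates record player location and reference, filtering sight and hearing by the enemy's abilities and range.
; A DoOnce-gated delay clears awareness after losing the player, with getters and setters exposing this state.
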(event OnTargetPerceptionUpdated(AIPerception)
  (params (Actor :type Actor%20Object%20Reference) (Stimulus :type AI%20Stimulus%20Structure))
  (bind (_age _expirationage _strength _stimuluslocation _receiverlocation _tag _bsuccessfullysensed) (Utilities|Struct|BreakAIStimulus Stimulus))
  (bind _enemy_info (Variables|Info|GetEnemy_Info))
  (bind (_sightinfo _hearinginfo _characteristics) (Utilities|Struct|BreakStruct_Enemy_Info _enemy_info))
  (bind (_cansee _sightdistance) (Utilities|Struct|BreakStruct_Enemy_Sight_Info _sightinfo))
  (bind (_canhear _hearingrange) (Utilities|Struct|BreakStruct_Enemy_Hearing_Info _hearinginfo))
  (if (Utilities|DoesObjectImplementInterface Actor "/Game/Characters/Player/BPI_Player.BPI_Player_C")
    (Variables|Sense|SetLastKnownCharacterLocation _stimuluslocation)
    (bind _returnvalue (Class|AIPerceptionSystem|GetSenseClassforStimulus Stimulus))
    (Variables|Sense|SetChasing_Character Actor)
    (if (Math|Boolean|ANDBoolean _bsuccessfullysensed (or (select (== _returnvalue "/Script/AIModule.AISense_Sight") (and _cansee (Utilities|Array|ContainsItem _characteristics "NewEnumerator11")) (and _canhear (Utilities|Array|ContainsItem _characteristics "NewEnumerator12"))) (Variables|Sense|GetSensing_Character)) (<= (Math|Vector|Distance(Vector) _stimuluslocation (Transformation|GetActorLocation (Pawn|GetControlledPawn))) (Math|Float|SelectFloat _sightdistance _hearingrange (== _returnvalue "/Script/AIModule.AISense_Sight"))))
      (Variables|Sense|SetSensing_Character true)
      (goto _label Reset)
      (elif (Variables|Sense|GetSensing_Character)
        (Utilities|FlowControl|DoOnce false :!label _label
          (:Completed
            (Utilities|FlowControl|Delay (.LoseAwarenessTime (Utilities|Struct|BreakStruct_Enemy_Info (Variables|Info|GetEnemy_Info))))
            (Variables|Sense|SetSensing_Character false)))
        (else
          (Utilities|FlowControl|Sequence
            (:then_0
              (goto _label Reset))
            (:then_1
              (Variables|Sense|SetSensing_Character false))))))))

(event EventSetCanSenseCharacter
  (params (Can :type Boolean))
  (Variables|Sense|SetSensing_Character Can))

(event EventSetChasingCharacterRef
  (params (New%20Character :type Actor%20Object%20Reference))
  (Variables|Sense|SetChasing_Character New%20Character))

(event EventBeginPlay
  ;[1 1 1] Run the behaviour tree on begin play
  (AI|RunBehaviorTree "/Game/Characters/Enemies/AI/Trees/BT_Enemy_Main.BT_Enemy_Main")
  (bind _all_enemy_info (Class|BPIEnemy|GetEnemyInfo(Message) (Pawn|GetControlledPawn)))
  (Variables|Info|SetEnemy_Info _all_enemy_info)
  (Utilities|FlowControl|Delay 0.2)
  (bind _all_enemy_info_2 (Class|BPIEnemy|GetEnemyInfo(Message) (Pawn|GetControlledPawn)))
  (Variables|Info|SetEnemy_Info _all_enemy_info_2))

(fn ConstructionScript)

(fn CanSenseCharacter
  (return (Variables|Sense|GetSensing_Character)))

(fn GetChasingCharacterRef
  (return (Variables|Sense|GetChasing_Character)))

(fn GetLastPlayerPosition
  (return (Variables|Sense|GetLastKnownCharacterLocation)))