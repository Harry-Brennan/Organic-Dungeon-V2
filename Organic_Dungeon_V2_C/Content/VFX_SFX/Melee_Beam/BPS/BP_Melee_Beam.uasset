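; Melee beam actor for a weapon's heavy attack that plays spawn audio, alerts AI with noise, configures its Niagara effect and self-destructs after three seconds.
; Niagara exports particle data back to the Blueprint, which sphere-traces at each position, ignoring instigator and weapon, and hits each actor once.
; Characters take weapon-defined damage, knockback and blood effects, while physics objects receive impulses.
; Every exported particle also triggers impact sound and slight camera shake.
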(event EventBeginPlay
  (bind _returnvalue (Transformation|GetActorLocation))
  (Audio|PlaySoundatLocation "/Game/VFX_SFX/Melee_Beam/Audio/Melee_Beam_Spawn_SC.Melee_Beam_Spawn_SC" _returnvalue "0, 0, 0" 1.0 1.0 0.0 0 0 0 0)
  (Class|AISenseHearing|ReportNoiseEvent _returnvalue 4.0 (Variables|Default|GetCharacter_Instigator) 0.0 "None")
  (Class|NiagaraComponent|SetVariableObject (Variables|Default|GetNiagara) "user.BP_Beam" self)
  (Class|NiagaraComponent|SetVariableVec2 (Variables|Default|GetNiagara) "user.Beam_Size" (Variables|Default|GetBeam_Size))
  (Niagara|SetNiagaraVariable(LinearColor) (Variables|Default|GetNiagara) "user.Beam_Colour" (Variables|Default|GetBeam_Colour))
  (Utilities|FlowControl|Delay 3.0)
  (Actor|DestroyActor))

(event EventParticleData
  (params (Data :type Array%20of%20Basic%20Particle%20Data%20Structures) (NiagaraSystem :type Niagara%20System%20Object%20Reference) (SimulationPositionOffset :type Vector%20%28by%20ref%29 :default "0, 0, 0"))
  (for _array_element Data
    (Utilities|FlowControl|Sequence
      (:then_0
        (bind (_outhits _returnvalue) (Collision|MultiSphereTraceForObjects (.Position (Utilities|Struct|BreakBasicParticleData _array_element)) (.Position (Utilities|Struct|BreakBasicParticleData _array_element)) (/ (.X (Math|Vector2D|BreakVector2D (Variables|Default|GetBeam_Size))) 1e+01) (Utilities|Array|MakeArray "ObjectTypeQuery3" "ObjectTypeQuery4" "ObjectTypeQuery8" "ObjectTypeQuery10" "ObjectTypeQuery9" "ObjectTypeQuery11") false (Utilities|Array|MakeArray (Variables|Default|GetCharacter_Instigator) (Variables|Default|GetWeapon_Instigator)) "None"))
        (if _returnvalue
          (bind _melee_info (Class|BPIMeleeWeapon|GetMeleeInfo(Message) (Variables|Default|GetWeapon_Instigator)))
          (for _array_element_2 _outhits
            (if (not (Utilities|Array|ContainsItem (Variables|Default|GetHit_Actors) (.HitActor (Collision|BreakHitResult _array_element_2))))
              (Utilities|Array|Add (Variables|Default|GetHit_Actors) (.HitActor (Collision|BreakHitResult _array_element_2)))
              (switch Utilities|FlowControl|Switch|SwitchonECollisionChannel (Collision|GetCollisionObjectType (.HitComponent (Collision|BreakHitResult _array_element_2)))
                (:ECC_Pawn
                  (Default|TakeDamage (Actor|GetComponentbyClass (.HitActor (Collision|BreakHitResult _array_element_2)) "/Game/Health/BPs/BPC_Health.BPC_Health_C") (.BeamDamage (Utilities|Struct|BreakStruct_Heavy_Attack_Info (.HeavyAttackInfo (Utilities|Struct|BreakStruct_Melee_Weapon _melee_info)))) (.Location (Collision|BreakHitResult _array_element_2)) (.HitActor (Collision|BreakHitResult _array_element_2)) (Variables|Default|GetCharacter_Instigator) :!label _label)
                  (Utilities|FlowControl|Sequence
                    (:then_0
                      (Camera|PlayWorldCameraShake "/Game/Weapons/BPs/BP_Melee_Hit_Camera_Shake.BP_Melee_Hit_Camera_Shake_C" (.Location (Collision|BreakHitResult _array_element_2)) (* (.BeamDamage (Utilities|Struct|BreakStruct_Heavy_Attack_Info (.HeavyAttackInfo (Utilities|Struct|BreakStruct_Melee_Weapon _melee_info)))) 1e+01) (* (* (.BeamDamage (Utilities|Struct|BreakStruct_Heavy_Attack_Info (.HeavyAttackInfo (Utilities|Struct|BreakStruct_Melee_Weapon _melee_info)))) 1e+01) 1.25)))
                    (:then_1
                      (Utilities|IsValid (Actor|GetComponentbyClass (.HitActor (Collision|BreakHitResult _array_element_2)) "/Game/VFX_SFX/Blood_Splatter/BPS/BPC_Blood_Effect.BPC_Blood_Effect_C")
                        (:Is%20Valid
                          (Default|BloodEffect (Actor|GetComponentbyClass (.HitActor (Collision|BreakHitResult _array_element_2)) "/Game/VFX_SFX/Blood_Splatter/BPS/BPC_Blood_Effect.BPC_Blood_Effect_C") (.Location (Collision|BreakHitResult _array_element_2)) (* (.ImpactNormal (Collision|BreakHitResult _array_element_2)) -1.0) (.HitActor (Collision|BreakHitResult _array_element_2)) (.BeamDamage (Utilities|Struct|BreakStruct_Heavy_Attack_Info (.HeavyAttackInfo (Utilities|Struct|BreakStruct_Melee_Weapon _melee_info)))))
                          (Audio|PlaySoundatLocation "/Game/VFX_SFX/Blood_Splatter/Audio/Impact_Audio/Body_Impact_SC.Body_Impact_SC" (.Location (Collision|BreakHitResult _array_element_2)) "0, 0, 0" 1.0 1.0 0.0 0 0 0 0))))
                    (:then_2
                      (bind _ascharacter (Utilities|Casting|CastToCharacter (.HitActor (Collision|BreakHitResult _array_element_2))))
                      (Character|LaunchCharacter _ascharacter (Math|Vector|MakeVector (.x (/ (Math|Vector|MakeVector (.X (Class|KismetMathLibrary|BreakVector3f (* (Math|Vector|GetForwardVector (Math|Rotator|FindLookatRotation (.ImpactPoint (Collision|BreakHitResult _array_element_2)) (Transformation|GetActorLocation (.HitActor (Collision|BreakHitResult _array_element_2))))) 5e+03))) (.Y (Class|KismetMathLibrary|BreakVector3f (* (Math|Vector|GetForwardVector (Math|Rotator|FindLookatRotation (.ImpactPoint (Collision|BreakHitResult _array_element_2)) (Transformation|GetActorLocation (.HitActor (Collision|BreakHitResult _array_element_2))))) 5e+03))) 0.0) 5.0)) (.y (/ (Math|Vector|MakeVector (.X (Class|KismetMathLibrary|BreakVector3f (* (Math|Vector|GetForwardVector (Math|Rotator|FindLookatRotation (.ImpactPoint (Collision|BreakHitResult _array_element_2)) (Transformation|GetActorLocation (.HitActor (Collision|BreakHitResult _array_element_2))))) 5e+03))) (.Y (Class|KismetMathLibrary|BreakVector3f (* (Math|Vector|GetForwardVector (Math|Rotator|FindLookatRotation (.ImpactPoint (Collision|BreakHitResult _array_element_2)) (Transformation|GetActorLocation (.HitActor (Collision|BreakHitResult _array_element_2))))) 5e+03))) 0.0) 5.0)) (/ (.Z (Class|KismetMathLibrary|BreakVector3f (* (Math|Vector|GetForwardVector (Math|Rotator|FindLookatRotation (.ImpactPoint (Collision|BreakHitResult _array_element_2)) (Transformation|GetActorLocation (.HitActor (Collision|BreakHitResult _array_element_2))))) 5e+03))) 4.0)) true true))))
                (:ECC_PhysicsBody
                  (Physics|AddImpulse (.HitComponent (Collision|BreakHitResult _array_element_2)) (* (Math|Vector|GetForwardVector (Math|Rotator|FindLookatRotation (.ImpactPoint (Collision|BreakHitResult _array_element_2)) (Transformation|GetActorLocation (.HitActor (Collision|BreakHitResult _array_element_2))))) 1.25e+03) "None" true :!label _label_2))
                (:ECC_GameTraceChannel2
                  (goto _label))
                (:ECC_GameTraceChannel3
                  (goto _label_2))
                (:ECC_GameTraceChannel4
                  (goto _label)))))))
      (:then_1
        (Camera|PlayWorldCameraShake "/Game/Movement/BP_Slight_Camera_Shake.BP_Slight_Camera_Shake_C" (.Position (Utilities|Struct|BreakBasicParticleData _array_element)) 2.5e+02 5e+02)
        (Audio|PlaySoundatLocation "/Game/VFX_SFX/Melee_Beam/Audio/Melee_Beam_Impact_SC.Melee_Beam_Impact_SC" (.Position (Utilities|Struct|BreakBasicParticleData _array_element)) "0, 0, 0" 1.0 1.0 0.0 0 0 0 0)))))

(fn ConstructionScript)