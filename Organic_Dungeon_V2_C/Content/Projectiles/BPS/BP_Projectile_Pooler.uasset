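; Projectile pool actor that supplies reusable BP_Projectile actors for shots instead of spawning one per shot.
; On BeginPlay it spawns MaxProjectiles projectiles, stores them in ProjectilePool and deactivates each.
; ShootProjectile activates the slot at CurrentProjectileIndex with shot transform, projectile, falloff and piercing data, then advances the index round-robin.
; A still-active projectile is reused anyway, with only a debug print as warning.
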(event Custom|Shoot%20Projectile
  (params (Projectile%20Info :type Struct%20Projectiles%20Structure) (Shot%20Location :type Vector) (Shot%20Rotation :type Rotator) (Falloff%20Info :type Struct%20Projectile%20Falloff%20Info%20Structure) (Piercing :type Boolean))
  (if (Variables|/Game/Projectiles/BPS/BP_Projectile.BP_Projectile_C|GetActive (Utilities|Array|Get(acopy) (Variables|PoolInfo|GetProjectile%20Pool) (Variables|PoolInfo|GetCurrent%20Projectile%20Index)))
    (Development|PrintString "USING A STILL ACTIVE PROJECTILE"))
  (Default|ActivateProjectile (Utilities|Array|Get(acopy) (Variables|PoolInfo|GetProjectile%20Pool) (Variables|PoolInfo|GetCurrent%20Projectile%20Index)) Projectile%20Info Shot%20Location Shot%20Rotation Falloff%20Info Piercing)
  (bind _result (Math|Integer|IncrementInt (Variables|PoolInfo|GetCurrent%20Projectile%20Index))
    (:%20%20
      (if (>= _result (Variables|PoolInfo|GetMax%20Projectiles))
        (Variables|PoolInfo|SetCurrent%20Projectile%20Index 0)))))

(event EventBeginPlay
  (for _index (range 1 (Variables|PoolInfo|GetMax%20Projectiles))
    (bind _returnvalue (Game|SpawnActorfromClass :Class "/Game/Projectiles/BPS/BP_Projectile.BP_Projectile_C" :CollisionHandlingOverride "Undefined" :TransformScaleMethod "MultiplyWithRoot" :Instigator 0))
    (Utilities|Array|Add (Variables|PoolInfo|GetProjectile%20Pool) _returnvalue)
    (Default|DeactivateProjectile _returnvalue)))

(fn ConstructionScript)