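; Configurable projectile actor that takes speed, gravity and mesh from its projectile info and DT_Projectiles, expiring at max range when falloff is enabled.
; On impact, its hit effect selects bullet-hole decals with particles and physics push, an explosion via BPCExplode, and/or distance-falloff damage through BPC_Health with blood effects.
; Piercing rounds use an overlap collision profile to keep flying, tracing backwards on overlap end to add exit holes.
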(event OnProjectileStop(ProjectileMovement)
  (params (ImpactResult :type Hit%20Result%20Structure%20%28by%20ref%29))
  (bind _returnvalue (Math|Random|RandomFloatinRange 5.0 15.0))
  (bind _returnvalue_2 (Math|Random|RandomFloatinRange 5.0 15.0))
  (bind _projectile_info (Variables|Default|GetProjectile_Info))
  (bind _projectile_info_2 (Variables|Default|GetProjectile_Info))
  (Utilities|Time|ClearandInvalidateTimerbyHandle (Variables|Default|GetEnd%20of%20Life%20Timer))
  (Variables|Default|SetHit%20Info ImpactResult)
  (Variables|Default|SetCurrently%20Piercing%20Object false)
  (Variables|HitInfo|SetHit%20Location (.Location (Collision|BreakHitResult (Variables|Default|GetHit%20Info))))
  (Variables|HitInfo|SetHit%20Impact%20Point (.ImpactPoint (Collision|BreakHitResult (Variables|Default|GetHit%20Info))))
  (Variables|HitInfo|SetHit%20Impact%20Normal (.ImpactNormal (Collision|BreakHitResult (Variables|Default|GetHit%20Info))))
  (Variables|HitInfo|SetHit%20Actor (.HitActor (Collision|BreakHitResult (Variables|Default|GetHit%20Info))))
  (Variables|HitInfo|SetHit%20Component (.HitComponent (Collision|BreakHitResult (Variables|Default|GetHit%20Info))))
  (switch Utilities|FlowControl|Switch|SwitchonEnum_On_Hit_Effects (.onhiteffect _projectile_info)
    (:NewEnumerator0
      (switch Utilities|FlowControl|Switch|SwitchonECollisionChannel (Collision|GetCollisionObjectType (Variables|HitInfo|GetHit%20Component)) :!label _label
        (:ECC_WorldStatic
          (Rendering|Decal|SpawnDecalatLocation "/Game/Projectiles/Bullet_Hole/M_Bullet_Hole.M_Bullet_Hole" (Math|Vector|MakeVector _returnvalue _returnvalue _returnvalue) (Variables|HitInfo|GetHit%20Impact%20Point) (Math|Conversions|RotationFromXVector (Variables|HitInfo|GetHit%20Impact%20Normal)) 1e+01 :!label _label_2)
          (Game|SpawnActorfromClass "/Game/VFX_SFX/Realistic_Starter_VFX_Pack_Vol2/Blueprints/Spawn_Particle.Spawn_Particle_C" (Math|Transform|MakeTransform (Variables|HitInfo|GetHit%20Impact%20Point) (Math|Conversions|RotationFromXVector (Variables|HitInfo|GetHit%20Impact%20Normal)) "0.100000,0.100000,0.100000") "AlwaysSpawn" "MultiplyWithRoot" 0 1.0 false "/Game/VFX_SFX/Realistic_Starter_VFX_Pack_Vol2/Particles/Explosion/P_Explosion_Big_A.P_Explosion_Big_A" 0 :!label _label_3)
          (Audio|PlaySoundatLocation "/Game/VFX_SFX/Sounds/Bullet_Impact/Bullet_Impact_SC.Bullet_Impact_SC" (Variables|HitInfo|GetHit%20Impact%20Point) "0, 0, 0" 1.0 1.0 0.0 0 0 0 0)
          (if (not (Variables|Default|GetPiercing))
            (Actor|DestroyActor)))
        (:ECC_WorldDynamic
          (goto _label_2))
        (:ECC_Pawn
          (if (not (Variables|Default|GetPiercing)) :!label _label_4
            (Actor|DestroyActor)))
        (:ECC_PhysicsBody
          (Physics|AddForce (Variables|HitInfo|GetHit%20Component) (+ (* (Transformation|GetActorUpVector) (* (.speed _projectile_info_2) 1e+01)) (* (Transformation|GetActorForwardVector) (* (.speed _projectile_info_2) 5e+01))) "None" true :!label _label_5)
          (Class|GameplayStatics|SpawnDecalAttached "/Game/Projectiles/Bullet_Hole/M_Bullet_Hole.M_Bullet_Hole" (Math|Vector|MakeVector _returnvalue_2 _returnvalue_2 _returnvalue_2) (Variables|HitInfo|GetHit%20Component) "None" (Variables|HitInfo|GetHit%20Impact%20Point) (Math|Conversions|RotationFromXVector (Variables|HitInfo|GetHit%20Impact%20Normal)) "KeepWorldPosition" 1e+01)
          (goto _label_3))
        (:ECC_GameTraceChannel1
          (goto _label_2))
        (:ECC_GameTraceChannel2
          (goto _label_4))
        (:ECC_GameTraceChannel3
          (goto _label_5))
        (:ECC_GameTraceChannel4
          (goto _label_4))))
    (:NewEnumerator1
      (Default|Explode (Variables|Default|GetBPC_Explode) (Variables|HitInfo|GetHit%20Location) (.explosiononhit _projectile_info) true (.speed _projectile_info) (.damage _projectile_info) (not (Variables|Default|GetPiercing))))
    (:NewEnumerator2
      (bind _damage_after_falloff (CallFunction|CalculateDamageFalloff (Variables|HitInfo|GetHit%20Location) :!label _label_6))
      (CallFunction|DealDamage _damage_after_falloff (Variables|HitInfo|GetHit%20Actor) (Variables|HitInfo|GetHit%20Location) (Variables|HitInfo|GetHit%20Impact%20Normal)))
    (:NewEnumerator3
      (Utilities|FlowControl|Sequence
        (:then_0
          (goto _label_6))
        (:then_1
          (goto _label))))))

(event OnComponentBeginOverlap(StaticMesh)
  (params (OverlappedComponent :type Primitive%20Component%20Object%20Reference) (OtherActor :type Actor%20Object%20Reference) (OtherComp :type Primitive%20Component%20Object%20Reference) (OtherBodyIndex :type Integer) (bFromSweep :type Boolean) (SweepResult :type Hit%20Result%20Structure%20%28by%20ref%29))
  (bind _returnvalue (Math|Random|RandomFloatinRange 5.0 15.0))
  (bind _returnvalue_2 (Math|Random|RandomFloatinRange 5.0 15.0))
  (bind _projectile_info (Variables|Default|GetProjectile_Info))
  (bind _projectile_info_2 (Variables|Default|GetProjectile_Info))
  (if (not (Variables|Default|GetCurrently%20Piercing%20Object))
    (Variables|Default|SetHit%20Info SweepResult)
    (Variables|Default|SetCurrently%20Piercing%20Object true)
    (Variables|HitInfo|SetHit%20Location (.Location (Collision|BreakHitResult (Variables|Default|GetHit%20Info))))
    (Variables|HitInfo|SetHit%20Impact%20Point (.ImpactPoint (Collision|BreakHitResult (Variables|Default|GetHit%20Info))))
    (Variables|HitInfo|SetHit%20Impact%20Normal (.ImpactNormal (Collision|BreakHitResult (Variables|Default|GetHit%20Info))))
    (Variables|HitInfo|SetHit%20Actor (.HitActor (Collision|BreakHitResult (Variables|Default|GetHit%20Info))))
    (Variables|HitInfo|SetHit%20Component (.HitComponent (Collision|BreakHitResult (Variables|Default|GetHit%20Info))))
    (switch Utilities|FlowControl|Switch|SwitchonEnum_On_Hit_Effects (.onhiteffect _projectile_info)
      (:NewEnumerator0
        (switch Utilities|FlowControl|Switch|SwitchonECollisionChannel (Collision|GetCollisionObjectType (Variables|HitInfo|GetHit%20Component)) :!label _label
          (:ECC_WorldStatic
            (Rendering|Decal|SpawnDecalatLocation "/Game/Projectiles/Bullet_Hole/M_Bullet_Hole.M_Bullet_Hole" (Math|Vector|MakeVector _returnvalue _returnvalue _returnvalue) (Variables|HitInfo|GetHit%20Impact%20Point) (Math|Conversions|RotationFromXVector (Variables|HitInfo|GetHit%20Impact%20Normal)) 1e+01 :!label _label_2)
            (Game|SpawnActorfromClass "/Game/VFX_SFX/Realistic_Starter_VFX_Pack_Vol2/Blueprints/Spawn_Particle.Spawn_Particle_C" (Math|Transform|MakeTransform (Variables|HitInfo|GetHit%20Impact%20Point) (Math|Conversions|RotationFromXVector (Variables|HitInfo|GetHit%20Impact%20Normal)) "0.100000,0.100000,0.100000") "AlwaysSpawn" "MultiplyWithRoot" 0 1.0 false "/Game/VFX_SFX/Realistic_Starter_VFX_Pack_Vol2/Particles/Explosion/P_Explosion_Big_A.P_Explosion_Big_A" 0 :!label _label_3)
            (Audio|PlaySoundatLocation "/Game/VFX_SFX/Sounds/Bullet_Impact/Bullet_Impact_SC.Bullet_Impact_SC" (Variables|HitInfo|GetHit%20Impact%20Point) "0, 0, 0" 1.0 1.0 0.0 0 0 0 0)
            (if (not (Variables|Default|GetPiercing))
              (Actor|DestroyActor)))
          (:ECC_WorldDynamic
            (goto _label_2))
          (:ECC_Pawn
            (if (not (Variables|Default|GetPiercing)) :!label _label_4
              (Actor|DestroyActor)))
          (:ECC_PhysicsBody
            (Physics|AddForce (Variables|HitInfo|GetHit%20Component) (+ (* (Transformation|GetActorUpVector) (* (.speed _projectile_info_2) 1e+01)) (* (Transformation|GetActorForwardVector) (* (.speed _projectile_info_2) 5e+01))) "None" true :!label _label_5)
            (Class|GameplayStatics|SpawnDecalAttached "/Game/Projectiles/Bullet_Hole/M_Bullet_Hole.M_Bullet_Hole" (Math|Vector|MakeVector _returnvalue_2 _returnvalue_2 _returnvalue_2) (Variables|HitInfo|GetHit%20Component) "None" (Variables|HitInfo|GetHit%20Impact%20Point) (Math|Conversions|RotationFromXVector (Variables|HitInfo|GetHit%20Impact%20Normal)) "KeepWorldPosition" 1e+01)
            (goto _label_3))
          (:ECC_GameTraceChannel1
            (goto _label_2))
          (:ECC_GameTraceChannel2
            (goto _label_4))
          (:ECC_GameTraceChannel3
            (goto _label_5))
          (:ECC_GameTraceChannel4
            (goto _label_4))))
      (:NewEnumerator1
        (Default|Explode (Variables|Default|GetBPC_Explode) (Variables|HitInfo|GetHit%20Location) (.explosiononhit _projectile_info) true (.speed _projectile_info) (.damage _projectile_info) (not (Variables|Default|GetPiercing))))
      (:NewEnumerator2
        (bind _damage_after_falloff (CallFunction|CalculateDamageFalloff (Variables|HitInfo|GetHit%20Location) :!label _label_6))
        (CallFunction|DealDamage _damage_after_falloff (Variables|HitInfo|GetHit%20Actor) (Variables|HitInfo|GetHit%20Location) (Variables|HitInfo|GetHit%20Impact%20Normal)))
      (:NewEnumerator3
        (Utilities|FlowControl|Sequence
          (:then_0
            (goto _label_6))
          (:then_1
            (goto _label)))))))

(event OnComponentEndOverlap(StaticMesh)
  (params (OverlappedComponent :type Primitive%20Component%20Object%20Reference) (OtherActor :type Actor%20Object%20Reference) (OtherComp :type Primitive%20Component%20Object%20Reference) (OtherBodyIndex :type Integer))
  (bind _returnvalue (Math|Random|RandomFloatinRange 5.0 15.0))
  (bind _returnvalue_2 (Math|Random|RandomFloatinRange 5.0 15.0))
  (bind _returnvalue_3 (Transformation|GetActorLocation))
  (bind _projectile_info (Variables|Default|GetProjectile_Info))
  (if (== OtherActor (.HitActor (Collision|BreakHitResult (stale OnComponentBeginOverlap(StaticMesh) SweepResult))))
    (Variables|Default|SetCurrently%20Piercing%20Object false)
    (switch Utilities|FlowControl|Switch|SwitchonECollisionChannel (Collision|GetCollisionObjectType (.HitComponent (Collision|BreakHitResult (stale OnComponentBeginOverlap(StaticMesh) SweepResult))))
      (:ECC_WorldStatic
        _)
      (:ECC_WorldDynamic
        _)
      (:ECC_PhysicsBody
        _)
      (:ECC_Destructible
        _)
      (:ECC_GameTraceChannel1
        _)
      (:ECC_GameTraceChannel3
        _))
    (bind (_outhit _returnvalue_4) (Collision|LineTraceByChannel _returnvalue_3 (+ _returnvalue_3 (* (Transformation|GetActorForwardVector) -1.5e+02)) "TraceTypeQuery1" false 0 "ForDuration"))
    (if _returnvalue_4
      (Variables|Default|SetHit%20Info _outhit)
      (Variables|HitInfo|SetHit%20Location (.Location (Collision|BreakHitResult (Variables|Default|GetHit%20Info))))
      (Variables|HitInfo|SetHit%20Impact%20Point (.ImpactPoint (Collision|BreakHitResult (Variables|Default|GetHit%20Info))))
      (Variables|HitInfo|SetHit%20Impact%20Normal (.ImpactNormal (Collision|BreakHitResult (Variables|Default|GetHit%20Info))))
      (Variables|HitInfo|SetHit%20Actor (.HitActor (Collision|BreakHitResult (Variables|Default|GetHit%20Info))))
      (Variables|HitInfo|SetHit%20Component (.HitComponent (Collision|BreakHitResult (Variables|Default|GetHit%20Info))))
      (switch Utilities|FlowControl|Switch|SwitchonEnum_On_Hit_Effects (Utilities|Struct|BreakStruct_Projectiles (Variables|Default|GetProjectile_Info))
        (:NewEnumerator0
          _)
        (:NewEnumerator3
          _))
      (switch Utilities|FlowControl|Switch|SwitchonECollisionChannel (Collision|GetCollisionObjectType (Variables|HitInfo|GetHit%20Component))
        (:ECC_WorldStatic
          (Rendering|Decal|SpawnDecalatLocation "/Game/Projectiles/Bullet_Hole/M_Bullet_Hole.M_Bullet_Hole" (Math|Vector|MakeVector _returnvalue _returnvalue _returnvalue) (Variables|HitInfo|GetHit%20Impact%20Point) (Math|Conversions|RotationFromXVector (Variables|HitInfo|GetHit%20Impact%20Normal)) 1e+01 :!label _label)
          (Game|SpawnActorfromClass "/Game/VFX_SFX/Realistic_Starter_VFX_Pack_Vol2/Blueprints/Spawn_Particle.Spawn_Particle_C" (Math|Transform|MakeTransform (Variables|HitInfo|GetHit%20Impact%20Point) (Math|Conversions|RotationFromXVector (Variables|HitInfo|GetHit%20Impact%20Normal)) "0.100000,0.100000,0.100000") "AlwaysSpawn" "MultiplyWithRoot" 0 1.0 false "/Game/VFX_SFX/Realistic_Starter_VFX_Pack_Vol2/Particles/Explosion/P_Explosion_Big_A.P_Explosion_Big_A" 0 :!label _label_2)
          (Audio|PlaySoundatLocation "/Game/VFX_SFX/Sounds/Bullet_Impact/Bullet_Impact_SC.Bullet_Impact_SC" (Variables|HitInfo|GetHit%20Impact%20Point) "0, 0, 0" 1.0 1.0 0.0 0 0 0 0)
          (if (not (Variables|Default|GetPiercing))
            (Actor|DestroyActor)))
        (:ECC_WorldDynamic
          (goto _label))
        (:ECC_Pawn
          (if (not (Variables|Default|GetPiercing)) :!label _label_3
            (Actor|DestroyActor)))
        (:ECC_PhysicsBody
          (Physics|AddForce (Variables|HitInfo|GetHit%20Component) (+ (* (Transformation|GetActorUpVector) (* (.speed _projectile_info) 1e+01)) (* (Transformation|GetActorForwardVector) (* (.speed _projectile_info) 5e+01))) "None" true :!label _label_4)
          (Class|GameplayStatics|SpawnDecalAttached "/Game/Projectiles/Bullet_Hole/M_Bullet_Hole.M_Bullet_Hole" (Math|Vector|MakeVector _returnvalue_2 _returnvalue_2 _returnvalue_2) (Variables|HitInfo|GetHit%20Component) "None" (Variables|HitInfo|GetHit%20Impact%20Point) (Math|Conversions|RotationFromXVector (Variables|HitInfo|GetHit%20Impact%20Normal)) "KeepWorldPosition" 1e+01)
          (goto _label_2))
        (:ECC_GameTraceChannel1
          (goto _label))
        (:ECC_GameTraceChannel2
          (goto _label_3))
        (:ECC_GameTraceChannel3
          (goto _label_4))
        (:ECC_GameTraceChannel4
          (goto _label_3))))))

(event Custom|Projectile%20END%20OF%20LIFE
  (bind _projectile_info (Variables|Default|GetProjectile_Info))
  (switch Utilities|FlowControl|Switch|SwitchonEnum_On_Hit_Effects (.onhiteffect (Variables|Default|GetProjectile_Info))
    (:NewEnumerator0
      (Game|SpawnActorfromClass "/Game/VFX_SFX/Realistic_Starter_VFX_Pack_Vol2/Blueprints/Spawn_Particle.Spawn_Particle_C" (Math|Transform|MakeTransform (Transformation|GetActorLocation) "0, 0, 0" "0.100000,0.100000,0.100000") "AlwaysSpawn" "MultiplyWithRoot" 0 1.0 false "/Game/VFX_SFX/Realistic_Starter_VFX_Pack_Vol2/Particles/Explosion/P_Explosion_Big_A.P_Explosion_Big_A" 0 :!label _label)
      (Actor|DestroyActor))
    (:NewEnumerator1
      (Default|Explode (Variables|Default|GetBPC_Explode) (Transformation|GetActorLocation) (.explosiononhit _projectile_info) true (.speed _projectile_info) (.damage _projectile_info) true))
    (:NewEnumerator2
      (goto _label))
    (:NewEnumerator3
      (goto _label))))

(event EventBeginPlay
  (bind _projectile_info (Variables|Default|GetProjectile_Info))
  (bind _falloff_info (Variables|Default|GetFalloff%20Info))
  (bind _projectilemovement (Variables|Default|GetProjectileMovement))
  (bind (_hasfalloff _maxrange) (Utilities|Struct|BreakStruct_Projectile_Falloff_Info _falloff_info))
  (bind _returnvalue (/ _maxrange (.speed _projectile_info)))
  (bind _output_get (Variables|/Script/Engine.ProjectileMovementComponent|SetInitialSpeed _projectilemovement (.speed _projectile_info)))
  (Variables|/Script/Engine.ProjectileMovementComponent|SetMaxSpeed _projectilemovement _output_get)
  (Components|StaticMesh|SetStaticMesh (Variables|Default|GetStaticMesh) (.mesh _projectile_info))
  (Variables|/Script/Engine.ProjectileMovementComponent|SetProjectileGravityScale (Variables|Default|GetProjectileMovement) (.gravity _projectile_info))
  (if _hasfalloff
    (Development|PrintString (Utilities|String|ToString(Float) _returnvalue))
    (bind _returnvalue_2 (Utilities|Time|SetTimerbyEvent (delegate Custom|Projectile%20END%20OF%20LIFE) _returnvalue))
    (Variables|Default|SetEnd%20of%20Life%20Timer _returnvalue_2)))

(fn ConstructionScript
  (bind _projectile_info (Variables|Default|GetProjectile_Info))
  (bind _projectilemovement (Variables|Default|GetProjectileMovement))
  (bind _staticmesh (Variables|Default|GetStaticMesh))
  (bind _returnvalue (Utilities|GetDataTableRow "/Game/Projectiles/Structs_DataTables/DT_Projectiles.DT_Projectiles" (Utilities|String|StringToName (Utilities|String|EnumtoString (.name _projectile_info))))
    (:then
      (bind _output_get (Variables|/Script/Engine.ProjectileMovementComponent|SetInitialSpeed _projectilemovement (.speed _projectile_info)))
      (Variables|/Script/Engine.ProjectileMovementComponent|SetMaxSpeed _projectilemovement _output_get)
      (Components|StaticMesh|SetStaticMesh (Variables|Default|GetStaticMesh) (.mesh _returnvalue))
      (Variables|/Script/Engine.ProjectileMovementComponent|SetProjectileGravityScale (Variables|Default|GetProjectileMovement) (.gravity _projectile_info))
      (if (Variables|Default|GetPiercing)
        (Collision|SetCollisionProfileName _staticmesh "Projectile_Piercing" true :!class /Script/Engine.PrimitiveComponent)
        (else
          (Collision|SetCollisionProfileName _staticmesh "Base_Projectile_Trace" true :!class /Script/Engine.PrimitiveComponent))))))

(fn DealDamage
  (params (Damage :type Float%20%28double-precision%29) (To%20Who :type Actor%20Object%20Reference) (Where :type Vector) (Normal :type Vector))
  (bind _returnvalue (Actor|GetComponentbyClass To%20Who "/Game/Health/BPs/BPC_Health.BPC_Health_C"))
  (bind _returnvalue_2 (Actor|GetComponentbyClass To%20Who "/Game/VFX_SFX/Blood_Splatter/BPS/BPC_Blood_Effect.BPC_Blood_Effect_C"))
  (Utilities|IsValid _returnvalue
    (:Is%20Valid
      (Default|TakeDamage _returnvalue Damage Where To%20Who (Components|GetOwner))
      (Utilities|IsValid _returnvalue_2
        (:Is%20Valid
          (Default|BloodEffect _returnvalue_2 Where Normal To%20Who Damage))
        (:Is%20Not%20Valid
          _))
      (Audio|PlaySoundatLocation "/Game/VFX_SFX/Blood_Splatter/Audio/Impact_Audio/Body_Impact_SC.Body_Impact_SC" Where "0, 0, 0" 1.0 1.0 0.0 0 0 0 0)
      (if (not (Variables|Default|GetPiercing))
        (Actor|DestroyActor)))))

(fn CalculateDamageFalloff
  (params (Hit%20Location :type Vector))
  (bind _projectile_info (Variables|Default|GetProjectile_Info))
  (bind _projectile_info_2 (Variables|Default|GetProjectile_Info))
  (bind _shot_location (Variables|Default|GetShot%20Location))
  (bind _damage (Utilities|Struct|BreakStruct_Projectiles _projectile_info))
  (bind _falloffinfo (Utilities|Struct|BreakStruct_Projectiles _projectile_info_2))
  (bind _returnvalue (Math|Vector|Distance(Vector) _shot_location Hit%20Location))
  (bind (_hasfalloff _maxrange _shouldclampdamage _mindamage _falloffstartrange) (Utilities|Struct|BreakStruct_Projectile_Falloff_Info _falloffinfo))
  (bind _returnvalue_2 (/ _returnvalue _maxrange))
  (bind _returnvalue_3 (- 1.0 _returnvalue_2))
  (bind _returnvalue_4 (* _damage _returnvalue_3))
  (bind _returnvalue_5 (Math|Float|Floor _returnvalue_4))
  (if (>= _returnvalue _falloffstartrange)
    (if _hasfalloff
      (if (>= _returnvalue _maxrange)
        (return (Math|Float|SelectFloat _mindamage 0.0 _shouldclampdamage))
        (else
          (return (Math|Float|SelectFloat (Math|Float|Clamp(Float) (Math|Conversions|ToFloat(Integer) _returnvalue_5) _mindamage _damage) (Math|Conversions|ToFloat(Integer) _returnvalue_5) _shouldclampdamage))))
      (else
        (return _damage)))
    (else
      (return _damage))))