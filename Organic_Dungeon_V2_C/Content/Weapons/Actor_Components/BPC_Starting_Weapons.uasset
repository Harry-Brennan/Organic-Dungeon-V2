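; Actor component that gives its owner its starting weapons and equips a starter weapon through BPC_Weaponry.
; On BeginPlay, after a short delay and only if the owner has a starter weapon, it spawns BP_Weapon actors from structs read via owner interface messages.
; A separate Updating_Weapons event rewrites those structs on the owner, filling them from weapon and projectile DataTables while retaining custom overrides.
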(event Custom|Updating_Weapons
  (Utilities|FlowControl|Sequence
    (:then_0
      (bind _starting_weapons (Class|BPICanHaveWeapon|GetStartingWeapons(Message) (Components|GetOwner)))
      (for (_array_element _array_index) _starting_weapons
        (Utilities|FlowControl|Sequence
          (:then_0
            (if (not (.CustomWeapon (Utilities|Struct|BreakStruct_Spawnable_Weapon _array_element)))
              ;[1 1 1] Setting starting weapon at index with info from starting weapon struct but this isn't a custom weapon so we're basically just using the name
              (CallFunction|UpdateNonCustomWeaponInfo _array_element _array_index false)))
          (:then_1
            (if (.CustomProjectile (Utilities|Struct|BreakStruct_Spawnable_Weapon _array_element))
              ;[1 1 1] Setting custom weapons that have custom projectiles
              (bind _returnvalue (Utilities|GetDataTableRow "/Game/Projectiles/Structs_DataTables/DT_Projectiles.DT_Projectiles" (Utilities|String|StringToName (Utilities|String|EnumtoString (.Name (Utilities|Struct|BreakStruct_Projectiles (.Projectile_Info (Utilities|Struct|BreakStruct_Ranged_Weapon (.Ranged_Info (Utilities|Struct|BreakStruct_Spawnable_Weapon _array_element)))))))))
                (:then
                  _)
                (:RowNotFound
                  _))
              (Class|BPICanHaveWeapon|SetStartingWeaponsIndex(Message) (Components|GetOwner) (Utilities|Struct|MakeStruct_Spawnable_Weapon (.CustomWeapon (Utilities|Struct|BreakStruct_Spawnable_Weapon _array_element)) (select (.CustomWeapon (Utilities|Struct|BreakStruct_Spawnable_Weapon _array_element)) true false) (.Base_Info (Utilities|Struct|BreakStruct_Spawnable_Weapon _array_element)) (Utilities|Struct|MakeStruct_Ranged_Weapon (.Starting_Ammo (Utilities|Struct|BreakStruct_Ranged_Weapon (.Ranged_Info (Utilities|Struct|BreakStruct_Spawnable_Weapon _array_element)))) (.Crosshair (Utilities|Struct|BreakStruct_Ranged_Weapon (.Ranged_Info (Utilities|Struct|BreakStruct_Spawnable_Weapon _array_element)))) (.Reload_Info (Utilities|Struct|BreakStruct_Ranged_Weapon (.Ranged_Info (Utilities|Struct|BreakStruct_Spawnable_Weapon _array_element)))) (.ProjectileName (Utilities|Struct|BreakStruct_Ranged_Weapon (.Ranged_Info (Utilities|Struct|BreakStruct_Spawnable_Weapon _array_element)))) (Utilities|Struct|MakeStruct_Projectiles (.Name (Utilities|Struct|BreakStruct_Projectiles _returnvalue)) (.Damage (Utilities|Struct|BreakStruct_Projectiles (.Projectile_Info (Utilities|Struct|BreakStruct_Ranged_Weapon (.Ranged_Info (Utilities|Struct|BreakStruct_Spawnable_Weapon _array_element)))))) (.Speed (Utilities|Struct|BreakStruct_Projectiles (.Projectile_Info (Utilities|Struct|BreakStruct_Ranged_Weapon (.Ranged_Info (Utilities|Struct|BreakStruct_Spawnable_Weapon _array_element)))))) (.Gravity (Utilities|Struct|BreakStruct_Projectiles (.Projectile_Info (Utilities|Struct|BreakStruct_Ranged_Weapon (.Ranged_Info (Utilities|Struct|BreakStruct_Spawnable_Weapon _array_element)))))) (.Mesh (Utilities|Struct|BreakStruct_Projectiles _returnvalue)) (.OnHitEffect (Utilities|Struct|BreakStruct_Projectiles (.Projectile_Info (Utilities|Struct|BreakStruct_Ranged_Weapon (.Ranged_Info (Utilities|Struct|BreakStruct_Spawnable_Weapon _array_element)))))) (.ExplosionOnHit (Utilities|Struct|BreakStruct_Projectiles (.Projectile_Info (Utilities|Struct|BreakStruct_Ranged_Weapon (.Ranged_Info (Utilities|Struct|BreakStruct_Spawnable_Weapon _array_element)))))) "(HasFalloff_3_A917AA1446B1BA23F4081CA3789978BF=False,MaxRange_4_C5A541AD479499D973D0788AA394DAB2=0.000000,ShouldClampDamage_7_5B2BE9764A451584341C5D83C4511C89=False,MinDamage_10_BB404A854189F80D4BFF7A91F9B95334=0.000000,FalloffStartRange_13_C382D74E41A093AE41B0F7BCD37FB054=0.000000)") (.Recoil (Utilities|Struct|BreakStruct_Ranged_Weapon (.Ranged_Info (Utilities|Struct|BreakStruct_Spawnable_Weapon _array_element)))) (.HitScan (Utilities|Struct|BreakStruct_Ranged_Weapon (.Ranged_Info (Utilities|Struct|BreakStruct_Spawnable_Weapon _array_element)))) (.Piercing (Utilities|Struct|BreakStruct_Ranged_Weapon (.Ranged_Info (Utilities|Struct|BreakStruct_Spawnable_Weapon _array_element)))) (.ShootParticle (Utilities|Struct|BreakStruct_Ranged_Weapon (.Ranged_Info (Utilities|Struct|BreakStruct_Spawnable_Weapon _array_element)))) (._Projectiles (Utilities|Struct|BreakStruct_Ranged_Weapon (.Ranged_Info (Utilities|Struct|BreakStruct_Spawnable_Weapon _array_element)))) (.Spread (Utilities|Struct|BreakStruct_Ranged_Weapon (.Ranged_Info (Utilities|Struct|BreakStruct_Spawnable_Weapon _array_element)))) (.Fire_Type (Utilities|Struct|BreakStruct_Ranged_Weapon (.Ranged_Info (Utilities|Struct|BreakStruct_Spawnable_Weapon _array_element)))) (.Burst_Info (Utilities|Struct|BreakStruct_Ranged_Weapon (.Ranged_Info (Utilities|Struct|BreakStruct_Spawnable_Weapon _array_element)))) (.Full_Auto_Info (Utilities|Struct|BreakStruct_Ranged_Weapon (.Ranged_Info (Utilities|Struct|BreakStruct_Spawnable_Weapon _array_element)))) (.Charged_Info (Utilities|Struct|BreakStruct_Ranged_Weapon (.Ranged_Info (Utilities|Struct|BreakStruct_Spawnable_Weapon _array_element)))) (.Charged_Burst_Info (Utilities|Struct|BreakStruct_Ranged_Weapon (.Ranged_Info (Utilities|Struct|BreakStruct_Spawnable_Weapon _array_element)))) (.Audio_Info (Utilities|Struct|BreakStruct_Ranged_Weapon (.Ranged_Info (Utilities|Struct|BreakStruct_Spawnable_Weapon _array_element))))) (.MeleeInfo (Utilities|Struct|BreakStruct_Spawnable_Weapon _array_element))) _array_index)
              (else
                ;[1 1 1] Setting custom weapon that doesn't have a custom projectile associated with it
                (bind _returnvalue_2 (Utilities|GetDataTableRow "/Game/Weapons/Structs_DataTables/DT_Ranged_Weapon_Info.DT_Ranged_Weapon_Info" (Utilities|String|StringToName (Utilities|String|EnumtoString (Utilities|Struct|BreakStruct_Weapon (.Base_Info (Utilities|Struct|BreakStruct_Spawnable_Weapon _array_element))))))
                  (:then
                    _)
                  (:RowNotFound
                    _))
                (bind _returnvalue_3 (Utilities|GetDataTableRow "/Game/Projectiles/Structs_DataTables/DT_Projectiles.DT_Projectiles" (Utilities|String|StringToName (Utilities|String|EnumtoString (.ProjectileName (Utilities|Struct|BreakStruct_Ranged_Weapon _returnvalue_2)))))
                  (:then
                    _)
                  (:RowNotFound
                    _))
                (bind _returnvalue_4 (Utilities|GetDataTableRow "/Game/Weapons/Structs_DataTables/DT_Basic_Weapon_Info.DT_Basic_Weapon_Info" (Utilities|String|StringToName (Utilities|String|EnumtoString (Utilities|Struct|BreakStruct_Weapon (.Base_Info (Utilities|Struct|BreakStruct_Spawnable_Weapon _array_element))))))
                  (:then
                    _)
                  (:RowNotFound
                    _))
                (Class|BPICanHaveWeapon|SetStartingWeaponsIndex(Message) (Components|GetOwner) (Utilities|Struct|MakeStruct_Spawnable_Weapon (.CustomWeapon (Utilities|Struct|BreakStruct_Spawnable_Weapon _array_element)) false (select (.CustomWeapon (Utilities|Struct|BreakStruct_Spawnable_Weapon _array_element)) (.Base_Info (Utilities|Struct|BreakStruct_Spawnable_Weapon _array_element)) _returnvalue_4) (Utilities|Struct|MakeStruct_Ranged_Weapon (.Starting_Ammo (Utilities|Struct|BreakStruct_Ranged_Weapon (select (.CustomWeapon (Utilities|Struct|BreakStruct_Spawnable_Weapon _array_element)) (.Ranged_Info (Utilities|Struct|BreakStruct_Spawnable_Weapon _array_element)) _returnvalue_2))) (.Crosshair (Utilities|Struct|BreakStruct_Ranged_Weapon _returnvalue_2)) (.Reload_Info (Utilities|Struct|BreakStruct_Ranged_Weapon (select (.CustomWeapon (Utilities|Struct|BreakStruct_Spawnable_Weapon _array_element)) (.Ranged_Info (Utilities|Struct|BreakStruct_Spawnable_Weapon _array_element)) _returnvalue_2))) (.ProjectileName (Utilities|Struct|BreakStruct_Ranged_Weapon _returnvalue_2)) _returnvalue_3 (.Recoil (Utilities|Struct|BreakStruct_Ranged_Weapon (select (.CustomWeapon (Utilities|Struct|BreakStruct_Spawnable_Weapon _array_element)) (.Ranged_Info (Utilities|Struct|BreakStruct_Spawnable_Weapon _array_element)) _returnvalue_2))) (.HitScan (Utilities|Struct|BreakStruct_Ranged_Weapon (select (.CustomWeapon (Utilities|Struct|BreakStruct_Spawnable_Weapon _array_element)) (.Ranged_Info (Utilities|Struct|BreakStruct_Spawnable_Weapon _array_element)) _returnvalue_2))) (.Piercing (Utilities|Struct|BreakStruct_Ranged_Weapon (select (.CustomWeapon (Utilities|Struct|BreakStruct_Spawnable_Weapon _array_element)) (.Ranged_Info (Utilities|Struct|BreakStruct_Spawnable_Weapon _array_element)) _returnvalue_2))) (.ShootParticle (Utilities|Struct|BreakStruct_Ranged_Weapon (select (.CustomWeapon (Utilities|Struct|BreakStruct_Spawnable_Weapon _array_element)) (.Ranged_Info (Utilities|Struct|BreakStruct_Spawnable_Weapon _array_element)) _returnvalue_2))) (._Projectiles (Utilities|Struct|BreakStruct_Ranged_Weapon (select (.CustomWeapon (Utilities|Struct|BreakStruct_Spawnable_Weapon _array_element)) (.Ranged_Info (Utilities|Struct|BreakStruct_Spawnable_Weapon _array_element)) _returnvalue_2))) (.Spread (Utilities|Struct|BreakStruct_Ranged_Weapon (select (.CustomWeapon (Utilities|Struct|BreakStruct_Spawnable_Weapon _array_element)) (.Ranged_Info (Utilities|Struct|BreakStruct_Spawnable_Weapon _array_element)) _returnvalue_2))) (.Fire_Type (Utilities|Struct|BreakStruct_Ranged_Weapon (select (.CustomWeapon (Utilities|Struct|BreakStruct_Spawnable_Weapon _array_element)) (.Ranged_Info (Utilities|Struct|BreakStruct_Spawnable_Weapon _array_element)) _returnvalue_2))) (.Burst_Info (Utilities|Struct|BreakStruct_Ranged_Weapon (select (.CustomWeapon (Utilities|Struct|BreakStruct_Spawnable_Weapon _array_element)) (.Ranged_Info (Utilities|Struct|BreakStruct_Spawnable_Weapon _array_element)) _returnvalue_2))) (.Full_Auto_Info (Utilities|Struct|BreakStruct_Ranged_Weapon (select (.CustomWeapon (Utilities|Struct|BreakStruct_Spawnable_Weapon _array_element)) (.Ranged_Info (Utilities|Struct|BreakStruct_Spawnable_Weapon _array_element)) _returnvalue_2))) (.Charged_Info (Utilities|Struct|BreakStruct_Ranged_Weapon (select (.CustomWeapon (Utilities|Struct|BreakStruct_Spawnable_Weapon _array_element)) (.Ranged_Info (Utilities|Struct|BreakStruct_Spawnable_Weapon _array_element)) _returnvalue_2))) (.Charged_Burst_Info (Utilities|Struct|BreakStruct_Ranged_Weapon (select (.CustomWeapon (Utilities|Struct|BreakStruct_Spawnable_Weapon _array_element)) (.Ranged_Info (Utilities|Struct|BreakStruct_Spawnable_Weapon _array_element)) _returnvalue_2))) (.Audio_Info (Utilities|Struct|BreakStruct_Ranged_Weapon (select (.CustomWeapon (Utilities|Struct|BreakStruct_Spawnable_Weapon _array_element)) (.Ranged_Info (Utilities|Struct|BreakStruct_Spawnable_Weapon _array_element)) _returnvalue_2)))) (.MeleeInfo (Utilities|Struct|BreakStruct_Spawnable_Weapon _array_element))) _array_index)))))))
    (:then_1
      ;[1 1 1] Setting starting weapon is not a custom weapon
      (bind _starter_weapon (Class|BPICanHaveWeapon|GetStarterWeapon(Message) (Components|GetOwner)))
      (Utilities|FlowControl|Sequence
        (:then_0
          (if (not (.CustomWeapon (Utilities|Struct|BreakStruct_Spawnable_Weapon _starter_weapon)))
            (CallFunction|UpdateNonCustomWeaponInfo _starter_weapon 0 true)))
        (:then_1
          ;[1 1 1] Setting starting weapon that has a custom projectile associated with it
          (if (.CustomProjectile (Utilities|Struct|BreakStruct_Spawnable_Weapon _starter_weapon))
            (bind _returnvalue_5 (Utilities|GetDataTableRow "/Game/Projectiles/Structs_DataTables/DT_Projectiles.DT_Projectiles" (Utilities|String|StringToName (Utilities|String|EnumtoString (.Name (Utilities|Struct|BreakStruct_Projectiles (.Projectile_Info (Utilities|Struct|BreakStruct_Ranged_Weapon (.Ranged_Info (Utilities|Struct|BreakStruct_Spawnable_Weapon _starter_weapon)))))))))
              (:then
                _)
              (:RowNotFound
                _))
            (Class|BPICanHaveWeapon|SetStarterWeapon(Message) (Components|GetOwner) (Utilities|Struct|MakeStruct_Spawnable_Weapon (.CustomWeapon (Utilities|Struct|BreakStruct_Spawnable_Weapon _starter_weapon)) (select (.CustomWeapon (Utilities|Struct|BreakStruct_Spawnable_Weapon _starter_weapon)) true false) (.Base_Info (Utilities|Struct|BreakStruct_Spawnable_Weapon _starter_weapon)) (Utilities|Struct|MakeStruct_Ranged_Weapon (.Starting_Ammo (Utilities|Struct|BreakStruct_Ranged_Weapon (.Ranged_Info (Utilities|Struct|BreakStruct_Spawnable_Weapon _starter_weapon)))) (.Crosshair (Utilities|Struct|BreakStruct_Ranged_Weapon (.Ranged_Info (Utilities|Struct|BreakStruct_Spawnable_Weapon _starter_weapon)))) (.Reload_Info (Utilities|Struct|BreakStruct_Ranged_Weapon (.Ranged_Info (Utilities|Struct|BreakStruct_Spawnable_Weapon _starter_weapon)))) (.ProjectileName (Utilities|Struct|BreakStruct_Ranged_Weapon (.Ranged_Info (Utilities|Struct|BreakStruct_Spawnable_Weapon _starter_weapon)))) (Utilities|Struct|MakeStruct_Projectiles (.Name (Utilities|Struct|BreakStruct_Projectiles _returnvalue_5)) (.Damage (Utilities|Struct|BreakStruct_Projectiles (.Projectile_Info (Utilities|Struct|BreakStruct_Ranged_Weapon (.Ranged_Info (Utilities|Struct|BreakStruct_Spawnable_Weapon _starter_weapon)))))) (.Speed (Utilities|Struct|BreakStruct_Projectiles (.Projectile_Info (Utilities|Struct|BreakStruct_Ranged_Weapon (.Ranged_Info (Utilities|Struct|BreakStruct_Spawnable_Weapon _starter_weapon)))))) (.Gravity (Utilities|Struct|BreakStruct_Projectiles (.Projectile_Info (Utilities|Struct|BreakStruct_Ranged_Weapon (.Ranged_Info (Utilities|Struct|BreakStruct_Spawnable_Weapon _starter_weapon)))))) (.Mesh (Utilities|Struct|BreakStruct_Projectiles _returnvalue_5)) (.OnHitEffect (Utilities|Struct|BreakStruct_Projectiles (.Projectile_Info (Utilities|Struct|BreakStruct_Ranged_Weapon (.Ranged_Info (Utilities|Struct|BreakStruct_Spawnable_Weapon _starter_weapon)))))) (.ExplosionOnHit (Utilities|Struct|BreakStruct_Projectiles (.Projectile_Info (Utilities|Struct|BreakStruct_Ranged_Weapon (.Ranged_Info (Utilities|Struct|BreakStruct_Spawnable_Weapon _starter_weapon)))))) "(HasFalloff_3_A917AA1446B1BA23F4081CA3789978BF=False,MaxRange_4_C5A541AD479499D973D0788AA394DAB2=0.000000,ShouldClampDamage_7_5B2BE9764A451584341C5D83C4511C89=False,MinDamage_10_BB404A854189F80D4BFF7A91F9B95334=0.000000,FalloffStartRange_13_C382D74E41A093AE41B0F7BCD37FB054=0.000000)") (.Recoil (Utilities|Struct|BreakStruct_Ranged_Weapon (.Ranged_Info (Utilities|Struct|BreakStruct_Spawnable_Weapon _starter_weapon)))) (.HitScan (Utilities|Struct|BreakStruct_Ranged_Weapon (.Ranged_Info (Utilities|Struct|BreakStruct_Spawnable_Weapon _starter_weapon)))) (.Piercing (Utilities|Struct|BreakStruct_Ranged_Weapon (.Ranged_Info (Utilities|Struct|BreakStruct_Spawnable_Weapon _starter_weapon)))) (.ShootParticle (Utilities|Struct|BreakStruct_Ranged_Weapon (.Ranged_Info (Utilities|Struct|BreakStruct_Spawnable_Weapon _starter_weapon)))) (._Projectiles (Utilities|Struct|BreakStruct_Ranged_Weapon (.Ranged_Info (Utilities|Struct|BreakStruct_Spawnable_Weapon _starter_weapon)))) (.Spread (Utilities|Struct|BreakStruct_Ranged_Weapon (.Ranged_Info (Utilities|Struct|BreakStruct_Spawnable_Weapon _starter_weapon)))) (.Fire_Type (Utilities|Struct|BreakStruct_Ranged_Weapon (.Ranged_Info (Utilities|Struct|BreakStruct_Spawnable_Weapon _starter_weapon)))) (.Burst_Info (Utilities|Struct|BreakStruct_Ranged_Weapon (.Ranged_Info (Utilities|Struct|BreakStruct_Spawnable_Weapon _starter_weapon)))) (.Full_Auto_Info (Utilities|Struct|BreakStruct_Ranged_Weapon (.Ranged_Info (Utilities|Struct|BreakStruct_Spawnable_Weapon _starter_weapon)))) (.Charged_Info (Utilities|Struct|BreakStruct_Ranged_Weapon (.Ranged_Info (Utilities|Struct|BreakStruct_Spawnable_Weapon _starter_weapon)))) (.Charged_Burst_Info (Utilities|Struct|BreakStruct_Ranged_Weapon (.Ranged_Info (Utilities|Struct|BreakStruct_Spawnable_Weapon _starter_weapon)))) (.Audio_Info (Utilities|Struct|BreakStruct_Ranged_Weapon (.Ranged_Info (Utilities|Struct|BreakStruct_Spawnable_Weapon _starter_weapon))))) (.MeleeInfo (Utilities|Struct|BreakStruct_Spawnable_Weapon _starter_weapon))))))))))

(event EventBeginPlay
  (bind _returnvalue (Components|GetOwner))
  (bind _returnvalue_2 (Actor|GetComponentbyClass _returnvalue "/Game/Weapons/Actor_Components/BPC_Weaponry.BPC_Weaponry_C"))
  ;[1 1 1] After short delay of spawning owner then get required info for initialising and setting starting weapons
  (Utilities|FlowControl|Delay 0.2)
  (bind _should_have_starter_weapon (Class|BPICanHaveWeapon|GetHasStarterWeapon(Message) (Components|GetOwner)))
  (if _should_have_starter_weapon
    (CallFunction|InitialiseStartingWeapons)
    (CallFunction|EquipStarterWeapon)
    (Default|EquipNextWeapon _returnvalue_2)
    (Default|EquipPreviousWeapon _returnvalue_2)))

(fn InitialiseStartingWeapons
  ;[1 1 1] Spawning the actual weapon blkueprints and then adding them via the weaponry component
  (bind _starting_weapons (Class|BPICanHaveWeapon|GetStartingWeapons(Message) (Components|GetOwner)))
  (for _array_element _starting_weapons
    (bind _returnvalue (Game|SpawnActorfromClass :Class "/Game/Weapons/BPs/BP_Weapon.BP_Weapon_C" :CollisionHandlingOverride "AlwaysSpawn" :TransformScaleMethod "MultiplyWithRoot" :Custom_Weapon? (.CustomWeapon (Utilities|Struct|BreakStruct_Spawnable_Weapon _array_element)) :Custom_Projectile (.CustomProjectile (Utilities|Struct|BreakStruct_Spawnable_Weapon _array_element)) :Info (.Base_Info (Utilities|Struct|BreakStruct_Spawnable_Weapon _array_element)) :Ranged_Info (.Ranged_Info (Utilities|Struct|BreakStruct_Spawnable_Weapon _array_element)) :Melee_Info (.MeleeInfo (Utilities|Struct|BreakStruct_Spawnable_Weapon _array_element)) :Instigator 0))
    (Default|AddWeapon (Actor|GetComponentbyClass (Components|GetOwner) "/Game/Weapons/Actor_Components/BPC_Weaponry.BPC_Weaponry_C") _returnvalue)))

(fn EquipStarterWeapon
  (bind _returnvalue (Components|GetOwner))
  (bind _returnvalue_2 (Actor|GetComponentbyClass _returnvalue "/Game/Weapons/Actor_Components/BPC_Weaponry.BPC_Weaponry_C"))
  ;[1 1 1] Spawning the starting weapon and adding to inventory and then equipping using weaponry component
  (bind _starter_weapon (Class|BPICanHaveWeapon|GetStarterWeapon(Message) (Components|GetOwner)))
  (bind _returnvalue_3 (Game|SpawnActorfromClass :Class "/Game/Weapons/BPs/BP_Weapon.BP_Weapon_C" :CollisionHandlingOverride "AlwaysSpawn" :TransformScaleMethod "MultiplyWithRoot" :Custom_Weapon? (.CustomWeapon (Utilities|Struct|BreakStruct_Spawnable_Weapon _starter_weapon)) :Custom_Projectile (.CustomProjectile (Utilities|Struct|BreakStruct_Spawnable_Weapon _starter_weapon)) :Info (.Base_Info (Utilities|Struct|BreakStruct_Spawnable_Weapon _starter_weapon)) :Ranged_Info (.Ranged_Info (Utilities|Struct|BreakStruct_Spawnable_Weapon _starter_weapon)) :Melee_Info (.MeleeInfo (Utilities|Struct|BreakStruct_Spawnable_Weapon _starter_weapon)) :Instigator 0))
  (Default|AddWeapon _returnvalue_2 _returnvalue_3)
  (Default|EquipWeapon _returnvalue_2 _returnvalue_3))

(fn UpdateNonCustomWeaponInfo
  (params (Weapon_Info :type Struct%20Spawnable%20Weapon%20Structure) (Array%20Index%20If%20Starting%20Weapons :type Integer) (Is_Starter_Weapon :type Boolean))
  (bind (_customprojectile _base_info) (Utilities|Struct|BreakStruct_Spawnable_Weapon Weapon_Info))
  (bind _returnvalue (Components|GetOwner))
  ;[1 1 1] Setting starting weapons based on passed info and then calling the corresponding functions in the blueprint actor that actually has the interface and functions to appropriately store the info
  (bind _returnvalue_2 (Utilities|GetDataTableRow "/Game/Weapons/Structs_DataTables/DT_Basic_Weapon_Info.DT_Basic_Weapon_Info" (Utilities|String|StringToName (Utilities|String|EnumtoString (Utilities|Struct|BreakStruct_Weapon _base_info))))
    (:then
      (Utilities|FlowControl|Sequence
        (:then_0
          (bind _returnvalue_3 (Utilities|GetDataTableRow "/Game/Weapons/Structs_DataTables/DT_Ranged_Weapon_Info.DT_Ranged_Weapon_Info" (Utilities|String|StringToName (Utilities|String|EnumtoString (.Name (Utilities|Struct|BreakStruct_Weapon _returnvalue_2)))))
            (:then
              (bind _returnvalue_4 (Utilities|GetDataTableRow "/Game/Projectiles/Structs_DataTables/DT_Projectiles.DT_Projectiles" (Utilities|String|StringToName (Utilities|String|EnumtoString (.Name (Utilities|Struct|BreakStruct_Projectiles (.Projectile_Info (Utilities|Struct|BreakStruct_Ranged_Weapon _returnvalue_3)))))))))))
        (:then_1
          (bind _returnvalue_5 (Utilities|GetDataTableRow "/Game/Weapons/Structs_DataTables/DT_Melee_Weapon_Info.DT_Melee_Weapon_Info" (Utilities|String|StringToName (Utilities|String|EnumtoString (.Name (Utilities|Struct|BreakStruct_Weapon _returnvalue_2)))))))
        (:then_2
          (if Is_Starter_Weapon
            (Class|BPICanHaveWeapon|SetStarterWeapon(Message) _returnvalue (Utilities|Struct|MakeStruct_Spawnable_Weapon false false (Utilities|Struct|MakeStruct_Weapon (.Name (Utilities|Struct|BreakStruct_Weapon _returnvalue_2)) (.Ranged (Utilities|Struct|BreakStruct_Weapon _returnvalue_2)) (.Icon (Utilities|Struct|BreakStruct_Weapon _returnvalue_2)) (.StaticMesh (Utilities|Struct|BreakStruct_Weapon _returnvalue_2)) (.BaseColour (Utilities|Struct|BreakStruct_Weapon _returnvalue_2))) (Utilities|Struct|MakeStruct_Ranged_Weapon (.Starting_Ammo (Utilities|Struct|BreakStruct_Ranged_Weapon _returnvalue_3)) (.Crosshair (Utilities|Struct|BreakStruct_Ranged_Weapon _returnvalue_3)) (.Reload_Info (Utilities|Struct|BreakStruct_Ranged_Weapon _returnvalue_3)) (.ProjectileName (Utilities|Struct|BreakStruct_Ranged_Weapon _returnvalue_3)) (select _customprojectile (Utilities|Struct|MakeStruct_Projectiles (.Name (Utilities|Struct|BreakStruct_Projectiles _returnvalue_4)) (.Damage (Utilities|Struct|BreakStruct_Projectiles (.Projectile_Info (Utilities|Struct|BreakStruct_Ranged_Weapon _returnvalue_3)))) (.Speed (Utilities|Struct|BreakStruct_Projectiles (.Projectile_Info (Utilities|Struct|BreakStruct_Ranged_Weapon _returnvalue_3)))) (.Gravity (Utilities|Struct|BreakStruct_Projectiles (.Projectile_Info (Utilities|Struct|BreakStruct_Ranged_Weapon _returnvalue_3)))) (.Mesh (Utilities|Struct|BreakStruct_Projectiles _returnvalue_4)) (.OnHitEffect (Utilities|Struct|BreakStruct_Projectiles (.Projectile_Info (Utilities|Struct|BreakStruct_Ranged_Weapon _returnvalue_3)))) (.ExplosionOnHit (Utilities|Struct|BreakStruct_Projectiles (.Projectile_Info (Utilities|Struct|BreakStruct_Ranged_Weapon _returnvalue_3)))) "(HasFalloff_3_A917AA1446B1BA23F4081CA3789978BF=False,MaxRange_4_C5A541AD479499D973D0788AA394DAB2=0.000000,ShouldClampDamage_7_5B2BE9764A451584341C5D83C4511C89=False,MinDamage_10_BB404A854189F80D4BFF7A91F9B95334=0.000000,FalloffStartRange_13_C382D74E41A093AE41B0F7BCD37FB054=0.000000)") _returnvalue_4) (.Recoil (Utilities|Struct|BreakStruct_Ranged_Weapon _returnvalue_3)) (.HitScan (Utilities|Struct|BreakStruct_Ranged_Weapon _returnvalue_3)) (.Piercing (Utilities|Struct|BreakStruct_Ranged_Weapon _returnvalue_3)) (.ShootParticle (Utilities|Struct|BreakStruct_Ranged_Weapon _returnvalue_3)) (._Projectiles (Utilities|Struct|BreakStruct_Ranged_Weapon _returnvalue_3)) (.Spread (Utilities|Struct|BreakStruct_Ranged_Weapon _returnvalue_3)) (.Fire_Type (Utilities|Struct|BreakStruct_Ranged_Weapon _returnvalue_3)) (.Burst_Info (Utilities|Struct|BreakStruct_Ranged_Weapon _returnvalue_3)) (.Full_Auto_Info (Utilities|Struct|BreakStruct_Ranged_Weapon _returnvalue_3)) (.Charged_Info (Utilities|Struct|BreakStruct_Ranged_Weapon _returnvalue_3)) (.Charged_Burst_Info (Utilities|Struct|BreakStruct_Ranged_Weapon _returnvalue_3)) (.Audio_Info (Utilities|Struct|BreakStruct_Ranged_Weapon _returnvalue_3))) (Utilities|Struct|MakeStruct_Melee_Weapon (.Crosshair (Utilities|Struct|BreakStruct_Melee_Weapon _returnvalue_5)) (.Combo_Amount (Utilities|Struct|BreakStruct_Melee_Weapon _returnvalue_5)) (.Damage (Utilities|Struct|BreakStruct_Melee_Weapon _returnvalue_5)) (.BlockingInfo (Utilities|Struct|BreakStruct_Melee_Weapon _returnvalue_5)) (.MeleeAudio (Utilities|Struct|BreakStruct_Melee_Weapon _returnvalue_5)) (.HeavyAttackInfo (Utilities|Struct|BreakStruct_Melee_Weapon _returnvalue_5)))))
            (else
              (Class|BPICanHaveWeapon|SetStartingWeaponsIndex(Message) _returnvalue (Utilities|Struct|MakeStruct_Spawnable_Weapon false false (Utilities|Struct|MakeStruct_Weapon (.Name (Utilities|Struct|BreakStruct_Weapon _returnvalue_2)) (.Ranged (Utilities|Struct|BreakStruct_Weapon _returnvalue_2)) (.Icon (Utilities|Struct|BreakStruct_Weapon _returnvalue_2)) (.StaticMesh (Utilities|Struct|BreakStruct_Weapon _returnvalue_2)) (.BaseColour (Utilities|Struct|BreakStruct_Weapon _returnvalue_2))) (Utilities|Struct|MakeStruct_Ranged_Weapon (.Starting_Ammo (Utilities|Struct|BreakStruct_Ranged_Weapon _returnvalue_3)) (.Crosshair (Utilities|Struct|BreakStruct_Ranged_Weapon _returnvalue_3)) (.Reload_Info (Utilities|Struct|BreakStruct_Ranged_Weapon _returnvalue_3)) (.ProjectileName (Utilities|Struct|BreakStruct_Ranged_Weapon _returnvalue_3)) (select _customprojectile (Utilities|Struct|MakeStruct_Projectiles (.Name (Utilities|Struct|BreakStruct_Projectiles _returnvalue_4)) (.Damage (Utilities|Struct|BreakStruct_Projectiles (.Projectile_Info (Utilities|Struct|BreakStruct_Ranged_Weapon _returnvalue_3)))) (.Speed (Utilities|Struct|BreakStruct_Projectiles (.Projectile_Info (Utilities|Struct|BreakStruct_Ranged_Weapon _returnvalue_3)))) (.Gravity (Utilities|Struct|BreakStruct_Projectiles (.Projectile_Info (Utilities|Struct|BreakStruct_Ranged_Weapon _returnvalue_3)))) (.Mesh (Utilities|Struct|BreakStruct_Projectiles _returnvalue_4)) (.OnHitEffect (Utilities|Struct|BreakStruct_Projectiles (.Projectile_Info (Utilities|Struct|BreakStruct_Ranged_Weapon _returnvalue_3)))) (.ExplosionOnHit (Utilities|Struct|BreakStruct_Projectiles (.Projectile_Info (Utilities|Struct|BreakStruct_Ranged_Weapon _returnvalue_3)))) "(HasFalloff_3_A917AA1446B1BA23F4081CA3789978BF=False,MaxRange_4_C5A541AD479499D973D0788AA394DAB2=0.000000,ShouldClampDamage_7_5B2BE9764A451584341C5D83C4511C89=False,MinDamage_10_BB404A854189F80D4BFF7A91F9B95334=0.000000,FalloffStartRange_13_C382D74E41A093AE41B0F7BCD37FB054=0.000000)") _returnvalue_4) (.Recoil (Utilities|Struct|BreakStruct_Ranged_Weapon _returnvalue_3)) (.HitScan (Utilities|Struct|BreakStruct_Ranged_Weapon _returnvalue_3)) (.Piercing (Utilities|Struct|BreakStruct_Ranged_Weapon _returnvalue_3)) (.ShootParticle (Utilities|Struct|BreakStruct_Ranged_Weapon _returnvalue_3)) (._Projectiles (Utilities|Struct|BreakStruct_Ranged_Weapon _returnvalue_3)) (.Spread (Utilities|Struct|BreakStruct_Ranged_Weapon _returnvalue_3)) (.Fire_Type (Utilities|Struct|BreakStruct_Ranged_Weapon _returnvalue_3)) (.Burst_Info (Utilities|Struct|BreakStruct_Ranged_Weapon _returnvalue_3)) (.Full_Auto_Info (Utilities|Struct|BreakStruct_Ranged_Weapon _returnvalue_3)) (.Charged_Info (Utilities|Struct|BreakStruct_Ranged_Weapon _returnvalue_3)) (.Charged_Burst_Info (Utilities|Struct|BreakStruct_Ranged_Weapon _returnvalue_3)) (.Audio_Info (Utilities|Struct|BreakStruct_Ranged_Weapon _returnvalue_3))) (Utilities|Struct|MakeStruct_Melee_Weapon (.Crosshair (Utilities|Struct|BreakStruct_Melee_Weapon _returnvalue_5)) (.Combo_Amount (Utilities|Struct|BreakStruct_Melee_Weapon _returnvalue_5)) (.Damage (Utilities|Struct|BreakStruct_Melee_Weapon _returnvalue_5)) (.BlockingInfo (Utilities|Struct|BreakStruct_Melee_Weapon _returnvalue_5)) (.MeleeAudio (Utilities|Struct|BreakStruct_Melee_Weapon _returnvalue_5)) (.HeavyAttackInfo (Utilities|Struct|BreakStruct_Melee_Weapon _returnvalue_5)))) Array%20Index%20If%20Starting%20Weapons))))))))