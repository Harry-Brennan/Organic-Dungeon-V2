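; Actor component that runs melee attacks, unarmed or with the equipped weapon, pulling damage from the owner or weapon and tracking light-attack combos.
; While the hitbox is open, Tick box-traces at the attacking bone or between weapon sockets, hitting each actor once per swing.
; Characters with health take damage, knockback, hitstop and blood effects; physics objects get impulses.
; Player owners also get crosshair animation and camera shake.
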(event Custom|Start_Melee_Attack
  (params (Unarmed%20Attack :type Boolean) (Heavy%20Attack :type Boolean))
  (bind _returnvalue (Components|GetOwner))
  (bind _returnvalue_2 (Components|GetOwner))
  (bind _returnvalue_3 (Actor|GetComponentbyClass _returnvalue "/Game/Weapons/Actor_Components/BPC_Attack_Handler.BPC_Attack_Handler_C"))
  (bind _returnvalue_4 (Actor|GetComponentbyClass _returnvalue_2 "/Game/Weapons/Actor_Components/BPC_Attack_Handler.BPC_Attack_Handler_C"))
  (if (Utilities|DoesObjectImplementInterface (Components|GetOwner) "/Game/Characters/Player/BPI_Player.BPI_Player_C")
    (Default|PlayHitCrosshairAnim (Actor|GetComponentbyClass (Components|GetOwner) "/Game/Characters/Player/BPC_HUD.BPC_HUD_C")))
  (if Unarmed%20Attack
    (Variables|Unarmed|SetUnarmed%20Attack true)
    (Variables|/Game/Weapons/Actor_Components/BPC_Attack_Handler.BPC_Attack_Handler_C|SetAttacking (Actor|GetComponentbyClass (Components|GetOwner) "/Game/Weapons/Actor_Components/BPC_Attack_Handler.BPC_Attack_Handler_C") true)
    (bind _info (Class|BPICanUnarmedAttack|GetUnarmedAttackInfo(Message) (Components|GetOwner)))
    (Variables|MeleeAttack|SetDamage (.damage _info))
    (Variables|Unarmed|SetUnarmed_Attack_Bone (.bone_attacking_with _info))
    (Variables|Unarmed|SetKnockbackForce (.knockbackforce _info))
    (Variables|Unarmed|SetKnockUpForce (.knockupforce _info))
    (elif Heavy%20Attack
      (Variables|Unarmed|SetUnarmed%20Attack false)
      (Variables|MeleeAttack|SetHeavy%20Attacking true)
      (bind _melee_info (Class|BPIMeleeWeapon|GetMeleeInfo(Message) (Variables|/Game/Weapons/Actor_Components/BPC_Weaponry.BPC_Weaponry_C|GetEquipped_Weapon (Actor|GetComponentbyClass (Components|GetOwner) "/Game/Weapons/Actor_Components/BPC_Weaponry.BPC_Weaponry_C"))))
      (Variables|MeleeAttack|SetDamage (.Damage (Utilities|Struct|BreakStruct_Heavy_Attack_Info (.heavyattackinfo _melee_info))))
      (Variables|/Game/Weapons/Actor_Components/BPC_Attack_Handler.BPC_Attack_Handler_C|SetAttacking_Melee_Weapon _returnvalue_4 (Variables|/Game/Weapons/Actor_Components/BPC_Weaponry.BPC_Weaponry_C|GetEquipped_Weapon (Actor|GetComponentbyClass (Components|GetOwner) "/Game/Weapons/Actor_Components/BPC_Weaponry.BPC_Weaponry_C")))
      (Variables|/Game/Weapons/Actor_Components/BPC_Attack_Handler.BPC_Attack_Handler_C|SetAttacking _returnvalue_4 true)
      (else
        (Variables|Unarmed|SetUnarmed%20Attack false)
        (Variables|MeleeAttack|SetHeavy%20Attacking false)
        (Variables|/Game/Weapons/Actor_Components/BPC_Attack_Handler.BPC_Attack_Handler_C|SetAttacking_Melee_Weapon _returnvalue_3 (Variables|/Game/Weapons/Actor_Components/BPC_Weaponry.BPC_Weaponry_C|GetEquipped_Weapon (Actor|GetComponentbyClass (Components|GetOwner) "/Game/Weapons/Actor_Components/BPC_Weaponry.BPC_Weaponry_C")))
        (Variables|/Game/Weapons/Actor_Components/BPC_Attack_Handler.BPC_Attack_Handler_C|SetAttacking _returnvalue_3 true)
        (bind _melee_info_2 (Class|BPIMeleeWeapon|GetMeleeInfo(Message) (Variables|/Game/Weapons/Actor_Components/BPC_Weaponry.BPC_Weaponry_C|GetEquipped_Weapon (Actor|GetComponentbyClass (Components|GetOwner) "/Game/Weapons/Actor_Components/BPC_Weaponry.BPC_Weaponry_C"))))
        (Variables|MeleeAttack|SetDamage (.damage _melee_info_2))
        (Math|Integer|IncrementInt (Variables|Meleeattack|GetCombo_Count)
          (:%20%20
            (if (>= (Variables|Meleeattack|GetCombo_Count) (.combo_amount _melee_info_2))
              (Variables|Meleeattack|SetCombo_Count 0))))))))

(event Custom|Melee_Attack_End
  (Utilities|FlowControl|Delay (Math|Float|SelectFloat 0.25 0.05 (Variables|Unarmed|GetUnarmed%20Attack)))
  (Variables|/Game/Weapons/Actor_Components/BPC_Attack_Handler.BPC_Attack_Handler_C|SetAttacking (Actor|GetComponentbyClass (Components|GetOwner) "/Game/Weapons/Actor_Components/BPC_Attack_Handler.BPC_Attack_Handler_C") false)
  (Variables|Unarmed|SetUnarmed%20Attack false))

(event Custom|End_Hitbox
  (Components|Tick|SetComponentTickEnabled false))

(event Custom|Start_Hitbox
  (Utilities|Array|Clear (Variables|Hitbox|GetHit_Actors))
  (Components|Tick|SetComponentTickEnabled true))

(event EventTick
  (params (DeltaSeconds :type Float%20%28single-precision%29))
  (bind _returnvalue (Components|GetOwner))
  (bind _returnvalue_2 (Components|GetOwner))
  (bind _returnvalue_3 (Components|GetOwner))
  (bind _returnvalue_4 (Components|GetOwner))
  (bind _returnvalue_5 (Components|GetOwner))
  (bind _returnvalue_6 (Components|GetOwner))
  (bind _array (Utilities|Array|MakeArray "ObjectTypeQuery10" "ObjectTypeQuery9" "ObjectTypeQuery8" "ObjectTypeQuery9" "ObjectTypeQuery11" "ObjectTypeQuery4"))
  (bind _hit_actors (Variables|Hitbox|GetHit_Actors))
  (bind _damage (Variables|MeleeAttack|GetDamage))
  (bind _unarmed_attack_bone (Variables|Unarmed|GetUnarmed_Attack_Bone))
  (bind _returnvalue_7 (Actor|GetComponentbyClass _returnvalue "/Game/Weapons/Actor_Components/BPC_Attack_Handler.BPC_Attack_Handler_C"))
  (bind _returnvalue_8 (Actor|GetComponentbyClass _returnvalue_2 "/Game/Weapons/Actor_Components/BPC_Attack_Handler.BPC_Attack_Handler_C"))
  (bind _returnvalue_9 (Actor|GetComponentbyClass _returnvalue_4 "/Game/Weapons/Actor_Components/BPC_Attack_Handler.BPC_Attack_Handler_C"))
  (bind _returnvalue_10 (Actor|GetComponentbyClass _returnvalue_3 "/Script/Engine.SkeletalMeshComponent"))
  (bind _returnvalue_11 (Actor|GetComponentbyClass _returnvalue_5 "/Game/Weapons/Actor_Components/BPC_Hitstop.BPC_Hitstop_C"))
  (bind _returnvalue_12 (Actor|GetComponentbyClass _returnvalue_6 "/Game/Weapons/Actor_Components/BPC_Attack_Handler.BPC_Attack_Handler_C"))
  (bind _returnvalue_13 (/ _damage 1e+03))
  (bind _returnvalue_14 (Transformation|GetSocketLocation _returnvalue_10 _unarmed_attack_bone))
  (bind _returnvalue_15 (+ 0.1 _returnvalue_13))
  (bind _attacking_melee_weapon (Variables|/Game/Weapons/Actor_Components/BPC_Attack_Handler.BPC_Attack_Handler_C|GetAttacking_Melee_Weapon _returnvalue_9))
  (bind _attacking_melee_weapon_2 (Variables|/Game/Weapons/Actor_Components/BPC_Attack_Handler.BPC_Attack_Handler_C|GetAttacking_Melee_Weapon _returnvalue_12))
  (bind _attacking_melee_weapon_3 (Variables|/Game/Weapons/Actor_Components/BPC_Attack_Handler.BPC_Attack_Handler_C|GetAttacking_Melee_Weapon _returnvalue_7))
  (bind _attacking_melee_weapon_4 (Variables|/Game/Weapons/Actor_Components/BPC_Attack_Handler.BPC_Attack_Handler_C|GetAttacking_Melee_Weapon _returnvalue_8))
  (if (Variables|Unarmed|GetUnarmed%20Attack)
    (bind (_outhits _returnvalue_16) (Class|KismetSystemLibrary|BoxTraceMultiforObjects _returnvalue_14 _returnvalue_14 "75.000000,75.000000,75.000000" (Transformation|GetSocketRotation _returnvalue_10 _unarmed_attack_bone) _array false (select (Utilities|IsValid _attacking_melee_weapon) (Utilities|Array|MakeArray (Components|GetOwner) _attacking_melee_weapon) (Utilities|Array|MakeArray (Components|GetOwner))) "ForDuration" true "(R=1.000000,G=0.000000,B=0.000000,A=1.000000)" "(R=0.000000,G=1.000000,B=0.000000,A=1.000000)" 1.0))
    (else
      (bind _static_mesh (Class|BPIMeleeWeapon|GetStaticMeshMelee(Message) _attacking_melee_weapon_4))
      (Class|BPIMeleeWeapon|GetMeleeInfo(Message) _attacking_melee_weapon_4)
      (bind (_outhits_2 _returnvalue_17) (Class|KismetSystemLibrary|BoxTraceMultiforObjects (Transformation|GetSocketLocation _static_mesh "HitBox_Top") (Transformation|GetSocketLocation _static_mesh "HitBox_Bottom") (Math|Conversions|ToVector(Float) (Math|Vector|Distance(Vector) (Transformation|GetSocketLocation _static_mesh "HitBox_Extent_Right") (Transformation|GetSocketLocation _static_mesh "HitBox_Extent_Left"))) (Transformation|GetWorldRotation _static_mesh) _array false (Utilities|Array|MakeArray (Components|GetOwner) (Variables|/Game/Weapons/Actor_Components/BPC_Attack_Handler.BPC_Attack_Handler_C|GetAttacking_Melee_Weapon (Actor|GetComponentbyClass (Components|GetOwner) "/Game/Weapons/Actor_Components/BPC_Attack_Handler.BPC_Attack_Handler_C"))) "ForOneFrame" true))))
  (if (select (Variables|Unarmed|GetUnarmed%20Attack) _returnvalue_16 _returnvalue_17)
    (for _array_element (select (Variables|Unarmed|GetUnarmed%20Attack) _outhits _outhits_2)
      (if (not (Utilities|Array|ContainsItem _hit_actors (.HitActor (Collision|BreakHitResult _array_element))))
        (Utilities|Array|Add _hit_actors (.HitActor (Collision|BreakHitResult _array_element)))
        (switch Utilities|FlowControl|Switch|SwitchonECollisionChannel (Collision|GetCollisionObjectType (.HitComponent (Collision|BreakHitResult _array_element)))
          (:ECC_Pawn
            (if (Utilities|DoesObjectImplementInterface (.HitActor (Collision|BreakHitResult _array_element)) "/Game/Health/Interfaces/BPI_Has_Health.BPI_Has_Health_C") :!label _label
              (Default|TakeDamage (Actor|GetComponentbyClass (.HitActor (Collision|BreakHitResult _array_element)) "/Game/Health/BPs/BPC_Health.BPC_Health_C") _damage (.Location (Collision|BreakHitResult _array_element)) (.HitActor (Collision|BreakHitResult _array_element)) (Components|GetOwner))
              (bind _ascharacter (Utilities|Casting|CastToCharacter (.HitActor (Collision|BreakHitResult _array_element))))
              (Character|LaunchCharacter _ascharacter (Math|Vector|MakeVector (.X (Class|KismetMathLibrary|BreakVector3f (/ (Math|Vector|SelectVector (+ (* (Math|Vector|GetUpVector (.HitComponent (Collision|BreakHitResult _array_element))) (Variables|Unarmed|GetKnockUpForce)) (* (Math|Vector|GetForwardVector (Math|Rotator|FindLookatRotation (Math|Vector|SelectVector (Transformation|GetSocketLocation (Actor|GetComponentbyClass (Components|GetOwner) "/Script/Engine.SkeletalMeshComponent") (Variables|Unarmed|GetUnarmed_Attack_Bone)) (Transformation|GetActorLocation (select (Utilities|IsValid _attacking_melee_weapon_2) _attacking_melee_weapon_2 _returnvalue_6)) (Variables|Unarmed|GetUnarmed%20Attack)) (Transformation|GetWorldLocation (.HitComponent (Collision|BreakHitResult _array_element))))) (Math|Float|SelectFloat (Variables|Unarmed|GetKnockbackForce) 9e+04 (Variables|Unarmed|GetUnarmed%20Attack)))) (* (Math|Vector|GetForwardVector (Math|Rotator|FindLookatRotation (Math|Vector|SelectVector (Transformation|GetSocketLocation (Actor|GetComponentbyClass (Components|GetOwner) "/Script/Engine.SkeletalMeshComponent") (Variables|Unarmed|GetUnarmed_Attack_Bone)) (Transformation|GetActorLocation (select (Utilities|IsValid _attacking_melee_weapon_2) _attacking_melee_weapon_2 _returnvalue_6)) (Variables|Unarmed|GetUnarmed%20Attack)) (Transformation|GetWorldLocation (.HitComponent (Collision|BreakHitResult _array_element))))) (Math|Float|SelectFloat (Variables|Unarmed|GetKnockbackForce) 9e+04 (Variables|Unarmed|GetUnarmed%20Attack))) (Variables|Unarmed|GetUnarmed%20Attack)) 75.0))) (.Y (Class|KismetMathLibrary|BreakVector3f (/ (Math|Vector|SelectVector (+ (* (Math|Vector|GetUpVector (.HitComponent (Collision|BreakHitResult _array_element))) (Variables|Unarmed|GetKnockUpForce)) (* (Math|Vector|GetForwardVector (Math|Rotator|FindLookatRotation (Math|Vector|SelectVector (Transformation|GetSocketLocation (Actor|GetComponentbyClass (Components|GetOwner) "/Script/Engine.SkeletalMeshComponent") (Variables|Unarmed|GetUnarmed_Attack_Bone)) (Transformation|GetActorLocation (select (Utilities|IsValid _attacking_melee_weapon_2) _attacking_melee_weapon_2 _returnvalue_6)) (Variables|Unarmed|GetUnarmed%20Attack)) (Transformation|GetWorldLocation (.HitComponent (Collision|BreakHitResult _array_element))))) (Math|Float|SelectFloat (Variables|Unarmed|GetKnockbackForce) 9e+04 (Variables|Unarmed|GetUnarmed%20Attack)))) (* (Math|Vector|GetForwardVector (Math|Rotator|FindLookatRotation (Math|Vector|SelectVector (Transformation|GetSocketLocation (Actor|GetComponentbyClass (Components|GetOwner) "/Script/Engine.SkeletalMeshComponent") (Variables|Unarmed|GetUnarmed_Attack_Bone)) (Transformation|GetActorLocation (select (Utilities|IsValid _attacking_melee_weapon_2) _attacking_melee_weapon_2 _returnvalue_6)) (Variables|Unarmed|GetUnarmed%20Attack)) (Transformation|GetWorldLocation (.HitComponent (Collision|BreakHitResult _array_element))))) (Math|Float|SelectFloat (Variables|Unarmed|GetKnockbackForce) 9e+04 (Variables|Unarmed|GetUnarmed%20Attack))) (Variables|Unarmed|GetUnarmed%20Attack)) 75.0))) (Math|Float|SelectFloat (.Z (Class|KismetMathLibrary|BreakVector3f (/ (Math|Vector|SelectVector (+ (* (Math|Vector|GetUpVector (.HitComponent (Collision|BreakHitResult _array_element))) (Variables|Unarmed|GetKnockUpForce)) (* (Math|Vector|GetForwardVector (Math|Rotator|FindLookatRotation (Math|Vector|SelectVector (Transformation|GetSocketLocation (Actor|GetComponentbyClass (Components|GetOwner) "/Script/Engine.SkeletalMeshComponent") (Variables|Unarmed|GetUnarmed_Attack_Bone)) (Transformation|GetActorLocation (select (Utilities|IsValid _attacking_melee_weapon_2) _attacking_melee_weapon_2 _returnvalue_6)) (Variables|Unarmed|GetUnarmed%20Attack)) (Transformation|GetWorldLocation (.HitComponent (Collision|BreakHitResult _array_element))))) (Math|Float|SelectFloat (Variables|Unarmed|GetKnockbackForce) 9e+04 (Variables|Unarmed|GetUnarmed%20Attack)))) (* (Math|Vector|GetForwardVector (Math|Rotator|FindLookatRotation (Math|Vector|SelectVector (Transformation|GetSocketLocation (Actor|GetComponentbyClass (Components|GetOwner) "/Script/Engine.SkeletalMeshComponent") (Variables|Unarmed|GetUnarmed_Attack_Bone)) (Transformation|GetActorLocation (select (Utilities|IsValid _attacking_melee_weapon_2) _attacking_melee_weapon_2 _returnvalue_6)) (Variables|Unarmed|GetUnarmed%20Attack)) (Transformation|GetWorldLocation (.HitComponent (Collision|BreakHitResult _array_element))))) (Math|Float|SelectFloat (Variables|Unarmed|GetKnockbackForce) 9e+04 (Variables|Unarmed|GetUnarmed%20Attack))) (Variables|Unarmed|GetUnarmed%20Attack)) 8.0))) 5e+01 (Variables|Unarmed|GetUnarmed%20Attack))) true true)
              (Utilities|FlowControl|Sequence
                (:then_0
                  (Utilities|IsValid (Actor|GetComponentbyClass (.HitActor (Collision|BreakHitResult _array_element)) "/Game/Weapons/Actor_Components/BPC_Hitstop.BPC_Hitstop_C")
                    (:Is%20Valid
                      (Default|StartHitstop (Actor|GetComponentbyClass (.HitActor (Collision|BreakHitResult _array_element)) "/Game/Weapons/Actor_Components/BPC_Hitstop.BPC_Hitstop_C") _returnvalue_15))
                    (:Is%20Not%20Valid
                      _))
                  (Utilities|IsValid _returnvalue_11
                    (:Is%20Valid
                      (Default|StartHitstop _returnvalue_11 _returnvalue_15))))
                (:then_1
                  (if (Utilities|DoesObjectImplementInterface (Components|GetOwner) "/Game/Characters/Player/BPI_Player.BPI_Player_C")
                    (Class|LegacyCameraShake|StartLegacyCameraShake (Game|GetPlayerCameraManager 0) "/Game/Weapons/BPs/BP_Melee_Hit_Camera_Shake.BP_Melee_Hit_Camera_Shake_C" 1.0 "CameraLocal" "0, 0, 0")))
                (:then_2
                  (Utilities|IsValid (Actor|GetComponentbyClass (.HitActor (Collision|BreakHitResult _array_element)) "/Game/VFX_SFX/Blood_Splatter/BPS/BPC_Blood_Effect.BPC_Blood_Effect_C")
                    (:Is%20Valid
                      (Default|BloodEffect (Actor|GetComponentbyClass (.HitActor (Collision|BreakHitResult _array_element)) "/Game/VFX_SFX/Blood_Splatter/BPS/BPC_Blood_Effect.BPC_Blood_Effect_C") (Math|Vector|SelectVector (Transformation|GetSocketLocation (Actor|GetComponentbyClass (Components|GetOwner) "/Script/Engine.SkeletalMeshComponent") (Variables|Unarmed|GetUnarmed_Attack_Bone)) (Math|Vector|SelectVector (Transformation|GetActorLocation _attacking_melee_weapon_3) (Transformation|GetActorLocation _returnvalue) (Utilities|IsValid _attacking_melee_weapon_3)) (Variables|Unarmed|GetUnarmed%20Attack)) (* (.Normal (Collision|BreakHitResult _array_element)) -1.0) (.HitActor (Collision|BreakHitResult _array_element)) _damage)
                      (Audio|PlaySoundatLocation "/Game/VFX_SFX/Blood_Splatter/Audio/Impact_Audio/Body_Impact_SC.Body_Impact_SC" (.Location (Collision|BreakHitResult _array_element)) "0, 0, 0" 1.0 1.0 0.0 0 0 0 0)))))))
          (:ECC_PhysicsBody
            (Physics|AddImpulse (.HitComponent (Collision|BreakHitResult _array_element)) (/ (+ (* (Math|Vector|GetUpVector (.HitComponent (Collision|BreakHitResult _array_element))) (Variables|Unarmed|GetKnockUpForce)) (* (Math|Vector|GetForwardVector (Math|Rotator|FindLookatRotation (Math|Vector|SelectVector (Transformation|GetSocketLocation (Actor|GetComponentbyClass (Components|GetOwner) "/Script/Engine.SkeletalMeshComponent") (Variables|Unarmed|GetUnarmed_Attack_Bone)) (Transformation|GetActorLocation (select (Utilities|IsValid _attacking_melee_weapon_2) _attacking_melee_weapon_2 _returnvalue_6)) (Variables|Unarmed|GetUnarmed%20Attack)) (Transformation|GetWorldLocation (.HitComponent (Collision|BreakHitResult _array_element))))) (Math|Float|SelectFloat (Variables|Unarmed|GetKnockbackForce) 9e+04 (Variables|Unarmed|GetUnarmed%20Attack)))) 1e+01) "None" true :!label _label_2)
            (if (Utilities|DoesObjectImplementInterface (Components|GetOwner) "/Game/Characters/Player/BPI_Player.BPI_Player_C")
              (Class|LegacyCameraShake|StartLegacyCameraShake (Game|GetPlayerCameraManager 0) "/Game/Weapons/BPs/BP_Melee_Hit_Camera_Shake.BP_Melee_Hit_Camera_Shake_C" 1.0 "CameraLocal" "0, 0, 0")))
          (:ECC_GameTraceChannel2
            (goto _label))
          (:ECC_GameTraceChannel3
            (goto _label_2))
          (:ECC_GameTraceChannel4
            (goto _label)))))))