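; Actor component that handles attack input for its owner, player or AI, routing unarmed, melee and ranged attacks to the weaponry, melee attack, ammo and shoot components.
; Ranged weapons branch by fire type into semi-auto, full-auto, burst, charge and charge-burst macros that gate CanFire with cooldowns and charging Niagara effects.
; Melee chooses light or heavy from hold time, updating the player crosshair.
; Tick refreshes CanFire from ammo and aiming, and cancels melee during weapon swaps.
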(event Custom|Handle_Attack
  (params (Unarmed%20Attack :type Boolean) (Heavy%20Attack :type Boolean))
  (bind _returnvalue (Components|GetOwner))
  (bind _returnvalue_2 (Actor|GetComponentbyClass _returnvalue "/Game/Weapons/Actor_Components/BPC_Weaponry.BPC_Weaponry_C"))
  (bind _equipped_weapon (Variables|/Game/Weapons/Actor_Components/BPC_Weaponry.BPC_Weaponry_C|GetEquipped_Weapon _returnvalue_2))
  (if Unarmed%20Attack
    ;[1 1 1] Unarmed Attack
    (Default|StartMeleeAttack (Actor|GetComponentbyClass (Components|GetOwner) "/Game/Weapons/Actor_Components/BPC_Melee_Attack.BPC_Melee_Attack_C") true false)
    (else
      (Utilities|IsValid _equipped_weapon
        (:Is%20Valid
          (bind _basics (Class|BPIWeapon|GetBasicInfo(Message) _equipped_weapon))
          (if (Utilities|Struct|BreakStruct_Weapon _basics)
            ;[1 1 1] If have ammo
            (if (> (Variables|/Game/Weapons/Actor_Components/BPC_Ammo.BPC_Ammo_C|GetCurrent_Ammo (Actor|GetComponentbyClass _equipped_weapon "/Game/Weapons/Actor_Components/BPC_Ammo.BPC_Ammo_C")) 0)
              ;[1 1 1] Shooting the equipped weapon's projectile and then if it is a full auto then we set can fire to false before doing a delay for the fire rate and then setting can fire back to true again
              (bind _ranged_info (Class|BPIRangedWeapon|GetRangedInfo(Message) _equipped_weapon))
              (bind _using_custom_projectile (Class|BPIRangedWeapon|GetCustomProjectile(Message) _equipped_weapon))
              (bind _returnvalue_3 (Utilities|GetDataTableRow "/Game/Projectiles/Structs_DataTables/DT_Projectiles.DT_Projectiles" (Utilities|String|StringToName (Utilities|String|EnumtoString (.ProjectileName (Utilities|Struct|BreakStruct_Ranged_Weapon _ranged_info)))))
                (:then
                  (Variables|Default|SetAttacking false)
                  (Default|Shoot (Actor|GetComponentbyClass _equipped_weapon "/Game/Weapons/Actor_Components/BPC_Shoot.BPC_Shoot_C") (select _using_custom_projectile (.Projectile_Info (Utilities|Struct|BreakStruct_Ranged_Weapon _ranged_info)) _returnvalue_3) _ranged_info)
                  (if (Utilities|Enum|Equal(Enum) (.Fire_Type (Utilities|Struct|BreakStruct_Ranged_Weapon _ranged_info)) "NewEnumerator2")
                    (Variables|Default|SetCan_Fire false)
                    (Utilities|FlowControl|Delay (Utilities|Struct|BreakStruct_Full_Auto_Info (.Full_Auto_Info (Utilities|Struct|BreakStruct_Ranged_Weapon _ranged_info))))
                    (Variables|Default|SetCan_Fire true)))))
            (else
              ;[1 1 1] Melee Attack
              (Default|StartMeleeAttack (Actor|GetComponentbyClass _returnvalue "/Game/Weapons/Actor_Components/BPC_Melee_Attack.BPC_Melee_Attack_C") false Heavy%20Attack)
              (if (Utilities|DoesObjectImplementInterface (Components|GetOwner) "/Game/Weapons/Unarmed_Attack/Interfaces/BPI_Can_Unarmed_Attack.BPI_Can_Unarmed_Attack_C")
                (Variables|/Game/Weapons/Actor_Components/BPC_Melee_Attack.BPC_Melee_Attack_C|SetUnarmed%20Attack (Actor|GetComponentbyClass (Components|GetOwner) "/Game/Weapons/Actor_Components/BPC_Melee_Attack.BPC_Melee_Attack_C") false)))))))))

(event Custom|End_Melee_Attack
  (params (Unarmed%20Attack :type Boolean))
  ;[1 1 1] Hitboxes and melee attack end
  (Default|MeleeAttackEnd (Actor|GetComponentbyClass (Components|GetOwner) "/Game/Weapons/Actor_Components/BPC_Melee_Attack.BPC_Melee_Attack_C")))

(event Custom|Start_Melee_Attack_HitBox
  (params (Unarmed%20Attack :type Boolean))
  ;[1 1 1] Hitboxes and melee attack end
  (Default|StartHitbox (Actor|GetComponentbyClass (Components|GetOwner) "/Game/Weapons/Actor_Components/BPC_Melee_Attack.BPC_Melee_Attack_C")))

(event Custom|Stop_Melee_Attack_HitBox
  (params (Unarmed%20Attack :type Boolean))
  ;[1 1 1] Hitboxes and melee attack end
  (Default|EndHitbox (Actor|GetComponentbyClass (Components|GetOwner) "/Game/Weapons/Actor_Components/BPC_Melee_Attack.BPC_Melee_Attack_C")))

(event Custom|Attack
  (params (Unarmed%20Attack :type Boolean) (Time :type Float%20%28double-precision%29))
  (bind _returnvalue (Components|GetOwner))
  (bind _returnvalue_2 (Components|GetOwner))
  (bind _returnvalue_3 (Actor|GetComponentbyClass _returnvalue "/Game/Weapons/Actor_Components/BPC_Weaponry.BPC_Weaponry_C"))
  (bind _returnvalue_4 (Actor|GetComponentbyClass _returnvalue_2 "/Game/Weapons/Actor_Components/BPC_Weaponry.BPC_Weaponry_C"))
  (bind _equipped_weapon (Variables|/Game/Weapons/Actor_Components/BPC_Weaponry.BPC_Weaponry_C|GetEquipped_Weapon _returnvalue_4))
  (bind _equipped_weapon_2 (Variables|/Game/Weapons/Actor_Components/BPC_Weaponry.BPC_Weaponry_C|GetEquipped_Weapon _returnvalue_3))
  (if Unarmed%20Attack
    ;[1 1 1] Unarmed attack branch
    (if (Variables|Default|GetAI%20Attacking?)
      (Utilities|FlowControl|Sequence
        (:then_0
          ;[1 1 1] Unarmed attack for AI or if the attack custom event is called
          (if (not (Variables|Default|GetAttacking)) :!label _label
            (Variables|/Game/Weapons/Actor_Components/BPC_Melee_Attack.BPC_Melee_Attack_C|SetUnarmed%20Attack (Actor|GetComponentbyClass (Components|GetOwner) "/Game/Weapons/Actor_Components/BPC_Melee_Attack.BPC_Melee_Attack_C") true)
            (CallFunction|HandleAttack true false)
            (Variables|/Game/Weapons/Actor_Components/BPC_Melee_Attack.BPC_Melee_Attack_C|SetCharging_Heavy (Actor|GetComponentbyClass (Components|GetOwner) "/Game/Weapons/Actor_Components/BPC_Melee_Attack.BPC_Melee_Attack_C") false)))
        (:then_1
          ;[1 1 1] Delay for manually calling attack function using the time parameter to delay attack input end custom event being called
          (Utilities|FlowControl|Delay Time :!label _label_2)
          (CallFunction|AttackInputEnd)))
      (else
        (goto _label)))
    (else
      (if (Variables|Default|GetAI%20Attacking?)
        (Utilities|FlowControl|Sequence
          (:then_0
            _)
          (:then_1
            (goto _label_2))))
      (Utilities|IsValid _equipped_weapon
        (:Is%20Valid
          ;[1 1 1] If ranged
          (bind _basics (Class|BPIWeapon|GetBasicInfo(Message) _equipped_weapon))
          (if (Utilities|Struct|BreakStruct_Weapon _basics)
            ;[1 1 1] Setting charging heavy and then checking if we can actually attack
            (Variables|/Game/Weapons/Actor_Components/BPC_Melee_Attack.BPC_Melee_Attack_C|SetCharging_Heavy (Actor|GetComponentbyClass (Components|GetOwner) "/Game/Weapons/Actor_Components/BPC_Melee_Attack.BPC_Melee_Attack_C") false)
            (if (Math|Boolean|ANDBoolean (not (Variables|Default|GetAttacking)) (Variables|Default|GetCan_Fire) (Variables|/Game/Weapons/Actor_Components/BPC_Aim.BPC_Aim_C|GetAiming? (Actor|GetComponentbyClass (Components|GetOwner) "/Game/Weapons/Actor_Components/BPC_Aim.BPC_Aim_C")))
              ;[1 1 1] Get ranged info and static mesh of equipped weaopn
              (bind _ranged_info (Class|BPIRangedWeapon|GetRangedInfo(Message) _equipped_weapon_2))
              (bind _static_mesh (Class|BPIRangedWeapon|GetStaticMesh(Message) _equipped_weapon_2))
              ;[1 1 1] Actual firing functionality based on the fire type of the ranged weapon
              ;;[1 1 1] Setting reference to ranged weapon mesh
              (Variables|Default|SetRanged%20Weapon%20Mesh _static_mesh)
              (switch Utilities|FlowControl|Switch|SwitchonEnum_Fire_Types (.Fire_Type (Utilities|Struct|BreakStruct_Ranged_Weapon _ranged_info))
                (:NewEnumerator1
                  (|SemiAuto))
                (:NewEnumerator2
                  (|FullAuto))
                (:NewEnumerator3
                  (|Burst (.Burst_Info (Utilities|Struct|BreakStruct_Ranged_Weapon _ranged_info))))
                (:NewEnumerator4
                  (|Charge (.Charged_Info (Utilities|Struct|BreakStruct_Ranged_Weapon _ranged_info)) (Math|Float|SelectFloat Time (stale Input|EnhancedActionEvents|EnhancedInputActionIA_Attack TriggeredSeconds) (Variables|Default|GetAI%20Attacking?)) (> (Variables|/Game/Weapons/Actor_Components/BPC_Ammo.BPC_Ammo_C|GetCurrent_Ammo (Actor|GetComponentbyClass (Variables|/Game/Weapons/Actor_Components/BPC_Weaponry.BPC_Weaponry_C|GetEquipped_Weapon (Actor|GetComponentbyClass (Components|GetOwner) "/Game/Weapons/Actor_Components/BPC_Weaponry.BPC_Weaponry_C")) "/Game/Weapons/Actor_Components/BPC_Ammo.BPC_Ammo_C")) 0)))
                (:NewEnumerator5
                  (|ChargeBurst (.Charged_Burst_Info (Utilities|Struct|BreakStruct_Ranged_Weapon _ranged_info)) (Math|Float|SelectFloat Time (stale Input|EnhancedActionEvents|EnhancedInputActionIA_Attack TriggeredSeconds) (Variables|Default|GetAI%20Attacking?)) (> (Variables|/Game/Weapons/Actor_Components/BPC_Ammo.BPC_Ammo_C|GetCurrent_Ammo (Actor|GetComponentbyClass (Variables|/Game/Weapons/Actor_Components/BPC_Weaponry.BPC_Weaponry_C|GetEquipped_Weapon (Actor|GetComponentbyClass (Components|GetOwner) "/Game/Weapons/Actor_Components/BPC_Weaponry.BPC_Weaponry_C")) "/Game/Weapons/Actor_Components/BPC_Ammo.BPC_Ammo_C")) 0)))))
            (else
              ;[1 1 1] Get melee info to get minimum charge time for the equipped melee weapon
              (bind _melee_info (Class|BPIMeleeWeapon|GetMeleeInfo(Message) (Variables|/Game/Weapons/Actor_Components/BPC_Weaponry.BPC_Weaponry_C|GetEquipped_Weapon (Actor|GetComponentbyClass (Components|GetOwner) "/Game/Weapons/Actor_Components/BPC_Weaponry.BPC_Weaponry_C"))))
              (if (< (Math|Float|SelectFloat Time (stale Input|EnhancedActionEvents|EnhancedInputActionIA_Attack TriggeredSeconds) (Variables|Default|GetAI%20Attacking?)) (Utilities|Struct|BreakStruct_Heavy_Attack_Info (Utilities|Struct|BreakStruct_Melee_Weapon _melee_info)))
                (Utilities|FlowControl|Sequence
                  (:then_0
                    (goto _label_3 Reset%20Do%20Once))
                  (:then_1
                    (goto _label_3 Melee%20Non%20Heavy)))
                (else
                  ;[1 1 1] Charging melee attack using attack input
                  (Variables|/Game/Weapons/Actor_Components/BPC_Melee_Attack.BPC_Melee_Attack_C|SetCharging_Heavy (Actor|GetComponentbyClass (Components|GetOwner) "/Game/Weapons/Actor_Components/BPC_Melee_Attack.BPC_Melee_Attack_C") true)
                  (|Changingcrosshair :!label _label_3))))))))))

(event Custom|Attack_Input_End
  (if (Utilities|Struct|BreakStruct_Weapon (stale Custom|Attack _basics))
    ;[1 1 1] Actual firing functionality based on the fire type of the ranged weapon
    ;;[1 1 1] Stopping attacking
    (Utilities|FlowControl|Sequence
      (:then_0
        (|SemiAuto) ; enters at Reset
      )
      (:then_1
        (|Charge (.Charged_Info (Utilities|Struct|BreakStruct_Ranged_Weapon (stale Custom|Attack _ranged_info))) (Math|Float|SelectFloat (stale Custom|Attack Time) (stale Input|EnhancedActionEvents|EnhancedInputActionIA_Attack TriggeredSeconds) (Variables|Default|GetAI%20Attacking?)) (> (Variables|/Game/Weapons/Actor_Components/BPC_Ammo.BPC_Ammo_C|GetCurrent_Ammo (Actor|GetComponentbyClass (Variables|/Game/Weapons/Actor_Components/BPC_Weaponry.BPC_Weaponry_C|GetEquipped_Weapon (Actor|GetComponentbyClass (Components|GetOwner) "/Game/Weapons/Actor_Components/BPC_Weaponry.BPC_Weaponry_C")) "/Game/Weapons/Actor_Components/BPC_Ammo.BPC_Ammo_C")) 0)) ; enters at Reset Niagara and Destroy Niagara
      )
      (:then_2
        (|Charge (.Charged_Info (Utilities|Struct|BreakStruct_Ranged_Weapon (stale Custom|Attack _ranged_info))) (Math|Float|SelectFloat (stale Custom|Attack Time) (stale Input|EnhancedActionEvents|EnhancedInputActionIA_Attack TriggeredSeconds) (Variables|Default|GetAI%20Attacking?)) (> (Variables|/Game/Weapons/Actor_Components/BPC_Ammo.BPC_Ammo_C|GetCurrent_Ammo (Actor|GetComponentbyClass (Variables|/Game/Weapons/Actor_Components/BPC_Weaponry.BPC_Weaponry_C|GetEquipped_Weapon (Actor|GetComponentbyClass (Components|GetOwner) "/Game/Weapons/Actor_Components/BPC_Weaponry.BPC_Weaponry_C")) "/Game/Weapons/Actor_Components/BPC_Ammo.BPC_Ammo_C")) 0)) ; enters at Reset
      )
      (:then_3
        (|ChargeBurst (.Charged_Burst_Info (Utilities|Struct|BreakStruct_Ranged_Weapon (stale Custom|Attack _ranged_info))) (Math|Float|SelectFloat (stale Custom|Attack Time) (stale Input|EnhancedActionEvents|EnhancedInputActionIA_Attack TriggeredSeconds) (Variables|Default|GetAI%20Attacking?)) (> (Variables|/Game/Weapons/Actor_Components/BPC_Ammo.BPC_Ammo_C|GetCurrent_Ammo (Actor|GetComponentbyClass (Variables|/Game/Weapons/Actor_Components/BPC_Weaponry.BPC_Weaponry_C|GetEquipped_Weapon (Actor|GetComponentbyClass (Components|GetOwner) "/Game/Weapons/Actor_Components/BPC_Weaponry.BPC_Weaponry_C")) "/Game/Weapons/Actor_Components/BPC_Ammo.BPC_Ammo_C")) 0)) ; enters at Finish Attack
      ))
    (else
      (Utilities|FlowControl|Sequence
        (:then_0
          (|MeleeAttackingAfterInputEnd (< (Math|Float|SelectFloat (stale Custom|Attack Time) (stale Input|EnhancedActionEvents|EnhancedInputActionIA_Attack TriggeredSeconds) (Variables|Default|GetAI%20Attacking?)) (Utilities|Struct|BreakStruct_Heavy_Attack_Info (Utilities|Struct|BreakStruct_Melee_Weapon (stale Custom|Attack _melee_info))))))
        (:then_1
          (Utilities|FlowControl|Sequence
            (:then_0
              (|Changingcrosshair) ; enters at Reset Do Once
            )
            (:then_1
              (|Changingcrosshair) ; enters at Melee Non Heavy
            )))))))

(event Input|EnhancedActionEvents|EnhancedInputActionIA_Attack
  (params (ActionValue :type Boolean) (ElapsedSeconds :type Float%20%28double-precision%29) (TriggeredSeconds :type Float%20%28double-precision%29) (InputAction :type Input%20Action%20Object%20Reference :default "/Game/Characters/Player/Input/Actions/IA_Attack.IA_Attack"))
  (bind _returnvalue (Components|GetOwner))
  (bind _returnvalue_2 (Components|GetOwner))
  (bind _returnvalue_3 (Actor|GetComponentbyClass _returnvalue "/Game/Weapons/Actor_Components/BPC_Weaponry.BPC_Weaponry_C"))
  (bind _returnvalue_4 (Actor|GetComponentbyClass _returnvalue_2 "/Game/Weapons/Actor_Components/BPC_Weaponry.BPC_Weaponry_C"))
  (bind _equipped_weapon (Variables|/Game/Weapons/Actor_Components/BPC_Weaponry.BPC_Weaponry_C|GetEquipped_Weapon _returnvalue_4))
  (bind _equipped_weapon_2 (Variables|/Game/Weapons/Actor_Components/BPC_Weaponry.BPC_Weaponry_C|GetEquipped_Weapon _returnvalue_3))
  (:Triggered
    (Utilities|IsValid _equipped_weapon
      (:Is%20Valid
        ;[1 1 1] If ranged
        (bind _basics (Class|BPIWeapon|GetBasicInfo(Message) _equipped_weapon))
        (if (Utilities|Struct|BreakStruct_Weapon _basics)
          ;[1 1 1] Setting charging heavy and then checking if we can actually attack
          (Variables|/Game/Weapons/Actor_Components/BPC_Melee_Attack.BPC_Melee_Attack_C|SetCharging_Heavy (Actor|GetComponentbyClass (Components|GetOwner) "/Game/Weapons/Actor_Components/BPC_Melee_Attack.BPC_Melee_Attack_C") false)
          (if (Math|Boolean|ANDBoolean (not (Variables|Default|GetAttacking)) (Variables|Default|GetCan_Fire) (Variables|/Game/Weapons/Actor_Components/BPC_Aim.BPC_Aim_C|GetAiming? (Actor|GetComponentbyClass (Components|GetOwner) "/Game/Weapons/Actor_Components/BPC_Aim.BPC_Aim_C")))
            ;[1 1 1] Get ranged info and static mesh of equipped weaopn
            (bind _ranged_info (Class|BPIRangedWeapon|GetRangedInfo(Message) _equipped_weapon_2))
            (bind _static_mesh (Class|BPIRangedWeapon|GetStaticMesh(Message) _equipped_weapon_2))
            ;[1 1 1] Actual firing functionality based on the fire type of the ranged weapon
            ;;[1 1 1] Setting reference to ranged weapon mesh
            (Variables|Default|SetRanged%20Weapon%20Mesh _static_mesh)
            (switch Utilities|FlowControl|Switch|SwitchonEnum_Fire_Types (.Fire_Type (Utilities|Struct|BreakStruct_Ranged_Weapon _ranged_info))
              (:NewEnumerator1
                (|SemiAuto :!label _label))
              (:NewEnumerator2
                (|FullAuto))
              (:NewEnumerator3
                (|Burst (.Burst_Info (Utilities|Struct|BreakStruct_Ranged_Weapon _ranged_info))))
              (:NewEnumerator4
                (|Charge (.Charged_Info (Utilities|Struct|BreakStruct_Ranged_Weapon _ranged_info)) (Math|Float|SelectFloat (stale Custom|Attack Time) TriggeredSeconds (Variables|Default|GetAI%20Attacking?)) (> (Variables|/Game/Weapons/Actor_Components/BPC_Ammo.BPC_Ammo_C|GetCurrent_Ammo (Actor|GetComponentbyClass (Variables|/Game/Weapons/Actor_Components/BPC_Weaponry.BPC_Weaponry_C|GetEquipped_Weapon (Actor|GetComponentbyClass (Components|GetOwner) "/Game/Weapons/Actor_Components/BPC_Weaponry.BPC_Weaponry_C")) "/Game/Weapons/Actor_Components/BPC_Ammo.BPC_Ammo_C")) 0) :!label _label_2))
              (:NewEnumerator5
                (|ChargeBurst (.Charged_Burst_Info (Utilities|Struct|BreakStruct_Ranged_Weapon _ranged_info)) (Math|Float|SelectFloat (stale Custom|Attack Time) TriggeredSeconds (Variables|Default|GetAI%20Attacking?)) (> (Variables|/Game/Weapons/Actor_Components/BPC_Ammo.BPC_Ammo_C|GetCurrent_Ammo (Actor|GetComponentbyClass (Variables|/Game/Weapons/Actor_Components/BPC_Weaponry.BPC_Weaponry_C|GetEquipped_Weapon (Actor|GetComponentbyClass (Components|GetOwner) "/Game/Weapons/Actor_Components/BPC_Weaponry.BPC_Weaponry_C")) "/Game/Weapons/Actor_Components/BPC_Ammo.BPC_Ammo_C")) 0) :!label _label_3))))
          (else
            ;[1 1 1] Get melee info to get minimum charge time for the equipped melee weapon
            (bind _melee_info (Class|BPIMeleeWeapon|GetMeleeInfo(Message) (Variables|/Game/Weapons/Actor_Components/BPC_Weaponry.BPC_Weaponry_C|GetEquipped_Weapon (Actor|GetComponentbyClass (Components|GetOwner) "/Game/Weapons/Actor_Components/BPC_Weaponry.BPC_Weaponry_C"))))
            (if (< (Math|Float|SelectFloat (stale Custom|Attack Time) TriggeredSeconds (Variables|Default|GetAI%20Attacking?)) (Utilities|Struct|BreakStruct_Heavy_Attack_Info (Utilities|Struct|BreakStruct_Melee_Weapon _melee_info)))
              (Utilities|FlowControl|Sequence :!label _label_4
                (:then_0
                  (goto _label_5 Reset%20Do%20Once))
                (:then_1
                  (goto _label_5 Melee%20Non%20Heavy)))
              (else
                ;[1 1 1] Charging melee attack using attack input
                (Variables|/Game/Weapons/Actor_Components/BPC_Melee_Attack.BPC_Melee_Attack_C|SetCharging_Heavy (Actor|GetComponentbyClass (Components|GetOwner) "/Game/Weapons/Actor_Components/BPC_Melee_Attack.BPC_Melee_Attack_C") true)
                (|Changingcrosshair :!label _label_5))))))))
  (:Canceled
    (if (Utilities|Struct|BreakStruct_Weapon _basics) :!label _label_6
      ;;[1 1 1] Stopping attacking
      (Utilities|FlowControl|Sequence
        (:then_0
          (goto _label Reset))
        (:then_1
          (goto _label_2 Reset%20Niagara%20and%20Destroy%20Niagara))
        (:then_2
          (goto _label_2 Reset))
        (:then_3
          (goto _label_3 Finish%20Attack)))
      (else
        (Utilities|FlowControl|Sequence
          (:then_0
            (|MeleeAttackingAfterInputEnd (< (Math|Float|SelectFloat (stale Custom|Attack Time) TriggeredSeconds (Variables|Default|GetAI%20Attacking?)) (Utilities|Struct|BreakStruct_Heavy_Attack_Info (Utilities|Struct|BreakStruct_Melee_Weapon _melee_info)))))
          (:then_1
            (goto _label_4))))))
  (:Completed
    (goto _label_6)))

(event EventTick
  (params (DeltaSeconds :type Float%20%28single-precision%29))
  (bind _returnvalue (Components|GetOwner))
  (bind _returnvalue_2 (Components|GetOwner))
  (bind _returnvalue_3 (Actor|GetComponentbyClass _returnvalue "/Game/Weapons/Actor_Components/BPC_Weaponry.BPC_Weaponry_C"))
  (bind _returnvalue_4 (Actor|GetComponentbyClass _returnvalue_2 "/Game/Weapons/Actor_Components/BPC_Melee_Attack.BPC_Melee_Attack_C"))
  (bind _equipped_weapon (Variables|/Game/Weapons/Actor_Components/BPC_Weaponry.BPC_Weaponry_C|GetEquipped_Weapon _returnvalue_3))
  (Utilities|FlowControl|Sequence
    (:then_0
      ;[1 1 1] Setting can fire
      (if (Utilities|IsValid _equipped_weapon)
        (Variables|Default|SetCan_Fire (and (> (Variables|/Game/Weapons/Actor_Components/BPC_Ammo.BPC_Ammo_C|GetCurrent_Ammo (Actor|GetComponentbyClass _equipped_weapon "/Game/Weapons/Actor_Components/BPC_Ammo.BPC_Ammo_C")) 0) (Variables|/Game/Weapons/Actor_Components/BPC_Aim.BPC_Aim_C|GetAiming? (Actor|GetComponentbyClass _returnvalue "/Game/Weapons/Actor_Components/BPC_Aim.BPC_Aim_C"))))))
    (:then_1
      ;[1 1 1] Setting charging heavy to be false if we are swapping weapons whilst attacking and then if we are doing an unarmed attack then we end the melee attack and stop melee attack passing unarmed attack true and if not then we do the same passing false
      (if (Variables|Default|GetAttacking)
        (if (Variables|/Game/Weapons/Actor_Components/BPC_Weaponry.BPC_Weaponry_C|GetSwapping_Weapons (Actor|GetComponentbyClass (Components|GetOwner) "/Game/Weapons/Actor_Components/BPC_Weaponry.BPC_Weaponry_C"))
          (Variables|/Game/Weapons/Actor_Components/BPC_Melee_Attack.BPC_Melee_Attack_C|SetCharging_Heavy _returnvalue_4 false)
          (if (Variables|/Game/Weapons/Actor_Components/BPC_Melee_Attack.BPC_Melee_Attack_C|GetUnarmed%20Attack _returnvalue_4)
            (CallFunction|EndMeleeAttack true)
            (CallFunction|StopMeleeAttackHitBox true)
            (else
              (CallFunction|EndMeleeAttack false)
              (CallFunction|StopMeleeAttackHitBox false))))))))

(fn GrapplingCheck
  (bind _returnvalue (Components|GetOwner))
  (bind _returnvalue_2 (Actor|GetComponentbyClass _returnvalue "/Game/Characters/Player/Grappling/BPC_Blood_Grapple_Swing.BPC_Blood_Grapple_Swing_C"))
  (return (not (Math|Boolean|ORBoolean (Variables|/Game/Characters/Player/Grappling/BPC_Blood_Grapple_Swing.BPC_Blood_Grapple_Swing_C|GetGrapple%20Pull? _returnvalue_2) (Variables|/Game/Characters/Player/Grappling/BPC_Blood_Grapple_Swing.BPC_Blood_Grapple_Swing_C|GetGrappled _returnvalue_2) (Variables|/Game/Characters/Player/Grappling/BPC_Blood_Grapple_Swing.BPC_Blood_Grapple_Swing_C|GetSwinging _returnvalue_2)))))