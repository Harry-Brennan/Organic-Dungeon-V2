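; Weapon recoil component that kicks the wielder's aim, launches them backward and shakes the player's camera.
; Start_Recoil stores the parameters and randomly picks left or right, then Tick offsets control rotation along vertical and horizontal curves until the duration elapses.
; Knockback launches the character opposite the aim, gated by movement mode and skipped while grapple-swinging.
; Camera shake runs only for BPI_Player owners, scaled by vertical recoil.
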(event Custom|Camera%20Shake
  (bind _output_get (Variables|Shake|SetCamera_Shake_Scale (Math|Float|Clamp(Float) (- (/ (Variables|RecoilAmounts|GetRecoil%20Amount%20Vertical) 1e+01) 0.5) 0.0 2.5)))
  (Class|LegacyCameraShake|StartLegacyCameraShake (Game|GetPlayerCameraManager 0) "/Game/Weapons/BPs/BP_Recoil_Camera_Shake.BP_Recoil_Camera_Shake_C" _output_get "World" "0, 0, 0"))

(event Custom|Physical%20Recoil
  (bind _aspawn (Utilities|Casting|CastToPawn (Components|GetOwner (Components|GetOwner))))
  (Variables|References|SetController (Pawn|GetController _aspawn))
  (Variables|Duration|SetRecoil_Percent 0.0)
  (Components|Tick|SetComponentTickEnabled true))

(event Custom|Start_Recoil
  (params (Recoil%20Duration :type Float%20%28double-precision%29) (Knockback%20Amount :type Float%20%28double-precision%29) (Vertical%20Recoil%20Curve :type Runtime%20Float%20Curve%20Structure) (Recoil%20Amount%20Vertical :type Float%20%28double-precision%29) (Horizontal%20Recoil%20Curve :type Runtime%20Float%20Curve%20Structure) (Recoil%20Amount%20Horizontal :type Float%20%28double-precision%29))
  (Variables|RecoilAmounts|SetRecoil%20Amount%20Vertical Recoil%20Amount%20Vertical)
  (Variables|Duration|SetRecoil_Duration Recoil%20Duration)
  (Variables|PhysicalKnockback|SetKnockback_Amount Knockback%20Amount)
  (Variables|RecoilAmounts|SetVertical%20Recoil%20Curve Vertical%20Recoil%20Curve)
  (Variables|RecoilAmounts|SetHorizontal%20Recoil%20Curve Horizontal%20Recoil%20Curve)
  (Variables|RecoilAmounts|SetRecoil%20Amount%20Horizontal Recoil%20Amount%20Horizontal)
  (Variables|RecoilAmounts|SetHorizontal%20Recoil%20Direction (Math|Random|RandomBoolwithWeight 0.5))
  (CallFunction|PhysicalRecoil)
  (if (Utilities|Enum|NotEqual(Enum) (Variables|/Game/Movement/BPC_Custom_Movement_Handler.BPC_Custom_Movement_Handler_C|GetCurrent_Movement_Mode (Actor|GetComponentbyClass (Components|GetOwner (Components|GetOwner)) "/Game/Movement/BPC_Custom_Movement_Handler.BPC_Custom_Movement_Handler_C")) "NewEnumerator0")
    (CallFunction|RecoilKnockback))
  (if (Utilities|DoesObjectImplementInterface (Components|GetOwner (Components|GetOwner)) "/Game/Characters/Player/BPI_Player.BPI_Player_C")
    (CallFunction|CameraShake)))

(event Custom|Stop_Recoil
  (Components|Tick|SetComponentTickEnabled false))

(event Custom|Recoil_Knockback
  (bind _returnvalue (Components|GetOwner))
  (bind _returnvalue_2 (Components|GetOwner))
  (bind _returnvalue_3 (Components|GetOwner _returnvalue))
  (bind _returnvalue_4 (Components|GetOwner _returnvalue_2))
  (bind _returnvalue_5 (Actor|GetComponentbyClass _returnvalue_4 "/Game/Movement/Grappling/BPC_Blood_Grapple_Swing.BPC_Blood_Grapple_Swing_C"))
  (Utilities|IsValid _returnvalue_5
    (:Is%20Valid
      (if (not (Variables|/Game/Movement/Grappling/BPC_Blood_Grapple_Swing.BPC_Blood_Grapple_Swing_C|GetSwinging _returnvalue_5))
        (bind _aspawn (Utilities|Casting|CastToPawn _returnvalue_3 :!label _label))
        (bind _ascharacter (Utilities|Casting|CastToCharacter _returnvalue_3))
        (Character|LaunchCharacter _ascharacter (* (Math|Vector|GetForwardVector (Pawn|GetControlRotation (Pawn|GetController _aspawn) :!class /Script/Engine.Controller)) (* (Variables|PhysicalKnockback|GetKnockback_Amount) -1.0)) false false)))
    (:Is%20Not%20Valid
      (goto _label))))

(event EventTick
  (params (DeltaSeconds :type Float%20%28single-precision%29))
  (bind _returnvalue (Class|ActorComponent|GetComponentTickInterval))
  (bind _recoil_duration (Variables|Duration|GetRecoil_Duration))
  (bind _controller (Variables|References|GetController))
  (bind _returnvalue_2 (Pawn|GetControlRotation _controller :!class /Script/Engine.Controller))
  (bind _returnvalue_3 (/ _recoil_duration _returnvalue))
  (bind (_roll _pitch _yaw) (Math|Rotator|BreakRotator _returnvalue_2))
  (bind _returnvalue_4 (/ 1.0 _returnvalue_3))
  (bind _output_get (Variables|Duration|SetRecoil_Percent (+ (Variables|Duration|GetRecoil_Percent) _returnvalue_4)))
  (if (>= _output_get 1.0)
    (CallFunction|StopRecoil)
    (else
      (Pawn|SetControlRotation (Variables|References|GetController) (Math|Rotator|MakeRotator (.Roll (Math|Rotator|BreakRotator (Math|Rotator|Lerp(Rotator) _returnvalue_2 (Math|Rotator|MakeRotator _roll (+ _pitch (* (* (Variables|RecoilAmounts|GetRecoil%20Amount%20Vertical) (Class|RecoilFunctionLibrary|GetRuntimeFloatCurveValue (Variables|RecoilAmounts|GetVertical%20Recoil%20Curve) (Variables|Duration|GetRecoil_Percent))) _returnvalue_4)) (Math|Float|SelectFloat (+ _yaw (* (* (Variables|RecoilAmounts|GetRecoil%20Amount%20Horizontal) (Class|RecoilFunctionLibrary|GetRuntimeFloatCurveValue (Variables|RecoilAmounts|GetHorizontal%20Recoil%20Curve) (Variables|Duration|GetRecoil_Percent))) _returnvalue_4)) (- _yaw (* (* (Variables|RecoilAmounts|GetRecoil%20Amount%20Horizontal) (Class|RecoilFunctionLibrary|GetRuntimeFloatCurveValue (Variables|RecoilAmounts|GetHorizontal%20Recoil%20Curve) (Variables|Duration|GetRecoil_Percent))) _returnvalue_4)) (Variables|RecoilAmounts|GetHorizontal%20Recoil%20Direction))) 1.0))) (.Pitch (Math|Rotator|BreakRotator (Math|Rotator|Lerp(Rotator) _returnvalue_2 (Math|Rotator|MakeRotator _roll (+ _pitch (* (* (Variables|RecoilAmounts|GetRecoil%20Amount%20Vertical) (Class|RecoilFunctionLibrary|GetRuntimeFloatCurveValue (Variables|RecoilAmounts|GetVertical%20Recoil%20Curve) (Variables|Duration|GetRecoil_Percent))) _returnvalue_4)) (Math|Float|SelectFloat (+ _yaw (* (* (Variables|RecoilAmounts|GetRecoil%20Amount%20Horizontal) (Class|RecoilFunctionLibrary|GetRuntimeFloatCurveValue (Variables|RecoilAmounts|GetHorizontal%20Recoil%20Curve) (Variables|Duration|GetRecoil_Percent))) _returnvalue_4)) (- _yaw (* (* (Variables|RecoilAmounts|GetRecoil%20Amount%20Horizontal) (Class|RecoilFunctionLibrary|GetRuntimeFloatCurveValue (Variables|RecoilAmounts|GetHorizontal%20Recoil%20Curve) (Variables|Duration|GetRecoil_Percent))) _returnvalue_4)) (Variables|RecoilAmounts|GetHorizontal%20Recoil%20Direction))) 1.0))) (.Yaw (Math|Rotator|BreakRotator (Math|Rotator|Lerp(Rotator) _returnvalue_2 (Math|Rotator|MakeRotator _roll (+ _pitch (* (* (Variables|RecoilAmounts|GetRecoil%20Amount%20Vertical) (Class|RecoilFunctionLibrary|GetRuntimeFloatCurveValue (Variables|RecoilAmounts|GetVertical%20Recoil%20Curve) (Variables|Duration|GetRecoil_Percent))) _returnvalue_4)) (Math|Float|SelectFloat (+ _yaw (* (* (Variables|RecoilAmounts|GetRecoil%20Amount%20Horizontal) (Class|RecoilFunctionLibrary|GetRuntimeFloatCurveValue (Variables|RecoilAmounts|GetHorizontal%20Recoil%20Curve) (Variables|Duration|GetRecoil_Percent))) _returnvalue_4)) (- _yaw (* (* (Variables|RecoilAmounts|GetRecoil%20Amount%20Horizontal) (Class|RecoilFunctionLibrary|GetRuntimeFloatCurveValue (Variables|RecoilAmounts|GetHorizontal%20Recoil%20Curve) (Variables|Duration|GetRecoil_Percent))) _returnvalue_4)) (Variables|RecoilAmounts|GetHorizontal%20Recoil%20Direction))) 1.0))))))))