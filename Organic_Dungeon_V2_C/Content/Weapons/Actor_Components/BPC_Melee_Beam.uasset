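; Melee weapon component that fires a BP_Melee_Beam projectile from the weapon, styled by its heavy attack info.
; Shoot_Beam shakes the camera for player wielders, clears HitActors, then traces from the wielder's head along control rotation.
; The beam spawns at the Projectile_Loc socket, aimed at the trace hit or end point and rolled against the mesh's roll.
; Beam size scales with the distance between the mesh's top and bottom hitbox sockets.
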(event Custom|Shoot_Beam
  (bind _returnvalue (Components|GetOwner))
  (bind _returnvalue_2 (Components|GetOwner))
  (bind _returnvalue_3 (Components|GetOwner))
  (bind _returnvalue_4 (Components|GetOwner))
  (bind _returnvalue_5 (Components|GetOwner _returnvalue_4))
  (bind _returnvalue_6 (Actor|GetComponentbyClass _returnvalue_5 "/Script/Engine.SkeletalMeshComponent"))
  (bind _returnvalue_7 (Transformation|GetSocketLocation _returnvalue_6 "head"))
  (if (Utilities|DoesObjectImplementInterface (Components|GetOwner (Components|GetOwner)) "/Game/Characters/Player/BPI_Player.BPI_Player_C")
    (Class|LegacyCameraShake|StartLegacyCameraShake (Game|GetPlayerCameraManager 0) "/Game/Weapons/BPs/BP_Melee_Hit_Camera_Shake.BP_Melee_Hit_Camera_Shake_C" 0.75 "CameraLocal" "0, 0, 0"))
  (Utilities|Array|Clear (Variables|Default|GetHit_Actors))
  (bind _aspawn (Utilities|Casting|CastToPawn _returnvalue_5))
  (bind _static_mesh (Class|BPIMeleeWeapon|GetStaticMeshMelee(Message) (Components|GetOwner)))
  (bind (_outhit _returnvalue_8) (Collision|LineTraceByChannel _returnvalue_7 (+ (* (Math|Vector|GetForwardVector (Pawn|GetControlRotation (Pawn|GetController _aspawn) :!class /Script/Engine.Controller)) 2.5e+03) _returnvalue_7) "TraceTypeQuery1" false (Utilities|Array|MakeArray _returnvalue (Components|GetOwner _returnvalue)) "None"))
  (bind _melee_info (Class|BPIMeleeWeapon|GetMeleeInfo(Message) _returnvalue_2))
  (Game|SpawnActorfromClass "/Game/VFX_SFX/Melee_Beam/BPS/BP_Melee_Beam.BP_Melee_Beam_C" (Math|Transform|MakeTransform (Transformation|GetSocketLocation _static_mesh "Projectile_Loc") (Math|Rotator|MakeRotator (* (.Roll (Math|Rotator|BreakRotator (Transformation|GetWorldRotation _static_mesh))) -1.0) (.pitch (Math|Rotator|FindLookatRotation (Transformation|GetActorLocation _returnvalue_2) (Math|Vector|SelectVector (.Location (Collision|BreakHitResult _outhit)) (.TraceEnd (Collision|BreakHitResult _outhit)) _returnvalue_8))) (.yaw (Math|Rotator|FindLookatRotation (Transformation|GetActorLocation _returnvalue_2) (Math|Vector|SelectVector (.Location (Collision|BreakHitResult _outhit)) (.TraceEnd (Collision|BreakHitResult _outhit)) _returnvalue_8)))) "1.000000,1.000000,1.000000") "Undefined" "MultiplyWithRoot" 0 (Utilities|Struct|BreakStruct_Heavy_Attack_Info (Utilities|Struct|BreakStruct_Melee_Weapon _melee_info)) (Math|Vector2D|MakeVector2D (* (Math|Vector|Distance(Vector) (Transformation|GetSocketLocation _static_mesh "HitBox_Top") (Transformation|GetSocketLocation _static_mesh "HitBox_Bottom")) 4.0) (* (Math|Vector|Distance(Vector) (Transformation|GetSocketLocation _static_mesh "HitBox_Top") (Transformation|GetSocketLocation _static_mesh "HitBox_Bottom")) 4.0)) (Components|GetOwner _returnvalue_3) _returnvalue_3 "0.000000,0.000000,0.000000" 0))