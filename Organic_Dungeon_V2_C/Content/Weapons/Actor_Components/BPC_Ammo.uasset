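; Weapon component that tracks ammo and runs timed reloads, reading reload settings from the owning weapon's ranged info.
; Starting a reload ends any attack input and enables Tick, which either adds rounds at percentage thresholds or refills an emptied magazine when time elapses.
; Reload steps play a sound and report noise.
; If the wielder implements BPI_Player, ammo changes update the equipped HUD slot's count, colour and animation.
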(event Custom|Decrease_Ammo
  (bind _returnvalue (Components|GetOwner))
  (bind _returnvalue_2 (Components|GetOwner))
  (bind _current_ammo (Variables|Default|GetCurrent_Ammo))
  (bind _max_ammo (Variables|Default|GetMax_Ammo))
  (bind _current_ammo_2 (Variables|Default|GetCurrent_Ammo))
  (bind _returnvalue_3 (Math|Conversions|ToFloat(Integer) _max_ammo))
  (bind _returnvalue_4 (Math|Conversions|ToFloat(Integer) _current_ammo))
  (bind _returnvalue_5 (Components|GetOwner _returnvalue))
  (bind _returnvalue_6 (Components|GetOwner _returnvalue_2))
  (bind _returnvalue_7 (Utilities|DoesObjectImplementInterface _returnvalue_5 "/Game/Characters/Player/BPI_Player.BPI_Player_C"))
  (bind _returnvalue_8 (Actor|GetComponentbyClass _returnvalue_6 "/Game/Characters/Player/BPC_HUD.BPC_HUD_C"))
  (bind _returnvalue_9 (/ _returnvalue_4 _returnvalue_3))
  (bind _hud_ref (Variables|/Game/Characters/Player/BPC_HUD.BPC_HUD_C|GetHUD_Ref _returnvalue_8))
  (bind _weapon_1 (Variables|/Game/UI/WBP_HUD.WBP_HUD_C|GetWeapon_1 _hud_ref))
  (bind _weapon_2 (Variables|/Game/UI/WBP_HUD.WBP_HUD_C|GetWeapon_2 _hud_ref))
  (bind _weapon_3 (Variables|/Game/UI/WBP_HUD.WBP_HUD_C|GetWeapon_3 _hud_ref))
  ;[1 1 1] Only able to decrease ammo if there is ammo to decrease
  (if (not (<= (Variables|Default|GetCurrent_Ammo) 0))
    (Math|Integer|DecrementInt (Variables|Default|GetCurrent_Ammo)
      (:%20%20
        ;[1 1 1] Resetting reload percentage and reloading seconds
        (Variables|Default|SetReload_Percent 0.0)
        (Variables|Default|SetReloading_Seconds 0.0)
        ;[1 1 1] Update ammo count in HUD and update the colour for the weapon image in the HUD and then play the ammo animation for the weapon in the HUD
        (if (Utilities|DoesObjectImplementInterface (Components|GetOwner (Components|GetOwner)) "/Game/Characters/Player/BPI_Player.BPI_Player_C")
          (switch int (Variables|/Game/UI/WBP_HUD.WBP_HUD_C|GetCurrently_Equipped_Weapon_Image_Relation _hud_ref)
            (:0
              (Default|UpdateImgColourforAmmo _weapon_1 _returnvalue_9)
              (Default|UpdateAmmoCount _weapon_1 _current_ammo_2 _returnvalue_7))
            (:1
              (Default|UpdateImgColourforAmmo _weapon_2 _returnvalue_9)
              (Default|UpdateAmmoCount _weapon_2 _current_ammo_2 _returnvalue_7))
            (:2
              (Default|UpdateImgColourforAmmo _weapon_3 _returnvalue_9)
              (Default|UpdateAmmoCount _weapon_3 _current_ammo_2 _returnvalue_7)))
          (Default|PlayAmmoAnimation (Variables|/Game/Characters/Player/BPC_HUD.BPC_HUD_C|GetHUD_Ref (Actor|GetComponentbyClass (Components|GetOwner (Components|GetOwner)) "/Game/Characters/Player/BPC_HUD.BPC_HUD_C")) true))))))

(event Custom|Reload
  (bind _returnvalue (Components|GetOwner))
  (bind _returnvalue_2 (Components|GetOwner))
  (bind _returnvalue_3 (Components|GetOwner _returnvalue))
  (bind _returnvalue_4 (Components|GetOwner _returnvalue_2))
  (bind _returnvalue_5 (Utilities|DoesObjectImplementInterface _returnvalue_3 "/Game/Characters/Player/BPI_Player.BPI_Player_C"))
  (bind _returnvalue_6 (Actor|GetComponentbyClass _returnvalue_4 "/Game/Characters/Player/BPC_HUD.BPC_HUD_C"))
  (bind _hud_ref (Variables|/Game/Characters/Player/BPC_HUD.BPC_HUD_C|GetHUD_Ref _returnvalue_6))
  (bind _weapon_1 (Variables|/Game/UI/WBP_HUD.WBP_HUD_C|GetWeapon_1 _hud_ref))
  (bind _weapon_2 (Variables|/Game/UI/WBP_HUD.WBP_HUD_C|GetWeapon_2 _hud_ref))
  (bind _weapon_3 (Variables|/Game/UI/WBP_HUD.WBP_HUD_C|GetWeapon_3 _hud_ref))
  ;[1 1 1] Can only reload if current ammo is less than max ammo
  (if (< (Variables|Default|GetCurrent_Ammo) (Variables|Default|GetMax_Ammo))
    (if (Variables|Default|GetReloading)
      ;[1 1 1] Stopping reload incase one is already active
      (CallFunction|StopReload)
      ;[1 1 1] If full reload then current ammo is set to 0 immediately since the by ammo reload starts on the ammo you already have
      (bind _ranged_info (Class|BPIRangedWeapon|GetRangedInfo(Message) (Components|GetOwner)))
      (switch Utilities|FlowControl|Switch|SwitchonEnum_Reload_Types (Utilities|Struct|BreakStruct_Reload_Info (.Reload_Info (Utilities|Struct|BreakStruct_Ranged_Weapon _ranged_info)))
        (:NewEnumerator0
          _)
        (:NewEnumerator1
          (Variables|Default|SetCurrent_Ammo 0)))
      (else
        ;[1 1 1] If full reload then set current ammo to 0 since the by ammo reload goes from what the current ammo already is
        (bind _ranged_info_2 (Class|BPIRangedWeapon|GetRangedInfo(Message) (Components|GetOwner)))
        (switch Utilities|FlowControl|Switch|SwitchonEnum_Reload_Types (Utilities|Struct|BreakStruct_Reload_Info (.Reload_Info (Utilities|Struct|BreakStruct_Ranged_Weapon _ranged_info_2)))
          (:NewEnumerator0
            _)
          (:NewEnumerator1
            (Variables|Default|SetCurrent_Ammo 0)))
        (CallFunction|StartReload)))
    (if (Utilities|DoesObjectImplementInterface (Components|GetOwner (Components|GetOwner)) "/Game/Characters/Player/BPI_Player.BPI_Player_C")
      ;[1 1 1] Update ammo count in HUD and update the colour for the weapon image in the HUD and then play the ammo animation for the weapon in the HUD
      (switch int (Variables|/Game/UI/WBP_HUD.WBP_HUD_C|GetCurrently_Equipped_Weapon_Image_Relation _hud_ref)
        (:0
          (Default|UpdateImgColourforAmmo _weapon_1 (/ (Math|Conversions|ToFloat(Integer) (Variables|Default|GetCurrent_Ammo)) (Math|Conversions|ToFloat(Integer) (Variables|Default|GetMax_Ammo))))
          (Default|UpdateAmmoCount _weapon_1 (Variables|Default|GetCurrent_Ammo) _returnvalue_5))
        (:1
          (Default|UpdateImgColourforAmmo _weapon_2 (/ (Math|Conversions|ToFloat(Integer) (Variables|Default|GetCurrent_Ammo)) (Math|Conversions|ToFloat(Integer) (Variables|Default|GetMax_Ammo))))
          (Default|UpdateAmmoCount _weapon_2 (Variables|Default|GetCurrent_Ammo) _returnvalue_5))
        (:2
          (Default|UpdateImgColourforAmmo _weapon_3 (/ (Math|Conversions|ToFloat(Integer) (Variables|Default|GetCurrent_Ammo)) (Math|Conversions|ToFloat(Integer) (Variables|Default|GetMax_Ammo))))
          (Default|UpdateAmmoCount _weapon_3 (Variables|Default|GetCurrent_Ammo) _returnvalue_5)))
      (Default|PlayAmmoAnimation (Variables|/Game/Characters/Player/BPC_HUD.BPC_HUD_C|GetHUD_Ref (Actor|GetComponentbyClass (Components|GetOwner (Components|GetOwner)) "/Game/Characters/Player/BPC_HUD.BPC_HUD_C")) true))))

(event Custom|Start_Reload
  (bind _returnvalue (Components|GetOwner))
  (bind _returnvalue_2 (Components|GetOwner _returnvalue))
  (bind _returnvalue_3 (Actor|GetComponentbyClass _returnvalue_2 "/Game/Weapons/Actor_Components/BPC_Attack_Handler.BPC_Attack_Handler_C"))
  (if (Variables|/Game/Weapons/Actor_Components/BPC_Attack_Handler.BPC_Attack_Handler_C|GetAttempting%20to%20Attack%20Input _returnvalue_3)
    (Default|AttackInputEnd _returnvalue_3))
  ;[1 1 1] Set starting ammo for reload to be the current ammo and reset reloading seconds and reload percent
  (Variables|Default|SetStarting_Ammo_For_Reload (Variables|Default|GetCurrent_Ammo))
  (Variables|Default|SetReloading_Seconds 0.0)
  (Variables|Default|SetReload_Percent 0.0)
  ;[1 1 1] Set reload time
  (bind _ranged_info (Class|BPIRangedWeapon|GetRangedInfo(Message) (Components|GetOwner)))
  (Variables|Default|SetReload_Time (Utilities|Struct|BreakStruct_Reload_Info (.Reload_Info (Utilities|Struct|BreakStruct_Ranged_Weapon _ranged_info))))
  ;[1 1 1] What reload percent needs to be to increase current ammo by 1
  (Variables|Default|SetReload_Threshold (/ 1.0 (Math|Conversions|ToFloat(Integer) (Variables|Default|GetMax_Ammo))))
  ;[1 1 1] Set reload percentage as current ammo out of max ammo
  (Variables|Default|SetReload_Percent (/ (Math|Conversions|ToFloat(Integer) (Variables|Default|GetCurrent_Ammo)) (Math|Conversions|ToFloat(Integer) (Variables|Default|GetMax_Ammo))))
  ;[1 1 1] Start reloading
  (Variables|Default|SetReloading true)
  (Components|Tick|SetComponentTickEnabled true))

(event Custom|Stop_Reload
  ;[1 1 1] Resetting variables and turning off the tick
  (Components|Tick|SetComponentTickEnabled false)
  (Variables|Default|SetReloading false)
  (Variables|Default|SetReloading_Seconds 0.0)
  (Variables|Default|SetReload_Percent 0.0))

(event Custom|Update_Max_Ammo
  (params (New%20Max%20Ammo :type Integer))
  ;[1 1 1] Updating the max ammo and setting the current ammo to be the max ammo and then also reloading just so it doesn't break anything when trying to reload next time
  (bind _output_get (Variables|Default|SetMax_Ammo New%20Max%20Ammo))
  (Variables|Default|SetCurrent_Ammo _output_get)
  (CallFunction|Reload))

(event EventTick
  (params (DeltaSeconds :type Float%20%28single-precision%29))
  (bind _returnvalue (Components|GetOwner))
  (bind _returnvalue_2 (Components|GetOwner))
  (bind _returnvalue_3 (Components|GetOwner))
  (bind _returnvalue_4 (Components|GetOwner))
  (bind _returnvalue_5 (Components|GetOwner))
  (bind _returnvalue_6 (Components|GetOwner))
  (bind _returnvalue_7 (Components|GetOwner _returnvalue))
  (bind _returnvalue_8 (Transformation|GetActorLocation _returnvalue_6))
  (bind _returnvalue_9 (Components|GetOwner _returnvalue_2))
  (bind _returnvalue_10 (Components|GetOwner _returnvalue_3))
  (bind _returnvalue_11 (Components|GetOwner _returnvalue_4))
  (bind _returnvalue_12 (Transformation|GetActorLocation _returnvalue_5))
  (bind _returnvalue_13 (Actor|GetComponentbyClass _returnvalue_7 "/Game/Characters/Player/BPC_HUD.BPC_HUD_C"))
  (bind _returnvalue_14 (Utilities|DoesObjectImplementInterface _returnvalue_10 "/Game/Characters/Player/BPI_Player.BPI_Player_C"))
  (bind _returnvalue_15 (Utilities|DoesObjectImplementInterface _returnvalue_11 "/Game/Characters/Player/BPI_Player.BPI_Player_C"))
  (bind _returnvalue_16 (Actor|GetComponentbyClass _returnvalue_9 "/Game/Characters/Player/BPC_HUD.BPC_HUD_C"))
  (bind _hud_ref (Variables|/Game/Characters/Player/BPC_HUD.BPC_HUD_C|GetHUD_Ref _returnvalue_13))
  (bind _hud_ref_2 (Variables|/Game/Characters/Player/BPC_HUD.BPC_HUD_C|GetHUD_Ref _returnvalue_16))
  (bind _weapon_1 (Variables|/Game/UI/WBP_HUD.WBP_HUD_C|GetWeapon_1 _hud_ref_2))
  (bind _weapon_2 (Variables|/Game/UI/WBP_HUD.WBP_HUD_C|GetWeapon_2 _hud_ref_2))
  (bind _weapon_3 (Variables|/Game/UI/WBP_HUD.WBP_HUD_C|GetWeapon_3 _hud_ref_2))
  (bind _weapon_1_2 (Variables|/Game/UI/WBP_HUD.WBP_HUD_C|GetWeapon_1 _hud_ref))
  (bind _weapon_2_2 (Variables|/Game/UI/WBP_HUD.WBP_HUD_C|GetWeapon_2 _hud_ref))
  (bind _weapon_3_2 (Variables|/Game/UI/WBP_HUD.WBP_HUD_C|GetWeapon_3 _hud_ref))
  ;[1 1 1] Increasing reloading seconds for the delta seconds of event tick
  (Variables|Default|SetReloading_Seconds (+ DeltaSeconds (Variables|Default|GetReloading_Seconds)))
  ;[1 1 1] Updating reload percentage of reloading seconds out of reload time
  (Variables|Default|SetReload_Percent (/ (Variables|Default|GetReloading_Seconds) (Variables|Default|GetReload_Time)))
  (switch Utilities|FlowControl|Switch|SwitchonEnum_Reload_Types (Utilities|Struct|BreakStruct_Reload_Info (.Reload_Info (Utilities|Struct|BreakStruct_Ranged_Weapon (stale Custom|Start_Reload _ranged_info))))
    (:NewEnumerator0
      (if (Math|Boolean|ANDBoolean (>= (Math|Float|%(Float) (Variables|Default|GetReload_Percent) (Variables|Default|GetReload_Threshold)) 0.0) (<= (Math|Float|%(Float) (Variables|Default|GetReload_Percent) (Variables|Default|GetReload_Threshold)) 0.02) (> (Variables|Default|GetReloading_Seconds) (/ (Variables|Default|GetReload_Time) 5e+01)))
        (Utilities|FlowControl|DoOnce false :!label _label
          (:Completed
            ;[1 1 1] Increment ammo
            (Math|Integer|IncrementInt (Variables|Default|GetCurrent_Ammo)
              (:%20%20
                (Utilities|FlowControl|Sequence
                  (:then_0
                    (if _returnvalue_14 :!label _label_2
                      ;[1 1 1] Update weapon HUD colour and ammo count
                      (switch int (Variables|/Game/UI/WBP_HUD.WBP_HUD_C|GetCurrently_Equipped_Weapon_Image_Relation _hud_ref_2)
                        (:0
                          (Default|UpdateImgColourforAmmo _weapon_1 (+ (/ (Math|Conversions|ToFloat(Integer) (Variables|Default|GetCurrent_Ammo)) (Math|Conversions|ToFloat(Integer) (Variables|Default|GetMax_Ammo))) (* (- 1.0 (/ (Math|Conversions|ToFloat(Integer) (Variables|Default|GetCurrent_Ammo)) (Math|Conversions|ToFloat(Integer) (Variables|Default|GetMax_Ammo)))) (Variables|Default|GetReload_Percent))))
                          (Default|UpdateAmmoCount _weapon_1 (Variables|Default|GetCurrent_Ammo) _returnvalue_15))
                        (:1
                          (Default|UpdateImgColourforAmmo _weapon_2 (+ (/ (Math|Conversions|ToFloat(Integer) (Variables|Default|GetCurrent_Ammo)) (Math|Conversions|ToFloat(Integer) (Variables|Default|GetMax_Ammo))) (* (- 1.0 (/ (Math|Conversions|ToFloat(Integer) (Variables|Default|GetCurrent_Ammo)) (Math|Conversions|ToFloat(Integer) (Variables|Default|GetMax_Ammo)))) (Variables|Default|GetReload_Percent))))
                          (Default|UpdateAmmoCount _weapon_2 (Variables|Default|GetCurrent_Ammo) _returnvalue_15))
                        (:2
                          (Default|UpdateImgColourforAmmo _weapon_3 (+ (/ (Math|Conversions|ToFloat(Integer) (Variables|Default|GetCurrent_Ammo)) (Math|Conversions|ToFloat(Integer) (Variables|Default|GetMax_Ammo))) (* (- 1.0 (/ (Math|Conversions|ToFloat(Integer) (Variables|Default|GetCurrent_Ammo)) (Math|Conversions|ToFloat(Integer) (Variables|Default|GetMax_Ammo)))) (Variables|Default|GetReload_Percent))))
                          (Default|UpdateAmmoCount _weapon_3 (Variables|Default|GetCurrent_Ammo) _returnvalue_15)))))
                  (:then_1
                    ;[1 1 1] Play sound and report noise
                    (Audio|PlaySoundatLocation (Utilities|Struct|BreakStruct_Ranged_Weapon_Audio (.Audio_Info (Utilities|Struct|BreakStruct_Ranged_Weapon (stale Custom|Start_Reload _ranged_info)))) _returnvalue_8 "0, 0, 0" 1.0 1.0 0.0 0 0 0 0)
                    (Class|AISenseHearing|ReportNoiseEvent _returnvalue_8 0.75 (Components|GetOwner (Components|GetOwner)) 0.0 "None")
                    (if (Utilities|DoesObjectImplementInterface (Components|GetOwner (Components|GetOwner)) "/Game/Characters/Player/BPI_Player.BPI_Player_C")
                      ;[1 1 1] Play reload animation if it is the player
                      (Default|PlayAmmoAnimation (Variables|/Game/Characters/Player/BPC_HUD.BPC_HUD_C|GetHUD_Ref (Actor|GetComponentbyClass (Components|GetOwner (Components|GetOwner)) "/Game/Characters/Player/BPC_HUD.BPC_HUD_C")) false))))))))
        (else
          (Utilities|FlowControl|Sequence
            (:then_0
              (goto _label Reset))
            (:then_1
              (goto _label_2)))))
      ;[1 1 1] reaching max ammo stops
      (if (>= (Variables|Default|GetCurrent_Ammo) (Variables|Default|GetMax_Ammo))
        (CallFunction|StopReload)))
    (:NewEnumerator1
      ;[1 1 1] If finished reloading
      (if (>= (Variables|Default|GetReload_Percent) 1.0)
        ;[1 1 1] Update current ammo and stop reloading
        (Variables|Default|SetCurrent_Ammo (Variables|Default|GetMax_Ammo))
        (CallFunction|StopReload)
        ;[1 1 1] Updating HUD weapon icon for ammo count and colour
        (if _returnvalue_14
          (switch int (Variables|/Game/UI/WBP_HUD.WBP_HUD_C|GetCurrently_Equipped_Weapon_Image_Relation _hud_ref)
            (:0
              (Default|UpdateImgColourforAmmo _weapon_1_2 (/ (Math|Conversions|ToFloat(Integer) (Variables|Default|GetCurrent_Ammo)) (Math|Conversions|ToFloat(Integer) (Variables|Default|GetMax_Ammo))))
              (Default|UpdateAmmoCount _weapon_1_2 (Variables|Default|GetCurrent_Ammo) _returnvalue_14))
            (:1
              (Default|UpdateImgColourforAmmo _weapon_2_2 (/ (Math|Conversions|ToFloat(Integer) (Variables|Default|GetCurrent_Ammo)) (Math|Conversions|ToFloat(Integer) (Variables|Default|GetMax_Ammo))))
              (Default|UpdateAmmoCount _weapon_2_2 (Variables|Default|GetCurrent_Ammo) _returnvalue_14))
            (:2
              (Default|UpdateImgColourforAmmo _weapon_3_2 (/ (Math|Conversions|ToFloat(Integer) (Variables|Default|GetCurrent_Ammo)) (Math|Conversions|ToFloat(Integer) (Variables|Default|GetMax_Ammo))))
              (Default|UpdateAmmoCount _weapon_3_2 (Variables|Default|GetCurrent_Ammo) _returnvalue_14)))
          (Default|PlayAmmoAnimation _hud_ref false))
        ;[1 1 1] Play reload sound and report noise
        (Audio|PlaySoundatLocation (Utilities|Struct|BreakStruct_Ranged_Weapon_Audio (.Audio_Info (Utilities|Struct|BreakStruct_Ranged_Weapon (stale Custom|Start_Reload _ranged_info)))) _returnvalue_12 "0, 0, 0" 1.0 1.0 0.0 0 0 0 0)
        (Class|AISenseHearing|ReportNoiseEvent _returnvalue_12 0.75 (Components|GetOwner (Components|GetOwner)) 0.0 "None")))))

(event EventBeginPlay
  ;[1 1 1] Setting up current ammo and reload time of the weapon that this component is attached to
  (Variables|Default|SetCurrent_Ammo (Variables|Default|GetMax_Ammo))
  (bind _basics (Class|BPIWeapon|GetBasicInfo(Message) (Components|GetOwner)))
  (Variables|Default|SetOwning%20Weapon%20is%20Ranged (Utilities|Struct|BreakStruct_Weapon _basics))
  (bind _ranged_info (Class|BPIRangedWeapon|GetRangedInfo(Message) (Components|GetOwner)))
  (Variables|Default|SetReload_Time (Utilities|Struct|BreakStruct_Reload_Info (Utilities|Struct|BreakStruct_Ranged_Weapon _ranged_info))))