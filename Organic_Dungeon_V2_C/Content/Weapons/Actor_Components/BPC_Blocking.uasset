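; Actor component that handles melee blocking for its owner, driven by the block input.
; Tick gates blocking on weapon, swap, aim, attack and cooldown state, and decays effectiveness over the weapon's maximum block time, triggering cooldown at zero.
; Timings and perfect-block stats come from the equipped weapon.
; Perfect Block, bound here to a debug key, sphere-traces to launch characters, push physics objects and destroy projectiles, then applies damage and gore after hitstop.
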(event Custom|Start_Blocking
  (bind _returnvalue (Components|GetOwner))
  (bind _returnvalue_2 (Actor|GetComponentbyClass _returnvalue "/Game/Weapons/Actor_Components/BPC_Weaponry.BPC_Weaponry_C"))
  (bind _equipped_weapon (Variables|/Game/Weapons/Actor_Components/BPC_Weaponry.BPC_Weaponry_C|GetEquipped_Weapon _returnvalue_2))
  (bind _returnvalue_3 (Transformation|GetActorLocation _equipped_weapon))
  (Variables|Times|SetBlocking_Duration 0.0)
  (Variables|Blocking|SetBlocking_Effectiveness 0.0)
  (bind _melee_info (Class|BPIMeleeWeapon|GetMeleeInfo(Message) (Variables|/Game/Weapons/Actor_Components/BPC_Weaponry.BPC_Weaponry_C|GetEquipped_Weapon (Actor|GetComponentbyClass (Components|GetOwner) "/Game/Weapons/Actor_Components/BPC_Weaponry.BPC_Weaponry_C"))))
  (Variables|Times|SetMax_Blocking_Time (.MaxBlockTime (Utilities|Struct|BreakStruct_Blocking_Info (.BlockingInfo (Utilities|Struct|BreakStruct_Melee_Weapon _melee_info)))))
  (Variables|Times|SetPerfect_Block_Threshold (.PerfectBlockThreshold (Utilities|Struct|BreakStruct_Blocking_Info (.BlockingInfo (Utilities|Struct|BreakStruct_Melee_Weapon _melee_info)))))
  (Variables|Times|SetBlocking_Cooldown_Time (.BlockCooldownTime (Utilities|Struct|BreakStruct_Blocking_Info (.BlockingInfo (Utilities|Struct|BreakStruct_Melee_Weapon _melee_info)))))
  (Variables|PerfectBlock|SetPerfect_Block_Radius (.PerfectBlockRadius (Utilities|Struct|BreakStruct_Blocking_Info (.BlockingInfo (Utilities|Struct|BreakStruct_Melee_Weapon _melee_info)))))
  (Variables|PerfectBlock|SetPerfect_Block_Knockback_Force (.PerfectBlockKnockbackForce (Utilities|Struct|BreakStruct_Blocking_Info (.BlockingInfo (Utilities|Struct|BreakStruct_Melee_Weapon _melee_info)))))
  (Variables|PerfectBlock|SetPerfect_Block_Damage (.PerfectBlockDamage (Utilities|Struct|BreakStruct_Blocking_Info (.BlockingInfo (Utilities|Struct|BreakStruct_Melee_Weapon _melee_info)))))
  (Variables|PerfectBlock|SetPerfect_Block_HItstop_Duration (.PerfectBlockHitstopDuration (Utilities|Struct|BreakStruct_Blocking_Info (.BlockingInfo (Utilities|Struct|BreakStruct_Melee_Weapon _melee_info)))))
  (Variables|Blocking|SetBlocking_Effectiveness 1.0)
  (Variables|Checks|SetBlocking true)
  (Audio|PlaySoundatLocation (Utilities|Struct|BreakStruct_Melee_Weapon_Audio (.MeleeAudio (Utilities|Struct|BreakStruct_Melee_Weapon _melee_info))) _returnvalue_3 "0, 0, 0" 1.0 1.0 0.0 0 0 0 0)
  (Class|AISenseHearing|ReportNoiseEvent _returnvalue_3 0.75 (Components|GetOwner) 0.0 "None"))

(event Custom|Stop_Blocking
  (Variables|Checks|SetBlocking false))

(event Custom|Blocking_Cooldown_CE
  (Variables|Checks|SetBlocking_Cooldown true)
  (Utilities|FlowControl|Delay (Variables|Times|GetBlocking_Cooldown_Time))
  (Variables|Checks|SetBlocking_Cooldown false))

(event Custom|Perfect_Block
  (bind _returnvalue (Components|GetOwner))
  (bind _returnvalue_2 (Components|GetOwner))
  (bind _returnvalue_3 (Components|GetOwner))
  (bind _returnvalue_4 (Components|GetOwner))
  (bind _perfect_block_damage (Variables|PerfectBlock|GetPerfect_Block_Damage))
  (bind _returnvalue_5 (Transformation|GetActorLocation _returnvalue_2))
  (bind _returnvalue_6 (Transformation|GetActorLocation _returnvalue_3))
  (Class|LegacyCameraShake|StartLegacyCameraShake (Game|GetPlayerCameraManager 0) "/Game/Projectiles/BPS/BP_Explosion_Camera_Shake.BP_Explosion_Camera_Shake_C" 2.0 "CameraLocal" "0, 0, 0")
  (bind _returnvalue_7 (Niagara|SpawnSystematLocation "/Game/VFX_SFX/Niagara/Ground_Slam/NS_Ground_Slam.NS_Ground_Slam" (Transformation|GetActorLocation (Components|GetOwner)) "0, 0, 0" "1.000000,1.000000,1.000000" true true "AutoRelease"))
  (Niagara|SetNiagaraVariable(LinearColor) _returnvalue_7 "user.Ground_Colour" (Math|Color|MakeColor 1.0 0.0 0.0))
  (Audio|PlaySoundatLocation "/Game/VFX_SFX/Sounds/Blocking/Perfect_Block_SC.Perfect_Block_SC" _returnvalue_6 "0, 0, 0" 5.0 1.0 0.0 0 0 0 0)
  (Class|AISenseHearing|ReportNoiseEvent _returnvalue_6 3.0 (Components|GetOwner (Components|GetOwner)) 0.0 "None")
  (Utilities|Array|Clear (Variables|PerfectBlock|GetPerfect_Block_Hit_Actors))
  (bind (_outhits _returnvalue_8) (Collision|MultiSphereTraceForObjects _returnvalue_5 _returnvalue_5 (Variables|PerfectBlock|GetPerfect_Block_Radius) (Utilities|Array|MakeArray "ObjectTypeQuery3" "ObjectTypeQuery4" "ObjectTypeQuery8" "ObjectTypeQuery10" "ObjectTypeQuery13" "ObjectTypeQuery9") false (Utilities|Array|MakeArray _returnvalue_4 (Variables|/Game/Weapons/Actor_Components/BPC_Weaponry.BPC_Weaponry_C|GetEquipped_Weapon (Actor|GetComponentbyClass _returnvalue_4 "/Game/Weapons/Actor_Components/BPC_Weaponry.BPC_Weaponry_C"))) "ForDuration"))
  (if _returnvalue_8
    (for _array_element _outhits
      (if (not (Utilities|Array|ContainsItem (Variables|PerfectBlock|GetPerfect_Block_Hit_Actors) (.HitActor (Collision|BreakHitResult _array_element))))
        (Utilities|Array|Add (Variables|PerfectBlock|GetPerfect_Block_Hit_Actors) (.HitActor (Collision|BreakHitResult _array_element)))
        (switch Utilities|FlowControl|Switch|SwitchonECollisionChannel (Collision|GetCollisionObjectType (.HitComponent (Collision|BreakHitResult _array_element)))
          (:ECC_Pawn
            (if (Utilities|DoesObjectImplementInterface (.HitActor (Collision|BreakHitResult _array_element)) "/Game/Health/Interfaces/BPI_Has_Health.BPI_Has_Health_C") :!label _label
              (bind _ascharacter (Utilities|Casting|CastToCharacter (.HitActor (Collision|BreakHitResult _array_element))))
              (Utilities|IsValid (Actor|GetComponentbyClass _ascharacter "/Game/Weapons/Actor_Components/BPC_Hitstop.BPC_Hitstop_C")
                (:Is%20Valid
                  (Default|StartHitstop (Actor|GetComponentbyClass _ascharacter "/Game/Weapons/Actor_Components/BPC_Hitstop.BPC_Hitstop_C") (Variables|PerfectBlock|GetPerfect_Block_HItstop_Duration)))
                (:Is%20Not%20Valid
                  _))
              (Character|LaunchCharacter _ascharacter (/ (+ (* (Math|Vector|GetForwardVector (Math|Rotator|FindLookatRotation (Transformation|GetActorLocation _returnvalue) (Transformation|GetWorldLocation (.HitComponent (Collision|BreakHitResult _array_element))))) (Variables|PerfectBlock|GetPerfect_Block_Knockback_Force)) (* (Transformation|GetActorUpVector _returnvalue) (/ (Variables|PerfectBlock|GetPerfect_Block_Knockback_Force) 2.0))) 5.0) true true)))
          (:ECC_PhysicsBody
            (Physics|AddImpulse (.HitComponent (Collision|BreakHitResult _array_element)) (* (Math|Vector|GetForwardVector (Math|Rotator|FindLookatRotation (Transformation|GetActorLocation _returnvalue) (Transformation|GetWorldLocation (.HitComponent (Collision|BreakHitResult _array_element))))) (Variables|PerfectBlock|GetPerfect_Block_Knockback_Force)) "None" true :!label _label_2))
          (:ECC_GameTraceChannel2
            (goto _label))
          (:ECC_GameTraceChannel3
            (goto _label_2))
          (:ECC_GameTraceChannel4
            (goto _label))
          (:ECC_GameTraceChannel7
            (Actor|DestroyActor (.HitActor (Collision|BreakHitResult _array_element)))))))
    (Utilities|FlowControl|Delay (Variables|PerfectBlock|GetPerfect_Block_HItstop_Duration))
    (for _array_element_2 (Variables|PerfectBlock|GetPerfect_Block_Hit_Actors)
      (Utilities|IsValid (Actor|GetComponentbyClass _array_element_2 "/Game/VFX_SFX/Blood_Splatter/BPS/BPC_Blood_Effect.BPC_Blood_Effect_C")
        (:Is%20Valid
          (Default|BloodEffect (Actor|GetComponentbyClass _array_element_2 "/Game/VFX_SFX/Blood_Splatter/BPS/BPC_Blood_Effect.BPC_Blood_Effect_C") (Transformation|GetActorLocation _array_element_2) (Transformation|GetActorLocation _array_element_2) _array_element_2 _perfect_block_damage)
          (Default|BloodEffect (Actor|GetComponentbyClass _array_element_2 "/Game/VFX_SFX/Blood_Splatter/BPS/BPC_Blood_Effect.BPC_Blood_Effect_C") (Transformation|GetActorLocation _array_element_2) (Transformation|GetActorLocation _array_element_2) _array_element_2 _perfect_block_damage))
        (:Is%20Not%20Valid
          _))
      (Audio|PlaySoundatLocation "/Game/VFX_SFX/Blood_Splatter/Audio/Impact_Audio/Body_Impact_SC.Body_Impact_SC" (Transformation|GetActorLocation _array_element_2) "0, 0, 0" 1.0 1.0 0.0 0 0 0 0)
      (Utilities|IsValid (Actor|GetComponentbyClass _array_element_2 "/Game/Health/BPs/BPC_Health.BPC_Health_C")
        (:Is%20Valid
          (Default|TakeDamage (Actor|GetComponentbyClass _array_element_2 "/Game/Health/BPs/BPC_Health.BPC_Health_C") (Variables|PerfectBlock|GetPerfect_Block_Damage) (Transformation|GetActorLocation _array_element_2) _array_element_2 (Components|GetOwner)))))
    (Game|SpawnActorfromClass "/Game/VFX_SFX/Bloodsplosion/BPs/BP_BloodSplosion.BP_BloodSplosion_C" (Math|Transform|MakeTransform (Transformation|GetActorLocation (Components|GetOwner)) "0, 0, 0" "1.000000,1.000000,1.000000") "Undefined" "MultiplyWithRoot" 0 250 0)))

(event Input|EnhancedActionEvents|EnhancedInputActionIA_Block
  (params (ActionValue :type Boolean) (ElapsedSeconds :type Float%20%28double-precision%29) (TriggeredSeconds :type Float%20%28double-precision%29) (InputAction :type Input%20Action%20Object%20Reference :default "/Game/Characters/Player/Input/Actions/IA_Block.IA_Block"))
  (bind _can_block (Variables|Checks|GetCan_Block))
  (:Triggered
    (if (not (Variables|Checks|GetBlocking)) :!label _label
      (if _can_block
        (CallFunction|StartBlocking))
      (elif (not _can_block)
        (CallFunction|StopBlocking))))
  (:Started
    (goto _label))
  (:Canceled
    (CallFunction|StopBlocking :!label _label_2)
    (Variables|Times|SetBlocking_Cooldown_Time (/ (Variables|Times|GetBlocking_Cooldown_Time) 5.0))
    (CallFunction|BlockingCooldownCE))
  (:Completed
    (goto _label_2)))

(event EventBeginPlay
  (Utilities|FlowControl|Delay 0.2)
  (Utilities|IsValid (Actor|GetComponentbyClass (Components|GetOwner) "/Game/Weapons/Actor_Components/BPC_Aim.BPC_Aim_C")
    (:Is%20Valid
      (Variables|Default|SetShould%20Check%20Aiming true))
    (:Is%20Not%20Valid
      (Variables|Default|SetShould%20Check%20Aiming false))))

(event EventTick
  (params (DeltaSeconds :type Float%20%28single-precision%29))
  (bind _returnvalue (Components|GetOwner))
  (bind _returnvalue_2 (Actor|GetComponentbyClass _returnvalue "/Game/Weapons/Actor_Components/BPC_Weaponry.BPC_Weaponry_C"))
  (bind _equipped_weapon (Variables|/Game/Weapons/Actor_Components/BPC_Weaponry.BPC_Weaponry_C|GetEquipped_Weapon _returnvalue_2))
  (Utilities|FlowControl|Sequence
    (:then_0
      (Utilities|IsValid _equipped_weapon
        (:Is%20Valid
          (bind _basics (Class|BPIWeapon|GetBasicInfo(Message) _equipped_weapon))
          (Variables|Checks|SetCan_Block (Math|Boolean|ANDBoolean (not (Variables|/Game/Weapons/Actor_Components/BPC_Weaponry.BPC_Weaponry_C|GetSwapping_Weapons _returnvalue_2)) (select (Variables|Default|GetShould%20Check%20Aiming) (not (Variables|/Game/Weapons/Actor_Components/BPC_Aim.BPC_Aim_C|GetAiming? (Actor|GetComponentbyClass _returnvalue "/Game/Weapons/Actor_Components/BPC_Aim.BPC_Aim_C"))) true) (not (Variables|/Game/Weapons/Actor_Components/BPC_Attack_Handler.BPC_Attack_Handler_C|GetAttacking (Actor|GetComponentbyClass _returnvalue "/Game/Weapons/Actor_Components/BPC_Attack_Handler.BPC_Attack_Handler_C"))) (not (.ranged _basics)) (not (Variables|Checks|GetBlocking_Cooldown)))))
        (:Is%20Not%20Valid
          (Variables|Checks|SetCan_Block false))))
    (:then_1
      (if (Variables|Checks|GetBlocking)
        (Variables|Times|SetBlocking_Duration (+ (Variables|Times|GetBlocking_Duration) DeltaSeconds))
        (bind _output_get (Variables|Blocking|SetBlocking_Effectiveness (Math|Float|Clamp(Float) (- 1.0 (/ (Variables|Times|GetBlocking_Duration) (Variables|Times|GetMax_Blocking_Time))))))
        (if (== _output_get 0.0)
          (Utilities|FlowControl|DoOnce false :!label _label
            (:Completed
              (bind _melee_info (Class|BPIMeleeWeapon|GetMeleeInfo(Message) (Variables|/Game/Weapons/Actor_Components/BPC_Weaponry.BPC_Weaponry_C|GetEquipped_Weapon (Actor|GetComponentbyClass (Components|GetOwner) "/Game/Weapons/Actor_Components/BPC_Weaponry.BPC_Weaponry_C"))))
              (Variables|Times|SetBlocking_Cooldown_Time (Utilities|Struct|BreakStruct_Blocking_Info (.BlockingInfo (Utilities|Struct|BreakStruct_Melee_Weapon _melee_info))))
              (CallFunction|BlockingCooldownCE)))
          (else
            (goto _label Reset)))))))

(event Input|KeyboardEvents|DebugKey6
  (params (Key :type Key%20Structure :default "None") (ActionValue :type Input%20Action%20Value%20Structure))
  (:Pressed
    (CallFunction|PerfectBlock)))