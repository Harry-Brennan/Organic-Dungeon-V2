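; Actor component that handles aiming down ranged weapons for its owner, driven by the IA_Aim input action.
; Tick refreshes CanAim from BPC_Weaponry, allowing it only for a valid ranged weapon while not swapping or reloading.
; Input starts or stops aiming on CanAim, which makes the Rolling check redundant.
; For BPI_Player owners, aim changes with ranged weapons update the BPC_HUD crosshair.
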(event Custom|Start_Aiming
  ;[1 1 1] Starting and stopping aiming based on if the equipped weapon is ranged
  (bind _basics (Class|BPIWeapon|GetBasicInfo(Message) (Variables|/Game/Weapons/Actor_Components/BPC_Weaponry.BPC_Weaponry_C|GetEquipped_Weapon (Actor|GetComponentbyClass (Components|GetOwner) "/Game/Weapons/Actor_Components/BPC_Weaponry.BPC_Weaponry_C"))))
  (if (.ranged _basics)
    (Variables|Default|SetAiming? true)
    ;[1 1 1] If Player then update crosshair
    (if (Utilities|DoesObjectImplementInterface (Components|GetOwner) "/Game/Characters/Player/BPI_Player.BPI_Player_C")
      (Default|UpdateCrosshair (Actor|GetComponentbyClass (Components|GetOwner) "/Game/Characters/Player/BPC_HUD.BPC_HUD_C") (Variables|Default|GetAiming?) false false))
    (else
      (Variables|Default|SetAiming? false))))

(event Custom|Stop_Aiming
  ;[1 1 1] Starting and stopping aiming based on if the equipped weapon is ranged
  (bind _basics (Class|BPIWeapon|GetBasicInfo(Message) (Variables|/Game/Weapons/Actor_Components/BPC_Weaponry.BPC_Weaponry_C|GetEquipped_Weapon (Actor|GetComponentbyClass (Components|GetOwner) "/Game/Weapons/Actor_Components/BPC_Weaponry.BPC_Weaponry_C"))))
  (if (.ranged _basics)
    (Variables|Default|SetAiming? false)
    ;[1 1 1] If Player then update crosshair
    (if (Utilities|DoesObjectImplementInterface (Components|GetOwner) "/Game/Characters/Player/BPI_Player.BPI_Player_C")
      (Default|UpdateCrosshair (Actor|GetComponentbyClass (Components|GetOwner) "/Game/Characters/Player/BPC_HUD.BPC_HUD_C") (Variables|Default|GetAiming?) false false))
    (else
      (Variables|Default|SetAiming? false))))

(event Custom|Attempt_Aiming
  ;[1 1 1] Aiming input action, can aim - can aim variable and not rolling or can aim
  (if (or (and (Variables|Default|GetCanAim?) (not (Variables|Default|GetRolling))) (Variables|Default|GetCanAim?))
    (CallFunction|StartAiming)
    (else
      (CallFunction|StopAiming))))

(event Input|EnhancedActionEvents|EnhancedInputActionIA_Aim
  (params (ActionValue :type Boolean) (ElapsedSeconds :type Float%20%28double-precision%29) (TriggeredSeconds :type Float%20%28double-precision%29) (InputAction :type Input%20Action%20Object%20Reference :default "/Game/Characters/Player/Input/Actions/IA_Aim.IA_Aim"))
  ;[1 1 1] Aiming input action, can aim - can aim variable and not rolling or can aim
  (:Triggered
    (if (or (and (Variables|Default|GetCanAim?) (not (Variables|Default|GetRolling))) (Variables|Default|GetCanAim?)) :!label _label
      (CallFunction|StartAiming)
      (else
        (CallFunction|StopAiming :!label _label_2))))
  (:Started
    (goto _label))
  (:Canceled
    (goto _label_2))
  (:Completed
    (goto _label_2)))

(event EventTick
  (params (DeltaSeconds :type Float%20%28single-precision%29))
  (bind _returnvalue (Components|GetOwner))
  (bind _returnvalue_2 (Components|GetOwner))
  (bind _returnvalue_3 (Actor|GetComponentbyClass _returnvalue_2 "/Game/Weapons/Actor_Components/BPC_Weaponry.BPC_Weaponry_C"))
  (bind _returnvalue_4 (Actor|GetComponentbyClass _returnvalue "/Game/Weapons/Actor_Components/BPC_Weaponry.BPC_Weaponry_C"))
  (bind _equipped_weapon (Variables|/Game/Weapons/Actor_Components/BPC_Weaponry.BPC_Weaponry_C|GetEquipped_Weapon _returnvalue_4))
  ;[1 1 1] Checking every 1/10 second if we can aim - if the equipped weapon is valid - if wer are not swapping a weapon or reloading
  (if (Utilities|IsValid _equipped_weapon)
    (bind _basics (Class|BPIWeapon|GetBasicInfo(Message) _equipped_weapon))
    (if (.ranged _basics)
      (if (or (Variables|/Game/Weapons/Actor_Components/BPC_Weaponry.BPC_Weaponry_C|GetSwapping_Weapons _returnvalue_3) (Variables|/Game/Weapons/Actor_Components/BPC_Ammo.BPC_Ammo_C|GetReloading (Actor|GetComponentbyClass (Variables|/Game/Weapons/Actor_Components/BPC_Weaponry.BPC_Weaponry_C|GetEquipped_Weapon _returnvalue_3) "/Game/Weapons/Actor_Components/BPC_Ammo.BPC_Ammo_C")))
        (Variables|Default|SetCanAim? false)
        (else
          (Variables|Default|SetCanAim? true)))
      (else
        (Variables|Default|SetCanAim? false)))
    (else
      (Variables|Default|SetCanAim? false))))