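; Sprint component that raises and restores the owning character's MaxWalkSpeed in response to the sprint input action.
; Starting reads speeds and transition times from the owner via messages, scaling top speed by a ground-angle multiplier.
; Start and stop notify BPC_Custom_Movement_Handler of mode changes.
; Component tick lerps walk speed over the startup or stopping time, switching itself off once the transition completes.
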(event EventBeginPlay
  (bind _output_get (Variables|Speeds|SetNormal_Walking_Speed (Variables|/Script/Engine.CharacterMovementComponent|GetMaxWalkSpeed (Actor|GetComponentbyClass (Components|GetOwner) "/Script/Engine.CharacterMovementComponent"))))
  (Class|BPICanSprint|UpdateNormalWalkingSpeed(Message) (Components|GetOwner) _output_get))

(event Custom|Start_Sprint
  (if (and (not (Variables|Status&Checks|GetSprinting)) (Variables|Status&Checks|GetCan_Sprint))
    (bind _sprint_info (Class|BPICanSprint|GetSprintInfo(Message) (Components|GetOwner)))
    (Variables|Speeds|SetNormal_Walking_Speed (.normal_walking_speed _sprint_info))
    (Variables|Speeds|SetMax_Sprint_Speed (* (Variables|Ground|GetGround_Angle_Multiplier) (.sprinting_max_speed _sprint_info)))
    (Variables|Speeds|SetSprint_Startup_Speed (.sprint_startup_speed _sprint_info))
    (Variables|Speeds|SetSprint_Stopping_Speed (.sprint_stopping_speed _sprint_info))
    (Variables|Status&Checks|SetStarting/Stopping true)
    (Components|Tick|SetComponentTickEnabled true)
    (Default|UpdateCustomMovementMode (Actor|GetComponentbyClass (Components|GetOwner) "/Game/Movement/BPC_Custom_Movement_Handler.BPC_Custom_Movement_Handler_C") "NewEnumerator1")
    (Variables|Status&Checks|SetSprinting true)
    (elif (not (Variables|Status&Checks|GetCan_Sprint))
      (Variables|Transitions|SetSprint_Percentage 0.0)
      (Variables|Status&Checks|SetSprinting false)
      (Default|TransitionfromMode (Actor|GetComponentbyClass (Components|GetOwner) "/Game/Movement/BPC_Custom_Movement_Handler.BPC_Custom_Movement_Handler_C") "NewEnumerator1"))))

(event Custom|Stop_Sprint
  (Variables|Status&Checks|SetStarting/Stopping false)
  (Variables|Transitions|SetSprint_Percentage 0.0)
  (Components|Tick|SetComponentTickEnabled true)
  (Variables|Status&Checks|SetSprinting false)
  (Default|TransitionfromMode (Actor|GetComponentbyClass (Components|GetOwner) "/Game/Movement/BPC_Custom_Movement_Handler.BPC_Custom_Movement_Handler_C") "NewEnumerator1"))

(event Input|EnhancedActionEvents|EnhancedInputActionIA_Sprint
  (params (ActionValue :type Boolean) (ElapsedSeconds :type Float%20%28double-precision%29) (TriggeredSeconds :type Float%20%28double-precision%29) (InputAction :type Input%20Action%20Object%20Reference :default "/Game/Characters/Player/Input/Actions/IA_Sprint.IA_Sprint"))
  (:Triggered
    (CallFunction|StartSprint)
    (Variables|Status&Checks|SetAttempting_To_Sprint true))
  (:Canceled
    (CallFunction|StopSprint :!label _label)
    (Variables|Status&Checks|SetAttempting_To_Sprint false))
  (:Completed
    (goto _label)))

(event EventTick
  (params (DeltaSeconds :type Float%20%28single-precision%29))
  (bind _returnvalue (Components|GetOwner))
  (bind _returnvalue_2 (Actor|GetComponentbyClass _returnvalue "/Script/Engine.CharacterMovementComponent"))
  (Variables|Transitions|SetSprint_Percentage (+ (Variables|Transitions|GetSprint_Percentage) (/ 1.0 (/ (Math|Float|SelectFloat (Variables|Speeds|GetSprint_Startup_Speed) (Variables|Speeds|GetSprint_Stopping_Speed) (Variables|Status&Checks|GetStarting/Stopping)) (Class|ActorComponent|GetComponentTickInterval)))))
  ;[1 1 1] Starting is true / stopping is false
  (if (Variables|Status&Checks|GetStarting/Stopping)
    (Variables|/Script/Engine.CharacterMovementComponent|SetMaxWalkSpeed _returnvalue_2 (Math|Float|Lerp (Variables|/Script/Engine.CharacterMovementComponent|GetMaxWalkSpeed _returnvalue_2) (Variables|Speeds|GetMax_Sprint_Speed) (Variables|Transitions|GetSprint_Percentage)))
    (else
      (Variables|/Script/Engine.CharacterMovementComponent|SetMaxWalkSpeed _returnvalue_2 (Math|Float|Lerp (Math|Float|Lerp (Variables|/Script/Engine.CharacterMovementComponent|GetMaxWalkSpeed _returnvalue_2) (Variables|Speeds|GetMax_Sprint_Speed) (Variables|Transitions|GetSprint_Percentage)) (Variables|Speeds|GetNormal_Walking_Speed) (Variables|Transitions|GetSprint_Percentage)))))
  (if (>= (Variables|Transitions|GetSprint_Percentage) 1.0)
    (Components|Tick|SetComponentTickEnabled false)))