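; Actor component that gives its owner a charge-limited dash along last movement input, or forward when there is none.
; Capsule traces step back from full distance to find the furthest spot with ground below and no Pawn-blocking hits.
; Tick turns on only during the dash, moving the owner there along a float curve without sweeping, so only the destination is validated.
; A cooldown timer restores all charges at once.
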(event Custom|Dash_Begin
  (bind _returnvalue (Components|GetOwner))
  (bind _returnvalue_2 (Components|GetOwner))
  (bind _returnvalue_3 (Transformation|GetActorLocation _returnvalue))
  (bind _instigator (Variables|/Script/Engine.Actor|GetInstigator _returnvalue_2))
  (bind _returnvalue_4 (Class|Pawn|GetLastMovementInputVector _instigator))
  (if (and (not (Variables|Debugging|GetDashing)) (> (Variables|Debugging|GetAvailable_Dash_Count) 0))
    (Variables|Debugging|SetDashing true)
    (Math|Integer|DecrementInt (Variables|Debugging|GetAvailable_Dash_Count)
      (:%20%20
        (CallFunction|DashCooldownBegin)
        (Variables|Debugging|SetAlpha 0.0)
        (Components|Tick|SetComponentTickEnabled false)
        (CallFunction|MoveOverTime (CallFunction|GetFurthestValidLocation _returnvalue_3 (+ _returnvalue_3 (* (Math|Vector|SelectVector (Transformation|GetActorForwardVector _returnvalue_2) _returnvalue_4 (Utilities|Operators|EqualEqual :A _returnvalue_4)) (Variables|Info|GetDash_Distance)))))))))

(event Custom|Move_Over_Time
  (params (Location :type Vector))
  (bind _output_get (Variables|Debugging|SetDash_Start_Location (Transformation|GetActorLocation (Components|GetOwner))))
  (Transformation|SetActorRotation (Components|GetOwner) (Math|Rotator|FindLookatRotation _output_get Location))
  (Components|Tick|SetComponentTickEnabled true))

(event Custom|Dash_Cooldown_Begin
  ;[1 1 1] Dash cooldowns
  (Utilities|Time|SetTimerbyEvent (delegate Custom|Reset_Dash_Cooldown) (Variables|Info|GetDash_Cooldown)))

(event Custom|Reset_Dash_Cooldown
  ;[1 1 1] Dash cooldowns
  (Variables|Debugging|SetAvailable_Dash_Count (Variables|Info|GetMax_Dash_Count)))

(event EventTick
  (params (DeltaSeconds :type Float%20%28single-precision%29))
  (Variables|Debugging|SetAlpha (+ (Variables|Debugging|GetAlpha) (Utilities|Operators|Divide 1.0 (Variables|Info|GetDash_Duration) 1e+02)))
  (Transformation|SetActorLocation (Components|GetOwner) (Math|Vector|Lerp(Vector) (Variables|Debugging|GetDash_Start_Location) (stale Custom|Move_Over_Time Location) (Math|Curves|GetFloatValue (Variables|Debugging|GetDash_Curve) (Variables|Debugging|GetAlpha))) false false)
  (if (>= (Variables|Debugging|GetAlpha) 1.0)
    (Components|Tick|SetComponentTickEnabled false)
    (Variables|Debugging|SetDashing false)))

(event EventBeginPlay
  ;[1 1 1] Setting capsule component and setting the available dash count to be the max dash count
  (bind _capsule (Class|BPICanDash|GetCapsuleCollision(Message) (Components|GetOwner)))
  (Variables|Default|SetCapsule_Component _capsule)
  (Variables|Debugging|SetAvailable_Dash_Count (Variables|Info|GetMax_Dash_Count)))

(event Input|MouseEvents|DebugKeyThumbMouseButton2
  (params (Key :type Key%20Structure) (ActionValue :type Input%20Action%20Value%20Structure))
  (:Pressed
    (CallFunction|DashBegin)))

(fn GetFurthestValidLocation
  (params (Start :type Vector) (End :type Vector))
  (bind _capsule_component (Variables|Default|GetCapsule_Component))
  (bind (_outradius _outhalfheight) (Class|CapsuleComponent|GetUnscaledCapsuleSize _capsule_component))
  (LocalVariables|SetDirection (Math|Vector|GetUnitDirection(Vector) Start End))
  (bind _output_get (LocalVariables|SetCapsule_Diameter (* (Variables|/Script/Engine.CapsuleComponent|GetCapsuleRadius (Variables|Default|GetCapsule_Component)) 2.0)))
  (bind _output_get_2 (LocalVariables|SetCapsule_Count (/ (Math|Vector|Distance(Vector) Start End) _output_get)))
  (for _index (range 0 _output_get_2)
    (LocalVariables|SetCurrent_Capsule_Location (+ (* (- (LocalVariables|GetCapsule_Count) _index) (LocalVariables|GetDirection) (LocalVariables|GetCapsule_Diameter)) Start))
    (bind _outhits (Class|KismetSystemLibrary|CapsuleTraceMultiforObjects (+ (* (- (LocalVariables|GetCapsule_Count) _index) (LocalVariables|GetDirection) (LocalVariables|GetCapsule_Diameter)) Start) (+ (* (- (LocalVariables|GetCapsule_Count) _index) (LocalVariables|GetDirection) (LocalVariables|GetCapsule_Diameter)) Start) _outradius _outhalfheight (Utilities|Array|MakeArray "ObjectTypeQuery1" "ObjectTypeQuery2" "ObjectTypeQuery3" "ObjectTypeQuery5" "ObjectTypeQuery6") false 0 "None" true))
    (bind _valid (CallFunction|IsValidLocation (LocalVariables|GetCurrent_Capsule_Location) _outhits))
    (if _valid
      (return (LocalVariables|GetCurrent_Capsule_Location))))
  (return Start))

(fn IsValidLocation
  (params (Location :type Vector) (Hits :type Array%20of%20Hit%20Result%20Structures))
  (bind _returnvalue (Collision|LineTraceByChannel Location (+ Location "0.000000,0.000000,-500.000000") "TraceTypeQuery1" false 0 "None"))
  (if _returnvalue
    (if (Utilities|Array|IsEmpty Hits)
      (return true)
      (else
        (for _array_element Hits
          (if (Utilities|Enum|Equal(Enum) (Collision|GetCollisionResponsetoChannel (.HitComponent (Collision|BreakHitResult _array_element)) "ECC_Pawn") "ECR_Block")
            (return false)))
        (return true)))
    (else
      (return false))))