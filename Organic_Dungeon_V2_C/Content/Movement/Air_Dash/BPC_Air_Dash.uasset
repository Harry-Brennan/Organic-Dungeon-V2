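; Actor component that gives its owning pawn a directional air dash, triggered by input while falling and off cooldown.
; The dash briefly switches movement to Flying, applies a velocity-change impulse along the last input direction, then restores Walking.
; It plays sound, reports AI noise, spawns Niagara between the feet and starts the cooldown.
; Owners implementing BPI_Player also get camera shake, HUD ability feedback and timed slow motion.
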(event Custom|Air_Dash
  (bind _returnvalue (Components|GetOwner))
  (bind _returnvalue_2 (Components|GetOwner))
  (bind _returnvalue_3 (Components|GetOwner))
  (bind _returnvalue_4 (Actor|GetComponentbyClass _returnvalue "/Script/Engine.SkeletalMeshComponent"))
  (bind _returnvalue_5 (Transformation|GetActorLocation _returnvalue_2))
  (bind _returnvalue_6 (Actor|GetComponentbyClass _returnvalue_3 "/Script/Engine.CharacterMovementComponent"))
  (bind _returnvalue_7 (Transformation|GetSocketLocation _returnvalue_4 "foot_l"))
  ;[1 1 1] Sound and noise event
  (Audio|PlaySoundatLocation "/Game/VFX_SFX/Air_Dash/Air_Dash_SC.Air_Dash_SC" _returnvalue_5 "0, 0, 0" 1.0 1.0 0.0 0 0 0 0)
  (Class|AISenseHearing|ReportNoiseEvent _returnvalue_5 2.0 (Components|GetOwner) 0.0 "None")
  (bind _aspawn (Utilities|Casting|CastToPawn _returnvalue_3))
  ;[1 1 1] Updating movement mode
  (Pawn|Components|CharacterMovement|SetMovementMode _returnvalue_6 "MOVE_Flying" 0)
  ;[1 1 1] Actual impulse force
  (Physics|AddImpulse _returnvalue_6 (* (Math|Vector|ClampVectorSize (Class|Pawn|GetLastMovementInputVector _aspawn) 0.0 1.0) (Variables|Strength|GetDash_Strength)) true)
  ;[1 1 1] Cooldown
  (CallFunction|AirDashCooldownCE)
  ;[1 1 1] Spawning double jump niagara at opposite rotation to dash direction and in between feet bones
  (Niagara|SpawnSystematLocation "/Game/VFX_SFX/Niagara/Double_Jump/NS_Double_Jump.NS_Double_Jump" (+ (* (Math|Vector|ClampVectorSize (Class|Pawn|GetLastMovementInputVector _aspawn) 0.0 1.0) 25.0) (+ _returnvalue_7 (/ (- (Transformation|GetSocketLocation _returnvalue_4 "foot_r") _returnvalue_7) 2.0))) (Math|Rotator|FindLookatRotation (+ (* (Math|Vector|ClampVectorSize (Class|Pawn|GetLastMovementInputVector _aspawn) 0.0 1.0) 25.0) (+ _returnvalue_7 (/ (- (Transformation|GetSocketLocation _returnvalue_4 "foot_r") _returnvalue_7) 2.0))) (Transformation|GetActorLocation (Components|GetOwner))))
  ;[1 1 1] Camera shake and then updating movement mode to walking
  (Utilities|FlowControl|Sequence
    (:then_0
      (if (Utilities|DoesObjectImplementInterface (Components|GetOwner) "/Game/Characters/Player/BPI_Player.BPI_Player_C")
        (CallFunction|AirDashCameraShake)
        (Default|UseMovementAbility (Actor|GetComponentbyClass (Components|GetOwner) "/Game/Characters/Player/BPC_HUD.BPC_HUD_C") "NewEnumerator1")
        (Default|AddSlowTime (Actor|GetComponentbyClass (Components|GetOwner) "/Game/Characters/Player/Slow_Time/BPC_Slow_Time_Manager.BPC_Slow_Time_Manager_C") (Variables|SlowTime|GetSlow%20Time%20Amount) "NewEnumerator8")
        (Utilities|Time|SetTimerbyFunctionName 0 "Stop Slow Time AD" (Variables|SlowTime|GetSlow%20Time%20Duration))))
    (:then_1
      (Utilities|FlowControl|Delay 0.2)
      (Pawn|Components|CharacterMovement|SetMovementMode _returnvalue_6 "MOVE_Walking" 0))))

(event Custom|Air_Dash_Cooldown_CE
  (bind _returnvalue (Components|GetOwner))
  ;[1 1 1] Dash cooldown
  (Variables|Cooldown|SetAir_Dash_Cooldown true)
  (Utilities|FlowControl|Delay (Variables|Cooldown|GetAir_Dash_Cooldown_Length))
  (Variables|Cooldown|SetAir_Dash_Cooldown false)
  (if (Utilities|DoesObjectImplementInterface _returnvalue "/Game/Characters/Player/BPI_Player.BPI_Player_C")
    (Default|ForciblyResetMovementAbility (Actor|GetComponentbyClass _returnvalue "/Game/Characters/Player/BPC_HUD.BPC_HUD_C") "NewEnumerator1")))

(event Custom|Air_Dash_Camera_Shake
  ;[1 1 1] Camera shake
  (Class|LegacyCameraShake|StartLegacyCameraShake (Game|GetPlayerCameraManager 0) "/Game/Movement/BP_Slight_Camera_Shake.BP_Slight_Camera_Shake_C" (+ (/ (Variables|Strength|GetDash_Strength) 7.5e+02) 2.0) "CameraLocal" "0, 0, 0")
  (Default|PlayHUDShake (Actor|GetComponentbyClass (Components|GetOwner) "/Game/Characters/Player/BPC_HUD.BPC_HUD_C")))

(event Input|EnhancedActionEvents|EnhancedInputActionIA_Air_Dash
  (params (ActionValue :type Boolean) (ElapsedSeconds :type Float%20%28double-precision%29) (TriggeredSeconds :type Float%20%28double-precision%29) (InputAction :type Input%20Action%20Object%20Reference :default "/Game/Characters/Player/Input/Actions/IA_Air_Dash.IA_Air_Dash"))
  ;[1 1 1] Input for air dash and being able to air dash based off of the falling and air dash cooldown variable
  (:Triggered
    (if (and (AI|Components|NavMovement|IsFalling (Actor|GetComponentbyClass (Components|GetOwner) "/Script/Engine.CharacterMovementComponent")) (not (Variables|Cooldown|GetAir_Dash_Cooldown)))
      (CallFunction|AirDash))))

(fn StopSlowTimeAD
  (Default|RemoveSlowTime (Actor|GetComponentbyClass (Components|GetOwner) "/Game/Characters/Player/Slow_Time/BPC_Slow_Time_Manager.BPC_Slow_Time_Manager_C") "NewEnumerator8"))