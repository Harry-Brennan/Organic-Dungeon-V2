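; Actor component that gives a character wall-running and wall jumps, with camera shake, tilt and slow-time extras for players.
; Tick uses side line traces, falling state, forward speed and cooldown to allow a run, then sphere traces each side.
; LaunchCharacter pushes the owner into and along the wall while gravity eases down.
; Losing the wall, nearing the floor or jumping off ends the run with a cooldown; the timed speed ramp is disconnected.
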(event EventBeginPlay
  (bind _wall_running_info (Class|BPICanWall-Run|GetWall-RunInfo(Message) (Components|GetOwner)))
  (Variables|Timing|SetMax_Wall_Run_Time (.max_wall_run_time _wall_running_info))
  (bind _capsule (Class|BPICanDash|GetCapsuleCollision(Message) (Components|GetOwner)))
  (Variables|Default|SetOwner_Capsule_Collision _capsule))

(fn WallRunMovement
  (params (Start :type Vector) (End :type Vector) (Direction :type Float%20%28double-precision%29))
  (bind _returnvalue (Components|GetOwner))
  (bind _returnvalue_2 (Actor|GetComponentbyClass _returnvalue "/Game/Characters/Player/BPC_Camera_Tilt.BPC_Camera_Tilt_C"))
  (bind (_outhit _returnvalue_3) (Collision|SphereTraceForObjects Start End 8.0 (Utilities|Array|MakeArray "ObjectTypeQuery7") false 0 (Variables|Traces|GetTrace%20Visibility)))
  (if _returnvalue_3
    (if (.ReturnValue (Utilities|WallRunVectorValidity (.ImpactNormal (Collision|BreakHitResult _outhit))))
      (Variables|Wall|SetWall_Run_Normal (.Vector2 (Utilities|WallRunVectorValidity (.ImpactNormal (Collision|BreakHitResult _outhit)))))
      ;[1 1 1] Stick character to wall
      (bind _ascharacter (Utilities|Casting|CastToCharacter (Components|GetOwner)))
      (Character|LaunchCharacter _ascharacter (Utilities|PlayertoWallVector) false false)
      ;[1 1 1] Move character forward
      (Character|LaunchCharacter _ascharacter (* (Math|Vector|CrossProduct (Variables|Wall|GetWall_Run_Normal) "0.000000,0.000000,1.000000") (* (Variables|Speed|GetWall_Run_Speed) Direction)) true (not (Variables|Status&Checks|GetWall_Run_Gravity)))
      (Default|UpdateCustomMovementMode (Actor|GetComponentbyClass (Components|GetOwner) "/Game/Movement/BPC_Custom_Movement_Handler.BPC_Custom_Movement_Handler_C") "NewEnumerator2")
      (CallFunction|StartCameraShake)
      (if (Utilities|DoesObjectImplementInterface _returnvalue "/Game/Characters/Player/BPI_Player.BPI_Player_C")
        (if (== Direction 1.0)
          (Default|WallrunningLeft _returnvalue_2)
          (else
            (Default|WallrunningRight _returnvalue_2))))
      (return true)
      (else
        (return false)))
    (else
      (return false))))

(fn EndWallRun
  (params (Wall_Run_Cooldown :type Float%20%28double-precision%29))
  (bind _returnvalue (Components|GetOwner))
  (if (Variables|Status&Checks|GetWall-Running)
    (Variables|Status&Checks|SetWall-Running false)
    (Variables|Status&Checks|SetWall_Run_Right false)
    (Variables|Status&Checks|SetWall_Run_Left false)
    (Variables|/Script/Engine.CharacterMovementComponent|SetGravityScale (Actor|GetComponentbyClass (Components|GetOwner) "/Script/Engine.CharacterMovementComponent") 2.5)
    (Variables|Status&Checks|SetWall_Run_Cooldown true)
    (Variables|Speed|SetWall_Run_Speed_Percentage 0.0)
    (Utilities|Time|SetTimerbyFunctionName 0 "Reset_Wall_Run_Cooldown" Wall_Run_Cooldown)
    (Default|TransitionfromMode (Actor|GetComponentbyClass (Components|GetOwner) "/Game/Movement/BPC_Custom_Movement_Handler.BPC_Custom_Movement_Handler_C") "NewEnumerator2")
    (CallFunction|ResetCameraShake)
    (Default|Cooldown (Actor|GetComponentbyClass (Components|GetOwner) "/Game/Movement/Double_Jump/BPC_Double_Jump.BPC_Double_Jump_C"))
    (Audio|Components|Audio|Stop (Variables|Sound|GetWall-Running_Sound))
    (if (Utilities|DoesObjectImplementInterface _returnvalue "/Game/Characters/Player/BPI_Player.BPI_Player_C")
      (Default|StoppingWallrunningTilt (Actor|GetComponentbyClass _returnvalue "/Game/Characters/Player/BPC_Camera_Tilt.BPC_Camera_Tilt_C"))
      (Default|RemoveSlowTime (Actor|GetComponentbyClass (Components|GetOwner) "/Game/Characters/Player/Slow_Time/BPC_Slow_Time_Manager.BPC_Slow_Time_Manager_C") "NewEnumerator5"))))

(fn LerpWallRunSpeed
  (params (Alpha :type Float%20%28double-precision%29))
  (Variables|Speed|SetWall_Run_Speed (Math|Float|Lerp (Variables|Speed|GetSpeed_At_Start_Of_Wall_Run) 7.5e+02 Alpha)))

(event Custom|Start_Camera_Shake
  (Utilities|FlowControl|DoOnce false
    (:Completed
      (if (Utilities|DoesObjectImplementInterface (Components|GetOwner) "/Game/Characters/Player/BPI_Player.BPI_Player_C")
        (Class|LegacyCameraShake|StartLegacyCameraShake (Game|GetPlayerCameraManager 0) "/Game/Movement/BP_Slight_Camera_Shake.BP_Slight_Camera_Shake_C" 1.0 "CameraLocal" "0, 0, 0")))))

(event Custom|Reset_Camera_Shake
  (Utilities|FlowControl|DoOnce false) ; enters at Reset
)

(event Custom|Reset_Wall_Run_Cooldown
  (Utilities|Time|ClearTimerbyFunctionName 0 "Reset_Wall_Run_Cooldown")
  (Variables|Status&Checks|SetWall_Run_Cooldown false))

(event Custom|Jump_Off_Wall
  (bind _wall_run_normal (Variables|Wall|GetWall_Run_Normal))
  (bind _jump_off_horizontal_force (Variables|JumpForce|GetJump_Off_Horizontal_Force))
  (if (Variables|Status&Checks|GetWall-Running)
    (CallFunction|EndWallRun 0.35)
    ;[1 1 1] Launch character in opposite direction to what wall you're running on
    (bind _ascharacter (Utilities|Casting|CastToCharacter (Components|GetOwner)))
    (Character|LaunchCharacter _ascharacter (Math|Vector|MakeVector (* (.x _wall_run_normal) _jump_off_horizontal_force) (* (.y _wall_run_normal) _jump_off_horizontal_force) (Variables|JumpForce|GetJump_Off_Vertical_Force)) false true)
    ;[1 1 1] If playe play camera shake
    (if (Utilities|DoesObjectImplementInterface (Components|GetOwner) "/Game/Characters/Player/BPI_Player.BPI_Player_C")
      (Class|LegacyCameraShake|StartLegacyCameraShake (Game|GetPlayerCameraManager 0) "/Game/Movement/BP_Slight_Camera_Shake.BP_Slight_Camera_Shake_C" 1.0 "CameraLocal" "0, 0, 0"))))

(event EventTick
  (params (DeltaSeconds :type Float%20%28single-precision%29))
  (bind _returnvalue (Components|GetOwner))
  (bind _returnvalue_2 (Components|GetOwner))
  (bind _returnvalue_3 (Components|GetOwner))
  (bind _returnvalue_4 (Components|GetOwner))
  (bind _returnvalue_5 (Components|GetOwner))
  (bind _returnvalue_6 (Components|GetOwner))
  (bind _returnvalue_7 (Components|GetOwner))
  (bind _returnvalue_8 (Components|GetOwner))
  (bind _array (Utilities|Array|MakeArray "ObjectTypeQuery7"))
  (bind _trace_visibility (Variables|Traces|GetTrace%20Visibility))
  (bind _returnvalue_9 (Transformation|GetActorLocation _returnvalue))
  (bind _returnvalue_10 (Actor|GetComponentbyClass _returnvalue_3 "/Script/Engine.CharacterMovementComponent"))
  (bind _returnvalue_11 (Actor|GetComponentbyClass _returnvalue_4 "/Script/Engine.CharacterMovementComponent"))
  (bind _returnvalue_12 (Transformation|GetActorLocation _returnvalue_6))
  (bind _returnvalue_13 (Transformation|GetActorRightVector _returnvalue_6))
  (bind _maxwalkspeed (Variables|/Script/Engine.CharacterMovementComponent|GetMaxWalkSpeed _returnvalue_10))
  (Utilities|FlowControl|Sequence
    (:then_0
      ;[1 1 1] Can wall run if falling, wall run cooldown not true and the horizontal velocity is greater than a specified amount
      (if (not (Variables|Status&Checks|GetWall-Running))
        (if (Variables|Status&Checks|GetAttempting%20to%20wall-run)
          (bind _returnvalue_14 (Collision|LineTraceForObjects _returnvalue_12 (+ _returnvalue_12 (* _returnvalue_13 1e+02)) _array false 0 _trace_visibility))
          (bind _returnvalue_15 (Collision|LineTraceForObjects _returnvalue_12 (+ _returnvalue_12 (* _returnvalue_13 -1e+02)) _array false 0 _trace_visibility))
          (if (Math|Boolean|ANDBoolean (AI|Components|NavMovement|IsFalling (Actor|GetComponentbyClass (Components|GetOwner) "/Script/Engine.CharacterMovementComponent")) (not (Variables|Status&Checks|GetWall_Run_Cooldown)) (>= (.x (Math|Vector|UnrotateVector (Variables|/Script/Engine.MovementComponent|GetVelocity (Actor|GetComponentbyClass _returnvalue_2 "/Script/Engine.CharacterMovementComponent")) (Transformation|GetActorRotation _returnvalue_2))) 75.0) (or _returnvalue_14 _returnvalue_15))
            (Variables|Status&Checks|SetCan_Wall_Run true)
            (else
              (Variables|Status&Checks|SetCan_Wall_Run false)
              (Utilities|FlowControl|Sequence
                (:then_0
                  (goto _label Reset))
                (:then_1
                  (goto _label_3 Reset)))))
          (else
            (Variables|Status&Checks|SetCan_Wall_Run false)))))
    (:then_1
      (if (Variables|Status&Checks|GetCan_Wall_Run)
        (Utilities|FlowControl|Sequence
          (:then_0
            (Utilities|FlowControl|DoOnce false :!label _label
              (:Completed
                (Variables|Timing|SetMax_Wall_Run_Time (Math|Float|Clamp(Float) (- (/ _maxwalkspeed 25.0) (/ _maxwalkspeed 1e+02)) 5.0 1e+01))
                (Variables|Speed|SetSpeed_At_Start_Of_Wall_Run (Math|Float|Clamp(Float) (* (.x (Math|Vector|UnrotateVector (Variables|/Script/Engine.MovementComponent|GetVelocity _returnvalue_10) (Transformation|GetActorRotation _returnvalue_3))) 2.0) 2.5e+03 99999.0))
                (if (Utilities|DoesObjectImplementInterface _returnvalue_5 "/Game/Characters/Player/BPI_Player.BPI_Player_C")
                  (Default|AddSlowTime (Actor|GetComponentbyClass _returnvalue_5 "/Game/Characters/Player/Slow_Time/BPC_Slow_Time_Manager.BPC_Slow_Time_Manager_C") (Variables|SlowTime|GetWall-Running%20Slow%20Time%20Amount) "NewEnumerator5")))))
          (:then_2
            (bind _on_wall (CallFunction|WallRunMovement (+ (* (Transformation|GetActorForwardVector _returnvalue_7) -15.0) (Transformation|GetActorLocation _returnvalue_7) (* (Transformation|GetActorRightVector _returnvalue_7) 5.0)) (.Right (Utilities|WallRunEndVectors)) -1.0))
            (if _on_wall
              (Variables|Status&Checks|SetWall-Running true)
              (Variables|Status&Checks|SetWall_Run_Right true)
              (Variables|Status&Checks|SetWall_Run_Left false)
              (Variables|/Script/Engine.CharacterMovementComponent|SetGravityScale _returnvalue_11 (Math|Interpolation|FInterpTo (Variables|/Script/Engine.CharacterMovementComponent|GetGravityScale _returnvalue_11) 0.25 (Utilities|Time|GetWorldDeltaSeconds) 1e+01) :!label _label_2)
              (Utilities|FlowControl|DoOnce false :!label _label_3
                (:Completed
                  (bind _returnvalue_16 (Audio|SpawnSoundAttached "/Game/VFX_SFX/Wall-Running/Wall-Running_Scrape_SC.Wall-Running_Scrape_SC" (Variables|/Script/Engine.Actor|GetRootComponent (Components|GetOwner)) "None" "0, 0, 0" "0, 0, 0" "KeepRelativeOffset" false 1.0 1.0 0.0 0 0))
                  (Variables|Sound|SetWall-Running_Sound _returnvalue_16)))
              (elif (Variables|Status&Checks|GetWall_Run_Right)
                (CallFunction|EndWallRun 1.0)
                (else
                  (bind _on_wall_2 (CallFunction|WallRunMovement (+ (* (Transformation|GetActorForwardVector _returnvalue_8) -15.0) (Transformation|GetActorLocation _returnvalue_8) (* (Transformation|GetActorRightVector _returnvalue_8) -5.0)) (.Left (Utilities|WallRunEndVectors)) 1.0))
                  (if _on_wall_2
                    (Variables|Status&Checks|SetWall-Running true)
                    (Variables|Status&Checks|SetWall_Run_Right false)
                    (Variables|Status&Checks|SetWall_Run_Left true)
                    (goto _label_2)
                    (else
                      (CallFunction|EndWallRun 1.0))))))))))
    (:then_2
      ;[1 1 1] Hit detection for if going to be touching the floor so should stop wall-running
      (if (Variables|Status&Checks|GetWall-Running)
        (bind _returnvalue_17 (Collision|LineTraceByChannel _returnvalue_9 (+ (* (Transformation|GetActorUpVector _returnvalue) -1.5e+02) _returnvalue_9) "TraceTypeQuery1" false 0 (Variables|Traces|GetTrace%20Visibility)))
        (if _returnvalue_17
          (CallFunction|EndWallRun 2.0))))))