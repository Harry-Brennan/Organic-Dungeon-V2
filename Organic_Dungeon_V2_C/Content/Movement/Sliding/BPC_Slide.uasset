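; Slide component for characters: starts above a minimum speed, locks move input, lowers friction, and ends on release, timeout or low speed.
; Tick pushes along the starting direction, traces slopes to adjust force and pitch, and blocks standing under obstacles.
; It also blends capsule height, launches characters in the path, and plays surface-based particles and sound.
; It notifies the movement handler, drives player camera tilt and slow time, and offers a slide-jump boost.
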(event EventBeginPlay
  (bind _slide_info (Class|BPICanSlide|GetSlidingInfo(Message) (Components|GetOwner)))
  (Variables|Speed|SetMin_Sliding_Speed (.min_slide_speed _slide_info)))

(event Custom|Slide_Jump_Boost
  (bind _returnvalue (Components|GetOwner))
  (bind _ascharacter (Utilities|Casting|CastToCharacter _returnvalue))
  (Character|LaunchCharacter _ascharacter (* (Transformation|GetActorUpVector _returnvalue) (Variables|JumpBoost|GetSlide_Jump_Force_Vertical)) false true))

(event Custom|Stop_Sliding
  (bind _returnvalue (Components|GetOwner))
  (bind _returnvalue_2 (Components|GetOwner))
  (bind _returnvalue_3 (Components|GetOwner))
  (bind _returnvalue_4 (Actor|GetComponentbyClass _returnvalue "/Script/Engine.CharacterMovementComponent"))
  (bind _returnvalue_5 (Transformation|GetActorRotation _returnvalue_2))
  (if (and (Variables|Checks&Status|GetCan_Stop_Sliding) (Variables|Checks&Status|GetSliding))
    (Variables|Checks&Status|SetStarting_Sliding false)
    (Variables|Transitioning|SetSliding_Transition_Percentage 0.0)
    (Variables|Time|SetSlide_Speed_Percentage 0.0)
    (Transformation|SetActorRotation _returnvalue_2 (Math|Rotator|MakeRotator (.roll _returnvalue_5) 0.0 (.yaw _returnvalue_5)))
    (Variables|Checks&Status|SetStopping_Sliding true)
    (Variables|Checks&Status|SetSliding false)
    (Variables|/Script/Engine.CharacterMovementComponent|SetBrakingDecelerationWalking _returnvalue_4 (Variables|CharacterMovementAssociated|GetNormal%20Braking%20Deceleration%20Walking))
    (Variables|/Script/Engine.CharacterMovementComponent|SetGroundFriction _returnvalue_4 (Variables|CharacterMovementAssociated|GetNormal%20Ground%20Friction))
    (Variables|Checks&Status|SetSlide_Cooldown true)
    (Default|TransitionfromMode (Actor|GetComponentbyClass (Components|GetOwner) "/Game/Movement/BPC_Custom_Movement_Handler.BPC_Custom_Movement_Handler_C") "NewEnumerator0")
    (bind _aspawn (Utilities|Casting|CastToPawn (Components|GetOwner)))
    (Input|SetIgnoreMoveInput (Pawn|GetController _aspawn) false)
    (if (Utilities|DoesObjectImplementInterface _returnvalue_3 "/Game/Characters/Player/BPI_Player.BPI_Player_C")
      (Default|RemoveSlowTime (Actor|GetComponentbyClass _returnvalue_3 "/Game/Characters/Player/Slow_Time/BPC_Slow_Time_Manager.BPC_Slow_Time_Manager_C") "NewEnumerator2"))
    (Utilities|FlowControl|Delay (Variables|Time|GetSlide_Cooldown_Length))
    (Variables|Checks&Status|SetSlide_Cooldown false)))

(event Custom|Start_Sliding
  (bind _returnvalue (Components|GetOwner))
  (bind _returnvalue_2 (Components|GetOwner))
  (bind _returnvalue_3 (Components|GetOwner))
  (bind _returnvalue_4 (Components|GetOwner))
  (bind _returnvalue_5 (Transformation|GetVelocity _returnvalue))
  (bind _returnvalue_6 (Transformation|GetActorRotation _returnvalue))
  (bind _returnvalue_7 (Actor|GetComponentbyClass _returnvalue_2 "/Script/Engine.CharacterMovementComponent"))
  (bind _returnvalue_8 (Transformation|GetActorRotation _returnvalue_3))
  (bind _returnvalue_9 (Actor|GetComponentbyClass _returnvalue_3 "/Script/Engine.CharacterMovementComponent"))
  (bind _returnvalue_10 (Math|Vector|UnrotateVector _returnvalue_5 _returnvalue_6))
  (bind _velocity (Variables|/Script/Engine.MovementComponent|GetVelocity _returnvalue_9))
  (bind _returnvalue_11 (Math|Vector|UnrotateVector _velocity _returnvalue_8))
  (if (Math|Boolean|ANDBoolean (Variables|Checks&Status|GetCan_Slide) (not (Variables|Checks&Status|GetSliding)) (not (Variables|Checks&Status|GetSlide_Cooldown)))
    (bind _slide_info (Class|BPICanSlide|GetSlidingInfo(Message) (Components|GetOwner)))
    (Variables|Speed|SetMin_Sliding_Speed (.min_slide_speed _slide_info))
    (Variables|Speed|SetBase_Movement_Speed (.base_movement_speed _slide_info))
    (if (>= (Math|Float|SelectFloat (* (.x _returnvalue_10) -1.0) (.x _returnvalue_10) (< (.x _returnvalue_10) 0.0)) (Variables|Speed|GetMin_Sliding_Speed))
      (Variables|Transitioning|SetSliding_Transition_Percentage 0.0)
      (bind _aspawn (Utilities|Casting|CastToPawn (Components|GetOwner)))
      (Input|SetIgnoreMoveInput (Pawn|GetController _aspawn) true)
      (Variables|Starting_Rot|SetRot_From_Velocity (Math|Conversions|RotationFromXVector _velocity))
      (bind _output_get (Variables|Speed|SetStart_Sliding_Speed (Math|Float|SelectFloat (* (.x _returnvalue_11) -1.0) (.x _returnvalue_11) (< (.x _returnvalue_11) 0.0))))
      (Variables|Speed|SetSlide_Speed _output_get)
      (Components|Tick|SetComponentTickEnabled true)
      (Variables|Checks&Status|SetStarting_Sliding true)
      (Variables|Checks&Status|SetSliding true)
      (Variables|Checks&Status|SetStopping_Sliding false)
      (Variables|/Script/Engine.CharacterMovementComponent|SetBrakingDecelerationWalking _returnvalue_7 (* (Variables|CharacterMovementAssociated|GetSliding%20Braking%20Deceleration%20Walking) (Math|Float|Clamp(Float) (/ (Math|Vector|VectorLength (Transformation|GetVelocity _returnvalue_2)) (Variables|CharacterMovementAssociated|GetMax%20Sliding%20Speed%20for%20Braking%20Deceleration%20Calc)))))
      (Variables|/Script/Engine.CharacterMovementComponent|SetGroundFriction _returnvalue_7 (Variables|CharacterMovementAssociated|GetSliding%20Ground%20Friction))
      (Default|UpdateCustomMovementMode (Actor|GetComponentbyClass (Components|GetOwner) "/Game/Movement/BPC_Custom_Movement_Handler.BPC_Custom_Movement_Handler_C") "NewEnumerator0")
      (if (Utilities|DoesObjectImplementInterface _returnvalue_4 "/Game/Characters/Player/BPI_Player.BPI_Player_C")
        (Default|AddSlowTime (Actor|GetComponentbyClass _returnvalue_4 "/Game/Characters/Player/Slow_Time/BPC_Slow_Time_Manager.BPC_Slow_Time_Manager_C") (Variables|SlowTime|GetSliding%20Slow%20Time%20Amount) "NewEnumerator2")))))

(event Input|EnhancedActionEvents|EnhancedInputActionIA_Slide
  (params (ActionValue :type Boolean) (ElapsedSeconds :type Float%20%28double-precision%29) (TriggeredSeconds :type Float%20%28double-precision%29) (InputAction :type Input%20Action%20Object%20Reference :default "/Game/Characters/Player/Input/Actions/IA_Slide.IA_Slide"))
  (:Triggered
    ;[1 1 1] call Start or stop sliding depending on input
    (CallFunction|StartSliding)
    ;[1 1 1] Attempting to slide keeps track of whether the player wants to start sliding
    (Variables|Checks&Status|SetAttempting_To_Slide true))
  (:Canceled
    (CallFunction|StopSliding :!label _label)
    (Variables|Checks&Status|SetAttempting_To_Slide false))
  (:Completed
    (goto _label)))

(event Custom|Check_Sliding_Down_Velocity
  ;[1 1 1] Unused barely working code for turning around the movement of the slide when reaching low speed whilst going up a slope
)

(event EventTick
  (params (DeltaSeconds :type Float%20%28single-precision%29))
  (bind _returnvalue (Components|GetOwner))
  (bind _returnvalue_2 (Components|GetOwner))
  (bind _returnvalue_3 (Components|GetOwner))
  (bind _returnvalue_4 (Components|GetOwner))
  (bind _returnvalue_5 (Components|GetOwner))
  (bind _returnvalue_6 (Components|GetOwner))
  (bind _returnvalue_7 (Components|GetOwner))
  (bind _returnvalue_8 (Components|GetOwner))
  (bind _returnvalue_9 (Components|GetOwner))
  (bind _rot_from_velocity (Variables|Starting_Rot|GetRot_From_Velocity))
  (bind _rot_from_velocity_2 (Variables|Starting_Rot|GetRot_From_Velocity))
  (bind _returnvalue_10 (Transformation|GetActorLocation _returnvalue))
  (bind _returnvalue_11 (Transformation|GetActorRotation _returnvalue_8))
  (bind _returnvalue_12 (Transformation|GetActorLocation _returnvalue_2))
  (bind _returnvalue_13 (Transformation|GetActorLocation _returnvalue_3))
  (bind _returnvalue_14 (Actor|GetComponentbyClass _returnvalue_5 "/Script/Engine.CharacterMovementComponent"))
  (bind _returnvalue_15 (Transformation|GetActorRotation _returnvalue_5))
  (bind _returnvalue_16 (Math|Vector|GetUpVector _rot_from_velocity))
  (bind _returnvalue_17 (Transformation|GetActorLocation _returnvalue_9))
  (bind _returnvalue_18 (* _returnvalue_16 -5e+01))
  (bind _velocity (Variables|/Script/Engine.MovementComponent|GetVelocity _returnvalue_14))
  (bind _returnvalue_19 (Math|Vector|UnrotateVector _velocity _returnvalue_15))
  (bind _returnvalue_20 (< (.x _returnvalue_19) 0.0))
  (bind _returnvalue_21 (* (.x _returnvalue_19) -1.0))
  (bind _returnvalue_22 (< (.y _returnvalue_19) 0.0))
  (bind _returnvalue_23 (* (.y _returnvalue_19) -1.0))
  (bind _returnvalue_24 (Math|Float|SelectFloat _returnvalue_21 (.x _returnvalue_19) _returnvalue_20))
  (bind _returnvalue_25 (Math|Float|SelectFloat _returnvalue_23 (.y _returnvalue_19) _returnvalue_22))
  (Utilities|FlowControl|Sequence
    (:then_0
      (if (Variables|Checks&Status|GetSliding)
        (Utilities|FlowControl|Sequence
          (:then_0
            ;[1 1 1] Changing the slide speed percentage based on if we are on a slope so if we are not on a slope then it passes time
            (Variables|Time|SetSlide_Speed_Percentage (Math|Float|SelectFloat 0.0 (Math|Float|Clamp(Float) (+ (Variables|Time|GetSlide_Speed_Percentage) (/ 1.0 (/ (Variables|Time|GetMax_Slide_Time) (Class|ActorComponent|GetComponentTickInterval))))) (Variables|Ground|GetOn_Slope)))
            ;[1 1 1] Lerping the slide speed down to 50 from starting based on the percentage of time for the maximum slide speed
            (Variables|Speed|SetSlide_Speed (Math|Float|Lerp (Variables|Speed|GetStart_Sliding_Speed) 5e+01 (Variables|Time|GetSlide_Speed_Percentage)))
            (if (Variables|Ground|GetOn_Slope)
              (if (Variables|Ground|GetGoing_Down_Slope)
                ;[1 1 1] Adding the actual force for the character moving in the direction they started sliding in and if they are on a slope then only doing it when going down the slope
                (Physics|AddForce (Actor|GetComponentbyClass (Components|GetOwner) "/Script/Engine.CharacterMovementComponent") (* (Math|Vector|GetForwardVector (Variables|Starting_Rot|GetRot_From_Velocity)) (* (Variables|Speed|GetSlide_Speed) 5.0)) :!label _label))
              (else
                (goto _label)))
            ;[1 1 1] Stopping sliding if velocity is nearly 0 / 25
            (if (Math|Boolean|ORBoolean (>= (Variables|Time|GetSlide_Speed_Percentage) 1.0) (and (<= _returnvalue_24 25.0) (< _returnvalue_25 1.0)) (and (<= _returnvalue_25 25.0) (< _returnvalue_24 1.0)))
              (Variables|Time|SetSlide_Cooldown_Length 2.0)
              (CallFunction|StopSliding)))
          (:then_1
            ;[1 1 1] Constantly doing checks to see if we can stop sliding based on if there is something above us
            (bind _returnvalue_26 (Collision|LineTraceForObjects _returnvalue_10 (+ (* (Transformation|GetActorUpVector _returnvalue) 1.5e+02) _returnvalue_10) (Utilities|Array|MakeArray "ObjectTypeQuery1" "ObjectTypeQuery2" "ObjectTypeQuery7" "ObjectTypeQuery4" "ObjectTypeQuery9" "ObjectTypeQuery11") false (Utilities|Array|MakeArray _returnvalue) (Variables|Traces|GetTrace%20Visibility) true "(R=1.000000,G=0.901964,B=0.000000,A=1.000000)"))
            (bind _output_get (Variables|Checks&Status|SetCan_Stop_Sliding (not _returnvalue_26)))
            (if (and _output_get (not (Variables|Checks&Status|GetAttempting_To_Slide)))
              (CallFunction|StopSliding)))
          (:then_2
            ;[1 1 1] Hit deftection for slope
            (bind _outhit (Collision|LineTraceForObjects _returnvalue_17 (Math|Vector|SelectVector (+ _returnvalue_17 _returnvalue_18) (+ _returnvalue_18 (* (Math|Vector|GetForwardVector _rot_from_velocity) 125.0) _returnvalue_17) (Variables|Ground|GetGoing_Down_Slope)) (Utilities|Array|MakeArray "ObjectTypeQuery1" "ObjectTypeQuery2" "ObjectTypeQuery7" "ObjectTypeQuery9" "ObjectTypeQuery11" "ObjectTypeQuery4") false 0 "ForDuration"))
            (bind _output_get_2 (Variables|Ground|SetGround_Normal (.Normal (Collision|BreakHitResult _outhit))))
            ;[1 1 1] Calculate angle of the slope
            (Variables|Ground|SetGround_Angle (Math|Float|Floor (Class|KismetMathLibrary|DegAcos (Math|Vector|DotProduct _output_get_2 "0.000000,0.000000,1.000000"))))
            ;[1 1 1] Check if we're on a slope
            (if (> (Variables|Ground|GetGround_Angle) 1)
              ;[1 1 1] Hit detection for checking if we are going down a slope or not
              (bind (_outhit_2 _returnvalue_27) (Collision|LineTraceByChannel _returnvalue_12 (+ (+ (* (Math|Vector|GetUpVector _rot_from_velocity_2) -5e+01) (* (Math|Vector|GetForwardVector _rot_from_velocity_2) 2.5e+02)) _returnvalue_12) "TraceTypeQuery1" false 0 "None"))
              (if (and _returnvalue_27 (== (.HitActor (Collision|BreakHitResult _outhit_2)) (.HitActor (Collision|BreakHitResult _outhit))))
                (Variables|Ground|SetOn_Slope true)
                (Variables|Ground|SetGoing_Down_Slope false)
                ;[1 1 1] Add force backwards from original rotation velocity if velocity is higher than 100
                (if (not (<= (.x (Math|Vector|UnrotateVector (Variables|/Script/Engine.MovementComponent|GetVelocity (Actor|GetComponentbyClass _returnvalue_7 "/Script/Engine.CharacterMovementComponent")) (Transformation|GetActorRotation _returnvalue_7))) 1e+02))
                  (Physics|AddForce (Actor|GetComponentbyClass (Components|GetOwner) "/Script/Engine.CharacterMovementComponent") (* (* (Math|Vector|GetForwardVector (Variables|Starting_Rot|GetRot_From_Velocity)) (* (Variables|Ground|GetGround_Angle) (Variables|Ground|GetAgainst_Slope_Speed_Multiplier))) -1.0))
                  (if (not (Variables|Checks&Status|GetStarting_Sliding)) :!label _label_2
                    ;[1 1 1] Set character rotation to match the slope angle
                    (Transformation|SetActorRotation _returnvalue_8 (Math|Rotator|MakeRotator (.roll _returnvalue_11) (Math|Interpolation|FInterpTo (.pitch _returnvalue_11) (.pitch (Math|Rotator|MakeRotfromZX (Variables|Ground|GetGround_Normal) (Transformation|GetActorForwardVector (Components|GetOwner)))) (Utilities|Time|GetWorldDeltaSeconds) 5.0) (.yaw _returnvalue_11)) :!label _label_3)))
                (else
                  (Variables|Ground|SetOn_Slope true)
                  (Variables|Ground|SetGoing_Down_Slope true)
                  ;[1 1 1] Add force forwards when going down the slope depending on the slope angle and slope speed multiplier
                  (Physics|AddForce (Actor|GetComponentbyClass (Components|GetOwner) "/Script/Engine.CharacterMovementComponent") (* (Math|Vector|GetForwardVector (Variables|Starting_Rot|GetRot_From_Velocity)) (* (* (Variables|Ground|GetGround_Angle) (Variables|Ground|GetSlope_Speed_Multiplier)) 5.0)))
                  (goto _label_2)))
              (else
                (Variables|Ground|SetOn_Slope false)
                (Variables|Ground|SetGoing_Down_Slope false)
                (goto _label_3))))
          (:then_3
            ;[1 1 1] Hit detection for launching other characters
            (CallFunction|SlideHitDetection))
          (:then_4
            ;[1 1 1] Particle effects when going faster than 10 units of velocity
            (if (> (Math|Vector|VectorLength (Variables|/Script/Engine.MovementComponent|GetVelocity (Actor|GetComponentbyClass (Components|GetOwner) "/Script/Engine.CharacterMovementComponent"))) 1e+01)
              (Utilities|FlowControl|DoOnce false :!label _label_4
                (:Completed
                  (CallFunction|StartSlidingParticles)
                  (goto _label_5 Reset))))))
        (else
          (Utilities|FlowControl|DoOnce false :!label _label_5
            (:Completed
              (CallFunction|StopSlidingParticles)
              (goto _label_4 Reset))))))
    (:then_1
      (if (Variables|Checks&Status|GetStarting_Sliding)
        ;[1 1 1] Sliding transition percentage
        (Variables|Transitioning|SetSliding_Transition_Percentage (Math|Float|Clamp(Float) (+ (Variables|Transitioning|GetSliding_Transition_Percentage) (/ 1.0 (/ 0.1 (Class|ActorComponent|GetComponentTickInterval))))))
        ;[1 1 1] Changing hitbox to be smaller for sliding
        (CallFunction|SlidingHitbox (Variables|Transitioning|GetSliding_Transition_Percentage))
        (if (Utilities|DoesObjectImplementInterface _returnvalue_4 "/Game/Characters/Player/BPI_Player.BPI_Player_C")
          ;[1 1 1] Camera tilt for starting sliding
          (Default|IntoSlidingCameraTilt (Actor|GetComponentbyClass _returnvalue_4 "/Game/Characters/Player/BPC_Camera_Tilt_Manager.BPC_Camera_Tilt_Manager_C")))
        (if (>= (Variables|Transitioning|GetSliding_Transition_Percentage) 1.0)
          (Variables|Checks&Status|SetStarting_Sliding false))
        ;[1 1 1] If we cannot slide anymore then we set the cooldown to be 0.1 so we cant just spam sliding and then we stop sliding
        (if (not (Variables|Checks&Status|GetCan_Slide)) :!label _label_6
          (Variables|Time|SetSlide_Cooldown_Length 0.1)
          (CallFunction|StopSliding))
        (elif (Variables|Checks&Status|GetStopping_Sliding)
          ;[1 1 1] Hit detection for being able to stop sliding when stopped sliding is already true as an extra check
          (bind _returnvalue_28 (Collision|LineTraceForObjects _returnvalue_13 (+ (* (Transformation|GetActorUpVector _returnvalue_3) 1.5e+02) _returnvalue_13) (Utilities|Array|MakeArray "ObjectTypeQuery1" "ObjectTypeQuery2" "ObjectTypeQuery7" "ObjectTypeQuery4" "ObjectTypeQuery9" "ObjectTypeQuery11") false (Utilities|Array|MakeArray _returnvalue_3) (Variables|Traces|GetTrace%20Visibility) true "(R=0.128230,G=0.000000,B=1.000000,A=1.000000)"))
          (if _returnvalue_28
            (Variables|Checks&Status|SetSliding true)
            (else
              (Variables|Checks&Status|SetSliding false)
              ;[1 1 1] Slide transition percentage
              (Variables|Transitioning|SetSliding_Transition_Percentage (Math|Float|Clamp(Float) (+ (Variables|Transitioning|GetSliding_Transition_Percentage) (/ 1.0 (/ 0.2 (Class|ActorComponent|GetComponentTickInterval))))))
              ;[1 1 1] Changing hit box of owner back to normal
              (CallFunction|RevertHitbox (Variables|Transitioning|GetSliding_Transition_Percentage))
              (if (Utilities|DoesObjectImplementInterface _returnvalue_6 "/Game/Characters/Player/BPI_Player.BPI_Player_C")
                ;[1 1 1] Camera tilt for ending sliding
                (Default|OutSlidingCameraTilt (Actor|GetComponentbyClass _returnvalue_6 "/Game/Characters/Player/BPC_Camera_Tilt_Manager.BPC_Camera_Tilt_Manager_C")))
              ;[1 1 1] End of sliding
              (if (>= (Variables|Transitioning|GetSliding_Transition_Percentage) 1.0)
                (Variables|Checks&Status|SetStopping_Sliding false)
                (Components|Tick|SetComponentTickEnabled false)
                (goto _label_6)
                (else
                  (goto _label_6)))))
          (else
            (goto _label_6)))))))

(event Custom|Sliding_Hitbox
  (params (Alpha :type Float%20%28double-precision%29))
  ;[1 1 1] Changing the half height of the character's capsule collision, this needs to be made more modular by getting the normal half height and the targeted half height
  (bind _capsule_hitbox (Class|BPICanSlide|GetHitbox(Message) (Components|GetOwner)))
  (Components|Capsule|SetCapsuleHalfHeight _capsule_hitbox (Math|Float|Lerp (Components|Capsule|GetUnscaledCapsuleHalfHeight _capsule_hitbox) 3e+01 Alpha) true)
  (bind _skeletal_mesh (Class|BPICanSlide|GetMesh(Message) (Components|GetOwner)))
  (Transformation|SetRelativeLocation _skeletal_mesh (Math|Vector|Lerp(Vector) (Variables|/Script/Engine.SceneComponent|GetRelativeLocation _skeletal_mesh) "0.000000,0.000000,-40.000000" Alpha) false false))

(event Custom|Revert_Hitbox
  (params (Alpha :type Float%20%28double-precision%29))
  ;[1 1 1] Changing the half height of the character's capsule collision, this needs to be made more modular by getting the normal half height and the targeted half height
  (bind _capsule_hitbox (Class|BPICanSlide|GetHitbox(Message) (Components|GetOwner)))
  (Components|Capsule|SetCapsuleHalfHeight _capsule_hitbox (Math|Float|Lerp (Components|Capsule|GetUnscaledCapsuleHalfHeight _capsule_hitbox) 9e+01 Alpha) true)
  (bind _skeletal_mesh (Class|BPICanSlide|GetMesh(Message) (Components|GetOwner)))
  (Transformation|SetRelativeLocation _skeletal_mesh (Math|Vector|Lerp(Vector) (Variables|/Script/Engine.SceneComponent|GetRelativeLocation _skeletal_mesh) "0.000000,0.000000,-89.000000" Alpha) false false))

(event Custom|Slide_Hit_Detection
  (bind _returnvalue (Components|GetOwner))
  (bind _returnvalue_2 (Components|GetOwner))
  (bind _returnvalue_3 (Components|GetOwner))
  (bind _rot_from_velocity (Variables|Starting_Rot|GetRot_From_Velocity))
  (bind _returnvalue_4 (Transformation|GetActorLocation _returnvalue_3))
  (bind _returnvalue_5 (Actor|GetComponentbyClass _returnvalue_2 "/Script/Engine.CharacterMovementComponent"))
  (bind _velocity (Variables|/Script/Engine.MovementComponent|GetVelocity _returnvalue_5))
  (bind _returnvalue_6 (Math|Vector|VectorLength _velocity))
  ;[1 1 1] Launching enemies out of the way of the sliding character
  (bind (_outhits _returnvalue_7) (Class|KismetSystemLibrary|BoxTraceMultiforObjects _returnvalue_4 (+ _returnvalue_4 (* (Math|Vector|GetForwardVector _rot_from_velocity) 1e+02)) "32.000000,32.000000,32.000000" _rot_from_velocity (Utilities|Array|MakeArray "ObjectTypeQuery3" "ObjectTypeQuery8" "ObjectTypeQuery10") false (Utilities|Array|MakeArray (Components|GetOwner)) (Variables|Traces|GetTrace%20Visibility) true))
  (if _returnvalue_7
    (for _array_element _outhits
      (bind _ascharacter (Utilities|Casting|CastToCharacter (.HitActor (Collision|BreakHitResult _array_element))))
      (Character|LaunchCharacter _ascharacter (+ (* (Transformation|GetActorForwardVector _returnvalue) _returnvalue_6) (* (Transformation|GetActorUpVector _returnvalue) (/ _returnvalue_6 2.0))) true true))
    (Audio|PlaySoundatLocation "/Game/VFX_SFX/Ground_Slam/Ground_Slam_Impact_SC.Ground_Slam_Impact_SC" (Transformation|GetActorLocation _returnvalue) "0, 0, 0" 1.0 1.0 0.0 0 0 0 0)))

(event Custom|Spawn_Slide_Particles
  (bind _returnvalue (Components|GetOwner))
  (bind _returnvalue_2 (Components|GetOwner))
  (bind _returnvalue_3 (Transformation|GetActorLocation _returnvalue_2))
  (bind _returnvalue_4 (Actor|GetComponentbyClass _returnvalue_2 "/Script/Engine.CharacterMovementComponent"))
  (bind _velocity (Variables|/Script/Engine.MovementComponent|GetVelocity _returnvalue_4))
  (bind _returnvalue_5 (Math|Conversions|RotationFromXVector _velocity))
  (bind _returnvalue_6 (Math|Vector|GetForwardVector _returnvalue_5))
  (bind _returnvalue_7 (* _returnvalue_6 5e+01))
  (bind _returnvalue_8 (+ _returnvalue_7 _returnvalue_3))
  (Transformation|SetActorLocation (Variables|Default|GetSliding_Particles) (+ (* (Math|Vector|GetForwardVector (Math|Conversions|RotationFromXVector (Variables|/Script/Engine.MovementComponent|GetVelocity (Actor|GetComponentbyClass _returnvalue "/Script/Engine.CharacterMovementComponent")))) 2.5e+02) (Transformation|GetActorLocation _returnvalue)) false false)
  (bind (_outhit _returnvalue_9) (Collision|LineTraceByChannel _returnvalue_8 (+ (* (Transformation|GetActorUpVector _returnvalue_2) -45.0) _returnvalue_8) "TraceTypeQuery1" false (Utilities|Array|MakeArray (Components|GetOwner)) (Variables|Traces|GetTrace%20Visibility) true "(R=0.000000,G=1.000000,B=0.459113,A=1.000000)" "(R=0.278180,G=0.000000,B=1.000000,A=1.000000)"))
  (if _returnvalue_9
    (Variables|Default|SetSurface_Sliding_On (Collision|GetSurfaceType _outhit))
    (Niagara|SetNiagaraVariable(LinearColor) (Variables|/Game/VFX_SFX/Niagara/Sliding_Particles/BP_Sliding_Particles.BP_Sliding_Particles_C|GetSlide_Particles (Variables|Default|GetSliding_Particles)) "user.Ground_Colour" (Utilities|Select :Index (Collision|GetSurfaceType _outhit) :SurfaceType_Default (Math|Color|MakeColor 0.0 0.0 0.0) :SurfaceType1 "" :SurfaceType2 "" :SurfaceType3 "" :SurfaceType4 ""))))

(event Custom|Start_Sliding_Particles
  (bind _returnvalue (Components|GetOwner))
  (bind _returnvalue_2 (Transformation|GetActorLocation _returnvalue))
  (bind _returnvalue_3 (Actor|GetComponentbyClass _returnvalue "/Script/Engine.CharacterMovementComponent"))
  (bind _velocity (Variables|/Script/Engine.MovementComponent|GetVelocity _returnvalue_3))
  (bind _returnvalue_4 (Math|Conversions|RotationFromXVector _velocity))
  (bind _returnvalue_5 (Math|Vector|GetForwardVector _returnvalue_4))
  (bind _returnvalue_6 (* _returnvalue_5 5e+01))
  (bind _returnvalue_7 (+ _returnvalue_6 _returnvalue_2))
  (bind _returnvalue_8 (Game|SpawnActorfromClass "/Game/VFX_SFX/Niagara/Sliding_Particles/BP_Sliding_Particles.BP_Sliding_Particles_C" (Math|Transform|MakeTransform _returnvalue_7 (Math|Rotator|FindLookatRotation _returnvalue_7 _returnvalue_2) "1.000000,1.000000,1.000000") "AlwaysSpawn" "MultiplyWithRoot" 0 0))
  (Variables|Default|SetSliding_Particles _returnvalue_8)
  (bind _returnvalue_9 (Utilities|Time|SetTimerbyEvent (delegate Custom|Spawn_Slide_Particles) 0.1 true))
  (bind _returnvalue_10 (Utilities|Time|SetTimerbyFunctionName 0 "Play_Slide_Sound" 0.1 true)))

(event Custom|Stop_Sliding_Particles
  (Actor|DestroyActor (Variables|Default|GetSliding_Particles))
  (Utilities|Time|ClearandInvalidateTimerbyHandle (stale Custom|Start_Sliding_Particles _returnvalue_9))
  (Utilities|Time|ClearandInvalidateTimerbyHandle (stale Custom|Start_Sliding_Particles _returnvalue_10)))

(event Custom|Play_Slide_Sound
  (Audio|PlaySoundatLocation (Utilities|Select :Index (Variables|Default|GetSurface_Sliding_On) :SurfaceType_Default "/Game/VFX_SFX/Sounds/Footfalls/Tile/Footstep_Tile_SC.Footstep_Tile_SC" :SurfaceType1 0 :SurfaceType2 0 :SurfaceType3 0 :SurfaceType4 0) (Transformation|GetActorLocation (Components|GetOwner)) "0, 0, 0" 1.0 1.0 0.0 0 0 0 0))