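; BPC_Double_Jump is a character component that provides upgradeable mid-air jumps with a limited count, refilled by a Cooldown event.
; Jumping cancels any ground slam, then launches the owner upward while keeping its forward speed, with sound, AI noise and Niagara between the feet.
; It also re-enables air dash.
; Owners implementing BPI_Player get HUD updates and camera shake, plus timed slow motion when air dash exists.
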(event EventBeginPlay
  (Variables|Jumps|SetAvailable_Jumps (Variables|Jumps|GetMax_Jumps)))

(fn StopSlowTimeDJ
  (Default|RemoveSlowTime (Actor|GetComponentbyClass (Components|GetOwner) "/Game/Characters/Player/Slow_Time/BPC_Slow_Time_Manager.BPC_Slow_Time_Manager_C") "NewEnumerator7"))

(event Custom|Cooldown
  (bind _returnvalue (Components|GetOwner))
  (Variables|Jumps|SetAvailable_Jumps (Variables|Jumps|GetMax_Jumps))
  (if (Utilities|DoesObjectImplementInterface _returnvalue "/Game/Characters/Player/BPI_Player.BPI_Player_C")
    (Default|ForciblyResetMovementAbility (Actor|GetComponentbyClass _returnvalue "/Game/Characters/Player/BPC_HUD.BPC_HUD_C") "NewEnumerator0")))

(event Custom|Double_Jump
  (bind _returnvalue (Components|GetOwner))
  (bind _returnvalue_2 (Components|GetOwner))
  (bind _returnvalue_3 (Components|GetOwner))
  (bind _returnvalue_4 (Components|GetOwner))
  (bind _returnvalue_5 (Components|GetOwner))
  (bind _returnvalue_6 (Components|GetOwner))
  (bind _returnvalue_7 (Actor|GetComponentbyClass _returnvalue "/Script/Engine.SkeletalMeshComponent"))
  (bind _returnvalue_8 (Actor|GetComponentbyClass _returnvalue_5 "/Game/Movement/Air_Dash/BPC_Air_Dash.BPC_Air_Dash_C"))
  (bind _returnvalue_9 (Actor|GetComponentbyClass _returnvalue_2 "/Game/Movement/Ground_Slam/BPC_Ground_Slam.BPC_Ground_Slam_C"))
  (bind _returnvalue_10 (Actor|GetComponentbyClass _returnvalue_3 "/Game/Characters/Player/BPC_HUD.BPC_HUD_C"))
  (bind _returnvalue_11 (Transformation|GetSocketLocation _returnvalue_7 "foot_l"))
  (bind _returnvalue_12 (Transformation|GetSocketLocation _returnvalue_7 "foot_r"))
  (bind _returnvalue_13 (- _returnvalue_12 _returnvalue_11))
  (bind _returnvalue_14 (/ _returnvalue_13 2.0))
  (bind _returnvalue_15 (+ _returnvalue_11 _returnvalue_14))
  ;[1 1 1] Check if we can double jump
  (if (Math|Boolean|ANDBoolean (> (Variables|Jumps|GetAvailable_Jumps) 0) (Variables|Status|GetCan_Double_Jump) (not (Variables|Status|GetAlready_Jumping)))
    (Utilities|IsValid _returnvalue_9
      (:Is%20Valid
        ;[1 1 1] Cancel ground slam
        (Default|StopGroundSlam _returnvalue_9))
      (:Is%20Not%20Valid
        _))
    (bind _ascharacter (Utilities|Casting|CastToCharacter (Components|GetOwner)))
    (Character|LaunchCharacter _ascharacter (+ (* (Transformation|GetActorUpVector _returnvalue_4) (Variables|Force|GetJump_Force)) (* (Transformation|GetActorForwardVector _returnvalue_4) (.x (Math|Vector|UnrotateVector (Variables|/Script/Engine.MovementComponent|GetVelocity (Actor|GetComponentbyClass _returnvalue_4 "/Script/Engine.CharacterMovementComponent")) (Transformation|GetActorRotation _returnvalue_4))))) true true)
    ;[1 1 1] Camera shake if player is owner
    (if (Utilities|DoesObjectImplementInterface (Components|GetOwner) "/Game/Characters/Player/BPI_Player.BPI_Player_C")
      (Class|LegacyCameraShake|StartLegacyCameraShake (Game|GetPlayerCameraManager 0) "/Game/Movement/BP_Slight_Camera_Shake.BP_Slight_Camera_Shake_C" 2.0 "CameraLocal" "0, 0, 0")
      (Default|PlayHUDShake _returnvalue_10)
      (Default|UseMovementAbility _returnvalue_10 "NewEnumerator0"))
    ;[1 1 1] Decrements available jumps
    (Math|Integer|DecrementInt (Variables|Jumps|GetAvailable_Jumps)
      (:%20%20
        ;[1 1 1] Play noise and report sound inbetween the 2 feet bones
        (Audio|PlaySoundatLocation "/Game/VFX_SFX/Double_Jump/Double_Jump_SC.Double_Jump_SC" _returnvalue_15 "0, 0, 0" 1.0 1.0 0.0 0 0 0 0)
        (Class|AISenseHearing|ReportNoiseEvent _returnvalue_15 1.5 (Components|GetOwner) 0.0 "None")
        ;[1 1 1] Spawn double jump niagara at point in between feet bones
        (Niagara|SpawnSystematLocation "/Game/VFX_SFX/Niagara/Double_Jump/NS_Double_Jump.NS_Double_Jump" _returnvalue_15)
        ;[1 1 1] Allows another air dash if the component is valid
        (Utilities|IsValid _returnvalue_8
          (:Is%20Valid
            (Variables|/Game/Movement/Air_Dash/BPC_Air_Dash.BPC_Air_Dash_C|SetAir_Dash_Cooldown _returnvalue_8 false)
            (if (Utilities|DoesObjectImplementInterface _returnvalue_6 "/Game/Characters/Player/BPI_Player.BPI_Player_C")
              (Default|ForciblyResetMovementAbility (Actor|GetComponentbyClass _returnvalue_6 "/Game/Characters/Player/BPC_HUD.BPC_HUD_C") "NewEnumerator1")
              (Default|AddSlowTime (Actor|GetComponentbyClass (Components|GetOwner) "/Game/Characters/Player/Slow_Time/BPC_Slow_Time_Manager.BPC_Slow_Time_Manager_C") (Variables|SlowTime|GetSlow%20Time%20Amount) "NewEnumerator7")
              (Utilities|Time|SetTimerbyFunctionName 0 "Stop Slow Time DJ" (Variables|SlowTime|GetSlow%20Time%20Duration)))))))))

(event Custom|Increase_Max_Jumps
  (params (Amount_To_Increase_By :type Integer))
  (bind _output_get (Variables|Jumps|SetMax_Jumps (+ (Variables|Jumps|GetMax_Jumps) Amount_To_Increase_By)))
  (Variables|Jumps|SetAvailable_Jumps _output_get))