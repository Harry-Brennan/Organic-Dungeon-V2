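; Flying-movement component that automatically triggers a gravity toggle on its owner at high speed.
; Each Tick it compares the owner's CharacterMovement velocity magnitude against MaxVel and checks that GravityScale is zero or below.
; When both hold, it sends a ToggleGravity interface message to the owner with fixed start, end and timing values, leaving the gravity change to the owner.
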(event EventTick
  (params (DeltaSeconds :type Float%20%28single-precision%29))
  (bind _returnvalue (Components|GetOwner))
  (bind _returnvalue_2 (Actor|GetComponentbyClass _returnvalue "/Script/Engine.CharacterMovementComponent"))
  (if (and (>= (Math|Vector|VectorLength (Variables|/Script/Engine.MovementComponent|GetVelocity _returnvalue_2)) (Variables|Default|GetMax_Vel)) (not (> (Variables|/Script/Engine.CharacterMovementComponent|GetGravityScale _returnvalue_2) 0.0)))
    (Class|BPICanFly|ToggleGravity(Message) (Components|GetOwner) 1.8 0.0 1.3)))