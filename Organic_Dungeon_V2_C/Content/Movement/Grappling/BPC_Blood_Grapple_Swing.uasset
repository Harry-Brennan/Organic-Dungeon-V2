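; Actor component for the blood grapple and swing ability, with cable, audio, HUD, camera shake and slow-time feedback.
; A camera box trace attaches a blade and cable to the hit, then collision type decides whether to launch the owner or yank the target.
; Some surfaces allow swinging: Tick applies force toward the hit until release, timeout with blinking cable, or optional obstruction check.
; Ending a swing launches along view direction, weaker at higher speed.
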(event EventTick
  (params (DeltaSeconds :type Float%20%28single-precision%29))
  (Variables|Checks|SetCan%20Grapple (not (Math|Boolean|ORBoolean (Variables|Checks|GetGrapple%20Cooldown) (Variables|Checks|GetGrapple%20Pull?) (Variables|Checks|GetGrappled) (Variables|Checks|GetSwinging))))
  (if (Variables|Checks|GetSwinging)
    (CallFunction|SwingForce)))

(event EventBeginPlay
  (bind _returnvalue (Components|GetOwner))
  (bind _returnvalue_2 (Actor|GetComponentbyClass _returnvalue "/Script/CableComponent.CableComponent"))
  (Utilities|FlowControl|Delay 0.2)
  (Utilities|IsValid _returnvalue_2
    (:Is%20Valid
      (Variables|Default|SetGrappling%20Cable%20 _returnvalue_2))
    (:Is%20Not%20Valid
      _))
  (bind _array_element (Utilities|Array|ForEachLoopwithBreak (Actor|GetComponentsByClass (Components|GetOwner) "/Script/Engine.ChildActorComponent") :!label _label)
    (:LoopBody
      (if (== (Variables|/Script/Engine.ChildActorComponent|GetChildActor _array_element) "/Game/Movement/Grappling/BP_Blood_Grapple_Blade.BP_Blood_Grapple_Blade")
        (goto _label Break)))
    (:Completed
      (Variables|Default|SetHeld%20Blood%20Grapple%20Child%20Actor _array_element)
      (Variables|Default|SetSwinging%20Continous%20Audio (Utilities|Array|Get(acopy) (Actor|GetComponentsbyTag (Components|GetOwner) "/Script/Engine.AudioComponent" "Swinging Audio"))))))

(fn GrappleCooldownFunc
  (Variables|Checks|SetGrapple%20Cooldown false))

(fn SwingForce
  (Physics|AddForce (Actor|GetComponentbyClass (Components|GetOwner) "/Script/Engine.CharacterMovementComponent") (* (Math|Vector|Normalize (- (Variables|Grapple|GetHit%20Location) (Transformation|GetActorLocation (Components|GetOwner)))) (* (Variables|Swinging|GetSwinging%20Force) (Variables|Swinging|GetSwinging%20Force%20Multiplier)))))

(fn SetupGrappleinHand
  (Development|SetHiddeninGame (Variables|Default|GetHeld%20Blood%20Grapple%20Child%20Actor) false false))

(fn PlaySwingingStretchSound
  (if (Variables|Checks|GetSwinging)
    (Audio|PlaySoundatLocation "/Game/VFX_SFX/Grappling/Swinging_Stretch_SC.Swinging_Stretch_SC" (Transformation|GetActorLocation (Components|GetOwner)) "0, 0, 0" 1.0 1.0 0.0 "/Game/VFX_SFX/Blood_Splatter/Audio/SA_Impact.SA_Impact" 0 0 0)
    (if (Variables|Checks|GetSwinging)
      (bind _returnvalue (Utilities|Time|SetTimerbyFunctionName 0 "Play Swinging Stretch Sound" (Math|Random|RandomFloatinRange 0.5 1.5)))
      (Variables|Swinging|SetSwinging%20Stretch%20Sound%20Timer _returnvalue))))

(fn GrappleSlowTimeStart
  (params (Slow%20Time%20Duration :type Float%20%28double-precision%29))
  (Development|PrintString "GRAPPLE SLOW TIME START")
  (Default|AddSlowTime (Actor|GetComponentbyClass (Components|GetOwner) "/Game/Characters/Player/Slow_Time/BPC_Slow_Time_Manager.BPC_Slow_Time_Manager_C") (Variables|SlowTime|GetGrapple%20Slow%20Time%20Amount) "NewEnumerator0")
  (Utilities|Time|SetTimerbyFunctionName 0 "Grapple Slow Time End" Slow%20Time%20Duration))

(fn GrappleSlowTimeEnd
  (Development|PrintString "GRAPPLE SLOW TIME END")
  (Default|RemoveSlowTime (Actor|GetComponentbyClass (Components|GetOwner) "/Game/Characters/Player/Slow_Time/BPC_Slow_Time_Manager.BPC_Slow_Time_Manager_C") "NewEnumerator0"))

(event Custom|Stop%20Swing
  (bind _returnvalue (Components|GetOwner))
  (bind _returnvalue_2 (Components|GetOwner))
  (bind _grappling_cable_ (Variables|Default|GetGrappling%20Cable%20))
  (bind _current_blood_grapple (Variables|Grapple|GetCurrent%20Blood%20Grapple))
  (bind _returnvalue_3 (Actor|GetComponentbyClass _returnvalue "/Game/Movement/Double_Jump/BPC_Double_Jump.BPC_Double_Jump_C"))
  (bind _returnvalue_4 (Actor|GetComponentbyClass _returnvalue_2 "/Script/Engine.CharacterMovementComponent"))
  (Variables|Checks|SetSwinging false)
  (Utilities|Time|ClearandInvalidateTimerbyHandle (Variables|Grapple|GetGrapple%20Cooldown%20Timer))
  (Variables|Checks|SetGrapple%20Cooldown false)
  (Variables|/Script/Engine.CharacterMovementComponent|SetGravityScale _returnvalue_4 1.75)
  (Variables|/Script/Engine.CharacterMovementComponent|SetAirControl _returnvalue_4 1.0)
  (Utilities|Time|ClearandInvalidateTimerbyHandle (Variables|Swinging|GetUpdating%20Cable%20Length%20Timer))
  (Utilities|Time|ClearandInvalidateTimerbyHandle (Variables|Swinging|GetSwinging%20Validity%20Check%20Timer))
  (Utilities|Time|ClearandInvalidateTimerbyHandle (Variables|Swinging|GetDisable%20Swinging%20From%20Collision%20Timer))
  (Utilities|Time|ClearandInvalidateTimerbyHandle (Variables|Swinging|GetSwinging%20Stretch%20Sound%20Timer))
  (Audio|PlaySoundatLocation "/Game/VFX_SFX/Grappling/Grapple_Pull_SC.Grapple_Pull_SC" (Transformation|GetActorLocation (Components|GetOwner)) "0, 0, 0" 1.0 1.0 0.0 0 0 0 0)
  (Components|Activation|Deactivate (Variables|Default|GetSwinging%20Continous%20Audio))
  (Development|SetHiddeninGame (Variables|Default|GetHeld%20Blood%20Grapple%20Child%20Actor) true false)
  (Rendering|Material|SetMaterial (Variables|/Game/Movement/Grappling/BP_Blood_Grapple_Blade.BP_Blood_Grapple_Blade_C|GetBlood%20Grapple%20SM (Variables|Grapple|GetCurrent%20Blood%20Grapple)) 0 "/Game/Assets/Materials/Grappling/M_Blood_Grapple.M_Blood_Grapple")
  (Utilities|IsValid _grappling_cable_
    (:Is%20Valid
      (Development|SetHiddeninGame _grappling_cable_ true false))
    (:Is%20Not%20Valid
      _))
  (Utilities|IsValid _current_blood_grapple
    (:Is%20Valid
      (Actor|SetLifeSpan _current_blood_grapple 4.0))
    (:Is%20Not%20Valid
      _))
  (Utilities|IsValid _returnvalue_3
    (:Is%20Valid
      (Default|Cooldown _returnvalue_3))
    (:Is%20Not%20Valid
      _))
  (bind _ascharacter (Utilities|Casting|CastToCharacter (Components|GetOwner))
    (:then
      (Character|LaunchCharacter _ascharacter (* (Math|Vector|GetForwardVector (Pawn|GetControlRotation _ascharacter :!class /Script/Engine.Pawn)) (* (Variables|Swinging|GetEnd%20Swing%20Launch%20Force) (- 1.0 (Math|Float|Clamp(Float) (/ (Math|Vector|VectorLength (Transformation|GetVelocity _ascharacter)) (Variables|Swinging|GetMax%20Velocity%20for%20Launch)))))) false false))
    (:CastFailed
      _))
  (if (Utilities|DoesObjectImplementInterface (Components|GetOwner) "/Game/Characters/Player/BPI_Player.BPI_Player_C")
    (Class|LegacyCameraShake|StartLegacyCameraShake (Game|GetPlayerCameraManager 0) "/Game/Movement/BP_Slight_Camera_Shake.BP_Slight_Camera_Shake_C" 4.0 "CameraLocal" "0, 0, 0")
    (Default|PlayGrappleCrosshairAnim (Actor|GetComponentbyClass (Components|GetOwner) "/Game/Characters/Player/BPC_HUD.BPC_HUD_C"))
    (Default|PlayHUDShake (Actor|GetComponentbyClass (Components|GetOwner) "/Game/Characters/Player/BPC_HUD.BPC_HUD_C"))
    (Default|ForciblyResetMovementAbility (Actor|GetComponentbyClass (Components|GetOwner) "/Game/Characters/Player/BPC_HUD.BPC_HUD_C") "NewEnumerator3")
    (Default|RemoveSlowTime (Actor|GetComponentbyClass (Components|GetOwner) "/Game/Characters/Player/Slow_Time/BPC_Slow_Time_Manager.BPC_Slow_Time_Manager_C") "NewEnumerator1")))

(event Custom|Start%20Swing
  (bind _returnvalue (Components|GetOwner))
  (bind _returnvalue_2 (Actor|GetComponentbyClass _returnvalue "/Script/Engine.CharacterMovementComponent"))
  (if (Variables|Checks|GetCan%20Swing)
    (Variables|Checks|SetSwinging true)
    (Utilities|Time|ClearandInvalidateTimerbyHandle (Variables|Grapple|GetGrapple%20Cooldown%20Timer))
    (Variables|/Script/Engine.CharacterMovementComponent|SetGravityScale _returnvalue_2 1.0)
    (Variables|/Script/Engine.CharacterMovementComponent|SetAirControl _returnvalue_2 1.0)
    (Variables|Checks|SetGrapple%20Cooldown false)
    (Components|Activation|Activate (Variables|Default|GetSwinging%20Continous%20Audio) false)
    (CallFunction|PlaySwingingStretchSound)
    (Default|AddSlowTime (Actor|GetComponentbyClass (Components|GetOwner) "/Game/Characters/Player/Slow_Time/BPC_Slow_Time_Manager.BPC_Slow_Time_Manager_C") (Variables|SlowTime|GetSwinging%20Slow%20Time%20Amount) "NewEnumerator1")
    (bind _returnvalue_3 (Utilities|Time|SetTimerbyEvent (delegate Custom|Update%20Length%20of%20Cable) 0.05 true))
    (Variables|Swinging|SetUpdating%20Cable%20Length%20Timer _returnvalue_3)
    (bind _returnvalue_4 (Utilities|Time|SetTimerbyEvent (delegate Custom|Swinging%20Countdown) (* (Variables|Swinging|GetMax%20Swing%20Time) 0.75)))
    (Variables|Swinging|SetSwinging%20Countdown%20Timer _returnvalue_4)
    (if (Variables|Swinging|GetShould%20Do%20Collision%20Check)
      (bind _returnvalue_5 (Utilities|Time|SetTimerbyEvent (delegate Custom|Swinging%20Validity%20Check) 0.1 true))
      (Variables|Swinging|SetSwinging%20Validity%20Check%20Timer _returnvalue_5))))

(event Custom|Update%20Length%20of%20Cable
  (Variables|/Script/CableComponent.CableComponent|SetCableLength (Variables|Default|GetGrappling%20Cable%20) (Math|Vector|Distance(Vector) (Transformation|GetActorLocation (Components|GetOwner)) (Transformation|GetActorLocation (Variables|Grapple|GetCurrent%20Blood%20Grapple)))))

(event Custom|Forcibly%20Stop%20Swinging
  (Variables|Checks|SetCan%20Swing false)
  (if (Variables|Checks|GetSwinging)
    (Utilities|FlowControl|Sequence
      (:then_0
        (Utilities|FlowControl|DoOnce false) ; enters at Reset
      )
      (:then_1
        (CallFunction|StopSwing))
      (:then_2
        (Utilities|Time|ClearandInvalidateTimerbyHandle (Variables|Swinging|GetSwinging%20Countdown%20Timer))))))

(event Custom|Swinging%20Countdown
  (bind _max_swing_time (Variables|Swinging|GetMax%20Swing%20Time))
  (bind _returnvalue (* _max_swing_time 0.03125))
  (if (Variables|Checks|GetSwinging)
    (Development|SetHiddeninGame (Variables|Default|GetGrappling%20Cable%20) true false)
    (Utilities|FlowControl|Delay _returnvalue)
    (if (Variables|Checks|GetSwinging)
      (Development|SetHiddeninGame (Variables|Default|GetGrappling%20Cable%20) false false)
      (Utilities|FlowControl|Delay _returnvalue)
      (if (Variables|Checks|GetSwinging)
        (Development|SetHiddeninGame (Variables|Default|GetGrappling%20Cable%20) true false)
        (Utilities|FlowControl|Delay _returnvalue)
        (if (Variables|Checks|GetSwinging)
          (Development|SetHiddeninGame (Variables|Default|GetGrappling%20Cable%20) false false)
          (Utilities|FlowControl|Delay _returnvalue)
          (if (Variables|Checks|GetSwinging)
            (Development|SetHiddeninGame (Variables|Default|GetGrappling%20Cable%20) true false)
            (Utilities|FlowControl|Delay _returnvalue)
            (if (Variables|Checks|GetSwinging)
              (Development|SetHiddeninGame (Variables|Default|GetGrappling%20Cable%20) false false)
              (Utilities|FlowControl|Delay _returnvalue)
              (if (Variables|Checks|GetSwinging)
                (Development|SetHiddeninGame (Variables|Default|GetGrappling%20Cable%20) true false)
                (Utilities|FlowControl|Delay _returnvalue)
                (if (Variables|Checks|GetSwinging)
                  (Development|SetHiddeninGame (Variables|Default|GetGrappling%20Cable%20) false false)
                  (Utilities|FlowControl|Delay _returnvalue)
                  (if (Variables|Checks|GetSwinging)
                    (CallFunction|ForciblyStopSwinging)))))))))))

(event Custom|Swinging%20Validity%20Check
  (bind _current_blood_grapple (Variables|Grapple|GetCurrent%20Blood%20Grapple))
  (Utilities|IsValid _current_blood_grapple
    (:Is%20Valid
      (bind _returnvalue (Collision|LineTraceForObjects (Transformation|GetSocketLocation (Actor|GetComponentbyClass (Components|GetOwner) "/Script/Engine.SkeletalMeshComponent") "Grappling_Socket_L") (Transformation|GetActorLocation _current_blood_grapple) (Utilities|Array|MakeArray "ObjectTypeQuery1" "ObjectTypeQuery2" "ObjectTypeQuery4" "ObjectTypeQuery9" "ObjectTypeQuery6" "ObjectTypeQuery7") false 0 "ForDuration"))
      (if _returnvalue
        (Utilities|FlowControl|DoOnce false :!label _label
          (:Completed
            (bind _returnvalue_2 (Utilities|Time|SetTimerbyEvent (delegate Custom|Disable%20Swinging%20From%20Collision) 0.25))
            (Variables|Swinging|SetDisable%20Swinging%20From%20Collision%20Timer _returnvalue_2)))
        (else
          (goto _label Reset))))))

(event Custom|Disable%20Swinging%20From%20Collision
  (if (stale Custom|Swinging%20Validity%20Check _returnvalue)
    (Utilities|Time|ClearandInvalidateTimerbyHandle (Variables|Swinging|GetSwinging%20Validity%20Check%20Timer))
    (CallFunction|ForciblyStopSwinging)))

(event Input|EnhancedActionEvents|EnhancedInputActionIA_Swing
  (params (ActionValue :type Boolean) (ElapsedSeconds :type Float%20%28double-precision%29) (TriggeredSeconds :type Float%20%28double-precision%29) (InputAction :type Input%20Action%20Object%20Reference :default "/Game/Characters/Player/Input/Actions/Grappling/IA_Swing.IA_Swing"))
  (:Triggered
    (if (Variables|Checks|GetCan%20Swing)
      (Utilities|FlowControl|DoOnce false :!label _label
        (:Completed
          (CallFunction|StartSwing)))))
  (:Completed
    (Variables|Checks|SetCan%20Swing false)
    (if (Variables|Checks|GetSwinging)
      (Utilities|FlowControl|Sequence
        (:then_0
          (goto _label Reset))
        (:then_1
          (CallFunction|StopSwing))
        (:then_2
          (Utilities|Time|ClearandInvalidateTimerbyHandle (Variables|Swinging|GetSwinging%20Countdown%20Timer)))))))

(event Custom|Grapple
  (bind _returnvalue (Components|GetOwner))
  (bind _returnvalue_2 (Components|GetOwner))
  (bind _returnvalue_3 (Game|GetPlayerCameraManager 0))
  (bind _returnvalue_4 (Components|GetOwner))
  (bind _grappling_cable_ (Variables|Default|GetGrappling%20Cable%20))
  (bind _returnvalue_5 (Utilities|DoesObjectImplementInterface _returnvalue_2 "/Game/Characters/Player/BPI_Player.BPI_Player_C"))
  (bind _returnvalue_6 (Camera|GetCameraLocation _returnvalue_3))
  (Variables|Checks|SetGrappled false)
  (Development|PrintString "Grapple")
  (Variables|Checks|SetGrapple%20Cooldown true)
  (bind _returnvalue_7 (Utilities|Time|SetTimerbyFunctionName 0 "Grapple Cooldown Func" (Variables|Grapple|GetGrapple%20Cooldown%20Duration)))
  (Variables|Grapple|SetGrapple%20Cooldown%20Timer _returnvalue_7)
  (bind (_outhit _returnvalue_8) (Class|KismetSystemLibrary|BoxTraceSingleforObjects _returnvalue_6 (+ _returnvalue_6 (* (Math|Vector|GetForwardVector (Pawn|GetControlRotation (Game|GetPlayerController 0) :!class /Script/Engine.Controller)) 2.5e+03)) "0.000000,25.000000,25.000000" (Pawn|GetControlRotation (Game|GetPlayerController 0) :!class /Script/Engine.Controller) (Utilities|Array|MakeArray "ObjectTypeQuery10" "ObjectTypeQuery9" "ObjectTypeQuery12" "ObjectTypeQuery14" "ObjectTypeQuery1" "ObjectTypeQuery2" "ObjectTypeQuery4" "ObjectTypeQuery7") false (Utilities|Array|MakeArray _returnvalue (Variables|/Game/Weapons/Actor_Components/BPC_Weaponry.BPC_Weaponry_C|GetEquipped_Weapon (Actor|GetComponentbyClass _returnvalue "/Game/Weapons/Actor_Components/BPC_Weaponry.BPC_Weaponry_C"))) "None" true))
  (if _returnvalue_8
    (Variables|Checks|SetGrapple%20Pull? true)
    (bind _output_get (Variables|Grapple|SetGrappled%20Actor (.HitActor (Collision|BreakHitResult _outhit))))
    (Variables|Grapple|SetGrappled%20Component (.HitComponent (Collision|BreakHitResult _outhit)))
    (Variables|Grapple|SetHit%20Location (.Location (Collision|BreakHitResult _outhit)))
    (CallFunction|SetupGrappleinHand)
    (if _returnvalue_5
      (Class|LegacyCameraShake|StartLegacyCameraShake (Game|GetPlayerCameraManager 0) "/Game/Movement/BP_Slight_Camera_Shake.BP_Slight_Camera_Shake_C" 4.0 "CameraLocal" "0, 0, 0"))
    (Utilities|IsValid (Actor|GetComponentbyClass _output_get "/Script/Engine.SkeletalMeshComponent")
      (:Is%20Valid
        (bind _returnvalue_9 (Game|SpawnActorfromClass "/Game/Movement/Grappling/BP_Blood_Grapple_Blade.BP_Blood_Grapple_Blade_C" (Math|Transform|MakeTransform (.BoneLocation (Class|SkinnedMeshComponent|FindClosestBoneK2 (Actor|GetComponentbyClass _output_get "/Script/Engine.SkeletalMeshComponent") (.ImpactPoint (Collision|BreakHitResult _outhit)) 1.0)) (Math|Rotator|FindLookatRotation (.Location (Collision|BreakHitResult _outhit)) (Transformation|GetActorLocation (Components|GetOwner))) "1.000000,1.000000,1.000000") "Undefined" "MultiplyWithRoot" _returnvalue_4 0))
        (Variables|Grapple|SetCurrent%20Blood%20Grapple _returnvalue_9)
        (Transformation|AttachComponentToComponent (Variables|Grapple|GetCurrent%20Blood%20Grapple) (Actor|GetComponentbyClass _output_get "/Script/Engine.SkeletalMeshComponent") (.ReturnValue (Class|SkinnedMeshComponent|FindClosestBoneK2 (Actor|GetComponentbyClass _output_get "/Script/Engine.SkeletalMeshComponent") (.ImpactPoint (Collision|BreakHitResult _outhit)) 1.0)) "KeepWorld" "KeepWorld" "KeepWorld" true))
      (:Is%20Not%20Valid
        (bind _returnvalue_10 (Game|SpawnActorfromClass "/Game/Movement/Grappling/BP_Blood_Grapple_Blade.BP_Blood_Grapple_Blade_C" (Math|Transform|MakeTransform (.Location (Collision|BreakHitResult _outhit)) (Math|Rotator|FindLookatRotation (.Location (Collision|BreakHitResult _outhit)) (Transformation|GetActorLocation (Components|GetOwner))) "1.000000,1.000000,1.000000") "Undefined" "MultiplyWithRoot" _returnvalue_4 0))
        (Variables|Grapple|SetCurrent%20Blood%20Grapple _returnvalue_10)
        (Transformation|AttachActorToActor (Variables|Grapple|GetCurrent%20Blood%20Grapple) (Variables|Grapple|GetGrappled%20Actor) "None" "KeepWorld" "KeepWorld" "KeepWorld" true)))
    (Development|SetHiddeninGame _grappling_cable_ false false)
    (Class|CableComponent|SetAttachEndtoComponent _grappling_cable_ (Variables|/Script/Engine.Actor|GetRootComponent (Variables|Grapple|GetCurrent%20Blood%20Grapple)) "None")
    (Variables|/Script/CableComponent.CableComponent|SetCableLength _grappling_cable_ (Math|Vector|Distance(Vector) (Transformation|GetActorLocation (Components|GetOwner)) (Transformation|GetActorLocation (Variables|Grapple|GetCurrent%20Blood%20Grapple))))
    (Rendering|Material|SetMaterial (Variables|/Game/Movement/Grappling/BP_Blood_Grapple_Blade.BP_Blood_Grapple_Blade_C|GetBlood%20Grapple%20SM (Variables|Grapple|GetCurrent%20Blood%20Grapple)) 0 "/Game/Assets/Materials/Grappling/M_Blood_Grapple_Active.M_Blood_Grapple_Active")
    (Audio|PlaySoundatLocation "/Game/VFX_SFX/Grappling/Grapple_SC.Grapple_SC" (Transformation|GetActorLocation (Variables|Grapple|GetCurrent%20Blood%20Grapple)) "0, 0, 0" 1.0 1.0 0.0 0 0 0 0)
    (Audio|PlaySoundatLocation "/Game/VFX_SFX/Grappling/Grapple_SC.Grapple_SC" (Transformation|GetActorLocation (Components|GetOwner)) "0, 0, 0" 1.0 1.0 0.0 0 0 0 0)
    (if (Utilities|DoesObjectImplementInterface (Components|GetOwner) "/Game/Characters/Player/BPI_Player.BPI_Player_C")
      (Default|PlayGrappleCrosshairAnim (Actor|GetComponentbyClass (Components|GetOwner) "/Game/Characters/Player/BPC_HUD.BPC_HUD_C"))
      (Default|PlayHUDShake (Actor|GetComponentbyClass (Components|GetOwner) "/Game/Characters/Player/BPC_HUD.BPC_HUD_C"))
      (Default|UseMovementAbility (Actor|GetComponentbyClass (Components|GetOwner) "/Game/Characters/Player/BPC_HUD.BPC_HUD_C") "NewEnumerator3"))
    (else
      (Variables|Checks|SetCan%20Swing false)
      (Variables|Checks|SetGrappled false)
      (Audio|PlaySoundatLocation "/Game/VFX_SFX/Grappling/Grapple_Miss_Sc.Grapple_Miss_Sc" (Transformation|GetActorLocation (Components|GetOwner)) "0, 0, 0" 1.0 1.0 0.0 0 0 0 0)
      (if _returnvalue_5
        (Default|UseMovementAbility (Actor|GetComponentbyClass (Components|GetOwner) "/Game/Characters/Player/BPC_HUD.BPC_HUD_C") "NewEnumerator3")))))

(event Input|EnhancedActionEvents|EnhancedInputActionIA_Grapple
  (params (ActionValue :type Boolean) (ElapsedSeconds :type Float%20%28double-precision%29) (TriggeredSeconds :type Float%20%28double-precision%29) (InputAction :type Input%20Action%20Object%20Reference :default "/Game/Characters/Player/Input/Actions/Grappling/IA_Grapple.IA_Grapple"))
  (:Triggered
    (if (Variables|Checks|GetCan%20Grapple)
      (Variables|Checks|SetGrappled true))))

(event Custom|Grapple%20Pull
  (Utilities|IsValid (Variables|Grapple|GetGrappled%20Actor)
    (:Is%20Valid
      (switch Utilities|FlowControl|Switch|SwitchonECollisionChannel (|Inputs)
        (:ECC_WorldStatic
          (Variables|Checks|SetCan%20Swing true :!label _label)
          (Utilities|FlowControl|Delay 0.15)
          (if (Variables|Checks|GetSwinging)
            (Variables|Checks|SetGrapple%20Pull? false)
            (else
              (CallFunction|GrappletoStationary))))
        (:ECC_WorldDynamic
          (goto _label))
        (:ECC_PhysicsBody
          (CallFunction|GrapplePullSmall :!label _label_2)
          (Variables|Checks|SetCan%20Swing false))
        (:ECC_GameTraceChannel1
          (goto _label))
        (:ECC_GameTraceChannel3
          (goto _label_2))
        (:ECC_GameTraceChannel4
          ;[1 1 1] Determine if enemy is big or small
          (if false
            (CallFunction|GrappletoMoving)
            (Variables|Checks|SetCan%20Swing false)
            (else
              (CallFunction|GrapplePullSmall)
              (Variables|Checks|SetCan%20Swing false))))
        (:ECC_GameTraceChannel6
          (CallFunction|GrappletoMoving)
          (Variables|Checks|SetCan%20Swing false))
        (:ECC_GameTraceChannel8
          (CallFunction|GrappletoStationary)
          (Variables|Checks|SetCan%20Swing false))))))

(event Custom|Grapple%20To%20Stationary
  (bind _returnvalue (Components|GetOwner))
  (bind _grapple_to_force (Variables|Grapple|GetGrapple%20To%20Force))
  (bind _returnvalue_2 (Actor|GetComponentbyClass _returnvalue "/Game/Movement/Double_Jump/BPC_Double_Jump.BPC_Double_Jump_C"))
  ;[1 1 1] Pull player towards grapple hook
  (Utilities|FlowControl|Delay (Variables|Grapple|GetPull%20Delay))
  (Development|PrintString "Grapple Hook")
  (bind _ascharacter (Utilities|Casting|CastToCharacter (Components|GetOwner)))
  (Character|LaunchCharacter _ascharacter (+ (* (Math|Vector|GetForwardVector (Math|Rotator|FindLookatRotation (Transformation|GetActorLocation (Components|GetOwner)) (Variables|Grapple|GetHit%20Location))) _grapple_to_force) (* (Transformation|GetActorUpVector (Components|GetOwner)) (/ _grapple_to_force 2.0))) true true)
  (Variables|Checks|SetGrapple%20Pull? false)
  (Variables|Checks|SetCan%20Swing false)
  (Audio|PlaySoundatLocation "/Game/VFX_SFX/Grappling/Grapple_Pull_SC.Grapple_Pull_SC" (Transformation|GetActorLocation (Variables|Grapple|GetCurrent%20Blood%20Grapple)) "0, 0, 0" 1.0 1.0 0.0 0 0 0 0)
  (Audio|PlaySoundatLocation "/Game/VFX_SFX/Grappling/Grapple_Pull_SC.Grapple_Pull_SC" (Transformation|GetActorLocation (Components|GetOwner)) "0, 0, 0" 1.0 1.0 0.0 0 0 0 0)
  (Actor|SetLifeSpan (Variables|Grapple|GetCurrent%20Blood%20Grapple) (Math|Float|SelectFloat 1.0 4.0 (Utilities|DoesObjectImplementInterface (Variables|Grapple|GetGrappled%20Actor) "/Game/Weapons/Interfaces/BPI_Weapon.BPI_Weapon_C")))
  (Utilities|FlowControl|Delay 0.05)
  (if (Utilities|DoesObjectImplementInterface (Components|GetOwner) "/Game/Characters/Player/BPI_Player.BPI_Player_C")
    (Class|LegacyCameraShake|StartLegacyCameraShake (Game|GetPlayerCameraManager 0) "/Game/Movement/BP_Slight_Camera_Shake.BP_Slight_Camera_Shake_C" 4.0 "CameraLocal" "0, 0, 0")
    (CallFunction|GrappleSlowTimeStart (Variables|SlowTime|GetGrapple%20Slow%20Time%20Duration))
    (Default|PlayHUDShake (Actor|GetComponentbyClass (Components|GetOwner) "/Game/Characters/Player/BPC_HUD.BPC_HUD_C"))
    (Default|PlayGrappleCrosshairAnim (Actor|GetComponentbyClass (Components|GetOwner) "/Game/Characters/Player/BPC_HUD.BPC_HUD_C")))
  (Utilities|IsValid _returnvalue_2
    (:Is%20Valid
      (Default|Cooldown _returnvalue_2))
    (:Is%20Not%20Valid
      _))
  (Development|SetHiddeninGame (Variables|Default|GetGrappling%20Cable%20) true false)
  (Development|SetHiddeninGame (Variables|Default|GetHeld%20Blood%20Grapple%20Child%20Actor) true false)
  (Rendering|Material|SetMaterial (Variables|/Game/Movement/Grappling/BP_Blood_Grapple_Blade.BP_Blood_Grapple_Blade_C|GetBlood%20Grapple%20SM (Variables|Grapple|GetCurrent%20Blood%20Grapple)) 0 "/Game/Assets/Materials/Grappling/M_Blood_Grapple.M_Blood_Grapple"))

(event Custom|Grapple%20Pull%20Small
  (bind _returnvalue (Components|GetOwner))
  (bind _returnvalue_2 (Components|GetOwner))
  (bind _grappled_actor (Variables|Grapple|GetGrappled%20Actor))
  (bind _returnvalue_3 (Actor|GetComponentbyClass _returnvalue "/Game/Movement/Double_Jump/BPC_Double_Jump.BPC_Double_Jump_C"))
  (bind _returnvalue_4 (Transformation|GetActorLocation _returnvalue_2))
  (bind _returnvalue_5 (Transformation|GetActorLocation _grappled_actor))
  (bind _returnvalue_6 (Math|Rotator|FindLookatRotation _returnvalue_5 _returnvalue_4))
  (bind _returnvalue_7 (Math|Vector|GetForwardVector _returnvalue_6))
  ;[1 1 1] Pull hit actor towards player and up a bit
  (Utilities|FlowControl|Delay (Variables|Grapple|GetPull%20Delay))
  (Development|PrintString "Grapple Pull Small")
  (bind _ascharacter (Utilities|Casting|CastToCharacter (Variables|Grapple|GetGrappled%20Actor))
    (:then
      (Character|LaunchCharacter _ascharacter (Math|Vector|SelectVector (* _returnvalue_7 (Variables|Grapple|GetGrapple%20Pull%20Force)) (+ (* (Transformation|GetActorUpVector (Variables|Grapple|GetGrappled%20Actor)) (Variables|Grapple|GetGrapple%20Pull%20Force)) (* _returnvalue_7 (/ (Variables|Grapple|GetGrapple%20Pull%20Force) 2.0))) (AI|Components|NavMovement|IsFalling (Variables|/Script/Engine.Character|GetCharacterMovement _ascharacter))) true true))
    (:CastFailed
      (Physics|AddImpulse (Variables|Grapple|GetGrappled%20Component) (+ (* (Math|Vector|GetUpVector (Variables|Grapple|GetGrappled%20Component)) (Variables|Grapple|GetGrapple%20To%20Force)) (* (Math|Vector|GetForwardVector (Math|Rotator|FindLookatRotation (Transformation|GetWorldLocation (Variables|Grapple|GetGrappled%20Component)) (Transformation|GetActorLocation (Components|GetOwner)))) (Variables|Grapple|GetGrapple%20To%20Force))) "None" false)))
  (Variables|Checks|SetGrapple%20Pull? false)
  (Variables|Checks|SetCan%20Swing false)
  (Audio|PlaySoundatLocation "/Game/VFX_SFX/Grappling/Grapple_Pull_SC.Grapple_Pull_SC" (Transformation|GetActorLocation (Variables|Grapple|GetCurrent%20Blood%20Grapple)) "0, 0, 0" 1.0 1.0 0.0 0 0 0 0)
  (Audio|PlaySoundatLocation "/Game/VFX_SFX/Grappling/Grapple_Pull_SC.Grapple_Pull_SC" (Transformation|GetActorLocation (Components|GetOwner)) "0, 0, 0" 1.0 1.0 0.0 0 0 0 0)
  (Actor|SetLifeSpan (Variables|Grapple|GetCurrent%20Blood%20Grapple) (Math|Float|SelectFloat 1.0 4.0 (Utilities|DoesObjectImplementInterface (Variables|Grapple|GetGrappled%20Actor) "/Game/Weapons/Interfaces/BPI_Weapon.BPI_Weapon_C")))
  (Utilities|FlowControl|Delay 0.05)
  (if (Utilities|DoesObjectImplementInterface (Components|GetOwner) "/Game/Characters/Player/BPI_Player.BPI_Player_C")
    (Class|LegacyCameraShake|StartLegacyCameraShake (Game|GetPlayerCameraManager 0) "/Game/Movement/BP_Slight_Camera_Shake.BP_Slight_Camera_Shake_C" 4.0 "CameraLocal" "0, 0, 0")
    (CallFunction|GrappleSlowTimeStart (Variables|SlowTime|GetGrapple%20Slow%20Time%20Duration))
    (Default|PlayHUDShake (Actor|GetComponentbyClass (Components|GetOwner) "/Game/Characters/Player/BPC_HUD.BPC_HUD_C"))
    (Default|PlayGrappleCrosshairAnim (Actor|GetComponentbyClass (Components|GetOwner) "/Game/Characters/Player/BPC_HUD.BPC_HUD_C")))
  (Utilities|IsValid _returnvalue_3
    (:Is%20Valid
      (Default|Cooldown _returnvalue_3))
    (:Is%20Not%20Valid
      _))
  (Development|SetHiddeninGame (Variables|Default|GetGrappling%20Cable%20) true false)
  (Development|SetHiddeninGame (Variables|Default|GetHeld%20Blood%20Grapple%20Child%20Actor) true false)
  (Rendering|Material|SetMaterial (Variables|/Game/Movement/Grappling/BP_Blood_Grapple_Blade.BP_Blood_Grapple_Blade_C|GetBlood%20Grapple%20SM (Variables|Grapple|GetCurrent%20Blood%20Grapple)) 0 "/Game/Assets/Materials/Grappling/M_Blood_Grapple.M_Blood_Grapple"))

(event Custom|Grapple%20To%20Moving
  (bind _returnvalue (Components|GetOwner))
  (bind _grapple_to_force (Variables|Grapple|GetGrapple%20To%20Force))
  (bind _returnvalue_2 (Actor|GetComponentbyClass _returnvalue "/Game/Movement/Double_Jump/BPC_Double_Jump.BPC_Double_Jump_C"))
  ;[1 1 1] Pull player towards hit actor
  (Utilities|FlowControl|Delay (Variables|Grapple|GetPull%20Delay))
  (Development|PrintString "Grapple Pull Big")
  (bind _ascharacter (Utilities|Casting|CastToCharacter (Components|GetOwner)))
  (Character|LaunchCharacter _ascharacter (+ (* (Math|Vector|GetForwardVector (Math|Rotator|FindLookatRotation (Transformation|GetActorLocation (Components|GetOwner)) (Variables|Grapple|GetHit%20Location))) _grapple_to_force) (* (Transformation|GetActorUpVector (Components|GetOwner)) (/ _grapple_to_force 2.0))) true true)
  (Variables|Checks|SetGrapple%20Pull? false)
  (Variables|Checks|SetCan%20Swing false)
  (Audio|PlaySoundatLocation "/Game/VFX_SFX/Grappling/Grapple_Pull_SC.Grapple_Pull_SC" (Transformation|GetActorLocation (Variables|Grapple|GetCurrent%20Blood%20Grapple)) "0, 0, 0" 1.0 1.0 0.0 0 0 0 0)
  (Audio|PlaySoundatLocation "/Game/VFX_SFX/Grappling/Grapple_Pull_SC.Grapple_Pull_SC" (Transformation|GetActorLocation (Components|GetOwner)) "0, 0, 0" 1.0 1.0 0.0 0 0 0 0)
  (Actor|SetLifeSpan (Variables|Grapple|GetCurrent%20Blood%20Grapple) (Math|Float|SelectFloat 1.0 4.0 (Utilities|DoesObjectImplementInterface (Variables|Grapple|GetGrappled%20Actor) "/Game/Weapons/Interfaces/BPI_Weapon.BPI_Weapon_C")))
  (Utilities|FlowControl|Delay 0.05)
  (if (Utilities|DoesObjectImplementInterface (Components|GetOwner) "/Game/Characters/Player/BPI_Player.BPI_Player_C")
    (Class|LegacyCameraShake|StartLegacyCameraShake (Game|GetPlayerCameraManager 0) "/Game/Movement/BP_Slight_Camera_Shake.BP_Slight_Camera_Shake_C" 4.0 "CameraLocal" "0, 0, 0")
    (CallFunction|GrappleSlowTimeStart (Variables|SlowTime|GetGrapple%20Slow%20Time%20Duration))
    (Default|PlayHUDShake (Actor|GetComponentbyClass (Components|GetOwner) "/Game/Characters/Player/BPC_HUD.BPC_HUD_C"))
    (Default|PlayGrappleCrosshairAnim (Actor|GetComponentbyClass (Components|GetOwner) "/Game/Characters/Player/BPC_HUD.BPC_HUD_C")))
  (Utilities|IsValid _returnvalue_2
    (:Is%20Valid
      (Default|Cooldown _returnvalue_2))
    (:Is%20Not%20Valid
      _))
  (Development|SetHiddeninGame (Variables|Default|GetGrappling%20Cable%20) true false)
  (Development|SetHiddeninGame (Variables|Default|GetHeld%20Blood%20Grapple%20Child%20Actor) true false)
  (Rendering|Material|SetMaterial (Variables|/Game/Movement/Grappling/BP_Blood_Grapple_Blade.BP_Blood_Grapple_Blade_C|GetBlood%20Grapple%20SM (Variables|Grapple|GetCurrent%20Blood%20Grapple)) 0 "/Game/Assets/Materials/Grappling/M_Blood_Grapple.M_Blood_Grapple"))