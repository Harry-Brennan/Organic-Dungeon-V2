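; BP_Blood_Grapple_Blade is the blood grapple blade actor used by the grappling movement, and it handles fading the blade out of view.
; BeginPlay creates a dynamic instance of the blood grapple material for the not-in-use look.
; FadeGrapple applies that instance to the mesh and runs a timeline, rate-scaled to the requested duration, that lerps opacity to zero before hiding the actor.
; StopFade halts the timeline.
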(event Custom|Fade%20Grapple
  (params (Time%20To%20Fade :type Float%20%28double-precision%29))
  (Rendering|Material|SetMaterial (Variables|Default|GetBlood%20Grapple%20SM) 0 (Variables|Default|GetGrapple%20Not%20In%20Use%20Material))
  (Components|Timeline|SetPlayRate (Variables|Default|GetLerp%20Opacity%20of%20Grapple) (/ 1.0 Time%20To%20Fade))
  (bind _lerp_grapple (Timeline|Lerp%20Opacity%20of%20Grapple PlayFromStart)
    (:Update
      (Rendering|Material|SetScalarParameterValue (Variables|Default|GetGrapple%20Not%20In%20Use%20Material) "Opacity" (Math|Float|Lerp 1.0 0.0 _lerp_grapple) :!class /Script/Engine.MaterialInstanceDynamic))
    (:Finished
      (Rendering|SetActorHiddenInGame true))))

(event Custom|Stop%20Fade
  (bind _lerp_grapple (Timeline|Lerp%20Opacity%20of%20Grapple Stop)
    (:Update
      (Rendering|Material|SetScalarParameterValue (Variables|Default|GetGrapple%20Not%20In%20Use%20Material) "Opacity" (Math|Float|Lerp 1.0 0.0 _lerp_grapple) :!class /Script/Engine.MaterialInstanceDynamic))
    (:Finished
      (Rendering|SetActorHiddenInGame true))))

(event EventBeginPlay
  (bind _returnvalue (Rendering|Material|CreateDynamicMaterialInstance (Variables|Default|GetBlood%20Grapple%20SM) 0 "/Game/Assets/Materials/Grappling/M_Blood_Grapple.M_Blood_Grapple" "None" :!class /Script/Engine.PrimitiveComponent))
  (Variables|Default|SetGrapple%20Not%20In%20Use%20Material _returnvalue))

(fn ConstructionScript)