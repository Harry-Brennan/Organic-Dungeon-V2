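; Weapon ammo component that tracks rounds, handles reloading and updates the equipped slot on the HUD when a player holds the weapon.
; Reload toggles a tick-driven timer, using timing and type from the weapon's ranged info.
; By Ammo reloads add rounds at progress thresholds through a modulo window and DoOnce, while Full reloads empty the count and refill on completion.
; Reload steps play a sound and report a noise event.
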(event Custom|Decrease_Ammo
  (bind _returnvalue (Components|GetOwner))
  (bind _current_ammo (Variables|Default|GetCurrent_Ammo))
  (bind _max_ammo (Variables|Default|GetMax_Ammo))
  (bind _current_ammo_2 (Variables|Default|GetCurrent_Ammo))
  (bind _returnvalue_2 (Math|Conversions|ToFloat(Integer) _max_ammo))
  (bind _returnvalue_3 (Math|Conversions|ToFloat(Integer) _current_ammo))
  (bind _returnvalue_4 (Components|GetOwner _returnvalue))
  (bind _returnvalue_5 (Actor|GetComponentbyClass _returnvalue_4 "/Game/Characters/Player/BPC_HUD.BPC_HUD_C"))
  (bind _returnvalue_6 (/ _returnvalue_3 _returnvalue_2))
  (bind _hud_ref (Variables|/Game/Characters/Player/BPC_HUD.BPC_HUD_C|GetHUD_Ref _returnvalue_5))
  (bind _weapon_1 (Variables|/Game/UI/WBP_HUD.WBP_HUD_C|GetWeapon_1 _hud_ref))
  (bind _weapon_2 (Variables|/Game/UI/WBP_HUD.WBP_HUD_C|GetWeapon_2 _hud_ref))
  (bind _weapon_3 (Variables|/Game/UI/WBP_HUD.WBP_HUD_C|GetWeapon_3 _hud_ref))
  (if (not (<= (Variables|Default|GetCurrent_Ammo) 0))
    (Math|Integer|DecrementInt (Variables|Default|GetCurrent_Ammo)
      (:%20%20
        (Variables|Default|SetReload_Percent 0.0)
        (Variables|Default|SetReloading_Seconds 0.0)
        (if (Utilities|DoesObjectImplementInterface (Components|GetOwner (Components|GetOwner)) "/Game/Characters/Player/BPI_Player.BPI_Player_C")
          (bind _basics (Class|BPIWeapon|GetBasicInfo(Message) (Components|GetOwner)))
          (switch int (Variables|/Game/UI/WBP_HUD.WBP_HUD_C|GetCurrently_Equipped_Weapon_Image_Relation _hud_ref)
            (:0
              (Default|UpdateImgColourforAmmo _weapon_1 _returnvalue_6)
              (Default|UpdateAmmoCount _weapon_1 _current_ammo_2 (.ranged _basics)))
            (:1
              (Default|UpdateImgColourforAmmo _weapon_2 _returnvalue_6)
              (Default|UpdateAmmoCount _weapon_2 _current_ammo_2 (.ranged _basics)))
            (:2
              (Default|UpdateImgColourforAmmo _weapon_3 _returnvalue_6)
              (Default|UpdateAmmoCount _weapon_3 _current_ammo_2 (.ranged _basics))))
          (Default|PlayAmmoAnimation (Variables|/Game/Characters/Player/BPC_HUD.BPC_HUD_C|GetHUD_Ref (Actor|GetComponentbyClass (Components|GetOwner (Components|GetOwner)) "/Game/Characters/Player/BPC_HUD.BPC_HUD_C")) true))))))

(event Custom|Reload
  (bind _returnvalue (Components|GetOwner))
  (bind _returnvalue_2 (Components|GetOwner _returnvalue))
  (bind _returnvalue_3 (Actor|GetComponentbyClass _returnvalue_2 "/Game/Characters/Player/BPC_HUD.BPC_HUD_C"))
  (bind _hud_ref (Variables|/Game/Characters/Player/BPC_HUD.BPC_HUD_C|GetHUD_Ref _returnvalue_3))
  (bind _weapon_1 (Variables|/Game/UI/WBP_HUD.WBP_HUD_C|GetWeapon_1 _hud_ref))
  (bind _weapon_2 (Variables|/Game/UI/WBP_HUD.WBP_HUD_C|GetWeapon_2 _hud_ref))
  (bind _weapon_3 (Variables|/Game/UI/WBP_HUD.WBP_HUD_C|GetWeapon_3 _hud_ref))
  (if (< (Variables|Default|GetCurrent_Ammo) (Variables|Default|GetMax_Ammo))
    (if (Variables|Default|GetReloading)
      (CallFunction|StopReload)
      (bind _ranged_info (Class|BPIRangedWeapon|GetRangedInfo(Message) (Components|GetOwner)))
      (switch Utilities|FlowControl|Switch|SwitchonEnum_Reload_Types (.Reload_Type (Utilities|Struct|BreakStruct_Reload_Info (.reload_info _ranged_info)))
        (:NewEnumerator0
          _)
        (:NewEnumerator1
          (Variables|Default|SetCurrent_Ammo 0)))
      (else
        (bind _ranged_info_2 (Class|BPIRangedWeapon|GetRangedInfo(Message) (Components|GetOwner)))
        (switch Utilities|FlowControl|Switch|SwitchonEnum_Reload_Types (.Reload_Type (Utilities|Struct|BreakStruct_Reload_Info (.reload_info _ranged_info_2)))
          (:NewEnumerator0
            _)
          (:NewEnumerator1
            (Variables|Default|SetCurrent_Ammo 0)))
        (CallFunction|StartReload)))
    (if (Utilities|DoesObjectImplementInterface (Components|GetOwner (Components|GetOwner)) "/Game/Characters/Player/BPI_Player.BPI_Player_C")
      (bind _basics (Class|BPIWeapon|GetBasicInfo(Message) (Components|GetOwner)))
      (switch int (Variables|/Game/UI/WBP_HUD.WBP_HUD_C|GetCurrently_Equipped_Weapon_Image_Relation _hud_ref)
        (:0
          (Default|UpdateImgColourforAmmo _weapon_1 (/ (Math|Conversions|ToFloat(Integer) (Variables|Default|GetCurrent_Ammo)) (Math|Conversions|ToFloat(Integer) (Variables|Default|GetMax_Ammo))))
          (Default|UpdateAmmoCount _weapon_1 (Variables|Default|GetCurrent_Ammo) (.ranged _basics)))
        (:1
          (Default|UpdateImgColourforAmmo _weapon_2 (/ (Math|Conversions|ToFloat(Integer) (Variables|Default|GetCurrent_Ammo)) (Math|Conversions|ToFloat(Integer) (Variables|Default|GetMax_Ammo))))
          (Default|UpdateAmmoCount _weapon_2 (Variables|Default|GetCurrent_Ammo) (.ranged _basics)))
        (:2
          (Default|UpdateImgColourforAmmo _weapon_3 (/ (Math|Conversions|ToFloat(Integer) (Variables|Default|GetCurrent_Ammo)) (Math|Conversions|ToFloat(Integer) (Variables|Default|GetMax_Ammo))))
          (Default|UpdateAmmoCount _weapon_3 (Variables|Default|GetCurrent_Ammo) (.ranged _basics))))
      (Default|PlayAmmoAnimation (Variables|/Game/Characters/Player/BPC_HUD.BPC_HUD_C|GetHUD_Ref (Actor|GetComponentbyClass (Components|GetOwner (Components|GetOwner)) "/Game/Characters/Player/BPC_HUD.BPC_HUD_C")) true))))

(event Custom|Start_Reload
  (Variables|Default|SetStarting_Ammo_For_Reload (Variables|Default|GetCurrent_Ammo))
  (Variables|Default|SetReloading_Seconds 0.0)
  (Variables|Default|SetReload_Percent 0.0)
  (bind _ranged_info (Class|BPIRangedWeapon|GetRangedInfo(Message) (Components|GetOwner)))
  (Variables|Default|SetReload_Time (.Reload_Time (Utilities|Struct|BreakStruct_Reload_Info (.reload_info _ranged_info))))
  ;[1 1 1] What reload percent needs to be to increase current ammo by 1
  (Variables|Default|SetReload_Threshold (/ 1.0 (Math|Conversions|ToFloat(Integer) (Variables|Default|GetMax_Ammo))))
  (Variables|Default|SetReload_Percent (/ (Math|Conversions|ToFloat(Integer) (Variables|Default|GetCurrent_Ammo)) (Math|Conversions|ToFloat(Integer) (Variables|Default|GetMax_Ammo))))
  (Variables|Default|SetReloading true)
  (Components|Tick|SetComponentTickEnabled true))

(event Custom|Stop_Reload
  (Components|Tick|SetComponentTickEnabled false)
  (Variables|Default|SetReloading false)
  (Variables|Default|SetReloading_Seconds 0.0)
  (Variables|Default|SetReload_Percent 0.0))

(event Custom|Update_Max_Ammo
  (params (New%20Max%20Ammo :type Integer))
  (bind _output_get (Variables|Default|SetMax_Ammo New%20Max%20Ammo))
  (Variables|Default|SetCurrent_Ammo _output_get)
  (CallFunction|Reload))

(event EventTick
  (params (DeltaSeconds :type Float%20%28single-precision%29))
  (bind _returnvalue (Components|GetOwner))
  (bind _returnvalue_2 (Components|GetOwner))
  (bind _returnvalue_3 (Components|GetOwner))
  (bind _returnvalue_4 (Components|GetOwner))
  (bind _returnvalue_5 (Components|GetOwner))
  (bind _returnvalue_6 (Transformation|GetActorLocation _returnvalue_5))
  (bind _returnvalue_7 (Components|GetOwner _returnvalue))
  (bind _returnvalue_8 (Components|GetOwner _returnvalue_2))
  (bind _returnvalue_9 (Transformation|GetActorLocation _returnvalue_3))
  (bind _returnvalue_10 (Components|GetOwner _returnvalue_4))
  (bind _returnvalue_11 (Utilities|DoesObjectImplementInterface _returnvalue_10 "/Game/Characters/Player/BPI_Player.BPI_Player_C"))
  (bind _returnvalue_12 (Actor|GetComponentbyClass _returnvalue_7 "/Game/Characters/Player/BPC_HUD.BPC_HUD_C"))
  (bind _returnvalue_13 (Actor|GetComponentbyClass _returnvalue_8 "/Game/Characters/Player/BPC_HUD.BPC_HUD_C"))
  (bind _hud_ref (Variables|/Game/Characters/Player/BPC_HUD.BPC_HUD_C|GetHUD_Ref _returnvalue_12))
  (bind _hud_ref_2 (Variables|/Game/Characters/Player/BPC_HUD.BPC_HUD_C|GetHUD_Ref _returnvalue_13))
  (bind _weapon_1 (Variables|/Game/UI/WBP_HUD.WBP_HUD_C|GetWeapon_1 _hud_ref))
  (bind _weapon_2 (Variables|/Game/UI/WBP_HUD.WBP_HUD_C|GetWeapon_2 _hud_ref))
  (bind _weapon_3 (Variables|/Game/UI/WBP_HUD.WBP_HUD_C|GetWeapon_3 _hud_ref))
  (bind _weapon_1_2 (Variables|/Game/UI/WBP_HUD.WBP_HUD_C|GetWeapon_1 _hud_ref_2))
  (bind _weapon_2_2 (Variables|/Game/UI/WBP_HUD.WBP_HUD_C|GetWeapon_2 _hud_ref_2))
  (bind _weapon_3_2 (Variables|/Game/UI/WBP_HUD.WBP_HUD_C|GetWeapon_3 _hud_ref_2))
  (Variables|Default|SetReloading_Seconds (+ DeltaSeconds (Variables|Default|GetReloading_Seconds)))
  (Development|PrintString (Utilities|String|ToString(Float) (Variables|Default|GetReloading_Seconds)))
  (Variables|Default|SetReload_Percent (/ (Variables|Default|GetReloading_Seconds) (Variables|Default|GetReload_Time)))
  (switch Utilities|FlowControl|Switch|SwitchonEnum_Reload_Types (.Reload_Type (Utilities|Struct|BreakStruct_Reload_Info (.reload_info (stale Custom|Start_Reload _ranged_info))))
    (:NewEnumerator0
      (if (Math|Boolean|ANDBoolean (>= (Math|Float|%(Float) (Variables|Default|GetReload_Percent) (Variables|Default|GetReload_Threshold)) 0.0) (<= (Math|Float|%(Float) (Variables|Default|GetReload_Percent) (Variables|Default|GetReload_Threshold)) 0.02) (> (Variables|Default|GetReloading_Seconds) (/ (Variables|Default|GetReload_Time) 5e+01)))
        (Utilities|FlowControl|DoOnce false :!label _label
          (:Completed
            (Math|Integer|IncrementInt (Variables|Default|GetCurrent_Ammo)
              (:%20%20
                (Utilities|FlowControl|Sequence
                  (:then_0
                    (if _returnvalue_11 :!label _label_2
                      (bind _basics (Class|BPIWeapon|GetBasicInfo(Message) (Components|GetOwner)))
                      (switch int (Variables|/Game/UI/WBP_HUD.WBP_HUD_C|GetCurrently_Equipped_Weapon_Image_Relation _hud_ref)
                        (:0
                          (Default|UpdateImgColourforAmmo _weapon_1 (+ (/ (Math|Conversions|ToFloat(Integer) (Variables|Default|GetCurrent_Ammo)) (Math|Conversions|ToFloat(Integer) (Variables|Default|GetMax_Ammo))) (* (- 1.0 (/ (Math|Conversions|ToFloat(Integer) (Variables|Default|GetCurrent_Ammo)) (Math|Conversions|ToFloat(Integer) (Variables|Default|GetMax_Ammo)))) (Variables|Default|GetReload_Percent))))
                          (Default|UpdateAmmoCount _weapon_1 (Variables|Default|GetCurrent_Ammo) (.ranged _basics)))
                        (:1
                          (Default|UpdateImgColourforAmmo _weapon_2 (+ (/ (Math|Conversions|ToFloat(Integer) (Variables|Default|GetCurrent_Ammo)) (Math|Conversions|ToFloat(Integer) (Variables|Default|GetMax_Ammo))) (* (- 1.0 (/ (Math|Conversions|ToFloat(Integer) (Variables|Default|GetCurrent_Ammo)) (Math|Conversions|ToFloat(Integer) (Variables|Default|GetMax_Ammo)))) (Variables|Default|GetReload_Percent))))
                          (Default|UpdateAmmoCount _weapon_2 (Variables|Default|GetCurrent_Ammo) (.ranged _basics)))
                        (:2
                          (Default|UpdateImgColourforAmmo _weapon_3 (+ (/ (Math|Conversions|ToFloat(Integer) (Variables|Default|GetCurrent_Ammo)) (Math|Conversions|ToFloat(Integer) (Variables|Default|GetMax_Ammo))) (* (- 1.0 (/ (Math|Conversions|ToFloat(Integer) (Variables|Default|GetCurrent_Ammo)) (Math|Conversions|ToFloat(Integer) (Variables|Default|GetMax_Ammo)))) (Variables|Default|GetReload_Percent))))
                          (Default|UpdateAmmoCount _weapon_3 (Variables|Default|GetCurrent_Ammo) (.ranged _basics))))))
                  (:then_1
                    (Audio|PlaySoundatLocation (.Reload_SC (Utilities|Struct|BreakStruct_Ranged_Weapon_Audio (.audio_info (stale Custom|Start_Reload _ranged_info)))) _returnvalue_6 "0, 0, 0" 1.0 1.0 0.0 0 0 0 0)
                    (Class|AISenseHearing|ReportNoiseEvent _returnvalue_6 0.75 (Components|GetOwner (Components|GetOwner)) 0.0 "None")
                    (if (Utilities|DoesObjectImplementInterface (Components|GetOwner (Components|GetOwner)) "/Game/Characters/Player/BPI_Player.BPI_Player_C")
                      (Default|PlayAmmoAnimation (Variables|/Game/Characters/Player/BPC_HUD.BPC_HUD_C|GetHUD_Ref (Actor|GetComponentbyClass (Components|GetOwner (Components|GetOwner)) "/Game/Characters/Player/BPC_HUD.BPC_HUD_C")) false))))))))
        (else
          (Utilities|FlowControl|Sequence
            (:then_0
              (goto _label Reset))
            (:then_1
              (goto _label_2)))))
      ;[1 1 1] reaching max ammo stops
      (if (>= (Variables|Default|GetCurrent_Ammo) (Variables|Default|GetMax_Ammo))
        (CallFunction|StopReload)))
    (:NewEnumerator1
      (if (>= (Variables|Default|GetReload_Percent) 1.0)
        (Variables|Default|SetCurrent_Ammo (Variables|Default|GetMax_Ammo))
        (CallFunction|StopReload)
        (if _returnvalue_11
          (bind _basics_2 (Class|BPIWeapon|GetBasicInfo(Message) (Components|GetOwner)))
          (switch int (Variables|/Game/UI/WBP_HUD.WBP_HUD_C|GetCurrently_Equipped_Weapon_Image_Relation _hud_ref_2)
            (:0
              (Default|UpdateImgColourforAmmo _weapon_1_2 (/ (Math|Conversions|ToFloat(Integer) (Variables|Default|GetCurrent_Ammo)) (Math|Conversions|ToFloat(Integer) (Variables|Default|GetMax_Ammo))))
              (Default|UpdateAmmoCount _weapon_1_2 (Variables|Default|GetCurrent_Ammo) (.ranged _basics_2)))
            (:1
              (Default|UpdateImgColourforAmmo _weapon_2_2 (/ (Math|Conversions|ToFloat(Integer) (Variables|Default|GetCurrent_Ammo)) (Math|Conversions|ToFloat(Integer) (Variables|Default|GetMax_Ammo))))
              (Default|UpdateAmmoCount _weapon_2_2 (Variables|Default|GetCurrent_Ammo) (.ranged _basics_2)))
            (:2
              (Default|UpdateImgColourforAmmo _weapon_3_2 (/ (Math|Conversions|ToFloat(Integer) (Variables|Default|GetCurrent_Ammo)) (Math|Conversions|ToFloat(Integer) (Variables|Default|GetMax_Ammo))))
              (Default|UpdateAmmoCount _weapon_3_2 (Variables|Default|GetCurrent_Ammo) (.ranged _basics_2))))
          (Default|PlayAmmoAnimation _hud_ref_2 false))
        (Audio|PlaySoundatLocation (.Reload_SC (Utilities|Struct|BreakStruct_Ranged_Weapon_Audio (.audio_info (stale Custom|Start_Reload _ranged_info)))) _returnvalue_9 "0, 0, 0" 1.0 1.0 0.0 0 0 0 0)
        (Class|AISenseHearing|ReportNoiseEvent _returnvalue_9 0.75 (Components|GetOwner (Components|GetOwner)) 0.0 "None")))))

(event EventBeginPlay
  (Variables|Default|SetCurrent_Ammo (Variables|Default|GetMax_Ammo))
  (bind _ranged_info (Class|BPIRangedWeapon|GetRangedInfo(Message) (Components|GetOwner)))
  (Variables|Default|SetReload_Time (.Reload_Time (Utilities|Struct|BreakStruct_Reload_Info (.reload_info _ranged_info)))))