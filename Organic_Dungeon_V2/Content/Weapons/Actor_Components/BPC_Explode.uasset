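; Explosion component that applies radial damage and knockback around a hit location, for projectile or other blasts.
; A multi-sphere trace finds each Pawn or PhysicsBody actor once, with debug drawing left on.
; Pawns with health take damage scaled by horizontal distance, characters are launched with optional blood effects, and physics bodies receive force.
; It then spawns particle, sound and camera shake, destroying the owner on request or whenever a physics body is hit.
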(fn Explode
  (params (Hit_Location :type Vector) (Explode%20Info :type Struct%20Explosion%20on%20Hit%20Structure) (From%20Projectile? :type Boolean) (Projectile%20Speed :type Float%20%28double-precision%29) (Damage :type Float%20%28double-precision%29) (Should%20Destroy%20Owner :type Boolean))
  (bind _returnvalue (Components|GetOwner))
  (bind _returnvalue_2 (Components|GetOwner))
  (bind _returnvalue_3 (Components|GetOwner))
  (bind (_x _y) (Class|KismetMathLibrary|BreakVector3f Hit_Location))
  (bind _explosionradius (Utilities|Struct|BreakStruct_Explosion_On_Hit Explode%20Info))
  (bind _returnvalue_4 (Transformation|GetActorUpVector _returnvalue))
  (bind _returnvalue_5 (Math|Float|SelectFloat Projectile%20Speed 2e+03 From%20Projectile?))
  (bind _returnvalue_6 (* _returnvalue_5 5.0))
  (bind _returnvalue_7 (* _returnvalue_4 _returnvalue_6))
  (Rendering|Debug|DrawDebugSphere Hit_Location 2e+01 12 "(R=1.000000,G=1.000000,B=1.000000,A=1.000000)" 5e+01 1.0)
  (Utilities|Array|Clear (LocalVariables|GetHit_Actors))
  (bind (_outhits _returnvalue_8) (Collision|MultiSphereTraceForObjects Hit_Location Hit_Location (.ExplosionRadius (Utilities|Struct|BreakStruct_Explosion_On_Hit Explode%20Info)) (Utilities|Array|MakeArray "ObjectTypeQuery4" "ObjectTypeQuery3") true 0 "ForDuration"))
  (if _returnvalue_8
    (for _array_element _outhits
      (LocalVariables|SetCurrent_Hit_Actor (.HitActor (Collision|BreakHitResult _array_element)))
      (if (not (Utilities|Array|ContainsItem (LocalVariables|GetHit_Actors) (Components|GetOwner (.HitComponent (Collision|BreakHitResult _array_element)))))
        (Utilities|Array|Add (LocalVariables|GetHit_Actors) (LocalVariables|GetCurrent_Hit_Actor))
        (switch Utilities|FlowControl|Switch|SwitchonECollisionChannel (Collision|GetCollisionObjectType (.HitComponent (Collision|BreakHitResult _array_element)))
          (:ECC_Pawn
            (if (Utilities|DoesObjectImplementInterface (LocalVariables|GetCurrent_Hit_Actor) "/Game/Health/Interfaces/BPI_Has_Health.BPI_Has_Health_C")
              (if (Utilities|IsValid (Actor|GetComponentbyClass (LocalVariables|GetCurrent_Hit_Actor) "/Game/Health/BPs/BPC_Health.BPC_Health_C"))
                (Default|TakeDamage (Actor|GetComponentbyClass (LocalVariables|GetCurrent_Hit_Actor) "/Game/Health/BPs/BPC_Health.BPC_Health_C") (Math|Conversions|ToFloat(Integer) (Math|Float|Floor (* Damage (- 1.0 (/ (- (Math|Vector|VectorLength (- (Math|Vector|MakeVector _x _y (.z (Transformation|GetActorLocation (LocalVariables|GetCurrent_Hit_Actor)))) (Math|Vector|MakeVector (.x (Transformation|GetActorLocation (LocalVariables|GetCurrent_Hit_Actor))) (.y (Transformation|GetActorLocation (LocalVariables|GetCurrent_Hit_Actor))) (.z (Transformation|GetActorLocation (LocalVariables|GetCurrent_Hit_Actor)))))) 75.0) (.ExplosionRadius (Utilities|Struct|BreakStruct_Explosion_On_Hit Explode%20Info))))))) (Transformation|GetActorLocation (LocalVariables|GetCurrent_Hit_Actor)) (LocalVariables|GetCurrent_Hit_Actor) (Components|GetOwner))
                (bind _ascharacter (Utilities|Casting|CastToCharacter (LocalVariables|GetCurrent_Hit_Actor)))
                (Character|LaunchCharacter _ascharacter (+ (/ _returnvalue_7 25.0) (/ (* (Math|Vector|GetForwardVector (Math|Rotator|FindLookatRotation Hit_Location (Transformation|GetWorldLocation (.HitComponent (Collision|BreakHitResult _array_element))))) (* _returnvalue_5 (.KnockbackAmount (Utilities|Struct|BreakStruct_Explosion_On_Hit Explode%20Info)))) 1.5e+02)) false false)
                (Utilities|IsValid (Actor|GetComponentbyClass (.HitActor (Collision|BreakHitResult _array_element)) "/Game/VFX_SFX/Blood_Splatter/BPS/BPC_Blood_Effect.BPC_Blood_Effect_C")
                  (:Is%20Valid
                    (Default|BloodEffect (Actor|GetComponentbyClass (.HitActor (Collision|BreakHitResult _array_element)) "/Game/VFX_SFX/Blood_Splatter/BPS/BPC_Blood_Effect.BPC_Blood_Effect_C") (.Location (Collision|BreakHitResult _array_element)) (.Normal (Collision|BreakHitResult _array_element)) (.HitActor (Collision|BreakHitResult _array_element)) (Math|Conversions|ToFloat(Integer) (Math|Float|Floor (* Damage (- 1.0 (/ (- (Math|Vector|VectorLength (- (Math|Vector|MakeVector _x _y (.z (Transformation|GetActorLocation (LocalVariables|GetCurrent_Hit_Actor)))) (Math|Vector|MakeVector (.x (Transformation|GetActorLocation (LocalVariables|GetCurrent_Hit_Actor))) (.y (Transformation|GetActorLocation (LocalVariables|GetCurrent_Hit_Actor))) (.z (Transformation|GetActorLocation (LocalVariables|GetCurrent_Hit_Actor)))))) 75.0) (.ExplosionRadius (Utilities|Struct|BreakStruct_Explosion_On_Hit Explode%20Info)))))))))))))
          (:ECC_PhysicsBody
            (Physics|AddForce (.HitComponent (Collision|BreakHitResult _array_element)) (+ _returnvalue_7 (* (Math|Vector|GetForwardVector (Math|Rotator|FindLookatRotation Hit_Location (Transformation|GetWorldLocation (.HitComponent (Collision|BreakHitResult _array_element))))) (* _returnvalue_5 (.KnockbackAmount (Utilities|Struct|BreakStruct_Explosion_On_Hit Explode%20Info))))) "None" true)
            (Utilities|IsValid _returnvalue_2
              (:Is%20Valid
                (Actor|DestroyActor _returnvalue_2))))))))
  (Game|SpawnActorfromClass "/Game/VFX_SFX/Realistic_Starter_VFX_Pack_Vol2/Blueprints/Spawn_Particle.Spawn_Particle_C" (Math|Transform|MakeTransform Hit_Location "0, 0, 0" "1.000000,1.000000,1.000000") "Undefined" "MultiplyWithRoot" 0 2.0 false "/Game/VFX_SFX/Realistic_Starter_VFX_Pack_Vol2/Particles/Explosion/P_Explosion_Big_A.P_Explosion_Big_A" 0)
  (Audio|PlaySoundatLocation "/Game/VFX_SFX/Sounds/Shots/Rocket/Explosion/Rocket_Explosion_SC.Rocket_Explosion_SC" (.Location (Collision|BreakHitResult _array_element)) "0, 0, 0" 1.0 1.0 0.0 0 0 0 0)
  (Camera|PlayWorldCameraShake "/Game/Projectiles/BPS/BP_Explosion_Camera_Shake.BP_Explosion_Camera_Shake_C" (.Location (Collision|BreakHitResult _array_element)) _explosionradius (* _explosionradius 4.0))
  (Utilities|IsValid _returnvalue_3
    (:Is%20Valid
      (if Should%20Destroy%20Owner
        (Actor|DestroyActor _returnvalue_3)))))