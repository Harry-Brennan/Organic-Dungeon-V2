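; BPC_Aim is an actor component that turns the owner's Aiming state on and off from the IA_Aim input action.
; Pressing or holding starts aiming while CanAim is true and stops it otherwise; releasing or canceling also stops it.
; For BPI_Player owners, both changes apply only when the weapon equipped in BPC_Player_Weaponry is ranged.
; Other owners set or clear Aiming directly.
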(event Custom|Start_Aiming
  (bind _returnvalue (Components|GetOwner))
  (if (Utilities|DoesObjectImplementInterface _returnvalue "/Game/Characters/Player/BPI_Player.BPI_Player_C")
    (bind _basics (Class|BPIWeapon|GetBasicInfo(Message) (Variables|/Game/Weapons/Actor_Components/BPC_Player_Weaponry.BPC_Player_Weaponry_C|GetEquipped_Weapon (Actor|GetComponentbyClass _returnvalue "/Game/Weapons/Actor_Components/BPC_Player_Weaponry.BPC_Player_Weaponry_C"))))
    (if (.ranged _basics)
      (Variables|Default|SetAiming? true))
    (else
      (Variables|Default|SetAiming? true))))

(event Custom|Stop_Aiming
  (bind _returnvalue (Components|GetOwner))
  (if (Utilities|DoesObjectImplementInterface _returnvalue "/Game/Characters/Player/BPI_Player.BPI_Player_C")
    (bind _basics (Class|BPIWeapon|GetBasicInfo(Message) (Variables|/Game/Weapons/Actor_Components/BPC_Player_Weaponry.BPC_Player_Weaponry_C|GetEquipped_Weapon (Actor|GetComponentbyClass _returnvalue "/Game/Weapons/Actor_Components/BPC_Player_Weaponry.BPC_Player_Weaponry_C"))))
    (if (.ranged _basics)
      (Variables|Default|SetAiming? false))
    (else
      (Variables|Default|SetAiming? false))))

(event Input|EnhancedActionEvents|EnhancedInputActionIA_Aim
  (params (ActionValue :type Boolean) (ElapsedSeconds :type Float%20%28double-precision%29) (TriggeredSeconds :type Float%20%28double-precision%29) (InputAction :type Input%20Action%20Object%20Reference :default "/Game/Characters/Player/Input/Actions/IA_Aim.IA_Aim"))
  (:Triggered
    (if (Variables|Default|GetCanAim?) :!label _label
      (CallFunction|StartAiming)
      (else
        (CallFunction|StopAiming :!label _label_2))))
  (:Started
    (goto _label))
  (:Canceled
    (goto _label_2))
  (:Completed
    (goto _label_2)))