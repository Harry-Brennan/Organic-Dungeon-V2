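; Actor component that manages its owner's weapon inventory, handling pickup, equipping and cycling through weapons.
; Stored weapons move to TargetPoints tagged "Inventory"; the equipped one snaps to the owner's Weapon_R socket.
; Cycling uses wrapped previous/next indexes, cancels reloads and updates HUD icons.
; Equipping plays a sound, reports noise, briefly flags SwappingWeapons and, for BPI_Player owners, updates the crosshair; only those owners respond to cycle inputs.
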(event Custom|Move_To_Inventory_Space
  (params (Weapon_To_Move :type Actor%20Object%20Reference))
  (bind _outactors (Actor|GetAllActorsOfClasswithTag "/Script/Engine.TargetPoint" "Inventory"))
  (for _array_element _outactors
    (Transformation|SetActorLocation Weapon_To_Move (Transformation|GetActorLocation _array_element) false false)))

(event Custom|Move_From_Inventory_Space
  (params (Weapon_To_Move :type Actor%20Object%20Reference) (End_Location :type Vector))
  (Transformation|SetActorLocation Weapon_To_Move End_Location false false))

(event Custom|Update_Next_&_Previous_Indexes
  (bind _weapons (Variables|Weapons|GetWeapons))
  (bind _equipped_weapon (Variables|Weapons|GetEquipped_Weapon))
  (bind _weapons_2 (Variables|Weapons|GetWeapons))
  (bind _equipped_weapon_2 (Variables|Weapons|GetEquipped_Weapon))
  (bind _returnvalue (Utilities|Array|FindItem _weapons _equipped_weapon))
  (bind _returnvalue_2 (Utilities|Array|FindItem _weapons_2 _equipped_weapon_2))
  (bind _returnvalue_3 (+ _returnvalue_2 1))
  (bind _returnvalue_4 (- _returnvalue 1))
  (Utilities|FlowControl|Sequence
    (:then_0
      (Variables|Swapping|SetNext_Weapon_Index (Math|Integer|SelectInt 0 _returnvalue_3 (> _returnvalue_3 (Utilities|Array|LastIndex _weapons_2)))))
    (:then_1
      (Variables|Swapping|SetPrevious_Weapon_Index (Math|Integer|SelectInt (Utilities|Array|LastIndex _weapons) _returnvalue_4 (< _returnvalue_4 0))))))

(event Custom|Equip_Previous_Weapon
  (bind _returnvalue (Components|GetOwner))
  (bind _equipped_weapon (Variables|Weapons|GetEquipped_Weapon))
  (bind _returnvalue_2 (Actor|GetComponentbyClass _equipped_weapon "/Game/Weapons/Actor_Components/BPC_Ammo.BPC_Ammo_C"))
  (bind _returnvalue_3 (Actor|GetComponentbyClass _returnvalue "/Game/Characters/Player/BPC_HUD.BPC_HUD_C"))
  (if (not (Utilities|Array|IsEmpty (Variables|Weapons|GetWeapons)))
    (if (Variables|/Game/Weapons/Actor_Components/BPC_Ammo.BPC_Ammo_C|GetReloading _returnvalue_2)
      (Default|StopReload _returnvalue_2))
    (CallFunction|UpdateNext&PreviousIndexes)
    (CallFunction|EquipWeapon (Utilities|Array|Get(acopy) (Variables|Weapons|GetWeapons) (Variables|Swapping|GetPrevious_Weapon_Index)))
    (Utilities|IsValid _returnvalue_3
      (:Is%20Valid
        (Default|SwapWeaponIcons _returnvalue_3 false)))))

(event Custom|Equip_Next_Weapon
  (bind _returnvalue (Components|GetOwner))
  (bind _equipped_weapon (Variables|Weapons|GetEquipped_Weapon))
  (bind _returnvalue_2 (Actor|GetComponentbyClass _returnvalue "/Game/Characters/Player/BPC_HUD.BPC_HUD_C"))
  (bind _returnvalue_3 (Actor|GetComponentbyClass _equipped_weapon "/Game/Weapons/Actor_Components/BPC_Ammo.BPC_Ammo_C"))
  (if (not (Utilities|Array|IsEmpty (Variables|Weapons|GetWeapons)))
    (if (Variables|/Game/Weapons/Actor_Components/BPC_Ammo.BPC_Ammo_C|GetReloading _returnvalue_3)
      (Default|StopReload _returnvalue_3))
    (CallFunction|UpdateNext&PreviousIndexes)
    (CallFunction|EquipWeapon (Utilities|Array|Get(acopy) (Variables|Weapons|GetWeapons) (Variables|Swapping|GetNext_Weapon_Index)))
    (Utilities|IsValid _returnvalue_2
      (:Is%20Valid
        (Default|SwapWeaponIcons _returnvalue_2 true)))))

(event Custom|Equip_Weapon
  (params (WeaponToEquip :type Actor%20Object%20Reference))
  (bind _returnvalue (Components|GetOwner))
  (bind _returnvalue_2 (Components|GetOwner))
  (bind _returnvalue_3 (Components|GetOwner))
  (bind _returnvalue_4 (Components|GetOwner))
  (bind _returnvalue_5 (Transformation|GetActorLocation _returnvalue_2))
  (bind _returnvalue_6 (Actor|GetComponentbyClass _returnvalue_3 "/Script/Engine.SkeletalMeshComponent"))
  (if (not (== WeaponToEquip (Variables|Weapons|GetEquipped_Weapon)))
    (CallFunction|DequipWeapon)
    (Class|BPIWeapon|UpdateCollision(Message) WeaponToEquip false)
    (CallFunction|MovefromInventorySpace WeaponToEquip (Transformation|GetSocketLocation _returnvalue_6 "Weapon_R"))
    (Transformation|AttachComponentToComponent WeaponToEquip _returnvalue_6 "Weapon_R" "SnapToTarget" "SnapToTarget" "KeepRelative" true)
    (Utilities|IsValid (Variables|Weapons|GetEquipped_Weapon)
      (:Is%20Valid
        (if (Variables|/Game/Weapons/Actor_Components/BPC_Ammo.BPC_Ammo_C|GetReloading (Actor|GetComponentbyClass (Variables|Weapons|GetEquipped_Weapon) "/Game/Weapons/Actor_Components/BPC_Ammo.BPC_Ammo_C"))
          (Default|StopReload (Actor|GetComponentbyClass (Variables|Weapons|GetEquipped_Weapon) "/Game/Weapons/Actor_Components/BPC_Ammo.BPC_Ammo_C"))))
      (:Is%20Not%20Valid
        _))
    (Variables|Weapons|SetEquipped_Weapon WeaponToEquip)
    (Utilities|FlowControl|Sequence
      (:then_0
        (CallFunction|UpdateNext&PreviousIndexes)
        (bind _basics (Class|BPIWeapon|GetBasicInfo(Message) (Variables|Weapons|GetEquipped_Weapon)))
        (if (.ranged _basics)
          (bind _ranged_info (Class|BPIRangedWeapon|GetRangedInfo(Message) (Variables|Weapons|GetEquipped_Weapon)))
          (Audio|PlaySoundatLocation (.reload_sc (Utilities|Struct|BreakStruct_Ranged_Weapon _ranged_info)) _returnvalue_5 "0, 0, 0" 1.0 1.0 0.0 0 0 0 0)
          (Class|AISenseHearing|ReportNoiseEvent _returnvalue_5 0.65 _returnvalue_4 0.0 "None")
          (if (Utilities|DoesObjectImplementInterface _returnvalue_4 "/Game/Characters/Player/BPI_Player.BPI_Player_C")
            (Default|UpdateCrosshair (Actor|GetComponentbyClass _returnvalue_4 "/Game/Characters/Player/BPC_HUD.BPC_HUD_C") false false false))
          (else
            (Audio|PlaySoundatLocation "/Game/VFX_SFX/Air_Dash/Air_Dash_SC.Air_Dash_SC" _returnvalue_5 "0, 0, 0" 1.0 1.0 0.0 0 0 0 0)
            (Class|AISenseHearing|ReportNoiseEvent _returnvalue_5 0.65 _returnvalue_2 0.0 "None")
            (if (Utilities|DoesObjectImplementInterface _returnvalue "/Game/Characters/Player/BPI_Player.BPI_Player_C")
              (Default|UpdateCrosshair (Actor|GetComponentbyClass _returnvalue "/Game/Characters/Player/BPC_HUD.BPC_HUD_C") true true false)))))
      (:then_1
        (Variables|Swapping|SetSwapping_Weapons true)
        (Utilities|FlowControl|Delay 0.1)
        (Variables|Swapping|SetSwapping_Weapons false)))))

(event Custom|Dequip_Weapon
  (bind _returnvalue (Components|GetOwner))
  (bind _equipped_weapon (Variables|Weapons|GetEquipped_Weapon))
  (Utilities|IsValid _equipped_weapon
    (:Is%20Valid
      (Transformation|DetachFromActor _equipped_weapon "KeepWorld" "KeepWorld" "KeepWorld")
      (Transformation|SetActorLocation _equipped_weapon (+ (Transformation|GetActorLocation _returnvalue) (* (Transformation|GetActorForwardVector _returnvalue) 5e+01)) false false)
      (Class|BPIWeapon|UpdateCollision(Message) _equipped_weapon true)
      (CallFunction|MovetoInventorySpace _equipped_weapon))))

(event Custom|Add_Weapon
  (params (WeaponToAdd :type Actor%20Object%20Reference))
  (bind _returnvalue (Components|GetOwner))
  (bind _returnvalue_2 (Actor|GetComponentbyClass _returnvalue "/Game/Characters/Player/BPC_HUD.BPC_HUD_C"))
  (Utilities|Array|Add (Variables|Weapons|GetWeapons) WeaponToAdd)
  (Class|BPIWeapon|UpdateCollision(Message) WeaponToAdd false)
  (Default|StopAnimatedRotation (Actor|GetComponentbyClass WeaponToAdd "/Game/Weapons/Actor_Components/BPC_Animated_Rotation.BPC_Animated_Rotation_C"))
  (CallFunction|MovetoInventorySpace WeaponToAdd)
  (CallFunction|EquipWeapon WeaponToAdd)
  (Actor|SetOwner WeaponToAdd (Components|GetOwner))
  (Utilities|IsValid _returnvalue_2
    (:Is%20Valid
      (Default|SwapWeaponIcons _returnvalue_2 true))))

(event Input|EnhancedActionEvents|EnhancedInputActionIA_Cycle_Next_Weapon
  (params (ActionValue :type Boolean) (ElapsedSeconds :type Float%20%28double-precision%29) (TriggeredSeconds :type Float%20%28double-precision%29) (InputAction :type Input%20Action%20Object%20Reference :default "/Game/Characters/Player/Input/Actions/IA_Cycle_Next_Weapon.IA_Cycle_Next_Weapon"))
  (:Triggered
    (if (Utilities|DoesObjectImplementInterface (Components|GetOwner) "/Game/Characters/Player/BPI_Player.BPI_Player_C")
      (CallFunction|EquipNextWeapon))))

(event Input|EnhancedActionEvents|EnhancedInputActionIA_Cycle_Previous_Weapon
  (params (ActionValue :type Boolean) (ElapsedSeconds :type Float%20%28double-precision%29) (TriggeredSeconds :type Float%20%28double-precision%29) (InputAction :type Input%20Action%20Object%20Reference :default "/Game/Characters/Player/Input/Actions/IA_Cycle_Previous_Weapon.IA_Cycle_Previous_Weapon"))
  (:Triggered
    (if (Utilities|DoesObjectImplementInterface (Components|GetOwner) "/Game/Characters/Player/BPI_Player.BPI_Player_C")
      (CallFunction|EquipPreviousWeapon))))