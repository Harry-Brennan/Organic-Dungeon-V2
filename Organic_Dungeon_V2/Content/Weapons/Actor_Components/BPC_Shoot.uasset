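; Weapon actor component that fires a ranged shot for its owning weapon, triggering ammo use, recoil, muzzle particle, sound, AI noise and crosshair animation.
; Each pellet spawns a BP_Projectile aimed at the point a camera-view line trace finds, with random spread.
; Hitscan weapons also sphere-trace along that spread direction, applying damage and blood effects directly.
; Piercing traces hit each actor along the line only once.
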(event Custom|Shoot
  (params (Projectile :type Struct%20Projectiles%20Structure) (Ranged_Info :type Struct%20Ranged%20Weapon%20Structure))
  (bind (_starting_ammo _crosshair _reload_info _projectilename _projectile_info _recoil _hitscan _piercing _shootparticle __projectiles _spread _fire_type _burst_info _full_auto_info _charged_info _charged_burst_info _audio_info) (Utilities|Struct|BreakStruct_Ranged_Weapon Ranged_Info))
  (bind _damage (Utilities|Struct|BreakStruct_Projectiles Projectile))
  (bind _damage_2 (Utilities|Struct|BreakStruct_Projectiles Projectile))
  (bind _returnvalue (Components|GetOwner))
  (bind _returnvalue_2 (Components|GetOwner))
  (bind _returnvalue_3 (Components|GetOwner))
  (bind _array (Utilities|Array|MakeArray "ObjectTypeQuery3" "ObjectTypeQuery1" "ObjectTypeQuery2"))
  (bind (_recoil_amount _recoil_duration _recoil_knockback) (Utilities|Struct|BreakStruct_Recoil_Info _recoil))
  (bind _returnvalue_4 (Components|GetOwner _returnvalue_2))
  (bind _returnvalue_5 (Components|GetOwner _returnvalue_3))
  (bind _returnvalue_6 (/ _spread 2.0))
  (bind _returnvalue_7 (- _returnvalue_6 _spread))
  (bind _shoot_transform (Class|BPIWeapon|GetShootTransform(Message) _returnvalue))
  (bind _static_mesh (Class|BPIRangedWeapon|GetStaticMesh(Message) (Components|GetOwner)))
  (Utilities|Array|Clear (Variables|Default|GetActors_To_Ignore))
  (Default|DecreaseAmmo (Actor|GetComponentbyClass (Components|GetOwner) "/Game/Weapons/Actor_Components/BPC_Ammo.BPC_Ammo_C"))
  (Default|StartRecoil (Actor|GetComponentbyClass (Components|GetOwner) "/Game/Weapons/Actor_Components/BPC_Recoil.BPC_Recoil_C") _recoil_amount _recoil_duration _recoil_knockback)
  (for _index (range 1 (._Projectiles (Utilities|Struct|BreakStruct_Ranged_Weapon Ranged_Info)))
    (bind _destination (CallFunction|AimTowardsCrosshair))
    (Variables|Default|SetSpread_Rand_Roll (Math|Random|RandomFloatinRange _returnvalue_7 _spread))
    (Variables|Default|SetSpread_Rand_Pitch (Math|Random|RandomFloatinRange _returnvalue_7 _spread))
    (Variables|Default|SetSpread_Rand_Yaw (Math|Random|RandomFloatinRange _returnvalue_7 _spread))
    (bind _returnvalue_8 (Game|SpawnActorfromClass "/Game/Projectiles/BPS/BP_Projectile.BP_Projectile_C" (Math|Transform|MakeTransform (.location _shoot_transform) (Math|Rotator|MakeRotator (+ (.Roll (Math|Rotator|BreakRotator (Math|Rotator|FindLookatRotation (.location _shoot_transform) _destination))) (Variables|Default|GetSpread_Rand_Roll)) (+ (.Pitch (Math|Rotator|BreakRotator (Math|Rotator|FindLookatRotation (.location _shoot_transform) _destination))) (Variables|Default|GetSpread_Rand_Pitch)) (+ (.Yaw (Math|Rotator|BreakRotator (Math|Rotator|FindLookatRotation (.location _shoot_transform) _destination))) (Variables|Default|GetSpread_Rand_Yaw))) "1.000000,1.000000,1.000000") "AlwaysSpawn" "MultiplyWithRoot" _returnvalue Projectile 0))
    (Utilities|Array|Add (Variables|Default|GetActors_To_Ignore) _returnvalue_8)
    (if _hitscan
      (bind _shoot_transform_2 (Class|BPIWeapon|GetShootTransform(Message) (Components|GetOwner)))
      (Utilities|Array|AppendArray (Variables|Default|GetActors_To_Ignore) (Utilities|Array|MakeArray _returnvalue_4 _returnvalue_4))
      (bind _outactors (Actor|GetAllActorsOfClass "/Game/Weapons/BPs/BP_Weapon.BP_Weapon_C"))
      (Utilities|Array|AppendArray (Variables|Default|GetActors_To_Ignore) _outactors)
      (if (.Piercing (Utilities|Struct|BreakStruct_Ranged_Weapon Ranged_Info))
        (Utilities|Array|Clear (Variables|Default|GetPierced_Actors))
        (bind (_outhits _returnvalue_9) (Collision|MultiSphereTraceForObjects (.location _shoot_transform_2) (+ (.location _shoot_transform_2) (* (Math|Vector|GetForwardVector (Math|Rotator|MakeRotator (+ (.Roll (Math|Rotator|BreakRotator (Math|Rotator|FindLookatRotation (.location _shoot_transform_2) _destination))) (Variables|Default|GetSpread_Rand_Roll)) (+ (.Pitch (Math|Rotator|BreakRotator (Math|Rotator|FindLookatRotation (.location _shoot_transform_2) _destination))) (Variables|Default|GetSpread_Rand_Pitch)) (+ (.Yaw (Math|Rotator|BreakRotator (Math|Rotator|FindLookatRotation (.location _shoot_transform_2) _destination))) (Variables|Default|GetSpread_Rand_Yaw)))) 5e+04)) 5.0 _array false (Variables|Default|GetActors_To_Ignore) (Variables|Default|GetTrace)))
        (if _returnvalue_9
          (for _array_element _outhits
            (if (not (Utilities|Array|ContainsItem (Variables|Default|GetPierced_Actors) (.HitActor (Collision|BreakHitResult _array_element))))
              (Utilities|Array|Add (Variables|Default|GetPierced_Actors) (.HitActor (Collision|BreakHitResult _array_element)))
              (if (Utilities|DoesObjectImplementInterface (.HitActor (Collision|BreakHitResult _array_element)) "/Game/Health/Interfaces/BPI_Has_Health.BPI_Has_Health_C")
                (Default|TakeDamage (Actor|GetComponentbyClass (.HitActor (Collision|BreakHitResult _array_element)) "/Game/Health/BPs/BPC_Health.BPC_Health_C") _damage (.Location (Collision|BreakHitResult _array_element)) (.HitActor (Collision|BreakHitResult _array_element)) (Components|GetOwner (Components|GetOwner))))
              (Utilities|IsValid (Actor|GetComponentbyClass (.HitActor (Collision|BreakHitResult _array_element)) "/Game/VFX_SFX/Blood_Splatter/BPS/BPC_Blood_Effect.BPC_Blood_Effect_C")
                (:Is%20Valid
                  (Default|BloodEffect (Actor|GetComponentbyClass (.HitActor (Collision|BreakHitResult _array_element)) "/Game/VFX_SFX/Blood_Splatter/BPS/BPC_Blood_Effect.BPC_Blood_Effect_C") (.Location (Collision|BreakHitResult _array_element)) (.Normal (Collision|BreakHitResult _array_element)) (.HitActor (Collision|BreakHitResult _array_element)) _damage)
                  (Default|BloodEffect (Actor|GetComponentbyClass (.HitActor (Collision|BreakHitResult _array_element)) "/Game/VFX_SFX/Blood_Splatter/BPS/BPC_Blood_Effect.BPC_Blood_Effect_C") (.Location (Collision|BreakHitResult _array_element)) (* (.Normal (Collision|BreakHitResult _array_element)) -1.0) (.HitActor (Collision|BreakHitResult _array_element)) _damage))
                (:Is%20Not%20Valid
                  _))
              (Audio|PlaySoundatLocation "/Game/VFX_SFX/Blood_Splatter/Audio/Impact_Audio/Body_Impact_SC.Body_Impact_SC" (.Location (Collision|BreakHitResult _array_element)) "0, 0, 0" 1.0 1.0 0.0 0 0 0 0))))
        (else
          (bind (_outhit _returnvalue_10) (Collision|SphereTraceForObjects (.location _shoot_transform_2) (+ (.location _shoot_transform_2) (* (Math|Vector|GetForwardVector (Math|Rotator|MakeRotator (+ (.Roll (Math|Rotator|BreakRotator (Math|Rotator|FindLookatRotation (.location _shoot_transform_2) _destination))) (Variables|Default|GetSpread_Rand_Roll)) (+ (.Pitch (Math|Rotator|BreakRotator (Math|Rotator|FindLookatRotation (.location _shoot_transform_2) _destination))) (Variables|Default|GetSpread_Rand_Pitch)) (+ (.Yaw (Math|Rotator|BreakRotator (Math|Rotator|FindLookatRotation (.location _shoot_transform_2) _destination))) (Variables|Default|GetSpread_Rand_Yaw)))) 5e+04)) 5.0 _array false (Variables|Default|GetActors_To_Ignore) (Variables|Default|GetTrace)))
          (if _returnvalue_10
            (if (Utilities|DoesObjectImplementInterface (.HitActor (Collision|BreakHitResult _outhit)) "/Game/Health/Interfaces/BPI_Has_Health.BPI_Has_Health_C")
              (Default|TakeDamage (Actor|GetComponentbyClass (.HitActor (Collision|BreakHitResult _outhit)) "/Game/Health/BPs/BPC_Health.BPC_Health_C") _damage_2 (.Location (Collision|BreakHitResult _outhit)) (.HitActor (Collision|BreakHitResult _outhit)) (Components|GetOwner (Components|GetOwner)))
              (Utilities|IsValid (Actor|GetComponentbyClass (.HitActor (Collision|BreakHitResult _outhit)) "/Game/VFX_SFX/Blood_Splatter/BPS/BPC_Blood_Effect.BPC_Blood_Effect_C")
                (:Is%20Valid
                  (Default|BloodEffect (Actor|GetComponentbyClass (.HitActor (Collision|BreakHitResult _outhit)) "/Game/VFX_SFX/Blood_Splatter/BPS/BPC_Blood_Effect.BPC_Blood_Effect_C") (.Location (Collision|BreakHitResult _outhit)) (.Normal (Collision|BreakHitResult _outhit)) (.HitActor (Collision|BreakHitResult _outhit)) _damage_2)
                  (Default|BloodEffect (Actor|GetComponentbyClass (.HitActor (Collision|BreakHitResult _outhit)) "/Game/VFX_SFX/Blood_Splatter/BPS/BPC_Blood_Effect.BPC_Blood_Effect_C") (.Location (Collision|BreakHitResult _outhit)) (* (.Normal (Collision|BreakHitResult _outhit)) -1.0) (.HitActor (Collision|BreakHitResult _outhit)) _damage_2))
                (:Is%20Not%20Valid
                  _))
              (Audio|PlaySoundatLocation "/Game/VFX_SFX/Blood_Splatter/Audio/Impact_Audio/Body_Impact_SC.Body_Impact_SC" (.Location (Collision|BreakHitResult _outhit)) "0, 0, 0" 1.0 1.0 0.0 0 0 0 0)))))))
  (bind _returnvalue_11 (Game|SpawnActorfromClass "/Game/VFX_SFX/Realistic_Starter_VFX_Pack_Vol2/Blueprints/Spawn_Particle.Spawn_Particle_C" (Math|Transform|MakeTransform (.location _shoot_transform) (.rotation _shoot_transform) "0.100000,0.100000,0.100000") "Undefined" "MultiplyWithRoot" 0 0.2 false _shootparticle 0))
  (Transformation|AttachComponentToComponent _returnvalue_11 _static_mesh "Shoot_Particle_Socket" "KeepWorld" "KeepWorld" "KeepRelative" true)
  (Audio|PlaySoundatLocation (.Shoot_SC (Utilities|Struct|BreakStruct_Ranged_Weapon_Audio _audio_info)) (.location _shoot_transform) "0, 0, 0" 1.0 1.0 0.0 0 0 0 0)
  (Class|AISenseHearing|ReportNoiseEvent (.location _shoot_transform) 6.0 (Components|GetOwner (Components|GetOwner)) 0.0 "None")
  (if (Utilities|DoesObjectImplementInterface _returnvalue_5 "/Game/Characters/Player/BPI_Player.BPI_Player_C")
    (Default|PlayHitCrosshairAnim (Actor|GetComponentbyClass _returnvalue_5 "/Game/Characters/Player/BPC_HUD.BPC_HUD_C"))))

(fn AimTowardsCrosshair
  (bind _aspawn (Utilities|Casting|CastToPawn (Components|GetOwner (Components|GetOwner))))
  (bind (_outhit _returnvalue) (Collision|LineTraceByChannel (.OutLocation (Actor|GetActorEyesViewPoint _aspawn)) (+ (* (Math|Vector|GetForwardVector (Pawn|GetControlRotation (Pawn|GetController _aspawn) :!class /Script/Engine.Controller)) 5e+04) (.OutLocation (Actor|GetActorEyesViewPoint _aspawn))) "TraceTypeQuery1" false (Utilities|Array|MakeArray (Components|GetOwner) (Components|GetOwner (Components|GetOwner))) (Variables|Default|GetTrace)))
  (return (Math|Vector|SelectVector (.Location (Collision|BreakHitResult _outhit)) (.TraceEnd (Collision|BreakHitResult _outhit)) _returnvalue)))