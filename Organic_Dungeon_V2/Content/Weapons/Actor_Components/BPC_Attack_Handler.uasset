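; Actor component that turns the owning player's attack input into ranged or melee attacks with the equipped weapon.
; Ranged input requires aiming and branches by fire type (semi-auto, full-auto, burst, charge, charge burst), using a delayed-loop macro for bursts.
; Handle Attack checks ammo and passes a DT_Projectiles row to BPC_Shoot, or starts BPC_Melee_Attack.
; Delays toggle CanFire for cooldowns, while Tick also rewrites it from ammo and aim state.
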(event Custom|Handle_Attack
  (bind _returnvalue (Components|GetOwner))
  (bind _returnvalue_2 (Actor|GetComponentbyClass _returnvalue "/Game/Weapons/Actor_Components/BPC_Player_Weaponry.BPC_Player_Weaponry_C"))
  (bind _equipped_weapon (Variables|/Game/Weapons/Actor_Components/BPC_Player_Weaponry.BPC_Player_Weaponry_C|GetEquipped_Weapon _returnvalue_2))
  (if (Utilities|DoesObjectImplementInterface _returnvalue "/Game/Characters/Player/BPI_Player.BPI_Player_C")
    (Utilities|IsValid _equipped_weapon
      (:Is%20Valid
        (bind _basics (Class|BPIWeapon|GetBasicInfo(Message) _equipped_weapon))
        (if (.ranged _basics)
          (if (> (Variables|/Game/Weapons/Actor_Components/BPC_Ammo.BPC_Ammo_C|GetCurrent_Ammo (Actor|GetComponentbyClass _equipped_weapon "/Game/Weapons/Actor_Components/BPC_Ammo.BPC_Ammo_C")) 0)
            (bind _ranged_info (Class|BPIRangedWeapon|GetRangedInfo(Message) _equipped_weapon))
            (bind _returnvalue_3 (Utilities|GetDataTableRow "/Game/Projectiles/Structs_DataTables/DT_Projectiles.DT_Projectiles" (Utilities|String|StringToName (Utilities|String|EnumtoString (.ProjectileName (Utilities|Struct|BreakStruct_Ranged_Weapon _ranged_info)))))
              (:then
                (Variables|Default|SetAttacking false)
                (Default|Shoot (Actor|GetComponentbyClass _equipped_weapon "/Game/Weapons/Actor_Components/BPC_Shoot.BPC_Shoot_C") _returnvalue_3 _ranged_info)
                (if (Utilities|Enum|Equal(Enum) (.Fire_Type (Utilities|Struct|BreakStruct_Ranged_Weapon _ranged_info)) "NewEnumerator2")
                  (Variables|Default|SetCan_Fire false)
                  (Utilities|FlowControl|Delay (Utilities|Struct|BreakStruct_Full_Auto_Info (.Full_Auto_Info (Utilities|Struct|BreakStruct_Ranged_Weapon _ranged_info))))
                  (Variables|Default|SetCan_Fire true)))
              (:RowNotFound
                (Development|PrintString "Projectile row not found"))))
          (else
            (Default|StartMeleeAttack (Actor|GetComponentbyClass _equipped_weapon "/Game/Weapons/Actor_Components/BPC_Melee_Attack.BPC_Melee_Attack_C"))))))))

(event Custom|End_Melee_Attack
  (Default|MeleeAttackEnd (Actor|GetComponentbyClass (Variables|/Game/Weapons/Actor_Components/BPC_Player_Weaponry.BPC_Player_Weaponry_C|GetEquipped_Weapon (Actor|GetComponentbyClass (Components|GetOwner) "/Game/Weapons/Actor_Components/BPC_Player_Weaponry.BPC_Player_Weaponry_C")) "/Game/Weapons/Actor_Components/BPC_Melee_Attack.BPC_Melee_Attack_C")))

(event Input|EnhancedActionEvents|EnhancedInputActionIA_Attack
  (params (ActionValue :type Boolean) (ElapsedSeconds :type Float%20%28double-precision%29) (TriggeredSeconds :type Float%20%28double-precision%29) (InputAction :type Input%20Action%20Object%20Reference :default "/Game/Characters/Player/Input/Actions/IA_Attack.IA_Attack"))
  (bind _returnvalue (Components|GetOwner))
  (bind _returnvalue_2 (Actor|GetComponentbyClass _returnvalue "/Game/Weapons/Actor_Components/BPC_Player_Weaponry.BPC_Player_Weaponry_C"))
  (bind _equipped_weapon (Variables|/Game/Weapons/Actor_Components/BPC_Player_Weaponry.BPC_Player_Weaponry_C|GetEquipped_Weapon _returnvalue_2))
  (bind _returnvalue_3 (Actor|GetComponentbyClass _equipped_weapon "/Game/Weapons/Actor_Components/BPC_Ammo.BPC_Ammo_C"))
  (:Triggered
    (bind _basics (Class|BPIWeapon|GetBasicInfo(Message) (Variables|/Game/Weapons/Actor_Components/BPC_Player_Weaponry.BPC_Player_Weaponry_C|GetEquipped_Weapon (Actor|GetComponentbyClass (Components|GetOwner) "/Game/Weapons/Actor_Components/BPC_Player_Weaponry.BPC_Player_Weaponry_C"))))
    (if (.ranged _basics)
      (if (Math|Boolean|ANDBoolean (not (Variables|Default|GetAttacking)) (Variables|Default|GetCan_Fire) (Variables|/Game/Weapons/Actor_Components/BPC_Aim.BPC_Aim_C|GetAiming? (Actor|GetComponentbyClass (Components|GetOwner) "/Game/Weapons/Actor_Components/BPC_Aim.BPC_Aim_C")))
        (bind _ranged_info (Class|BPIRangedWeapon|GetRangedInfo(Message) (Variables|/Game/Weapons/Actor_Components/BPC_Player_Weaponry.BPC_Player_Weaponry_C|GetEquipped_Weapon (Actor|GetComponentbyClass (Components|GetOwner) "/Game/Weapons/Actor_Components/BPC_Player_Weaponry.BPC_Player_Weaponry_C"))))
        (switch Utilities|FlowControl|Switch|SwitchonEnum_Fire_Types (.fire_type _ranged_info)
          (:NewEnumerator1
            (Utilities|FlowControl|DoOnce false :!label _label
              (:Completed
                (Development|PrintString "HANDLING ATTACK FROM STARTED")
                (CallFunction|HandleAttack)
                (if (and (Utilities|DoesObjectImplementInterface _returnvalue "/Game/Characters/Player/BPI_Player.BPI_Player_C") (Variables|/Game/Weapons/Actor_Components/BPC_Ammo.BPC_Ammo_C|GetReloading _returnvalue_3)) :!label _label_2
                  (Default|StopReload _returnvalue_3)))))
          (:NewEnumerator2
            (if (Variables|Default|GetCan_Fire)
              (Development|PrintString "HANDLING ATTACK FROM TRIGGERED")
              (CallFunction|HandleAttack)
              (goto _label_2)))
          (:NewEnumerator3
            (if (Variables|Default|GetCan_Fire)
              (Variables|Default|SetCan_Fire false)
              (Utilities|BurstLoopDelayFire 1 (._Burst_Projectiles (Utilities|Struct|BreakStruct_Burst_Info (.burst_info _ranged_info))) (.Time_Between_Burst_Rounds (Utilities|Struct|BreakStruct_Burst_Info (.burst_info _ranged_info)))
                (:Loop%20Body
                  (CallFunction|HandleAttack)
                  (goto _label_2))
                (:Completed
                  (Utilities|FlowControl|Delay (.Time_Between_Bursts (Utilities|Struct|BreakStruct_Burst_Info (.burst_info _ranged_info))))
                  (Variables|Default|SetCan_Fire true)))))
          (:NewEnumerator4
            (if (>= TriggeredSeconds (.Charge_Time (Utilities|Struct|BreakStruct_Charge_Info (.charged_info _ranged_info))))
              (Variables|Default|SetCan_Fire false)
              (CallFunction|HandleAttack)
              (Utilities|FlowControl|Sequence
                (:then_0
                  (goto _label_2))
                (:then_1
                  (Utilities|FlowControl|Delay (.Recharge_Time (Utilities|Struct|BreakStruct_Charge_Info (.charged_info _ranged_info))))
                  (Variables|Default|SetCan_Fire true)))))
          (:NewEnumerator5
            (Development|PrintString (Utilities|String|ToString(Float) TriggeredSeconds))
            (if (>= TriggeredSeconds (.Charge_Time (Utilities|Struct|BreakStruct_Charged_Burst_Info (.charged_burst_info _ranged_info))))
              (Variables|Default|SetCan_Fire false)
              (Utilities|BurstLoopDelayFire 1 (._Burst_Projectiles (Utilities|Struct|BreakStruct_Charged_Burst_Info (.charged_burst_info _ranged_info))) (.Time_Between_Burst_Shots (Utilities|Struct|BreakStruct_Charged_Burst_Info (.charged_burst_info _ranged_info)))
                (:Loop%20Body
                  (CallFunction|HandleAttack))
                (:Completed
                  (Utilities|FlowControl|Delay (.Charge_Cooldown (Utilities|Struct|BreakStruct_Charged_Burst_Info (.charged_burst_info _ranged_info))))
                  (Variables|Default|SetCan_Fire true)))))))
      (elif (not (Variables|Default|GetAttacking))
        (CallFunction|HandleAttack))))
  (:Canceled
    (if (.ranged _basics) :!label _label_3
      (goto _label Reset)))
  (:Completed
    (goto _label_3)))

(event EventTick
  (params (DeltaSeconds :type Float%20%28single-precision%29))
  (bind _returnvalue (Components|GetOwner))
  (bind _returnvalue_2 (Actor|GetComponentbyClass _returnvalue "/Game/Weapons/Actor_Components/BPC_Player_Weaponry.BPC_Player_Weaponry_C"))
  (bind _equipped_weapon (Variables|/Game/Weapons/Actor_Components/BPC_Player_Weaponry.BPC_Player_Weaponry_C|GetEquipped_Weapon _returnvalue_2))
  (if (Utilities|IsValid _equipped_weapon)
    (Variables|Default|SetCan_Fire (and (> (Variables|/Game/Weapons/Actor_Components/BPC_Ammo.BPC_Ammo_C|GetCurrent_Ammo (Actor|GetComponentbyClass _equipped_weapon "/Game/Weapons/Actor_Components/BPC_Ammo.BPC_Ammo_C")) 0) (Variables|/Game/Weapons/Actor_Components/BPC_Aim.BPC_Aim_C|GetAiming? (Actor|GetComponentbyClass _returnvalue "/Game/Weapons/Actor_Components/BPC_Aim.BPC_Aim_C"))))))