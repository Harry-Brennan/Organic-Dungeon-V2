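; Actor component that gives its owning actor a spinning, vertically bobbing animation, started on BeginPlay and switchable through Start and Stop events that toggle its tick.
; Each tick advances the yaw using FInterpTo toward a target always 180 degrees ahead, scaled by RotateRate.
; A ping-pong percentage between -1 and 1, stepped by VerticalTime and the tick interval instead of delta time, drives an extrapolating Lerp around the starting height.
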(event Custom|Start_Animated_Rotation
  (Variables|Default|SetStartZ (.z (Transformation|GetActorLocation (Components|GetOwner))))
  (Variables|Default|SetTargetZ (+ (Variables|Default|GetStartZ) (/ (Variables|Default|GetVertical_Range) 2.0)))
  (Components|Tick|SetComponentTickEnabled true))

(event Custom|Stop_Animated_Rotation
  (Components|Tick|SetComponentTickEnabled false))

(event EventTick
  (params (DeltaSeconds :type Float%20%28single-precision%29))
  (bind _returnvalue (Components|GetOwner))
  (bind _returnvalue_2 (Class|ActorComponent|GetComponentTickInterval))
  (bind _returnvalue_3 (Components|GetOwner))
  (bind _vertical_time (Variables|Default|GetVertical_Time))
  (bind _returnvalue_4 (Transformation|GetActorLocation _returnvalue))
  (bind _returnvalue_5 (Transformation|GetActorRotation _returnvalue_3))
  (bind _returnvalue_6 (/ _vertical_time _returnvalue_2))
  (bind _returnvalue_7 (/ 2.0 _returnvalue_6))
  (Transformation|SetActorRotation (Components|GetOwner) (Math|Rotator|MakeRotator (.roll _returnvalue_5) (.pitch _returnvalue_5) (Math|Interpolation|FInterpTo (.yaw _returnvalue_5) (+ (.yaw _returnvalue_5) 1.8e+02) DeltaSeconds (Variables|Default|GetRotateRate))))
  (Utilities|FlowControl|Sequence
    (:then_0
      (if (and (>= (Variables|Default|GetVertical_Percent) 1.0) (Variables|Default|GetDirection))
        (Variables|Default|SetDirection false)
        (elif (and (<= (Variables|Default|GetVertical_Percent) -1.0) (not (Variables|Default|GetDirection)))
          (Variables|Default|SetDirection true))))
    (:then_1
      (Variables|Default|SetVertical_Percent (Math|Float|SelectFloat (+ (Variables|Default|GetVertical_Percent) _returnvalue_7) (- (Variables|Default|GetVertical_Percent) _returnvalue_7) (Variables|Default|GetDirection)))
      (Transformation|SetActorLocation (Components|GetOwner) (Math|Vector|MakeVector (.x _returnvalue_4) (.y _returnvalue_4) (Math|Float|Lerp (Variables|Default|GetStartZ) (Variables|Default|GetTargetZ) (Variables|Default|GetVertical_Percent))) false false))))

(event EventBeginPlay
  (CallFunction|StartAnimatedRotation))