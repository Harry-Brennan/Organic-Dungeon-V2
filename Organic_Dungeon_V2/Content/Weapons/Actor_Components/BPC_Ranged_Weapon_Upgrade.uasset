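; Actor component that upgrades one chosen area of its owning ranged weapon's stats.
; Upgrade reads the weapon's info by message, rebuilds the struct through a Select that swaps in only that area, and writes it back.
; Explosion on Hit upgrades also override the on-hit effect with a fixed enum value.
; Ammo upgrades refresh BPC_Ammo's max, projectile upgrades send a custom-projectile update, and every upgrade sends a custom-weapon update.
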(event Custom|Upgrade
  (params (Upgrade%20Area :type Enum_Ranged_Info_Options%20Enum :default "NewEnumerator0") (New%20Info :type Struct%20Ranged%20Weapon%20Structure))
  (bind _returnvalue (Components|GetOwner))
  (bind _returnvalue_2 (Components|GetOwner))
  (Utilities|UpdateRangedInfo (Components|GetOwner) Upgrade%20Area New%20Info)
  (switch Utilities|FlowControl|Switch|SwitchonEnum_Ranged_Info_Options Upgrade%20Area
    (:NewEnumerator0
      (bind _ranged_info (Class|BPIRangedWeapon|GetRangedInfo(Message) _returnvalue_2))
      (Default|UpdateMaxAmmo (Actor|GetComponentbyClass _returnvalue_2 "/Game/Weapons/Actor_Components/BPC_Ammo.BPC_Ammo_C") (.starting_ammo _ranged_info)))
    (:NewEnumerator1
      _)
    (:NewEnumerator2
      _)
    (:NewEnumerator3
      (Class|BPIWeapon|UpdateCustomProjectile(Message) _returnvalue true :!label _label))
    (:NewEnumerator4
      (goto _label))
    (:NewEnumerator5
      (goto _label))
    (:NewEnumerator6
      (goto _label))
    (:NewEnumerator7
      (goto _label))
    (:NewEnumerator16
      _)
    (:NewEnumerator12
      _)
    (:NewEnumerator11
      _)
    (:NewEnumerator13
      _)
    (:NewEnumerator14
      _)
    (:NewEnumerator15
      _)
    (:NewEnumerator17
      _)
    (:NewEnumerator20
      _)
    (:NewEnumerator18
      _)
    (:NewEnumerator19
      _))
  (Class|BPIWeapon|UpdateCustomWeapon(Message) _returnvalue true))

(fn UpdateRangedInfo
  (params (New%20Info :type Struct%20Ranged%20Weapon%20Structure) (Old%20Info :type Struct%20Ranged%20Weapon%20Structure) (Info%20To%20Change :type Enum_Ranged_Info_Options%20Enum :default "NewEnumerator0"))
  (bind (_starting_ammo _crosshair _reload_info _projectilename _projectile_info _recoil _hitscan _piercing _shootparticle __projectiles _spread _fire_type _burst_info _full_auto_info _charged_info _charged_burst_info) (Utilities|Struct|BreakStruct_Ranged_Weapon New%20Info))
  (bind (_starting_ammo_2 _crosshair_2 _reload_info_2 _projectilename_2 _projectile_info_2 _recoil_2 _hitscan_2 _piercing_2 _shootparticle_2 __projectiles_2 _spread_2 _fire_type_2 _burst_info_2 _full_auto_info_2 _charged_info_2 _charged_burst_info_2 _audio_info) (Utilities|Struct|BreakStruct_Ranged_Weapon Old%20Info))
  (bind (_starting_ammo_3 _crosshair_3 _reload_info_3 _projectilename_3 _projectile_info_3 _recoil_3 _hitscan_3 _piercing_3 _shootparticle_3 __projectiles_3 _spread_3 _fire_type_3 _burst_info_3 _full_auto_info_3 _charged_info_3 _charged_burst_info_3 _audio_info_2) (Utilities|Struct|BreakStruct_Ranged_Weapon Old%20Info))
  (bind (_starting_ammo_4 _crosshair_4 _reload_info_4 _projectilename_4 _projectile_info_4 _recoil_4 _hitscan_4 _piercing_4 _shootparticle_4 __projectiles_4 _spread_4 _fire_type_4 _burst_info_4 _full_auto_info_4 _charged_info_4 _charged_burst_info_4 _audio_info_3) (Utilities|Struct|BreakStruct_Ranged_Weapon Old%20Info))
  (bind (_starting_ammo_5 _crosshair_5 _reload_info_5 _projectilename_5 _projectile_info_5 _recoil_5 _hitscan_5 _piercing_5 _shootparticle_5 __projectiles_5 _spread_5 _fire_type_5 _burst_info_5 _full_auto_info_5 _charged_info_5 _charged_burst_info_5 _audio_info_4) (Utilities|Struct|BreakStruct_Ranged_Weapon Old%20Info))
  (bind (_starting_ammo_6 _crosshair_6 _reload_info_6 _projectilename_6 _projectile_info_6 _recoil_6 _hitscan_6 _piercing_6 _shootparticle_6 __projectiles_6 _spread_6 _fire_type_6 _burst_info_6 _full_auto_info_6 _charged_info_6 _charged_burst_info_6 _audio_info_5) (Utilities|Struct|BreakStruct_Ranged_Weapon Old%20Info))
  (bind (_starting_ammo_7 _crosshair_7 _reload_info_7 _projectilename_7 _projectile_info_7 _recoil_7 _hitscan_7 _piercing_7 _shootparticle_7 __projectiles_7 _spread_7 _fire_type_7 _burst_info_7 _full_auto_info_7 _charged_info_7 _charged_burst_info_7 _audio_info_6) (Utilities|Struct|BreakStruct_Ranged_Weapon Old%20Info))
  (bind (_starting_ammo_8 _crosshair_8 _reload_info_8 _projectilename_8 _projectile_info_8 _recoil_8 _hitscan_8 _piercing_8 _shootparticle_8 __projectiles_8 _spread_8 _fire_type_8 _burst_info_8 _full_auto_info_8 _charged_info_8 _charged_burst_info_8 _audio_info_7) (Utilities|Struct|BreakStruct_Ranged_Weapon Old%20Info))
  (bind (_starting_ammo_9 _crosshair_9 _reload_info_9 _projectilename_9 _projectile_info_9 _recoil_9 _hitscan_9 _piercing_9 _shootparticle_9 __projectiles_9 _spread_9 _fire_type_9 _burst_info_9 _full_auto_info_9 _charged_info_9 _charged_burst_info_9 _audio_info_8) (Utilities|Struct|BreakStruct_Ranged_Weapon Old%20Info))
  (bind (_starting_ammo_10 _crosshair_10 _reload_info_10 _projectilename_10 _projectile_info_10 _recoil_10 _hitscan_10 _piercing_10 _shootparticle_10 __projectiles_10 _spread_10 _fire_type_10 _burst_info_10 _full_auto_info_10 _charged_info_10 _charged_burst_info_10 _audio_info_9) (Utilities|Struct|BreakStruct_Ranged_Weapon Old%20Info))
  (bind (_starting_ammo_11 _crosshair_11 _reload_info_11 _projectilename_11 _projectile_info_11 _recoil_11 _hitscan_11 _piercing_11 _shootparticle_11 __projectiles_11 _spread_11 _fire_type_11 _burst_info_11 _full_auto_info_11 _charged_info_11 _charged_burst_info_11 _audio_info_10) (Utilities|Struct|BreakStruct_Ranged_Weapon Old%20Info))
  (bind (_starting_ammo_12 _crosshair_12 _reload_info_12 _projectilename_12 _projectile_info_12 _recoil_12 _hitscan_12 _piercing_12 _shootparticle_12 __projectiles_12 _spread_12 _fire_type_12 _burst_info_12 _full_auto_info_12 _charged_info_12 _charged_burst_info_12 _audio_info_11) (Utilities|Struct|BreakStruct_Ranged_Weapon Old%20Info))
  (bind (_starting_ammo_13 _crosshair_13 _reload_info_13 _projectilename_13 _projectile_info_13 _recoil_13 _hitscan_13 _piercing_13 _shootparticle_13 __projectiles_13 _spread_13 _fire_type_13 _burst_info_13 _full_auto_info_13 _charged_info_13 _charged_burst_info_13 _audio_info_12) (Utilities|Struct|BreakStruct_Ranged_Weapon Old%20Info))
  (bind (_starting_ammo_14 _crosshair_14 _reload_info_14 _projectilename_14 _projectile_info_14 _recoil_14 _hitscan_14 _piercing_14 _shootparticle_14 __projectiles_14 _spread_14 _fire_type_14 _burst_info_14 _full_auto_info_14 _charged_info_14 _charged_burst_info_14 _audio_info_13) (Utilities|Struct|BreakStruct_Ranged_Weapon Old%20Info))
  (bind (_starting_ammo_15 _crosshair_15 _reload_info_15 _projectilename_15 _projectile_info_15 _recoil_15 _hitscan_15 _piercing_15 _shootparticle_15 __projectiles_15 _spread_15 _fire_type_15 _burst_info_15 _full_auto_info_15 _charged_info_15 _charged_burst_info_15 _audio_info_14) (Utilities|Struct|BreakStruct_Ranged_Weapon Old%20Info))
  (bind (_starting_ammo_16 _crosshair_16 _reload_info_16 _projectilename_16 _projectile_info_16 _recoil_16 _hitscan_16 _piercing_16 _shootparticle_16 __projectiles_16 _spread_16 _fire_type_16 _burst_info_16 _full_auto_info_16 _charged_info_16 _charged_burst_info_16 _audio_info_15) (Utilities|Struct|BreakStruct_Ranged_Weapon Old%20Info))
  (bind (_starting_ammo_17 _crosshair_17 _reload_info_17 _projectilename_17 _projectile_info_17 _recoil_17 _hitscan_17 _piercing_17 _shootparticle_17 __projectiles_17 _spread_17 _fire_type_17 _burst_info_17 _full_auto_info_17 _charged_info_17 _charged_burst_info_17 _audio_info_16) (Utilities|Struct|BreakStruct_Ranged_Weapon Old%20Info))
  (bind (_starting_ammo_18 _crosshair_18 _reload_info_18 _projectilename_18 _projectile_info_18 _recoil_18 _hitscan_18 _piercing_18 _shootparticle_18 __projectiles_18 _spread_18 _fire_type_18 _burst_info_18 _full_auto_info_18 _charged_info_18 _charged_burst_info_18 _audio_info_17) (Utilities|Struct|BreakStruct_Ranged_Weapon Old%20Info))
  (bind (_starting_ammo_19 _crosshair_19 _reload_info_19 _projectilename_19 _projectile_info_19 _recoil_19 _hitscan_19 _piercing_19 _shootparticle_19 __projectiles_19 _spread_19 _fire_type_19 _burst_info_19 _full_auto_info_19 _charged_info_19 _charged_burst_info_19 _audio_info_18) (Utilities|Struct|BreakStruct_Ranged_Weapon Old%20Info))
  (bind (_name _damage _speed _gravity _mesh) (Utilities|Struct|BreakStruct_Projectiles _projectile_info_2))
  (bind (_name_2 _damage_2 _speed_2 _gravity_2 _mesh_2 _onhiteffect _explosiononhit) (Utilities|Struct|BreakStruct_Projectiles _projectile_info_3))
  (bind (_name_3 _damage_3 _speed_3 _gravity_3 _mesh_3 _onhiteffect_2 _explosiononhit_2) (Utilities|Struct|BreakStruct_Projectiles _projectile_info_4))
  (bind (_name_4 _damage_4 _speed_4 _gravity_4 _mesh_4 _onhiteffect_3 _explosiononhit_3) (Utilities|Struct|BreakStruct_Projectiles _projectile_info_5))
  (bind (_recoil_amount _recoil_duration _recoil_knockback) (Utilities|Struct|BreakStruct_Recoil_Info _recoil))
  (bind (_reload_type _reload_time) (Utilities|Struct|BreakStruct_Reload_Info _reload_info))
  (bind (_name_5 _damage_5 _speed_5 _gravity_5 _mesh_5 _onhiteffect_4 _explosiononhit_4) (Utilities|Struct|BreakStruct_Projectiles _projectile_info))
  (bind (_explosionradius _knockbackamount) (Utilities|Struct|BreakStruct_Explosion_On_Hit _explosiononhit_4))
  (return (Utilities|Select :Index Info%20To%20Change :NewEnumerator0 (Utilities|Struct|MakeStruct_Ranged_Weapon _starting_ammo _crosshair_7 _reload_info_7 _projectilename_7 _projectile_info_7 _recoil_7 _hitscan_7 _piercing_7 _shootparticle_7 __projectiles_7 _spread_7 _fire_type_7 _burst_info_7 _full_auto_info_7 _charged_info_7 _charged_burst_info_7 _audio_info_6) :NewEnumerator1 (Utilities|Struct|MakeStruct_Ranged_Weapon _starting_ammo_17 _crosshair_17 (Utilities|Struct|MakeStruct_Reload_Info _reload_type (.Reload_Time (Utilities|Struct|BreakStruct_Reload_Info _reload_info_17)) 0) _projectilename_17 _projectile_info_17 _recoil_17 _hitscan_17 _piercing_17 _shootparticle_17 __projectiles_17 _spread_17 _fire_type_17 _burst_info_17 _full_auto_info_17 _charged_info_17 _charged_burst_info_17 _audio_info_16) :NewEnumerator2 (Utilities|Struct|MakeStruct_Ranged_Weapon _starting_ammo_18 _crosshair_18 (Utilities|Struct|MakeStruct_Reload_Info (.Reload_Type (Utilities|Struct|BreakStruct_Reload_Info _reload_info_18)) _reload_time 0) _projectilename_18 _projectile_info_18 _recoil_18 _hitscan_18 _piercing_18 _shootparticle_18 __projectiles_18 _spread_18 _fire_type_18 _burst_info_18 _full_auto_info_18 _charged_info_18 _charged_burst_info_18 _audio_info_17) :NewEnumerator3 (Utilities|Struct|MakeStruct_Ranged_Weapon _starting_ammo_6 _crosshair_6 _reload_info_6 _projectilename _projectile_info_6 _recoil_6 _hitscan_6 _piercing_6 _shootparticle_6 __projectiles_6 _spread_6 _fire_type_6 _burst_info_6 _full_auto_info_6 _charged_info_6 _charged_burst_info_6 _audio_info_5) :NewEnumerator4 (Utilities|Struct|MakeStruct_Ranged_Weapon _starting_ammo_3 _crosshair_3 _reload_info_3 _projectilename_3 (Utilities|Struct|MakeStruct_Projectiles _name_2 _damage_5 _speed_2 0.75 _mesh_2 _onhiteffect _explosiononhit) _recoil_3 _hitscan_3 _piercing_3 _shootparticle_3 __projectiles_3 _spread_3 _fire_type_3 _burst_info_3 _full_auto_info_3 _charged_info_3 _charged_burst_info_3 _audio_info_2) :NewEnumerator5 (Utilities|Struct|MakeStruct_Ranged_Weapon _starting_ammo_4 _crosshair_4 _reload_info_4 _projectilename_4 (Utilities|Struct|MakeStruct_Projectiles _name_3 _damage_3 _speed_5 0.75 _mesh_3 _onhiteffect_2 _explosiononhit_2) _recoil_4 _hitscan_4 _piercing_4 _shootparticle_4 __projectiles_4 _spread_4 _fire_type_4 _burst_info_4 _full_auto_info_4 _charged_info_4 _charged_burst_info_4 _audio_info_3) :NewEnumerator6 (Utilities|Struct|MakeStruct_Ranged_Weapon _starting_ammo_5 _crosshair_5 _reload_info_5 _projectilename_5 (Utilities|Struct|MakeStruct_Projectiles _name_4 _damage_4 _speed_4 0.75 _mesh_4 _onhiteffect_4 _explosiononhit_3) _recoil_5 _hitscan_5 _piercing_5 _shootparticle_5 __projectiles_5 _spread_5 _fire_type_5 _burst_info_5 _full_auto_info_5 _charged_info_5 _charged_burst_info_5 _audio_info_4) :NewEnumerator7 (Utilities|Struct|MakeStruct_Ranged_Weapon _starting_ammo_2 _crosshair_2 _reload_info_2 _projectilename_2 (Utilities|Struct|MakeStruct_Projectiles _name _damage _speed 0.75 _mesh "NewEnumerator1" (Utilities|Struct|MakeStruct_Explosion_On_Hit _explosionradius _knockbackamount)) _recoil_2 _hitscan_2 _piercing_2 _shootparticle_2 __projectiles_2 _spread_2 _fire_type_2 _burst_info_2 _full_auto_info_2 _charged_info_2 _charged_burst_info_2 _audio_info) :NewEnumerator16 (Utilities|Struct|MakeStruct_Ranged_Weapon _starting_ammo_8 _crosshair_8 _reload_info_8 _projectilename_8 _projectile_info_8 (Utilities|Struct|MakeStruct_Recoil_Info _recoil_amount _recoil_duration _recoil_knockback) _hitscan_8 _piercing_8 _shootparticle_8 __projectiles_8 _spread_8 _fire_type_8 _burst_info_8 _full_auto_info_8 _charged_info_8 _charged_burst_info_8 _audio_info_7) :NewEnumerator12 (Utilities|Struct|MakeStruct_Ranged_Weapon _starting_ammo_9 _crosshair_9 _reload_info_9 _projectilename_9 _projectile_info_9 _recoil_9 _hitscan _piercing_9 _shootparticle_9 __projectiles_9 _spread_9 _fire_type_9 _burst_info_9 _full_auto_info_9 _charged_info_9 _charged_burst_info_9 _audio_info_8) :NewEnumerator11 (Utilities|Struct|MakeStruct_Ranged_Weapon _starting_ammo_10 _crosshair_10 _reload_info_10 _projectilename_10 _projectile_info_10 _recoil_10 _hitscan_10 _piercing _shootparticle_10 __projectiles_10 _spread_10 _fire_type_10 _burst_info_10 _full_auto_info_10 _charged_info_10 _charged_burst_info_10 _audio_info_9) :NewEnumerator13 (Utilities|Struct|MakeStruct_Ranged_Weapon _starting_ammo_11 _crosshair_11 _reload_info_11 _projectilename_11 _projectile_info_11 _recoil_11 _hitscan_11 _piercing_11 _shootparticle_11 __projectiles _spread_11 _fire_type_11 _burst_info_11 _full_auto_info_11 _charged_info_11 _charged_burst_info_11 _audio_info_10) :NewEnumerator14 (Utilities|Struct|MakeStruct_Ranged_Weapon _starting_ammo_12 _crosshair_12 _reload_info_12 _projectilename_12 _projectile_info_12 _recoil_12 _hitscan_12 _piercing_12 _shootparticle_12 __projectiles_12 _spread _fire_type_12 _burst_info_12 _full_auto_info_12 _charged_info_12 _charged_burst_info_12 _audio_info_11) :NewEnumerator15 (Utilities|Struct|MakeStruct_Ranged_Weapon _starting_ammo_13 _crosshair_13 _reload_info_13 _projectilename_13 _projectile_info_13 _recoil_13 _hitscan_13 _piercing_13 _shootparticle_13 __projectiles_13 _spread_13 _fire_type _burst_info_13 _full_auto_info_13 _charged_info_13 _charged_burst_info_13 _audio_info_12) :NewEnumerator17 (Utilities|Struct|MakeStruct_Ranged_Weapon _starting_ammo_14 _crosshair_14 _reload_info_14 _projectilename_14 _projectile_info_14 _recoil_14 _hitscan_14 _piercing_14 _shootparticle_14 __projectiles_14 _spread_14 _fire_type_14 _burst_info _full_auto_info_14 _charged_info_14 _charged_burst_info_14 _audio_info_13) :NewEnumerator20 (Utilities|Struct|MakeStruct_Ranged_Weapon _starting_ammo_15 _crosshair_15 _reload_info_15 _projectilename_15 _projectile_info_15 _recoil_15 _hitscan_15 _piercing_15 _shootparticle_15 __projectiles_15 _spread_15 _fire_type_15 _burst_info_15 _full_auto_info _charged_info_15 _charged_burst_info_15 _audio_info_14) :NewEnumerator18 (Utilities|Struct|MakeStruct_Ranged_Weapon _starting_ammo_16 _crosshair_16 _reload_info_16 _projectilename_16 _projectile_info_16 _recoil_16 _hitscan_16 _piercing_16 _shootparticle_16 __projectiles_16 _spread_16 _fire_type_16 _burst_info_16 _full_auto_info_16 _charged_info _charged_burst_info_16 _audio_info_15) :NewEnumerator19 (Utilities|Struct|MakeStruct_Ranged_Weapon _starting_ammo_19 _crosshair_19 _reload_info_19 _projectilename_19 _projectile_info_19 _recoil_19 _hitscan_19 _piercing_19 _shootparticle_19 __projectiles_19 _spread_19 _fire_type_19 _burst_info_19 _full_auto_info_19 _charged_info_19 _charged_burst_info _audio_info_18))))