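; Actor component that spawns its owner's starting weapons and starter weapon as BP_Weapon actors in BPC_Weaponry.
; After a short BeginPlay delay, if the owner has a starter weapon, it adds them all, equips the starter, then cycles next and previous.
; A separate Updating_Weapons event rebuilds the owner's weapon structs through interface messages, filling non-custom weapons and projectile data from name-keyed DataTables.
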(event Custom|Updating_Weapons
  (Utilities|FlowControl|Sequence
    (:then_0
      (bind _starting_weapons (Class|BPICanHaveWeapon|GetStartingWeapons(Message) (Components|GetOwner)))
      (for (_array_element _array_index) _starting_weapons
        (Utilities|FlowControl|Sequence
          (:then_0
            (if (not (.CustomWeapon (Utilities|Struct|BreakStruct_Spawnable_Weapon _array_element)))
              (CallFunction|UpdateNonCustomWeaponInfo _array_element _array_index false)))
          (:then_1
            (if (.CustomProjectile (Utilities|Struct|BreakStruct_Spawnable_Weapon _array_element))
              (bind _returnvalue (Utilities|GetDataTableRow "/Game/Projectiles/Structs_DataTables/DT_Projectiles.DT_Projectiles" (Utilities|String|StringToName (Utilities|String|EnumtoString (.Name (Utilities|Struct|BreakStruct_Projectiles (.Projectile_Info (Utilities|Struct|BreakStruct_Ranged_Weapon (.Ranged_Info (Utilities|Struct|BreakStruct_Spawnable_Weapon _array_element)))))))))
                (:then
                  _)
                (:RowNotFound
                  _))
              (Class|BPICanHaveWeapon|SetStartingWeaponsIndex(Message) (Components|GetOwner) (Utilities|Struct|MakeStruct_Spawnable_Weapon (.CustomWeapon (Utilities|Struct|BreakStruct_Spawnable_Weapon _array_element)) (select (.CustomWeapon (Utilities|Struct|BreakStruct_Spawnable_Weapon _array_element)) true false) (.Base_Info (Utilities|Struct|BreakStruct_Spawnable_Weapon _array_element)) (Utilities|Struct|MakeStruct_Ranged_Weapon (.Starting_Ammo (Utilities|Struct|BreakStruct_Ranged_Weapon (.Ranged_Info (Utilities|Struct|BreakStruct_Spawnable_Weapon _array_element)))) (.Crosshair (Utilities|Struct|BreakStruct_Ranged_Weapon (.Ranged_Info (Utilities|Struct|BreakStruct_Spawnable_Weapon _array_element)))) (.Reload_Info (Utilities|Struct|BreakStruct_Ranged_Weapon (.Ranged_Info (Utilities|Struct|BreakStruct_Spawnable_Weapon _array_element)))) (.ProjectileName (Utilities|Struct|BreakStruct_Ranged_Weapon (.Ranged_Info (Utilities|Struct|BreakStruct_Spawnable_Weapon _array_element)))) (Utilities|Struct|MakeStruct_Projectiles (.Name (Utilities|Struct|BreakStruct_Projectiles _returnvalue)) (.Damage (Utilities|Struct|BreakStruct_Projectiles (.Projectile_Info (Utilities|Struct|BreakStruct_Ranged_Weapon (.Ranged_Info (Utilities|Struct|BreakStruct_Spawnable_Weapon _array_element)))))) (.Speed (Utilities|Struct|BreakStruct_Projectiles (.Projectile_Info (Utilities|Struct|BreakStruct_Ranged_Weapon (.Ranged_Info (Utilities|Struct|BreakStruct_Spawnable_Weapon _array_element)))))) (.Gravity (Utilities|Struct|BreakStruct_Projectiles (.Projectile_Info (Utilities|Struct|BreakStruct_Ranged_Weapon (.Ranged_Info (Utilities|Struct|BreakStruct_Spawnable_Weapon _array_element)))))) (.Mesh (Utilities|Struct|BreakStruct_Projectiles _returnvalue)) (.OnHitEffect (Utilities|Struct|BreakStruct_Projectiles (.Projectile_Info (Utilities|Struct|BreakStruct_Ranged_Weapon (.Ranged_Info (Utilities|Struct|BreakStruct_Spawnable_Weapon _array_element)))))) (.ExplosionOnHit (Utilities|Struct|BreakStruct_Projectiles (.Projectile_Info (Utilities|Struct|BreakStruct_Ranged_Weapon (.Ranged_Info (Utilities|Struct|BreakStruct_Spawnable_Weapon _array_element))))))) (.Recoil (Utilities|Struct|BreakStruct_Ranged_Weapon (.Ranged_Info (Utilities|Struct|BreakStruct_Spawnable_Weapon _array_element)))) (.HitScan (Utilities|Struct|BreakStruct_Ranged_Weapon (.Ranged_Info (Utilities|Struct|BreakStruct_Spawnable_Weapon _array_element)))) (.Piercing (Utilities|Struct|BreakStruct_Ranged_Weapon (.Ranged_Info (Utilities|Struct|BreakStruct_Spawnable_Weapon _array_element)))) (.ShootParticle (Utilities|Struct|BreakStruct_Ranged_Weapon (.Ranged_Info (Utilities|Struct|BreakStruct_Spawnable_Weapon _array_element)))) (._Projectiles (Utilities|Struct|BreakStruct_Ranged_Weapon (.Ranged_Info (Utilities|Struct|BreakStruct_Spawnable_Weapon _array_element)))) (.Spread (Utilities|Struct|BreakStruct_Ranged_Weapon (.Ranged_Info (Utilities|Struct|BreakStruct_Spawnable_Weapon _array_element)))) (.Fire_Type (Utilities|Struct|BreakStruct_Ranged_Weapon (.Ranged_Info (Utilities|Struct|BreakStruct_Spawnable_Weapon _array_element)))) (.Burst_Info (Utilities|Struct|BreakStruct_Ranged_Weapon (.Ranged_Info (Utilities|Struct|BreakStruct_Spawnable_Weapon _array_element)))) (.Full_Auto_Info (Utilities|Struct|BreakStruct_Ranged_Weapon (.Ranged_Info (Utilities|Struct|BreakStruct_Spawnable_Weapon _array_element)))) (.Charged_Info (Utilities|Struct|BreakStruct_Ranged_Weapon (.Ranged_Info (Utilities|Struct|BreakStruct_Spawnable_Weapon _array_element)))) (.Charged_Burst_Info (Utilities|Struct|BreakStruct_Ranged_Weapon (.Ranged_Info (Utilities|Struct|BreakStruct_Spawnable_Weapon _array_element)))) (.Audio_Info (Utilities|Struct|BreakStruct_Ranged_Weapon (.Ranged_Info (Utilities|Struct|BreakStruct_Spawnable_Weapon _array_element))))) (.Melee_Info (Utilities|Struct|BreakStruct_Spawnable_Weapon _array_element))) _array_index)
              (else
                (bind _returnvalue_2 (Utilities|GetDataTableRow "/Game/Weapons/Structs_DataTables/DT_Ranged_Weapon_Info.DT_Ranged_Weapon_Info" (Utilities|String|StringToName (Utilities|String|EnumtoString (.Name (Utilities|Struct|BreakStruct_Weapon (.Base_Info (Utilities|Struct|BreakStruct_Spawnable_Weapon _array_element)))))))
                  (:then
                    _)
                  (:RowNotFound
                    _))
                (bind _returnvalue_3 (Utilities|GetDataTableRow "/Game/Projectiles/Structs_DataTables/DT_Projectiles.DT_Projectiles" (Utilities|String|StringToName (Utilities|String|EnumtoString (.ProjectileName (Utilities|Struct|BreakStruct_Ranged_Weapon _returnvalue_2)))))
                  (:then
                    _)
                  (:RowNotFound
                    _))
                (bind _returnvalue_4 (Utilities|GetDataTableRow "/Game/Weapons/Structs_DataTables/DT_Basic_Weapon_Info.DT_Basic_Weapon_Info" (Utilities|String|StringToName (Utilities|String|EnumtoString (.Name (Utilities|Struct|BreakStruct_Weapon (.Base_Info (Utilities|Struct|BreakStruct_Spawnable_Weapon _array_element)))))))
                  (:then
                    _)
                  (:RowNotFound
                    _))
                (Class|BPICanHaveWeapon|SetStartingWeaponsIndex(Message) (Components|GetOwner) (Utilities|Struct|MakeStruct_Spawnable_Weapon (.CustomWeapon (Utilities|Struct|BreakStruct_Spawnable_Weapon _array_element)) false (select (.CustomWeapon (Utilities|Struct|BreakStruct_Spawnable_Weapon _array_element)) (.Base_Info (Utilities|Struct|BreakStruct_Spawnable_Weapon _array_element)) _returnvalue_4) (Utilities|Struct|MakeStruct_Ranged_Weapon (.Starting_Ammo (Utilities|Struct|BreakStruct_Ranged_Weapon (select (.CustomWeapon (Utilities|Struct|BreakStruct_Spawnable_Weapon _array_element)) (.Ranged_Info (Utilities|Struct|BreakStruct_Spawnable_Weapon _array_element)) _returnvalue_2))) (.Crosshair (Utilities|Struct|BreakStruct_Ranged_Weapon _returnvalue_2)) (.Reload_Info (Utilities|Struct|BreakStruct_Ranged_Weapon (select (.CustomWeapon (Utilities|Struct|BreakStruct_Spawnable_Weapon _array_element)) (.Ranged_Info (Utilities|Struct|BreakStruct_Spawnable_Weapon _array_element)) _returnvalue_2))) (.ProjectileName (Utilities|Struct|BreakStruct_Ranged_Weapon _returnvalue_2)) _returnvalue_3 (.Recoil (Utilities|Struct|BreakStruct_Ranged_Weapon (select (.CustomWeapon (Utilities|Struct|BreakStruct_Spawnable_Weapon _array_element)) (.Ranged_Info (Utilities|Struct|BreakStruct_Spawnable_Weapon _array_element)) _returnvalue_2))) (.HitScan (Utilities|Struct|BreakStruct_Ranged_Weapon (select (.CustomWeapon (Utilities|Struct|BreakStruct_Spawnable_Weapon _array_element)) (.Ranged_Info (Utilities|Struct|BreakStruct_Spawnable_Weapon _array_element)) _returnvalue_2))) (.Piercing (Utilities|Struct|BreakStruct_Ranged_Weapon (select (.CustomWeapon (Utilities|Struct|BreakStruct_Spawnable_Weapon _array_element)) (.Ranged_Info (Utilities|Struct|BreakStruct_Spawnable_Weapon _array_element)) _returnvalue_2))) (.ShootParticle (Utilities|Struct|BreakStruct_Ranged_Weapon (select (.CustomWeapon (Utilities|Struct|BreakStruct_Spawnable_Weapon _array_element)) (.Ranged_Info (Utilities|Struct|BreakStruct_Spawnable_Weapon _array_element)) _returnvalue_2))) (._Projectiles (Utilities|Struct|BreakStruct_Ranged_Weapon (select (.CustomWeapon (Utilities|Struct|BreakStruct_Spawnable_Weapon _array_element)) (.Ranged_Info (Utilities|Struct|BreakStruct_Spawnable_Weapon _array_element)) _returnvalue_2))) (.Spread (Utilities|Struct|BreakStruct_Ranged_Weapon (select (.CustomWeapon (Utilities|Struct|BreakStruct_Spawnable_Weapon _array_element)) (.Ranged_Info (Utilities|Struct|BreakStruct_Spawnable_Weapon _array_element)) _returnvalue_2))) (.Fire_Type (Utilities|Struct|BreakStruct_Ranged_Weapon (select (.CustomWeapon (Utilities|Struct|BreakStruct_Spawnable_Weapon _array_element)) (.Ranged_Info (Utilities|Struct|BreakStruct_Spawnable_Weapon _array_element)) _returnvalue_2))) (.Burst_Info (Utilities|Struct|BreakStruct_Ranged_Weapon (select (.CustomWeapon (Utilities|Struct|BreakStruct_Spawnable_Weapon _array_element)) (.Ranged_Info (Utilities|Struct|BreakStruct_Spawnable_Weapon _array_element)) _returnvalue_2))) (.Full_Auto_Info (Utilities|Struct|BreakStruct_Ranged_Weapon (select (.CustomWeapon (Utilities|Struct|BreakStruct_Spawnable_Weapon _array_element)) (.Ranged_Info (Utilities|Struct|BreakStruct_Spawnable_Weapon _array_element)) _returnvalue_2))) (.Charged_Info (Utilities|Struct|BreakStruct_Ranged_Weapon (select (.CustomWeapon (Utilities|Struct|BreakStruct_Spawnable_Weapon _array_element)) (.Ranged_Info (Utilities|Struct|BreakStruct_Spawnable_Weapon _array_element)) _returnvalue_2))) (.Charged_Burst_Info (Utilities|Struct|BreakStruct_Ranged_Weapon (select (.CustomWeapon (Utilities|Struct|BreakStruct_Spawnable_Weapon _array_element)) (.Ranged_Info (Utilities|Struct|BreakStruct_Spawnable_Weapon _array_element)) _returnvalue_2))) (.Audio_Info (Utilities|Struct|BreakStruct_Ranged_Weapon (select (.CustomWeapon (Utilities|Struct|BreakStruct_Spawnable_Weapon _array_element)) (.Ranged_Info (Utilities|Struct|BreakStruct_Spawnable_Weapon _array_element)) _returnvalue_2)))) (.Melee_Info (Utilities|Struct|BreakStruct_Spawnable_Weapon _array_element))) _array_index)))))))
    (:then_1
      (bind _starter_weapon (Class|BPICanHaveWeapon|GetStarterWeapon(Message) (Components|GetOwner)))
      (Utilities|FlowControl|Sequence
        (:then_0
          (if (not (.CustomWeapon (Utilities|Struct|BreakStruct_Spawnable_Weapon _starter_weapon)))
            (CallFunction|UpdateNonCustomWeaponInfo _starter_weapon 0 true)))
        (:then_1
          (if (.CustomProjectile (Utilities|Struct|BreakStruct_Spawnable_Weapon _starter_weapon))
            (bind _returnvalue_5 (Utilities|GetDataTableRow "/Game/Projectiles/Structs_DataTables/DT_Projectiles.DT_Projectiles" (Utilities|String|StringToName (Utilities|String|EnumtoString (.Name (Utilities|Struct|BreakStruct_Projectiles (.Projectile_Info (Utilities|Struct|BreakStruct_Ranged_Weapon (.Ranged_Info (Utilities|Struct|BreakStruct_Spawnable_Weapon _starter_weapon)))))))))
              (:then
                _)
              (:RowNotFound
                _))
            (Class|BPICanHaveWeapon|SetStarterWeapon(Message) (Components|GetOwner) (Utilities|Struct|MakeStruct_Spawnable_Weapon (.CustomWeapon (Utilities|Struct|BreakStruct_Spawnable_Weapon _starter_weapon)) (select (.CustomWeapon (Utilities|Struct|BreakStruct_Spawnable_Weapon _starter_weapon)) true false) (.Base_Info (Utilities|Struct|BreakStruct_Spawnable_Weapon _starter_weapon)) (Utilities|Struct|MakeStruct_Ranged_Weapon (.Starting_Ammo (Utilities|Struct|BreakStruct_Ranged_Weapon (.Ranged_Info (Utilities|Struct|BreakStruct_Spawnable_Weapon _starter_weapon)))) (.Crosshair (Utilities|Struct|BreakStruct_Ranged_Weapon (.Ranged_Info (Utilities|Struct|BreakStruct_Spawnable_Weapon _starter_weapon)))) (.Reload_Info (Utilities|Struct|BreakStruct_Ranged_Weapon (.Ranged_Info (Utilities|Struct|BreakStruct_Spawnable_Weapon _starter_weapon)))) (.ProjectileName (Utilities|Struct|BreakStruct_Ranged_Weapon (.Ranged_Info (Utilities|Struct|BreakStruct_Spawnable_Weapon _starter_weapon)))) (Utilities|Struct|MakeStruct_Projectiles (.Name (Utilities|Struct|BreakStruct_Projectiles _returnvalue_5)) (.Damage (Utilities|Struct|BreakStruct_Projectiles (.Projectile_Info (Utilities|Struct|BreakStruct_Ranged_Weapon (.Ranged_Info (Utilities|Struct|BreakStruct_Spawnable_Weapon _starter_weapon)))))) (.Speed (Utilities|Struct|BreakStruct_Projectiles (.Projectile_Info (Utilities|Struct|BreakStruct_Ranged_Weapon (.Ranged_Info (Utilities|Struct|BreakStruct_Spawnable_Weapon _starter_weapon)))))) (.Gravity (Utilities|Struct|BreakStruct_Projectiles (.Projectile_Info (Utilities|Struct|BreakStruct_Ranged_Weapon (.Ranged_Info (Utilities|Struct|BreakStruct_Spawnable_Weapon _starter_weapon)))))) (.Mesh (Utilities|Struct|BreakStruct_Projectiles _returnvalue_5)) (.OnHitEffect (Utilities|Struct|BreakStruct_Projectiles (.Projectile_Info (Utilities|Struct|BreakStruct_Ranged_Weapon (.Ranged_Info (Utilities|Struct|BreakStruct_Spawnable_Weapon _starter_weapon)))))) (.ExplosionOnHit (Utilities|Struct|BreakStruct_Projectiles (.Projectile_Info (Utilities|Struct|BreakStruct_Ranged_Weapon (.Ranged_Info (Utilities|Struct|BreakStruct_Spawnable_Weapon _starter_weapon))))))) (.Recoil (Utilities|Struct|BreakStruct_Ranged_Weapon (.Ranged_Info (Utilities|Struct|BreakStruct_Spawnable_Weapon _starter_weapon)))) (.HitScan (Utilities|Struct|BreakStruct_Ranged_Weapon (.Ranged_Info (Utilities|Struct|BreakStruct_Spawnable_Weapon _starter_weapon)))) (.Piercing (Utilities|Struct|BreakStruct_Ranged_Weapon (.Ranged_Info (Utilities|Struct|BreakStruct_Spawnable_Weapon _starter_weapon)))) (.ShootParticle (Utilities|Struct|BreakStruct_Ranged_Weapon (.Ranged_Info (Utilities|Struct|BreakStruct_Spawnable_Weapon _starter_weapon)))) (._Projectiles (Utilities|Struct|BreakStruct_Ranged_Weapon (.Ranged_Info (Utilities|Struct|BreakStruct_Spawnable_Weapon _starter_weapon)))) (.Spread (Utilities|Struct|BreakStruct_Ranged_Weapon (.Ranged_Info (Utilities|Struct|BreakStruct_Spawnable_Weapon _starter_weapon)))) (.Fire_Type (Utilities|Struct|BreakStruct_Ranged_Weapon (.Ranged_Info (Utilities|Struct|BreakStruct_Spawnable_Weapon _starter_weapon)))) (.Burst_Info (Utilities|Struct|BreakStruct_Ranged_Weapon (.Ranged_Info (Utilities|Struct|BreakStruct_Spawnable_Weapon _starter_weapon)))) (.Full_Auto_Info (Utilities|Struct|BreakStruct_Ranged_Weapon (.Ranged_Info (Utilities|Struct|BreakStruct_Spawnable_Weapon _starter_weapon)))) (.Charged_Info (Utilities|Struct|BreakStruct_Ranged_Weapon (.Ranged_Info (Utilities|Struct|BreakStruct_Spawnable_Weapon _starter_weapon)))) (.Charged_Burst_Info (Utilities|Struct|BreakStruct_Ranged_Weapon (.Ranged_Info (Utilities|Struct|BreakStruct_Spawnable_Weapon _starter_weapon)))) (.Audio_Info (Utilities|Struct|BreakStruct_Ranged_Weapon (.Ranged_Info (Utilities|Struct|BreakStruct_Spawnable_Weapon _starter_weapon))))) (.Melee_Info (Utilities|Struct|BreakStruct_Spawnable_Weapon _starter_weapon))))))))))

(event EventBeginPlay
  (bind _returnvalue (Components|GetOwner))
  (bind _returnvalue_2 (Actor|GetComponentbyClass _returnvalue "/Game/Weapons/Actor_Components/BPC_Weaponry.BPC_Weaponry_C"))
  (Utilities|FlowControl|Delay 0.2)
  (bind _should_have_starter_weapon (Class|BPICanHaveWeapon|GetHasStarterWeapon(Message) (Components|GetOwner)))
  (if _should_have_starter_weapon
    (CallFunction|InitialiseStartingWeapons)
    (CallFunction|EquipStarterWeapon)
    (Default|EquipNextWeapon _returnvalue_2)
    (Default|EquipPreviousWeapon _returnvalue_2)))

(fn InitialiseStartingWeapons
  (bind _starting_weapons (Class|BPICanHaveWeapon|GetStartingWeapons(Message) (Components|GetOwner)))
  (for _array_element _starting_weapons
    (bind _returnvalue (Game|SpawnActorfromClass :Class "/Game/Weapons/BPs/BP_Weapon.BP_Weapon_C" :CollisionHandlingOverride "AlwaysSpawn" :TransformScaleMethod "MultiplyWithRoot" :Custom_Weapon? (.CustomWeapon (Utilities|Struct|BreakStruct_Spawnable_Weapon _array_element)) :Custom_Projectile (.CustomProjectile (Utilities|Struct|BreakStruct_Spawnable_Weapon _array_element)) :Info (.Base_Info (Utilities|Struct|BreakStruct_Spawnable_Weapon _array_element)) :Ranged_Info (.Ranged_Info (Utilities|Struct|BreakStruct_Spawnable_Weapon _array_element)) :Melee_Info (.Melee_Info (Utilities|Struct|BreakStruct_Spawnable_Weapon _array_element)) :Instigator 0))
    (Default|AddWeapon (Actor|GetComponentbyClass (Components|GetOwner) "/Game/Weapons/Actor_Components/BPC_Weaponry.BPC_Weaponry_C") _returnvalue)))

(fn EquipStarterWeapon
  (bind _returnvalue (Components|GetOwner))
  (bind _returnvalue_2 (Actor|GetComponentbyClass _returnvalue "/Game/Weapons/Actor_Components/BPC_Weaponry.BPC_Weaponry_C"))
  (bind _starter_weapon (Class|BPICanHaveWeapon|GetStarterWeapon(Message) (Components|GetOwner)))
  (bind _returnvalue_3 (Game|SpawnActorfromClass :Class "/Game/Weapons/BPs/BP_Weapon.BP_Weapon_C" :CollisionHandlingOverride "AlwaysSpawn" :TransformScaleMethod "MultiplyWithRoot" :Custom_Weapon? (.CustomWeapon (Utilities|Struct|BreakStruct_Spawnable_Weapon _starter_weapon)) :Custom_Projectile (.CustomProjectile (Utilities|Struct|BreakStruct_Spawnable_Weapon _starter_weapon)) :Info (.Base_Info (Utilities|Struct|BreakStruct_Spawnable_Weapon _starter_weapon)) :Ranged_Info (.Ranged_Info (Utilities|Struct|BreakStruct_Spawnable_Weapon _starter_weapon)) :Melee_Info (.Melee_Info (Utilities|Struct|BreakStruct_Spawnable_Weapon _starter_weapon)) :Instigator 0))
  (Default|AddWeapon _returnvalue_2 _returnvalue_3)
  (Default|EquipWeapon _returnvalue_2 _returnvalue_3))

(fn UpdateNonCustomWeaponInfo
  (params (Weapon_Info :type Struct%20Spawnable%20Weapon%20Structure) (Array%20Index%20If%20Starting%20Weapons :type Integer) (Is_Starter_Weapon :type Boolean))
  (bind (_customweapon _customprojectile _base_info) (Utilities|Struct|BreakStruct_Spawnable_Weapon Weapon_Info))
  (bind _returnvalue (Components|GetOwner))
  (bind _returnvalue_2 (Utilities|GetDataTableRow "/Game/Weapons/Structs_DataTables/DT_Basic_Weapon_Info.DT_Basic_Weapon_Info" (Utilities|String|StringToName (Utilities|String|EnumtoString (.Name (Utilities|Struct|BreakStruct_Weapon _base_info)))))
    (:then
      (Utilities|FlowControl|Sequence
        (:then_0
          (bind _returnvalue_3 (Utilities|GetDataTableRow "/Game/Weapons/Structs_DataTables/DT_Ranged_Weapon_Info.DT_Ranged_Weapon_Info" (Utilities|String|StringToName (Utilities|String|EnumtoString (.Name (Utilities|Struct|BreakStruct_Weapon _returnvalue_2)))))
            (:then
              (bind _returnvalue_4 (Utilities|GetDataTableRow "/Game/Projectiles/Structs_DataTables/DT_Projectiles.DT_Projectiles" (Utilities|String|StringToName (Utilities|String|EnumtoString (.Name (Utilities|Struct|BreakStruct_Projectiles (.Projectile_Info (Utilities|Struct|BreakStruct_Ranged_Weapon _returnvalue_3)))))))))
            (:RowNotFound
              (Development|PrintString "Hello"))))
        (:then_1
          (bind _returnvalue_5 (Utilities|GetDataTableRow "/Game/Weapons/Structs_DataTables/DT_Melee_Weapon_Info.DT_Melee_Weapon_Info" (Utilities|String|StringToName (Utilities|String|EnumtoString (.Name (Utilities|Struct|BreakStruct_Weapon _returnvalue_2)))))))
        (:then_2
          (if Is_Starter_Weapon
            (Class|BPICanHaveWeapon|SetStarterWeapon(Message) _returnvalue (Utilities|Struct|MakeStruct_Spawnable_Weapon false false (Utilities|Struct|MakeStruct_Weapon (.Name (Utilities|Struct|BreakStruct_Weapon _returnvalue_2)) (.Ranged (Utilities|Struct|BreakStruct_Weapon _returnvalue_2)) (.Icon (Utilities|Struct|BreakStruct_Weapon _returnvalue_2)) (.StaticMesh (Utilities|Struct|BreakStruct_Weapon _returnvalue_2)) (.BaseColour (Utilities|Struct|BreakStruct_Weapon _returnvalue_2))) (Utilities|Struct|MakeStruct_Ranged_Weapon (.Starting_Ammo (Utilities|Struct|BreakStruct_Ranged_Weapon _returnvalue_3)) (.Crosshair (Utilities|Struct|BreakStruct_Ranged_Weapon _returnvalue_3)) (.Reload_Info (Utilities|Struct|BreakStruct_Ranged_Weapon _returnvalue_3)) (.ProjectileName (Utilities|Struct|BreakStruct_Ranged_Weapon _returnvalue_3)) (select _customprojectile (Utilities|Struct|MakeStruct_Projectiles (.Name (Utilities|Struct|BreakStruct_Projectiles _returnvalue_4)) (.Damage (Utilities|Struct|BreakStruct_Projectiles (.Projectile_Info (Utilities|Struct|BreakStruct_Ranged_Weapon _returnvalue_3)))) (.Speed (Utilities|Struct|BreakStruct_Projectiles (.Projectile_Info (Utilities|Struct|BreakStruct_Ranged_Weapon _returnvalue_3)))) (.Gravity (Utilities|Struct|BreakStruct_Projectiles (.Projectile_Info (Utilities|Struct|BreakStruct_Ranged_Weapon _returnvalue_3)))) (.Mesh (Utilities|Struct|BreakStruct_Projectiles _returnvalue_4)) (.OnHitEffect (Utilities|Struct|BreakStruct_Projectiles (.Projectile_Info (Utilities|Struct|BreakStruct_Ranged_Weapon _returnvalue_3)))) (.ExplosionOnHit (Utilities|Struct|BreakStruct_Projectiles (.Projectile_Info (Utilities|Struct|BreakStruct_Ranged_Weapon _returnvalue_3))))) _returnvalue_4) (.Recoil (Utilities|Struct|BreakStruct_Ranged_Weapon _returnvalue_3)) (.HitScan (Utilities|Struct|BreakStruct_Ranged_Weapon _returnvalue_3)) (.Piercing (Utilities|Struct|BreakStruct_Ranged_Weapon _returnvalue_3)) (.ShootParticle (Utilities|Struct|BreakStruct_Ranged_Weapon _returnvalue_3)) (._Projectiles (Utilities|Struct|BreakStruct_Ranged_Weapon _returnvalue_3)) (.Spread (Utilities|Struct|BreakStruct_Ranged_Weapon _returnvalue_3)) (.Fire_Type (Utilities|Struct|BreakStruct_Ranged_Weapon _returnvalue_3)) (.Burst_Info (Utilities|Struct|BreakStruct_Ranged_Weapon _returnvalue_3)) (.Full_Auto_Info (Utilities|Struct|BreakStruct_Ranged_Weapon _returnvalue_3)) (.Charged_Info (Utilities|Struct|BreakStruct_Ranged_Weapon _returnvalue_3)) (.Charged_Burst_Info (Utilities|Struct|BreakStruct_Ranged_Weapon _returnvalue_3)) (.Audio_Info (Utilities|Struct|BreakStruct_Ranged_Weapon _returnvalue_3))) (Utilities|Struct|MakeStruct_Melee_Weapon (.Combo_Amount (Utilities|Struct|BreakStruct_Melee_Weapon _returnvalue_5)) (.Damage (Utilities|Struct|BreakStruct_Melee_Weapon _returnvalue_5)) "(MaxBlockTime_4_97BBC6444E50D6FB4E678480412D012C=2.500000,PerfectBlockThreshold_5_EE51B64145963B84D81495B86490ABAC=0.250000,BlockCooldownTime_8_EA325A6D4CFBBEA541F83388897D7125=1.750000,PerfectBlockRadius_11_F02A35F24ECB870B782958B892563501=350.000000,PerfectBlockKnockbackForce_13_06F91F3649F0DA11420F5CBA025E150A=6500.000000,PerfectBlockDamage_15_21CDD1304D59BBE6BB770F8AE746C5ED=50.000000,PerfectBlockHitstopDuration_17_3BD6FD304CAFB89BB5537BB9BA0393B8=0.250000)" "(AttackSound_2_968CB2B8450766B08C46478BF96E73CD=None)")))
            (else
              (Class|BPICanHaveWeapon|SetStartingWeaponsIndex(Message) _returnvalue (Utilities|Struct|MakeStruct_Spawnable_Weapon false false (Utilities|Struct|MakeStruct_Weapon (.Name (Utilities|Struct|BreakStruct_Weapon _returnvalue_2)) (.Ranged (Utilities|Struct|BreakStruct_Weapon _returnvalue_2)) (.Icon (Utilities|Struct|BreakStruct_Weapon _returnvalue_2)) (.StaticMesh (Utilities|Struct|BreakStruct_Weapon _returnvalue_2)) (.BaseColour (Utilities|Struct|BreakStruct_Weapon _returnvalue_2))) (Utilities|Struct|MakeStruct_Ranged_Weapon (.Starting_Ammo (Utilities|Struct|BreakStruct_Ranged_Weapon _returnvalue_3)) (.Crosshair (Utilities|Struct|BreakStruct_Ranged_Weapon _returnvalue_3)) (.Reload_Info (Utilities|Struct|BreakStruct_Ranged_Weapon _returnvalue_3)) (.ProjectileName (Utilities|Struct|BreakStruct_Ranged_Weapon _returnvalue_3)) (select _customprojectile (Utilities|Struct|MakeStruct_Projectiles (.Name (Utilities|Struct|BreakStruct_Projectiles _returnvalue_4)) (.Damage (Utilities|Struct|BreakStruct_Projectiles (.Projectile_Info (Utilities|Struct|BreakStruct_Ranged_Weapon _returnvalue_3)))) (.Speed (Utilities|Struct|BreakStruct_Projectiles (.Projectile_Info (Utilities|Struct|BreakStruct_Ranged_Weapon _returnvalue_3)))) (.Gravity (Utilities|Struct|BreakStruct_Projectiles (.Projectile_Info (Utilities|Struct|BreakStruct_Ranged_Weapon _returnvalue_3)))) (.Mesh (Utilities|Struct|BreakStruct_Projectiles _returnvalue_4)) (.OnHitEffect (Utilities|Struct|BreakStruct_Projectiles (.Projectile_Info (Utilities|Struct|BreakStruct_Ranged_Weapon _returnvalue_3)))) (.ExplosionOnHit (Utilities|Struct|BreakStruct_Projectiles (.Projectile_Info (Utilities|Struct|BreakStruct_Ranged_Weapon _returnvalue_3))))) _returnvalue_4) (.Recoil (Utilities|Struct|BreakStruct_Ranged_Weapon _returnvalue_3)) (.HitScan (Utilities|Struct|BreakStruct_Ranged_Weapon _returnvalue_3)) (.Piercing (Utilities|Struct|BreakStruct_Ranged_Weapon _returnvalue_3)) (.ShootParticle (Utilities|Struct|BreakStruct_Ranged_Weapon _returnvalue_3)) (._Projectiles (Utilities|Struct|BreakStruct_Ranged_Weapon _returnvalue_3)) (.Spread (Utilities|Struct|BreakStruct_Ranged_Weapon _returnvalue_3)) (.Fire_Type (Utilities|Struct|BreakStruct_Ranged_Weapon _returnvalue_3)) (.Burst_Info (Utilities|Struct|BreakStruct_Ranged_Weapon _returnvalue_3)) (.Full_Auto_Info (Utilities|Struct|BreakStruct_Ranged_Weapon _returnvalue_3)) (.Charged_Info (Utilities|Struct|BreakStruct_Ranged_Weapon _returnvalue_3)) (.Charged_Burst_Info (Utilities|Struct|BreakStruct_Ranged_Weapon _returnvalue_3)) (.Audio_Info (Utilities|Struct|BreakStruct_Ranged_Weapon _returnvalue_3))) (Utilities|Struct|MakeStruct_Melee_Weapon (.Combo_Amount (Utilities|Struct|BreakStruct_Melee_Weapon _returnvalue_5)) (.Damage (Utilities|Struct|BreakStruct_Melee_Weapon _returnvalue_5)) "(MaxBlockTime_4_97BBC6444E50D6FB4E678480412D012C=2.500000,PerfectBlockThreshold_5_EE51B64145963B84D81495B86490ABAC=0.250000,BlockCooldownTime_8_EA325A6D4CFBBEA541F83388897D7125=1.750000,PerfectBlockRadius_11_F02A35F24ECB870B782958B892563501=350.000000,PerfectBlockKnockbackForce_13_06F91F3649F0DA11420F5CBA025E150A=6500.000000,PerfectBlockDamage_15_21CDD1304D59BBE6BB770F8AE746C5ED=50.000000,PerfectBlockHitstopDuration_17_3BD6FD304CAFB89BB5537BB9BA0393B8=0.250000)" "(AttackSound_2_968CB2B8450766B08C46478BF96E73CD=None)")) Array%20Index%20If%20Starting%20Weapons))))))))