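; Pickup weapon actor, melee or ranged, that adds itself to an overlapping player's weaponry component if not already held.
; Construction script fills stats from data tables by weapon name, or keeps custom values, then sets mesh, interact radius, max ammo and rotation animation.
; A second pass resolves projectile data, with custom projectiles taking only name and mesh from the table.
; Getters expose info, mesh and shoot transform.
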(event OnComponentBeginOverlap(Interact_Collision)
  (params (OverlappedComponent :type Primitive%20Component%20Object%20Reference) (OtherActor :type Actor%20Object%20Reference) (OtherComp :type Primitive%20Component%20Object%20Reference) (OtherBodyIndex :type Integer) (bFromSweep :type Boolean) (SweepResult :type Hit%20Result%20Structure%20%28by%20ref%29))
  (if (or (Utilities|DoesObjectImplementInterface OtherActor "/Game/Characters/Shared_Interfaces/BPI_Can_Aim.BPI_Can_Aim_C") (Utilities|DoesObjectImplementInterface OtherActor "/Game/Characters/Shared_Interfaces/BPI_Can_Melee_Attack.BPI_Can_Melee_Attack_C"))
    (if (and (Utilities|DoesObjectImplementInterface OtherActor "/Game/Characters/Player/BPI_Player.BPI_Player_C") (not (Utilities|Array|ContainsItem (Variables|/Game/Weapons/Actor_Components/BPC_Weaponry.BPC_Weaponry_C|GetWeapons (Actor|GetComponentbyClass OtherActor "/Game/Weapons/Actor_Components/BPC_Weaponry.BPC_Weaponry_C")) self)))
      (Default|AddWeapon (Actor|GetComponentbyClass OtherActor "/Game/Weapons/Actor_Components/BPC_Weaponry.BPC_Weaponry_C") self))))

(event EventUpdateRangedInfo
  (params (New_Ranged_Info :type Struct%20Ranged%20Weapon%20Structure))
  (Variables|Info|SetRanged_Info New_Ranged_Info))

(event EventUpdateCustomProjectile
  (params (Is%20Custom :type Boolean))
  (Variables|Info|SetCustom_Projectile Is%20Custom))

(event EventUpdateCollision
  (params (Collision_Enabled :type Boolean))
  (Collision|SetActorEnableCollision Collision_Enabled))

(event EventUpdateCustomWeapon
  (params (Is%20Custom :type Boolean))
  (Variables|Info|SetCustom_Weapon? Is%20Custom))

(fn ConstructionScript
  (bind _bpc_animated_rotation (Variables|AnimatedRotation|GetBPC_Animated_Rotation))
  (bind _animated_rotation_info (Variables|AnimatedRotation|GetAnimated_Rotation_Info))
  (Variables|/Game/Weapons/Actor_Components/BPC_Animated_Rotation.BPC_Animated_Rotation_C|SetRotateRate _bpc_animated_rotation (.rotate_rate _animated_rotation_info))
  (Variables|/Game/Weapons/Actor_Components/BPC_Animated_Rotation.BPC_Animated_Rotation_C|SetVertical_Range _bpc_animated_rotation (.vertical_range _animated_rotation_info))
  (Variables|/Game/Weapons/Actor_Components/BPC_Animated_Rotation.BPC_Animated_Rotation_C|SetVertical_Time _bpc_animated_rotation (.vertical_time _animated_rotation_info))
  (Utilities|FlowControl|Sequence
    (:then_0
      (if (Variables|Info|GetCustom_Weapon?)
        (Components|Sphere|SetSphereRadius (Variables|Default|GetInteract_Collision) (Variables|Interaction|GetInteract_Radius) true)
        (Components|StaticMesh|SetStaticMesh (Variables|Default|GetWeapon_Static_Mesh) (.staticmesh (Variables|Info|GetInfo)))
        (Variables|/Game/Weapons/Actor_Components/BPC_Ammo.BPC_Ammo_C|SetMax_Ammo (Variables|Default|GetBPC_Ammo) (.starting_ammo (Variables|Info|GetRanged_Info)))
        (Variables|Info|SetInfo (Utilities|RandomWeaponBaseColour (Variables|Info|GetInfo)))
        (else
          (Variables|Info|SetCustom_Projectile false)
          (bind _returnvalue (Utilities|GetDataTableRow "/Game/Weapons/Structs_DataTables/DT_Basic_Weapon_Info.DT_Basic_Weapon_Info" (Utilities|String|StringToName (Utilities|String|EnumtoString (.name (Variables|Info|GetInfo)))))
            (:then
              (bind _output_get (Variables|Info|SetInfo (Utilities|RandomWeaponBaseColour _returnvalue)))
              (if (.ranged _output_get)
                (bind _returnvalue_2 (Utilities|GetDataTableRow "/Game/Weapons/Structs_DataTables/DT_Ranged_Weapon_Info.DT_Ranged_Weapon_Info" (Utilities|String|StringToName (Utilities|String|EnumtoString (.name (Variables|Info|GetInfo)))))
                  (:then
                    (Variables|Info|SetRanged_Info _returnvalue_2)))
                (else
                  (bind _returnvalue_3 (Utilities|GetDataTableRow "/Game/Weapons/Structs_DataTables/DT_Melee_Weapon_Info.DT_Melee_Weapon_Info" (Utilities|String|StringToName (Utilities|String|EnumtoString (.name (Variables|Info|GetInfo)))))
                    (:then
                      (Variables|Info|SetMelee_Info _returnvalue_3)))))
              (Components|Sphere|SetSphereRadius (Variables|Default|GetInteract_Collision) (Variables|Interaction|GetInteract_Radius) true)
              (Components|StaticMesh|SetStaticMesh (Variables|Default|GetWeapon_Static_Mesh) (.staticmesh (Variables|Info|GetInfo)))
              (Variables|/Game/Weapons/Actor_Components/BPC_Ammo.BPC_Ammo_C|SetMax_Ammo (Variables|Default|GetBPC_Ammo) (.starting_ammo (Variables|Info|GetRanged_Info))))))))
    (:then_1
      (if (Variables|Info|GetCustom_Projectile)
        (Variables|Info|SetCustom_Weapon? true)
        (bind _returnvalue_4 (Utilities|GetDataTableRow "/Game/Projectiles/Structs_DataTables/DT_Projectiles.DT_Projectiles" (Utilities|String|StringToName (Utilities|String|EnumtoString (.projectilename (Variables|Info|GetRanged_Info)))))
          (:then
            (Variables|Info|SetRanged_Info (Utilities|Struct|MakeStruct_Ranged_Weapon (.starting_ammo (Variables|Info|GetRanged_Info)) (.crosshair (Variables|Info|GetRanged_Info)) (.reload_info (Variables|Info|GetRanged_Info)) (.projectilename (Variables|Info|GetRanged_Info)) (Utilities|Struct|MakeStruct_Projectiles (.Name (Utilities|Struct|BreakStruct_Projectiles _returnvalue_4)) (.Damage (Utilities|Struct|BreakStruct_Projectiles (.projectile_info (Variables|Info|GetRanged_Info)))) (.Speed (Utilities|Struct|BreakStruct_Projectiles (.projectile_info (Variables|Info|GetRanged_Info)))) (.Gravity (Utilities|Struct|BreakStruct_Projectiles (.projectile_info (Variables|Info|GetRanged_Info)))) (.Mesh (Utilities|Struct|BreakStruct_Projectiles _returnvalue_4)) (.OnHitEffect (Utilities|Struct|BreakStruct_Projectiles (.projectile_info (Variables|Info|GetRanged_Info)))) (.ExplosionOnHit (Utilities|Struct|BreakStruct_Projectiles (.projectile_info (Variables|Info|GetRanged_Info))))) (.recoil (Variables|Info|GetRanged_Info)) (.hitscan (Variables|Info|GetRanged_Info)) (.piercing (Variables|Info|GetRanged_Info)) (.shootparticle (Variables|Info|GetRanged_Info)) (._projectiles (Variables|Info|GetRanged_Info)) (.spread (Variables|Info|GetRanged_Info)) (.fire_type (Variables|Info|GetRanged_Info)) (.burst_info (Variables|Info|GetRanged_Info)) (.full_auto_info (Variables|Info|GetRanged_Info)) (.charged_info (Variables|Info|GetRanged_Info)) (.charged_burst_info (Variables|Info|GetRanged_Info)) (.audio_info (Variables|Info|GetRanged_Info))))))
        (else
          (if (Variables|Info|GetCustom_Weapon?)
            _
            (else
              (Variables|Info|SetCustom_Weapon? false)))
          (bind _returnvalue_5 (Utilities|GetDataTableRow "/Game/Weapons/Structs_DataTables/DT_Ranged_Weapon_Info.DT_Ranged_Weapon_Info" (Utilities|String|StringToName (Utilities|String|EnumtoString (.name (Variables|Info|GetInfo)))))
            (:then
              (bind _returnvalue_6 (Utilities|GetDataTableRow "/Game/Projectiles/Structs_DataTables/DT_Projectiles.DT_Projectiles" (Utilities|String|StringToName (Utilities|String|EnumtoString (.ProjectileName (Utilities|Struct|BreakStruct_Ranged_Weapon _returnvalue_5)))))
                (:then
                  (Variables|Info|SetRanged_Info (Utilities|Struct|MakeStruct_Ranged_Weapon (.starting_ammo (Variables|Info|GetRanged_Info)) (.crosshair (Variables|Info|GetRanged_Info)) (.reload_info (Variables|Info|GetRanged_Info)) (.ProjectileName (Utilities|Struct|BreakStruct_Ranged_Weapon _returnvalue_5)) _returnvalue_6 (.recoil (Variables|Info|GetRanged_Info)) (.hitscan (Variables|Info|GetRanged_Info)) (.piercing (Variables|Info|GetRanged_Info)) (.shootparticle (Variables|Info|GetRanged_Info)) (._projectiles (Variables|Info|GetRanged_Info)) (.spread (Variables|Info|GetRanged_Info)) (.fire_type (Variables|Info|GetRanged_Info)) (.burst_info (Variables|Info|GetRanged_Info)) (.full_auto_info (Variables|Info|GetRanged_Info)) (.charged_info (Variables|Info|GetRanged_Info)) (.charged_burst_info (Variables|Info|GetRanged_Info)) (.audio_info (Variables|Info|GetRanged_Info)))))))))))))

(fn GetBasicInfo
  (return (Variables|Info|GetInfo)))

(fn GetCustomProjectile
  (return (Variables|Info|GetCustom_Projectile)))

(fn GetMeleeInfo
  (return (Variables|Info|GetMelee_Info)))

(fn GetRangedInfo
  (return (Variables|Info|GetRanged_Info)))

(fn GetShootTransform
  (return (Transformation|GetWorldTransform (Variables|Default|GetShoot_Transform))))

(fn GetStaticMesh
  (return (Variables|Default|GetWeapon_Static_Mesh)))

(fn GetStaticMeshMelee
  (return (Variables|Default|GetWeapon_Static_Mesh)))