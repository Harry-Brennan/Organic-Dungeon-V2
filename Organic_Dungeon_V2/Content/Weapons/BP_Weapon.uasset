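; BP_Weapon is a weapon actor that players pick up by overlapping its interaction sphere.
; The construction script sizes the sphere from InteractRadius and sets the mesh from the weapon's Info data.
; On overlap, an actor implementing BPI_Player receives the weapon through its BPC_Player_Weaponry component, unless it already holds it.
; Getters expose basic, melee and ranged info, the mesh and the shoot transform, while an event toggles actor collision.
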(event OnComponentBeginOverlap(Interact_Collision)
  (params (OverlappedComponent :type Primitive%20Component%20Object%20Reference) (OtherActor :type Actor%20Object%20Reference) (OtherComp :type Primitive%20Component%20Object%20Reference) (OtherBodyIndex :type Integer) (bFromSweep :type Boolean) (SweepResult :type Hit%20Result%20Structure%20%28by%20ref%29))
  (if (and (Utilities|DoesObjectImplementInterface OtherActor "/Game/Characters/Player/BPI_Player.BPI_Player_C") (not (Utilities|Array|ContainsItem (Variables|/Game/Weapons/BPC_Player_Weaponry.BPC_Player_Weaponry_C|GetWeapons (Actor|GetComponentbyClass OtherActor "/Game/Weapons/BPC_Player_Weaponry.BPC_Player_Weaponry_C")) self)))
    (Default|AddWeapon (Actor|GetComponentbyClass OtherActor "/Game/Weapons/BPC_Player_Weaponry.BPC_Player_Weaponry_C") self)))

(event EventUpdateCollision
  (params (Collision_Enabled :type Boolean))
  (Collision|SetActorEnableCollision Collision_Enabled))

(fn ConstructionScript
  (Components|Sphere|SetSphereRadius (Variables|Default|GetInteract_Collision) (Variables|Interaction|GetInteract_Radius) true)
  (Components|StaticMesh|SetStaticMesh (Variables|Default|GetWeapon_Static_Mesh) (.staticmesh (Variables|Default|GetInfo))))

(fn GetBasicInfo
  (return (Variables|Default|GetInfo)))

(fn GetMeleeInfo
  (return (Variables|Default|GetMelee_Info)))

(fn GetRangedInfo
  (return (Variables|Default|GetRanged_Info)))

(fn GetShootTransform
  (return (Transformation|GetWorldTransform (Variables|Default|GetShoot_Transform))))

(fn GetStaticMesh
  (return (Variables|Default|GetWeapon_Static_Mesh)))