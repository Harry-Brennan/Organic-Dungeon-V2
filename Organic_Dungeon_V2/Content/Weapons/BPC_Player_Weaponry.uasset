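; Player weaponry component that keeps the list of collected weapons and handles adding, equipping and input-driven cycling between them.
; Stored weapons remain world actors, moved to an "Inventory"-tagged TargetPoint; the equipped one attaches to the owner's Weapon_R socket.
; Adding a weapon stops its rotation animation, equips it and sets its owner.
; Cycling wraps around the list, cancels active reloads through BPC_Ammo and swaps icons through BPC_HUD.
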(event Custom|Move_To_Inventory_Space
  (params (Weapon_To_Move :type Actor%20Object%20Reference))
  (bind _outactors (Actor|GetAllActorsOfClasswithTag "/Script/Engine.TargetPoint" "Inventory"))
  (for _array_element _outactors
    (Transformation|SetActorLocation Weapon_To_Move (Transformation|GetActorLocation _array_element) false false)))

(event Custom|Move_From_Inventory_Space
  (params (Weapon_To_Move :type Actor%20Object%20Reference) (End_Location :type Vector))
  (Transformation|SetActorLocation Weapon_To_Move End_Location false false))

(event Custom|Update_Next_&_Previous_Indexes
  (bind _weapons (Variables|Default|GetWeapons))
  (bind _equipped_weapon (Variables|Default|GetEquipped_Weapon))
  (bind _weapons_2 (Variables|Default|GetWeapons))
  (bind _equipped_weapon_2 (Variables|Default|GetEquipped_Weapon))
  (bind _returnvalue (Utilities|Array|FindItem _weapons _equipped_weapon))
  (bind _returnvalue_2 (Utilities|Array|FindItem _weapons_2 _equipped_weapon_2))
  (bind _returnvalue_3 (+ _returnvalue_2 1))
  (bind _returnvalue_4 (- _returnvalue 1))
  (Utilities|FlowControl|Sequence
    (:then_0
      (Variables|Default|SetNext_Weapon_Index (Math|Integer|SelectInt 0 _returnvalue_3 (> _returnvalue_3 (Utilities|Array|LastIndex _weapons_2)))))
    (:then_1
      (Variables|Default|SetPrevious_Weapon_Index (Math|Integer|SelectInt (Utilities|Array|LastIndex _weapons) _returnvalue_4 (< _returnvalue_4 0))))))

(event Custom|Equip_Previous_Weapon
  (bind _equipped_weapon (Variables|Default|GetEquipped_Weapon))
  (bind _returnvalue (Actor|GetComponentbyClass _equipped_weapon "/Game/Weapons/BPC_Ammo.BPC_Ammo_C"))
  (if (not (Utilities|Array|IsEmpty (Variables|Default|GetWeapons)))
    (if (Variables|/Game/Weapons/BPC_Ammo.BPC_Ammo_C|GetReloading _returnvalue)
      (Default|StopReload _returnvalue))
    (CallFunction|UpdateNext&PreviousIndexes)
    (CallFunction|EquipWeapon (Utilities|Array|Get(acopy) (Variables|Default|GetWeapons) (Variables|Default|GetPrevious_Weapon_Index)))
    (Default|SwapWeaponIcons (Actor|GetComponentbyClass (Components|GetOwner) "/Game/Characters/Player/BPC_HUD.BPC_HUD_C") false)))

(event Custom|Equip_Next_Weapon
  (bind _equipped_weapon (Variables|Default|GetEquipped_Weapon))
  (bind _returnvalue (Actor|GetComponentbyClass _equipped_weapon "/Game/Weapons/BPC_Ammo.BPC_Ammo_C"))
  (if (not (Utilities|Array|IsEmpty (Variables|Default|GetWeapons)))
    (if (Variables|/Game/Weapons/BPC_Ammo.BPC_Ammo_C|GetReloading _returnvalue)
      (Default|StopReload _returnvalue))
    (CallFunction|UpdateNext&PreviousIndexes)
    (CallFunction|EquipWeapon (Utilities|Array|Get(acopy) (Variables|Default|GetWeapons) (Variables|Default|GetNext_Weapon_Index)))
    (Default|SwapWeaponIcons (Actor|GetComponentbyClass (Components|GetOwner) "/Game/Characters/Player/BPC_HUD.BPC_HUD_C") true)))

(event Custom|Equip_Weapon
  (params (WeaponToEquip :type Actor%20Object%20Reference))
  (bind _returnvalue (Components|GetOwner))
  (bind _returnvalue_2 (Actor|GetComponentbyClass _returnvalue "/Script/Engine.SkeletalMeshComponent"))
  (if (not (== WeaponToEquip (Variables|Default|GetEquipped_Weapon)))
    (Development|PrintString (Utilities|String|Append "EQUIPPING: " (Utilities|GetDisplayName WeaponToEquip)))
    (CallFunction|DequipWeapon)
    (Class|BPIWeapon|UpdateCollision(Message) WeaponToEquip false)
    (CallFunction|MovefromInventorySpace WeaponToEquip (Transformation|GetSocketLocation _returnvalue_2 "Weapon_R"))
    (Transformation|AttachComponentToComponent WeaponToEquip _returnvalue_2 "Weapon_R" "SnapToTarget" "SnapToTarget" "KeepRelative" true)
    (Utilities|IsValid (Variables|Default|GetEquipped_Weapon)
      (:Is%20Valid
        (if (Variables|/Game/Weapons/BPC_Ammo.BPC_Ammo_C|GetReloading (Actor|GetComponentbyClass (Variables|Default|GetEquipped_Weapon) "/Game/Weapons/BPC_Ammo.BPC_Ammo_C"))
          (Default|StopReload (Actor|GetComponentbyClass (Variables|Default|GetEquipped_Weapon) "/Game/Weapons/BPC_Ammo.BPC_Ammo_C"))))
      (:Is%20Not%20Valid
        _))
    (Variables|Default|SetEquipped_Weapon WeaponToEquip)
    (CallFunction|UpdateNext&PreviousIndexes)))

(event Custom|Dequip_Weapon
  (bind _returnvalue (Components|GetOwner))
  (bind _equipped_weapon (Variables|Default|GetEquipped_Weapon))
  (Development|PrintString (Utilities|String|Append "DEQUIPPING: " (Utilities|GetDisplayName (Variables|Default|GetEquipped_Weapon))))
  (Utilities|IsValid _equipped_weapon
    (:Is%20Valid
      (Transformation|DetachFromActor _equipped_weapon "KeepWorld" "KeepWorld" "KeepWorld")
      (Transformation|SetActorLocation _equipped_weapon (+ (Transformation|GetActorLocation _returnvalue) (* (Transformation|GetActorForwardVector _returnvalue) 5e+01)) false false)
      (Class|BPIWeapon|UpdateCollision(Message) _equipped_weapon true)
      (CallFunction|MovetoInventorySpace _equipped_weapon))))

(event Custom|Add_Weapon
  (params (WeaponToAdd :type Actor%20Object%20Reference))
  (Development|PrintString (Utilities|String|Append "ADDING THIS TO INVENTORY:" (Utilities|GetDisplayName WeaponToAdd)))
  (Utilities|Array|Add (Variables|Default|GetWeapons) WeaponToAdd)
  (Class|BPIWeapon|UpdateCollision(Message) WeaponToAdd false)
  (Default|StopAnimatedRotation (Actor|GetComponentbyClass WeaponToAdd "/Game/Weapons/BPC_Animated_Rotation.BPC_Animated_Rotation_C"))
  (CallFunction|MovetoInventorySpace WeaponToAdd)
  (CallFunction|EquipWeapon WeaponToAdd)
  (Default|SwapWeaponIcons (Actor|GetComponentbyClass (Components|GetOwner) "/Game/Characters/Player/BPC_HUD.BPC_HUD_C") true)
  (Actor|SetOwner WeaponToAdd (Components|GetOwner)))

(event Input|EnhancedActionEvents|EnhancedInputActionIA_Cycle_Next_Weapon
  (params (ActionValue :type Boolean) (ElapsedSeconds :type Float%20%28double-precision%29) (TriggeredSeconds :type Float%20%28double-precision%29) (InputAction :type Input%20Action%20Object%20Reference :default "/Game/Characters/Player/Input/Actions/IA_Cycle_Next_Weapon.IA_Cycle_Next_Weapon"))
  (:Triggered
    (CallFunction|EquipNextWeapon)))

(event Input|EnhancedActionEvents|EnhancedInputActionIA_Cycle_Previous_Weapon
  (params (ActionValue :type Boolean) (ElapsedSeconds :type Float%20%28double-precision%29) (TriggeredSeconds :type Float%20%28double-precision%29) (InputAction :type Input%20Action%20Object%20Reference :default "/Game/Characters/Player/Input/Actions/IA_Cycle_Previous_Weapon.IA_Cycle_Previous_Weapon"))
  (:Triggered
    (CallFunction|EquipPreviousWeapon)))