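; Actor component that makes its owning actor spin around yaw and bob up and down around its starting height.
; It starts on BeginPlay, and its start and stop events toggle component tick, with start also recording the current Z.
; Tick eases yaw toward an always-moving target for continuous spin, and eases Z between the VerticalRange limits, flipping direction near each.
; RotateRate drives both the spin and bob speeds.
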(event Custom|Start_Animated_Rotation
  (Variables|Default|SetStartZ (.z (Transformation|GetActorLocation (Components|GetOwner))))
  (Components|Tick|SetComponentTickEnabled true))

(event Custom|Stop_Animated_Rotation
  (Components|Tick|SetComponentTickEnabled false))

(event EventTick
  (params (DeltaSeconds :type Float%20%28single-precision%29))
  (bind _returnvalue (Components|GetOwner))
  (bind _returnvalue_2 (Components|GetOwner))
  (bind _startz (Variables|Default|GetStartZ))
  (bind _vertical_range (Variables|Default|GetVertical_Range))
  (bind _returnvalue_3 (Transformation|GetActorLocation _returnvalue))
  (bind _returnvalue_4 (Transformation|GetActorRotation _returnvalue_2))
  (bind _returnvalue_5 (/ _vertical_range 2.0))
  (Transformation|SetActorRotation (Components|GetOwner) (Math|Rotator|MakeRotator (.roll _returnvalue_4) (.pitch _returnvalue_4) (Math|Interpolation|FInterpTo (.yaw _returnvalue_4) (+ (.yaw _returnvalue_4) 1.8e+02) DeltaSeconds (Variables|Default|GetRotateRate))))
  (Utilities|FlowControl|Sequence
    (:then_0
      (if (and (not (Variables|Default|GetDirection)) (Math|Float|NearlyEqual(Float) (+ (Variables|Default|GetStartZ) (/ (Variables|Default|GetVertical_Range) 2.0)) (.z _returnvalue_3) 5.0))
        (Variables|Default|SetDirection true)
        (elif (and (Variables|Default|GetDirection) (Math|Float|NearlyEqual(Float) (- (Variables|Default|GetStartZ) (/ (Variables|Default|GetVertical_Range) 2.0)) (.z _returnvalue_3) 5.0))
          (Variables|Default|SetDirection false))))
    (:then_1
      (Variables|Default|SetTargetZ (Math|Float|SelectFloat (- _startz _returnvalue_5) (+ _startz _returnvalue_5) (Variables|Default|GetDirection)))
      (Transformation|SetActorLocation (Components|GetOwner) (Math|Vector|MakeVector (.x _returnvalue_3) (.y _returnvalue_3) (Math|Interpolation|FInterpTo (.z _returnvalue_3) (Variables|Default|GetTargetZ) DeltaSeconds (Variables|Default|GetRotateRate))) false false))))

(event EventBeginPlay
  (CallFunction|StartAnimatedRotation))