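; Weapon inventory component that lets its owning actor collect, equip, dequip and cycle through weapons.
; Added weapons join an array, have pickup rotation stopped, and are teleported to an "Inventory"-tagged TargetPoint instead of being destroyed.
; Equipping dequips the current weapon, then attaches the new one to the owner's hand_r socket, toggling collision through UpdateCollisionMessage.
; Next and previous events wrap around the array using a stored index.
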(event Custom|Equip_Weapon
  (params (WeaponToEquip :type Actor%20Object%20Reference))
  (bind _returnvalue (Components|GetOwner))
  (bind _returnvalue_2 (Actor|GetComponentbyClass _returnvalue "/Script/Engine.SkeletalMeshComponent"))
  (if (not (== WeaponToEquip (Variables|Default|GetEquipped_Weapon)))
    (Development|PrintString (Utilities|String|Append "EQUIPPING: " (Utilities|GetDisplayName WeaponToEquip)))
    (CallFunction|DequipWeapon)
    (Class|BPIWeapon|UpdateCollision(Message) WeaponToEquip false)
    (CallFunction|MovefromInventorySpace WeaponToEquip (Transformation|GetSocketLocation _returnvalue_2 "hand_r"))
    (Transformation|AttachComponentToComponent WeaponToEquip _returnvalue_2 "hand_r" "SnapToTarget" "SnapToTarget" "KeepRelative" true)
    (Variables|Default|SetEquipped_Weapon WeaponToEquip)))

(event Custom|Equip_Previous_Weapon
  (bind _weapons (Variables|Default|GetWeapons))
  (if (not (Utilities|Array|IsEmpty (Variables|Default|GetWeapons)))
    (bind _output_get (Variables|Default|SetNext_Weapon_Index (Math|Integer|SelectInt (Utilities|Array|LastIndex _weapons) (- (Utilities|Array|FindItem _weapons (Variables|Default|GetEquipped_Weapon)) 1) (<= (Variables|Default|GetNext_Weapon_Index) 0))))
    (Development|PrintString (Utilities|String|Append "Current Weapon Index:" (Utilities|String|ToString(Integer) _output_get)))
    (CallFunction|EquipWeapon (Utilities|Array|Get(acopy) (Variables|Default|GetWeapons) (Variables|Default|GetNext_Weapon_Index)))))

(event Custom|Add_Weapon
  (params (WeaponToAdd :type Actor%20Object%20Reference))
  (Development|PrintString (Utilities|String|Append "ADDING THIS TO INVENTORY:" (Utilities|GetDisplayName WeaponToAdd)))
  (Utilities|Array|Add (Variables|Default|GetWeapons) WeaponToAdd)
  (Class|BPIWeapon|UpdateCollision(Message) WeaponToAdd false)
  (Default|StopAnimatedRotation (Actor|GetComponentbyClass WeaponToAdd "/Game/Weapons/BPC_Animated_Rotation.BPC_Animated_Rotation_C"))
  (CallFunction|MovetoInventorySpace WeaponToAdd))

(event Custom|Equip_Next_Weapon
  (bind _weapons (Variables|Default|GetWeapons))
  (if (not (Utilities|Array|IsEmpty (Variables|Default|GetWeapons)))
    (bind _output_get (Variables|Default|SetNext_Weapon_Index (Math|Integer|SelectInt 0 (+ (Utilities|Array|FindItem _weapons (Variables|Default|GetEquipped_Weapon)) 1) (>= (Variables|Default|GetNext_Weapon_Index) (Utilities|Array|LastIndex _weapons)))))
    (Development|PrintString (Utilities|String|Append "Current Weapon Index:" (Utilities|String|ToString(Integer) _output_get)))
    (CallFunction|EquipWeapon (Utilities|Array|Get(acopy) (Variables|Default|GetWeapons) (Variables|Default|GetNext_Weapon_Index)))))

(event Custom|Dequip_Weapon
  (bind _returnvalue (Components|GetOwner))
  (bind _equipped_weapon (Variables|Default|GetEquipped_Weapon))
  (Development|PrintString (Utilities|String|Append "DEQUIPPING: " (Utilities|GetDisplayName (Variables|Default|GetEquipped_Weapon))))
  (Utilities|IsValid _equipped_weapon
    (:Is%20Valid
      (Transformation|DetachFromActor _equipped_weapon "KeepWorld" "KeepWorld" "KeepWorld")
      (Transformation|SetActorLocation _equipped_weapon (+ (Transformation|GetActorLocation _returnvalue) (* (Transformation|GetActorForwardVector _returnvalue) 5e+01)) false false)
      (Class|BPIWeapon|UpdateCollision(Message) _equipped_weapon true)
      (CallFunction|MovetoInventorySpace _equipped_weapon))
    (:Is%20Not%20Valid
      (Development|PrintString "equipped weapon not valid"))))

(event Custom|Move_To_Inventory_Space
  (params (Weapon_To_Move :type Actor%20Object%20Reference))
  (bind _outactors (Actor|GetAllActorsOfClasswithTag "/Script/Engine.TargetPoint" "Inventory"))
  (for _array_element _outactors
    (Transformation|SetActorLocation Weapon_To_Move (Transformation|GetActorLocation _array_element) false false)))

(event Custom|Move_From_Inventory_Space
  (params (Weapon_To_Move :type Actor%20Object%20Reference) (End_Location :type Vector))
  (Transformation|SetActorLocation Weapon_To_Move End_Location false false))