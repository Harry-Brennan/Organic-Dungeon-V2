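; Weapon ammo component that tracks the current count and handles an interruptible, incremental reload.
; Reload toggles ticking, which grows a reload percentage and converts it to whole rounds until the magazine is full.
; When the owner's owner implements BPI_Player, reload time comes from the equipped weapon, otherwise a default applies.
; For players it also drives the HUD's weapon-slot colour and ammo animation through BPC_HUD.
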(event Custom|Decrease_Ammo
  (bind _returnvalue (Components|GetOwner))
  (bind _current_ammo (Variables|Default|GetCurrent_Ammo))
  (bind _max_ammo (Variables|Default|GetMax_Ammo))
  (bind _returnvalue_2 (Math|Conversions|ToFloat(Integer) _max_ammo))
  (bind _returnvalue_3 (Math|Conversions|ToFloat(Integer) _current_ammo))
  (bind _returnvalue_4 (Components|GetOwner _returnvalue))
  (bind _returnvalue_5 (Actor|GetComponentbyClass _returnvalue_4 "/Game/Characters/Player/BPC_HUD.BPC_HUD_C"))
  (bind _returnvalue_6 (/ _returnvalue_3 _returnvalue_2))
  (bind _hud_ref (Variables|/Game/Characters/Player/BPC_HUD.BPC_HUD_C|GetHUD_Ref _returnvalue_5))
  (if (not (<= (Variables|Default|GetCurrent_Ammo) 0))
    (Math|Integer|DecrementInt (Variables|Default|GetCurrent_Ammo)
      (:%20%20
        (Variables|Default|SetReload_Percent 0.0)
        (if (Utilities|DoesObjectImplementInterface (Components|GetOwner (Components|GetOwner)) "/Game/Characters/Player/BPI_Player.BPI_Player_C")
          (Development|PrintString (Utilities|String|ToString(Float) _returnvalue_6))
          (switch int (Variables|/Game/UI/WBP_HUD.WBP_HUD_C|GetCurrently_Equipped_Weapon_Image_Relation _hud_ref)
            (:0
              (Default|UpdateImgColourforAmmo (Variables|/Game/UI/WBP_HUD.WBP_HUD_C|GetWeapon_1 _hud_ref) _returnvalue_6))
            (:1
              (Default|UpdateImgColourforAmmo (Variables|/Game/UI/WBP_HUD.WBP_HUD_C|GetWeapon_2 _hud_ref) _returnvalue_6))
            (:2
              (Default|UpdateImgColourforAmmo (Variables|/Game/UI/WBP_HUD.WBP_HUD_C|GetWeapon_3 _hud_ref) _returnvalue_6)))
          (Default|PlayAmmoAnimation (Variables|/Game/Characters/Player/BPC_HUD.BPC_HUD_C|GetHUD_Ref (Actor|GetComponentbyClass (Components|GetOwner (Components|GetOwner)) "/Game/Characters/Player/BPC_HUD.BPC_HUD_C")) true))))))

(event Custom|Reload
  (bind _returnvalue (Components|GetOwner))
  (bind _current_ammo (Variables|Default|GetCurrent_Ammo))
  (bind _max_ammo (Variables|Default|GetMax_Ammo))
  (bind _returnvalue_2 (Math|Conversions|ToFloat(Integer) _max_ammo))
  (bind _returnvalue_3 (Math|Conversions|ToFloat(Integer) _current_ammo))
  (bind _returnvalue_4 (Components|GetOwner _returnvalue))
  (bind _returnvalue_5 (Actor|GetComponentbyClass _returnvalue_4 "/Game/Characters/Player/BPC_HUD.BPC_HUD_C"))
  (bind _returnvalue_6 (/ _returnvalue_3 _returnvalue_2))
  (bind _hud_ref (Variables|/Game/Characters/Player/BPC_HUD.BPC_HUD_C|GetHUD_Ref _returnvalue_5))
  (if (Variables|Default|GetReloading)
    (CallFunction|StopReload)
    (if (Utilities|DoesObjectImplementInterface (Components|GetOwner (Components|GetOwner)) "/Game/Characters/Player/BPI_Player.BPI_Player_C")
      (switch int (Variables|/Game/UI/WBP_HUD.WBP_HUD_C|GetCurrently_Equipped_Weapon_Image_Relation _hud_ref)
        (:0
          (Default|UpdateImgColourforAmmo (Variables|/Game/UI/WBP_HUD.WBP_HUD_C|GetWeapon_1 _hud_ref) _returnvalue_6))
        (:1
          (Default|UpdateImgColourforAmmo (Variables|/Game/UI/WBP_HUD.WBP_HUD_C|GetWeapon_2 _hud_ref) _returnvalue_6))
        (:2
          (Default|UpdateImgColourforAmmo (Variables|/Game/UI/WBP_HUD.WBP_HUD_C|GetWeapon_3 _hud_ref) _returnvalue_6)))
      (Default|PlayAmmoAnimation (Variables|/Game/Characters/Player/BPC_HUD.BPC_HUD_C|GetHUD_Ref (Actor|GetComponentbyClass (Components|GetOwner (Components|GetOwner)) "/Game/Characters/Player/BPC_HUD.BPC_HUD_C")) true))
    (else
      (CallFunction|StartReload))))

(event Custom|Start_Reload
  (bind _returnvalue (Components|GetOwner))
  (bind _returnvalue_2 (Components|GetOwner _returnvalue))
  (bind _returnvalue_3 (Utilities|DoesObjectImplementInterface _returnvalue_2 "/Game/Characters/Player/BPI_Player.BPI_Player_C"))
  (Variables|Default|SetStarting_Ammo_For_Reload (Variables|Default|GetCurrent_Ammo))
  (Variables|Default|SetReloading true)
  (if _returnvalue_3
    (bind _ranged_info (Class|BPIRangedWeapon|GetRangedInfo(Message) (Variables|/Game/Weapons/BPC_Player_Weaponry.BPC_Player_Weaponry_C|GetEquipped_Weapon (Actor|GetComponentbyClass _returnvalue_2 "/Game/Weapons/BPC_Player_Weaponry.BPC_Player_Weaponry_C")))))
  (Variables|Default|SetReload_Time (Math|Float|SelectFloat (.reload_time _ranged_info) 3.0 _returnvalue_3))
  ;[1 1 1] What reload percent needs to be to increase current ammo by 1
  (bind _output_get (Variables|Default|SetReload_Threshold (/ 1.0 (Math|Conversions|ToFloat(Integer) (Variables|Default|GetMax_Ammo)))))
  (Development|PrintString (Utilities|String|Append "RELOAD THRESHOLD : " (Utilities|String|ToString(Float) _output_get)))
  (bind _output_get_2 (Variables|Default|SetReload_Percent (/ (Math|Conversions|ToFloat(Integer) (Variables|Default|GetCurrent_Ammo)) (Math|Conversions|ToFloat(Integer) (Variables|Default|GetMax_Ammo)))))
  (if (> _output_get_2 0.0)
    (Variables|Default|SetReload_Time (* (Variables|Default|GetReload_Time) _output_get_2)))
  (Components|Tick|SetComponentTickEnabled true))

(event Custom|Stop_Reload
  (Variables|Default|SetReloading false)
  (Components|Tick|SetComponentTickEnabled false))

(event EventTick
  (params (DeltaSeconds :type Float%20%28single-precision%29))
  (bind _returnvalue (Components|GetOwner))
  (bind _returnvalue_2 (Components|GetOwner _returnvalue))
  (bind _returnvalue_3 (Actor|GetComponentbyClass _returnvalue_2 "/Game/Characters/Player/BPC_HUD.BPC_HUD_C"))
  (bind _hud_ref (Variables|/Game/Characters/Player/BPC_HUD.BPC_HUD_C|GetHUD_Ref _returnvalue_3))
  (bind _output_get (Variables|Default|SetReload_Percent (+ (Variables|Default|GetReload_Percent) (/ 1.0 (/ (Variables|Default|GetReload_Time) (Class|ActorComponent|GetComponentTickInterval))))))
  (Development|PrintString (Utilities|String|Append "RELOAD PERCENT : " (Utilities|String|ToString(Float) _output_get)))
  (bind _output_get_2 (Variables|Default|SetCurrent_Ammo (Math|Float|Truncate (/ (Variables|Default|GetReload_Percent) (Variables|Default|GetReload_Threshold)))))
  (Development|PrintString (Utilities|String|Append "CURRENT AMMO" (Utilities|String|ToString(Integer) _output_get_2)))
  (if (Utilities|DoesObjectImplementInterface (Components|GetOwner (Components|GetOwner)) "/Game/Characters/Player/BPI_Player.BPI_Player_C")
    (switch int (Variables|/Game/UI/WBP_HUD.WBP_HUD_C|GetCurrently_Equipped_Weapon_Image_Relation _hud_ref)
      (:0
        (Default|UpdateImgColourforAmmo (Variables|/Game/UI/WBP_HUD.WBP_HUD_C|GetWeapon_1 _hud_ref) (Variables|Default|GetReload_Percent)))
      (:1
        (Default|UpdateImgColourforAmmo (Variables|/Game/UI/WBP_HUD.WBP_HUD_C|GetWeapon_2 _hud_ref) (Variables|Default|GetReload_Percent)))
      (:2
        (Default|UpdateImgColourforAmmo (Variables|/Game/UI/WBP_HUD.WBP_HUD_C|GetWeapon_3 _hud_ref) (Variables|Default|GetReload_Percent))))
    (if (and (!= (Variables|Default|GetCurrent_Ammo) (Variables|Default|GetStarting_Ammo_For_Reload)) (and (>= (Math|Integer|%(Integer) (Math|Float|Truncate (* (Variables|Default|GetReload_Percent) 1e+02)) (Math|Float|Truncate (* (Variables|Default|GetReload_Threshold) 1e+02))) 0) (<= (Math|Integer|%(Integer) (Math|Float|Truncate (* (Variables|Default|GetReload_Percent) 1e+02)) (Math|Float|Truncate (* (Variables|Default|GetReload_Threshold) 1e+02))) 1)))
      (Default|PlayAmmoAnimation (Variables|/Game/Characters/Player/BPC_HUD.BPC_HUD_C|GetHUD_Ref (Actor|GetComponentbyClass (Components|GetOwner (Components|GetOwner)) "/Game/Characters/Player/BPC_HUD.BPC_HUD_C")) false)))
  ;[1 1 1] reaching max ammo stops
  (if (>= _output_get_2 (Variables|Default|GetMax_Ammo))
    (CallFunction|StopReload)
    (Variables|Default|SetReload_Percent 0.0)))

(event EventBeginPlay
  (Variables|Default|SetCurrent_Ammo (Variables|Default|GetMax_Ammo)))