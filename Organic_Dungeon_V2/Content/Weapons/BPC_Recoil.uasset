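; Weapon recoil component that kicks player 0's aim upward, knocks back the wielding character and shakes the camera.
; Start_Recoil sets a clamped pitch target, launches the owner's owner opposite its aim, and scales camera shake by recoil amount for BPI_Player implementers.
; Tick, enabled only during recoil, lerps control pitch to the target, then back toward the original, stopping within half the recoil amount.
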(event Custom|Camera%20Shake
  (bind _output_get (Variables|Default|SetCamera_Shake_Scale (Math|Float|Clamp(Float) (- (/ (Variables|Default|GetRecoil_Amount) 1e+01) 0.5) 0.0 2.5)))
  (Class|LegacyCameraShake|StartLegacyCameraShake (Game|GetPlayerCameraManager 0) "/Game/Weapons/BP_Recoil_Camera_Shake.BP_Recoil_Camera_Shake_C" _output_get "World" "0, 0, 0"))

(event Custom|Physical%20Recoil
  (Development|PrintString "PHYSICAL RECOIL")
  (Variables|Default|SetRecoil_Percent 0.0)
  (Variables|Default|SetOriginal_Aim_Rot (Pawn|GetControlRotation (Game|GetPlayerController 0) :!class /Script/Engine.Controller))
  (Variables|Default|SetRecoil_Active true)
  (Components|Tick|SetComponentTickEnabled true))

(event Custom|Start_Recoil
  (params (Recoil_Amount :type Float%20%28double-precision%29) (Recoil_Duration :type Float%20%28double-precision%29) (Knockback_Amount :type Float%20%28double-precision%29))
  (bind _returnvalue (Game|GetPlayerController 0))
  (bind _returnvalue_2 (Game|GetPlayerController 0))
  (bind _returnvalue_3 (Pawn|GetControlRotation _returnvalue :!class /Script/Engine.Controller))
  (bind _returnvalue_4 (Pawn|GetControlRotation _returnvalue_2 :!class /Script/Engine.Controller))
  (Variables|Default|SetRecoil_Amount Recoil_Amount)
  (Variables|Default|SetRecoil_Duration Recoil_Duration)
  (Variables|Default|SetKnockback_Amount Knockback_Amount)
  (Variables|Default|SetTarget_Aim_Rot (Math|Rotator|MakeRotator (.roll _returnvalue_3) (Math|Float|Clamp(Float) (+ (Math|Float|SelectFloat (- (.pitch _returnvalue_4) 3.6e+02) (.pitch _returnvalue_4) (>= (.pitch _returnvalue_4) 1.8e+02)) (Variables|Default|GetRecoil_Amount)) -9e+01 9e+01) (.yaw _returnvalue_3)))
  (CallFunction|PhysicalRecoil)
  (CallFunction|RecoilKnockback)
  (if (Utilities|DoesObjectImplementInterface (Components|GetOwner (Components|GetOwner)) "/Game/Characters/Player/BPI_Player.BPI_Player_C")
    (CallFunction|CameraShake)))

(event Custom|Recoil_Return
  (Development|PrintString "RECOIL RETURN")
  (Variables|Default|SetRecoil_Percent 0.0)
  (Variables|Default|SetRecoil_Active false))

(event Custom|Stop_Recoil
  (Components|Tick|SetComponentTickEnabled false))

(event Custom|Recoil_Knockback
  (bind _returnvalue (Components|GetOwner))
  (bind _returnvalue_2 (Components|GetOwner _returnvalue))
  (bind _aspawn (Utilities|Casting|CastToPawn _returnvalue_2))
  (bind _ascharacter (Utilities|Casting|CastToCharacter _returnvalue_2))
  (Development|PrintString (Utilities|String|ToString(Vector) (* (Math|Vector|GetForwardVector (Pawn|GetControlRotation (Pawn|GetController _aspawn) :!class /Script/Engine.Controller)) (* (Variables|Default|GetKnockback_Amount) -1.0))) true true "(R=1.000000,G=0.000000,B=0.050593,A=1.000000)")
  (Character|LaunchCharacter _ascharacter (* (Math|Vector|GetForwardVector (Pawn|GetControlRotation (Pawn|GetController _aspawn) :!class /Script/Engine.Controller)) (* (Variables|Default|GetKnockback_Amount) -1.0)) false false))

(event EventTick
  (params (DeltaSeconds :type Float%20%28single-precision%29))
  (bind _returnvalue (Game|GetPlayerController 0))
  (bind _returnvalue_2 (Game|GetPlayerController 0))
  (bind _returnvalue_3 (Game|GetPlayerController 0))
  (bind _target_aim_rot (Variables|Default|GetTarget_Aim_Rot))
  (bind _returnvalue_4 (Pawn|GetControlRotation _returnvalue_2 :!class /Script/Engine.Controller))
  (bind _returnvalue_5 (Pawn|GetControlRotation _returnvalue :!class /Script/Engine.Controller))
  (bind _returnvalue_6 (Pawn|GetControlRotation _returnvalue_3 :!class /Script/Engine.Controller))
  (bind (_roll _pitch _yaw) (Math|Rotator|BreakRotator _returnvalue_4))
  (bind _output_get (Variables|Default|SetRecoil_Percent (+ (Variables|Default|GetRecoil_Percent) (/ 1.0 (/ (Variables|Default|GetRecoil_Duration) (Class|ActorComponent|GetComponentTickInterval))))))
  (if (and (Variables|Default|GetRecoil_Active) (<= _output_get 1.0))
    (Pawn|SetControlRotation (Game|GetPlayerController 0) (Math|Rotator|Lerp(Rotator) (Math|Rotator|MakeRotator (.roll _returnvalue_5) (.pitch _returnvalue_5) (.yaw _returnvalue_5)) (Math|Rotator|MakeRotator (.roll _returnvalue_5) (.pitch (Variables|Default|GetTarget_Aim_Rot)) (.yaw _returnvalue_5)) (Variables|Default|GetRecoil_Percent) true))
    (if (or (Utilities|Operators|EqualEqual _returnvalue_6 _target_aim_rot 1.0) (>= (.Pitch (Math|Rotator|BreakRotator _returnvalue_6)) (.Pitch (Math|Rotator|BreakRotator _target_aim_rot))))
      (CallFunction|RecoilReturn))
    (else
      (Development|PrintString "RETURNING RECOIL")
      (Pawn|SetControlRotation (Game|GetPlayerController 0) (Math|Rotator|Lerp(Rotator) _returnvalue_4 (Math|Rotator|MakeRotator _roll (.pitch (Variables|Default|GetOriginal_Aim_Rot)) _yaw) (Variables|Default|GetRecoil_Percent) true))
      (if (<= (.Pitch (Math|Rotator|BreakRotator _returnvalue_4)) (+ (.Pitch (Math|Rotator|BreakRotator (Variables|Default|GetOriginal_Aim_Rot))) (/ (Variables|Default|GetRecoil_Amount) 2.0)))
        (CallFunction|StopRecoil)))))