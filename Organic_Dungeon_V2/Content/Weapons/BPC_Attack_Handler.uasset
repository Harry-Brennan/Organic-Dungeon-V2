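; Attack handler component that turns IA_Attack input into shots from the player's equipped weapon.
; The weapon's fire type selects semi-auto (DoOnce reset on release), full-auto (delay-gated by fire rate) or burst (custom delayed-loop macro with cooldown).
; Handle_Attack checks for BPI_Player, a valid weapon and ammo, then passes a DT_Projectiles row to the weapon's BPC_Shoot.
; Melee attacks only print a placeholder message.
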(event Custom|Handle_Attack
  (bind _returnvalue (Components|GetOwner))
  (bind _returnvalue_2 (Actor|GetComponentbyClass _returnvalue "/Game/Weapons/BPC_Player_Weaponry.BPC_Player_Weaponry_C"))
  (bind _equipped_weapon (Variables|/Game/Weapons/BPC_Player_Weaponry.BPC_Player_Weaponry_C|GetEquipped_Weapon _returnvalue_2))
  (if (Utilities|DoesObjectImplementInterface _returnvalue "/Game/Characters/Player/BPI_Player.BPI_Player_C")
    (Utilities|IsValid _equipped_weapon
      (:Is%20Valid
        (bind _basics (Class|BPIWeapon|GetBasicInfo(Message) _equipped_weapon))
        (if (.ranged _basics)
          (if (> (Variables|/Game/Weapons/BPC_Ammo.BPC_Ammo_C|GetCurrent_Ammo (Actor|GetComponentbyClass _equipped_weapon "/Game/Weapons/BPC_Ammo.BPC_Ammo_C")) 0)
            (bind _ranged_info (Class|BPIRangedWeapon|GetRangedInfo(Message) _equipped_weapon))
            (bind _returnvalue_3 (Utilities|GetDataTableRow "/Game/Projectiles/DT_Projectiles.DT_Projectiles" (Utilities|String|StringToName (Utilities|String|EnumtoString (.ProjectileName (Utilities|Struct|BreakStruct_Ranged_Weapon _ranged_info)))))
              (:then
                (Variables|Default|SetAttacking false)
                (Default|Shoot (Actor|GetComponentbyClass _equipped_weapon "/Game/Weapons/BPC_Shoot.BPC_Shoot_C") _returnvalue_3 _ranged_info)
                (if (Utilities|Enum|Equal(Enum) (.Fire_Type (Utilities|Struct|BreakStruct_Ranged_Weapon _ranged_info)) "NewEnumerator2")
                  (Variables|Default|SetCan_Fire false)
                  (Utilities|FlowControl|Delay (.Fire_Rate (Utilities|Struct|BreakStruct_Ranged_Weapon _ranged_info)))
                  (Variables|Default|SetCan_Fire true)))
              (:RowNotFound
                (Development|PrintString "Projectile row not found"))))
          (else
            (Development|PrintString "Melee attack")))))))

(event Input|EnhancedActionEvents|EnhancedInputActionIA_Attack
  (params (ActionValue :type Boolean) (ElapsedSeconds :type Float%20%28double-precision%29) (TriggeredSeconds :type Float%20%28double-precision%29) (InputAction :type Input%20Action%20Object%20Reference :default "/Game/Characters/Player/Input/Actions/IA_Attack.IA_Attack"))
  (:Triggered
    (if (not (and (Variables|Default|GetAttacking) (Variables|Default|GetCan_Fire)))
      (bind _ranged_info (Class|BPIRangedWeapon|GetRangedInfo(Message) (Variables|/Game/Weapons/BPC_Player_Weaponry.BPC_Player_Weaponry_C|GetEquipped_Weapon (Actor|GetComponentbyClass (Components|GetOwner) "/Game/Weapons/BPC_Player_Weaponry.BPC_Player_Weaponry_C"))))
      (switch Utilities|FlowControl|Switch|SwitchonEnum_Fire_Types (.fire_type _ranged_info)
        (:NewEnumerator1
          (Utilities|FlowControl|DoOnce false :!label _label
            (:Completed
              (Development|PrintString "HANDLING ATTACK FROM STARTED")
              (CallFunction|HandleAttack))))
        (:NewEnumerator2
          (if (Variables|Default|GetCan_Fire)
            (Development|PrintString "HANDLING ATTACK FROM TRIGGERED")
            (CallFunction|HandleAttack)))
        (:NewEnumerator3
          (if (Variables|Default|GetCan_Fire)
            (Variables|Default|SetCan_Fire false)
            (Utilities|BurstLoopDelayFire 1 (._burst_projectiles _ranged_info) (.time_between_burst _ranged_info)
              (:Loop%20Body
                (CallFunction|HandleAttack))
              (:Completed
                (Utilities|FlowControl|Delay (.fire_rate _ranged_info))
                (Variables|Default|SetCan_Fire true))))))))
  (:Canceled
    (goto _label Reset))
  (:Completed
    (goto _label Reset)))