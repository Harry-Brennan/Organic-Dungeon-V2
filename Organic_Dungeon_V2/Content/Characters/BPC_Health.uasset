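; BPC_Health is a health component that tracks current and max health, shown as a row of hearts for owners implementing BPI_Player.
; For players, BeginPlay fills WBP_Health from the HUD component; heal and damage toggle and animate individual WBP_Heart widgets.
; Max-health changes add or remove hearts, with increases recounting current health from filled hearts.
; Four debug keys exercise these events, and Death is an empty stub.
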(event Custom|Take_Damage
  (params (Damage_To_Take :type Float%20%28double-precision%29))
  (bind _health_widget (Variables|Default|GetHealth_Widget))
  (bind _hearts_wrapbox (Variables|/Game/UI/WBP_Health.WBP_Health_C|GetHearts_WrapBox _health_widget))
  (bind _returnvalue (Class|PanelWidget|GetAllChildren _hearts_wrapbox))
  (bind _output_get (Variables|Default|SetCurrent_Health (- (Variables|Default|GetCurrent_Health) (Math|Float|Floor Damage_To_Take))))
  (if (<= _output_get 0)
    (CallFunction|Death)
    (elif (Utilities|DoesObjectImplementInterface (Components|GetOwner) "/Game/Characters/Player/BPI_Player.BPI_Player_C")
      (bind _array_index (Utilities|Array|ForEachLoopwithBreak _returnvalue :!label _label)
        (:LoopBody
          (bind _aswbp_heart (Utilities|Casting|CastToWBP_Heart (Utilities|Array|Get(acopy) _returnvalue (- (Utilities|Array|Length _returnvalue) _array_index))))
          (if (Variables|/Game/UI/WBP_Heart.WBP_Heart_C|GetFilled? _aswbp_heart)
            (Variables|/Game/UI/WBP_Heart.WBP_Heart_C|SetFilled? _aswbp_heart false)
            (Default|PlayTakeDamageAnim _aswbp_heart)
            (goto _label Break)))))))

(event Custom|Death)

(event Custom|Heal
  (if (Utilities|DoesObjectImplementInterface (Components|GetOwner) "/Game/Characters/Player/BPI_Player.BPI_Player_C")
    (bind _array_element (Utilities|Array|ForEachLoopwithBreak (Class|PanelWidget|GetAllChildren (Variables|/Game/UI/WBP_Health.WBP_Health_C|GetHearts_WrapBox (Variables|Default|GetHealth_Widget))) :!label _label)
      (:LoopBody
        (bind _aswbp_heart (Utilities|Casting|CastToWBP_Heart _array_element))
        (if (not (Variables|/Game/UI/WBP_Heart.WBP_Heart_C|GetFilled? _aswbp_heart))
          (Variables|/Script/UMG.Image|SetColorAndOpacity (Variables|/Game/UI/WBP_Heart.WBP_Heart_C|GetHeart_Filled_Img _aswbp_heart) (Math|Color|MakeColor 1.0 1.0 1.0))
          (Variables|/Game/UI/WBP_Heart.WBP_Heart_C|SetFilled? _aswbp_heart true)
          (Math|Integer|IncrementInt (Variables|Default|GetCurrent_Health)
            (:%20%20
              (Default|PlayHealAnim _aswbp_heart)
              (goto _label Break))))))
    (else
      (Math|Integer|IncrementInt (Variables|Default|GetCurrent_Health)))))

(event EventBeginPlay
  (if (Utilities|DoesObjectImplementInterface (Components|GetOwner) "/Game/Characters/Player/BPI_Player.BPI_Player_C")
    (bind _array_element (Utilities|Array|ForEachLoopwithBreak (Actor|GetComponentsByClass (Components|GetOwner) "/Script/UMG.WidgetComponent") :!label _label)
      (:LoopBody
        (bind _aswbp_health (Utilities|Casting|CastToWBP_Health (UserInterface|GetWidget _array_element)))
        (goto _label Break))
      (:Completed
        (Variables|Default|SetHealth_Widget (select (Utilities|DoesObjectImplementInterface (Components|GetOwner) "/Game/Characters/Player/BPI_Player.BPI_Player_C") (Variables|/Game/UI/WBP_HUD.WBP_HUD_C|GetWBP_Health (Variables|/Game/Characters/Player/BPC_HUD.BPC_HUD_C|GetHUD_Ref (Actor|GetComponentbyClass (Components|GetOwner) "/Game/Characters/Player/BPC_HUD.BPC_HUD_C"))) _aswbp_health))
        (for _index (range 1 (Variables|Default|GetMax_Health))
          (Default|AddHeart (Variables|Default|GetHealth_Widget)))))))

(event Input|KeyboardEvents|DebugKey1
  (params (Key :type Key%20Structure :default "None") (ActionValue :type Input%20Action%20Value%20Structure))
  (:Pressed
    (CallFunction|TakeDamage 0.0)))

(event Input|KeyboardEvents|DebugKey2
  (params (Key :type Key%20Structure :default "None") (ActionValue :type Input%20Action%20Value%20Structure))
  (:Pressed
    (CallFunction|Heal)))

(event Input|KeyboardEvents|DebugKey3
  (params (Key :type Key%20Structure :default "None") (ActionValue :type Input%20Action%20Value%20Structure))
  (:Pressed
    (CallFunction|DecreaseMaxHealth)))

(event Input|KeyboardEvents|DebugKey4
  (params (Key :type Key%20Structure :default "None") (ActionValue :type Input%20Action%20Value%20Structure))
  (:Pressed
    (CallFunction|IncreaseMaxHealth)))

(event Custom|Increase_Max_Health
  (bind _health_widget (Variables|Default|GetHealth_Widget))
  (bind _hearts_wrapbox (Variables|/Game/UI/WBP_Health.WBP_Health_C|GetHearts_WrapBox _health_widget))
  (bind _returnvalue (Class|PanelWidget|GetAllChildren _hearts_wrapbox))
  (Math|Integer|IncrementInt (Variables|Default|GetMax_Health)
    (:%20%20
      (Default|AddHeart _health_widget)
      (bind _array_element (Utilities|Array|ForEachLoopwithBreak _returnvalue :!label _label)
        (:LoopBody
          (bind _aswbp_heart (Utilities|Casting|CastToWBP_Heart _array_element))
          (if (not (Variables|/Game/UI/WBP_Heart.WBP_Heart_C|GetFilled? _aswbp_heart))
            (Default|PlayHealAnim _aswbp_heart)
            (Variables|/Game/UI/WBP_Heart.WBP_Heart_C|SetFilled? _aswbp_heart true)
            (bind _aswbp_heart_2 (Utilities|Casting|CastToWBP_Heart (Class|PanelWidget|GetChildat _hearts_wrapbox (Utilities|Array|LastIndex _returnvalue))))
            (Variables|/Script/UMG.Image|SetColorAndOpacity (Variables|/Game/UI/WBP_Heart.WBP_Heart_C|GetHeart_Filled_Img _aswbp_heart_2) (Math|Color|MakeColor 0.0 0.0 0.0))
            (Variables|/Game/UI/WBP_Heart.WBP_Heart_C|SetFilled? _aswbp_heart_2 false)
            (goto _label Break)))
        (:Completed
          (Variables|Default|SetCurrent_Health 0)
          (for _array_element_2 (Class|PanelWidget|GetAllChildren (Variables|/Game/UI/WBP_Health.WBP_Health_C|GetHearts_WrapBox (Variables|Default|GetHealth_Widget)))
            (bind _aswbp_heart_3 (Utilities|Casting|CastToWBP_Heart _array_element_2))
            (if (Variables|/Game/UI/WBP_Heart.WBP_Heart_C|GetFilled? _aswbp_heart_3)
              (Math|Integer|IncrementInt (Variables|Default|GetCurrent_Health)
                (:%20%20
                  (Default|PlayHealAnim _aswbp_heart_3))))))))))

(event Custom|Decrease_Max_Health
  (Math|Integer|DecrementInt (Variables|Default|GetMax_Health)
    (:%20%20
      (if (> (Variables|Default|GetCurrent_Health) (Variables|Default|GetMax_Health))
        (Variables|Default|SetCurrent_Health (Variables|Default|GetMax_Health)))
      (Class|PanelWidget|RemoveChildat (Variables|/Game/UI/WBP_Health.WBP_Health_C|GetHearts_WrapBox (Variables|Default|GetHealth_Widget)) (Utilities|Array|LastIndex (Class|PanelWidget|GetAllChildren (Variables|/Game/UI/WBP_Health.WBP_Health_C|GetHearts_WrapBox (Variables|Default|GetHealth_Widget)))))
      (if (<= (Variables|Default|GetMax_Health) 0)
        (CallFunction|Death)))))