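; Player character component that rolls the camera through control rotation for strafing, sliding and wall running.
; Tick leans it with local sideways velocity, pausing near vertical pitch and while BPC_Slide or BPC_WallRunning state flags are set.
; Separate slide and wall-run events each apply one FInterpTo step per call toward their tilt.
; Wallrunning_Left has no DeltaTime wired, and Stopping_Wallrunning_Tilt is empty.
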(event Custom|Into_Sliding
  (bind _controller (Variables|Default|GetController))
  (bind _sliding_camera_tilt_amount (Variables|Default|GetSliding_Camera_Tilt_Amount))
  (bind _returnvalue (Pawn|GetControlRotation _controller :!class /Script/Engine.Controller))
  (Pawn|SetControlRotation _controller (Math|Rotator|MakeRotator (Math|Float|Clamp(Float) (Math|Interpolation|FInterpTo (.roll (Transformation|GetWorldRotation (Variables|Default|GetCamera))) _sliding_camera_tilt_amount (Utilities|Time|GetWorldDeltaSeconds) 2.0) (* _sliding_camera_tilt_amount -1.0) _sliding_camera_tilt_amount) (.pitch _returnvalue) (.yaw _returnvalue))))

(event Custom|Out_Sliding
  (bind _controller (Variables|Default|GetController))
  (bind _returnvalue (Pawn|GetControlRotation _controller :!class /Script/Engine.Controller))
  (Pawn|SetControlRotation _controller (Math|Rotator|MakeRotator (Math|Interpolation|FInterpTo (.roll (Transformation|GetWorldRotation (Variables|Default|GetCamera))) 0.0 (Utilities|Time|GetWorldDeltaSeconds) 2.0) (.pitch _returnvalue) (.yaw _returnvalue))))

(event Custom|Wallrunning_Left
  (bind _controller (Variables|Default|GetController))
  (bind _returnvalue (Pawn|GetControlRotation _controller :!class /Script/Engine.Controller))
  (Pawn|SetControlRotation _controller (Math|Rotator|MakeRotator (Math|Interpolation|FInterpTo (.roll (Transformation|GetWorldRotation (Variables|Default|GetCamera))) (Variables|Default|GetWallrunning_Camera_Tilt_Amount) 0.0 2.0) (.pitch _returnvalue) (.yaw _returnvalue))))

(event Custom|Wallrunning_Right
  (bind _controller (Variables|Default|GetController))
  (bind _returnvalue (Pawn|GetControlRotation _controller :!class /Script/Engine.Controller))
  (Pawn|SetControlRotation _controller (Math|Rotator|MakeRotator (Math|Interpolation|FInterpTo (.roll (Transformation|GetWorldRotation (Variables|Default|GetCamera))) (* (Variables|Default|GetWallrunning_Camera_Tilt_Amount) -1.0) (Utilities|Time|GetWorldDeltaSeconds) 2.0) (.pitch _returnvalue) (.yaw _returnvalue))))

(event Custom|Stopping_Wallrunning_Tilt)

(event EventBeginPlay
  (Variables|Default|SetCamera (Actor|GetComponentbyClass (Components|GetOwner) "/Script/Engine.CameraComponent"))
  (bind _ascharacter (Utilities|Casting|CastToCharacter (Components|GetOwner)))
  (Variables|Default|SetController (Pawn|GetController _ascharacter)))

(event EventTick
  (params (DeltaSeconds :type Float%20%28single-precision%29))
  (bind _returnvalue (Components|GetOwner))
  (bind _returnvalue_2 (Components|GetOwner))
  (bind _returnvalue_3 (Utilities|Time|GetWorldDeltaSeconds))
  (bind _camera (Variables|Default|GetCamera))
  (bind _controller (Variables|Default|GetController))
  (bind _controller_2 (Variables|Default|GetController))
  (bind _returnvalue_4 (Actor|GetComponentbyClass _returnvalue "/Game/Movement/Sliding/BPC_Slide.BPC_Slide_C"))
  (bind _returnvalue_5 (Pawn|GetControlRotation _controller_2 :!class /Script/Engine.Controller))
  (bind _returnvalue_6 (Transformation|GetVelocity _returnvalue_2))
  (bind _returnvalue_7 (Transformation|GetActorRotation _returnvalue_2))
  (bind _returnvalue_8 (Pawn|GetControlRotation _controller :!class /Script/Engine.Controller))
  (bind _returnvalue_9 (Transformation|GetWorldRotation _camera))
  (bind _returnvalue_10 (Actor|GetComponentbyClass _returnvalue "/Game/Movement/Wall-Running/BPC_Wall-Running.BPC_Wall-Running_C"))
  (bind _returnvalue_11 (Math|Vector|UnrotateVector _returnvalue_6 _returnvalue_7))
  (bind _returnvalue_12 (/ (.y _returnvalue_11) 1e+03))
  (bind _returnvalue_13 (* _returnvalue_12 4.0))
  (bind _returnvalue_14 (Math|Interpolation|FInterpTo (.roll _returnvalue_9) _returnvalue_13 _returnvalue_3 2.0))
  (if (Math|Boolean|ANDBoolean (Math|Boolean|ANDBoolean (not (Variables|/Game/Movement/Sliding/BPC_Slide.BPC_Slide_C|GetSliding _returnvalue_4)) (not (Variables|/Game/Movement/Sliding/BPC_Slide.BPC_Slide_C|GetStarting_Sliding _returnvalue_4)) (not (Variables|/Game/Movement/Sliding/BPC_Slide.BPC_Slide_C|GetStopping_Sliding _returnvalue_4)) (not (Variables|/Game/Movement/Wall-Running/BPC_Wall-Running.BPC_Wall-Running_C|GetCan_Wall_Run _returnvalue_10)) (not (Variables|/Game/Movement/Wall-Running/BPC_Wall-Running.BPC_Wall-Running_C|GetWall_Run_Right _returnvalue_10)) (not (Variables|/Game/Movement/Wall-Running/BPC_Wall-Running.BPC_Wall-Running_C|GetWall_Run_Left _returnvalue_10))) (not (or (and (>= (.pitch _returnvalue_5) 85.0) (<= (.pitch _returnvalue_5) 255.0)) (and (<= (.pitch _returnvalue_5) 275.0) (>= (.pitch _returnvalue_5) 255.0)))) (not (Math|Float|NearlyEqual(Float) (.roll _returnvalue_9) _returnvalue_14 0.002)))
    (Pawn|SetControlRotation _controller (Math|Rotator|MakeRotator (Math|Float|Clamp(Float) _returnvalue_14 -4.0 4.0) (.pitch _returnvalue_8) (.yaw _returnvalue_8)))))