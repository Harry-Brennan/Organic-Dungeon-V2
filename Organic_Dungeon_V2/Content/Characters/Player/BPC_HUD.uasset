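; Player HUD component that creates the HUD widget and relays weapon icon swaps, crosshair visibility and texture, and hit crosshair animation to it.
; Once ticking is enabled shortly after BeginPlay, it polls sibling aim, attack, slide, jump, wall-run, sprint and weaponry components each frame.
; The AvailableAction helper turns those states into key-hint prompts, adding or removing each on the available-actions widget.
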(event Custom|Swap_Weapon_Icons
  (params (Next? :type Boolean))
  (Default|UpdateEquippedWeaponUI (Variables|Default|GetHUD_Ref) Next?))

(event Custom|Update_Crosshair
  (params (Aiming :type Boolean))
  (bind _ranged_info (Class|BPIRangedWeapon|GetRangedInfo(Message) (Variables|/Game/Weapons/Actor_Components/BPC_Weaponry.BPC_Weaponry_C|GetEquipped_Weapon (Actor|GetComponentbyClass (Components|GetOwner) "/Game/Weapons/Actor_Components/BPC_Weaponry.BPC_Weaponry_C"))))
  (Default|UpdateCrosshairVisibility (Variables|Default|GetHUD_Ref) Aiming (.crosshair _ranged_info)))

(event Custom|Play_Hit_Crosshair_Anim
  (Default|PlayFireAnim (Variables|/Game/UI/WBP_HUD.WBP_HUD_C|GetWBP_Crosshair (Variables|Default|GetHUD_Ref))))

(event EventTick
  (params (DeltaSeconds :type Float%20%28single-precision%29))
  (bind _returnvalue (Components|GetOwner))
  (bind _returnvalue_2 (Components|GetOwner))
  (bind _returnvalue_3 (Components|GetOwner))
  (bind _returnvalue_4 (Actor|GetComponentbyClass _returnvalue_3 "/Game/Weapons/Actor_Components/BPC_Attack_Handler.BPC_Attack_Handler_C"))
  (bind _returnvalue_5 (Actor|GetComponentbyClass _returnvalue_2 "/Game/Weapons/Actor_Components/BPC_Weaponry.BPC_Weaponry_C"))
  (bind _returnvalue_6 (Actor|GetComponentbyClass _returnvalue_3 "/Game/Movement/Sliding/BPC_Slide.BPC_Slide_C"))
  (bind _returnvalue_7 (Actor|GetComponentbyClass _returnvalue "/Game/Weapons/Actor_Components/BPC_Weaponry.BPC_Weaponry_C"))
  (bind _equipped_weapon (Variables|/Game/Weapons/Actor_Components/BPC_Weaponry.BPC_Weaponry_C|GetEquipped_Weapon _returnvalue_5))
  (bind _sliding (Variables|/Game/Movement/Sliding/BPC_Slide.BPC_Slide_C|GetSliding _returnvalue_6))
  (bind _equipped_weapon_2 (Variables|/Game/Weapons/Actor_Components/BPC_Weaponry.BPC_Weaponry_C|GetEquipped_Weapon _returnvalue_7))
  (Utilities|FlowControl|Sequence
    (:then_0
      ;[1 1 1] Aiming
      (Utilities|AvailableAction (Variables|/Game/Weapons/Actor_Components/BPC_Aim.BPC_Aim_C|GetCanAim? (Actor|GetComponentbyClass (Components|GetOwner) "/Game/Weapons/Actor_Components/BPC_Aim.BPC_Aim_C")) "AIM - LEFT MOUSE"))
    (:then_1
      ;[1 1 1] firing ranged weapon
      (Utilities|AvailableAction (and (Variables|/Game/Weapons/Actor_Components/BPC_Attack_Handler.BPC_Attack_Handler_C|GetCan_Fire _returnvalue_4) (not (Variables|/Game/Weapons/Actor_Components/BPC_Attack_Handler.BPC_Attack_Handler_C|GetAttacking _returnvalue_4))) "FIRE - RIGHT MOUSE"))
    (:then_2
      ;[1 1 1] Sliding
      (Utilities|AvailableAction (and (Variables|/Game/Movement/Sliding/BPC_Slide.BPC_Slide_C|GetCan_Slide _returnvalue_6) (not _sliding)) "SLIDE - CONTROL"))
    (:then_3
      ;[1 1 1] Stopping sliding
      (Utilities|AvailableAction (and (Variables|/Game/Movement/Sliding/BPC_Slide.BPC_Slide_C|GetCan_Stop_Sliding _returnvalue_6) _sliding) "STOP SLIDING - RELEASE CONTROL"))
    (:then_4
      ;[1 1 1] Reloading ranged
      (if (Utilities|IsValid _equipped_weapon)
        (bind _basics (Class|BPIWeapon|GetBasicInfo(Message) _equipped_weapon))
        (Utilities|AvailableAction (.ranged _basics) "RELOAD - R")))
    (:then_5
      ;[1 1 1] Double jump
      (Utilities|AvailableAction (Variables|/Game/Movement/Double_Jump/BPC_Double_Jump.BPC_Double_Jump_C|GetCan_Double_Jump (Actor|GetComponentbyClass (Components|GetOwner) "/Game/Movement/Double_Jump/BPC_Double_Jump.BPC_Double_Jump_C")) "DOUBLE JUMP - SPACE"))
    (:then_6
      ;[1 1 1] Slide jump
      (Utilities|AvailableAction (Variables|/Game/Movement/Sliding/BPC_Slide.BPC_Slide_C|GetSliding (Actor|GetComponentbyClass (Components|GetOwner) "/Game/Movement/Sliding/BPC_Slide.BPC_Slide_C")) "SLIDE JUMP - SPACE"))
    (:then_7
      ;[1 1 1] Wall-run jump
      (Utilities|AvailableAction (Variables|/Game/Movement/Wall-Running/BPC_Wall-Running.BPC_Wall-Running_C|GetWall-Running (Actor|GetComponentbyClass (Components|GetOwner) "/Game/Movement/Wall-Running/BPC_Wall-Running.BPC_Wall-Running_C")) "WALL-RUN JUMP - SPACE"))
    (:then_8
      ;[1 1 1] Sprinting
      (Utilities|AvailableAction (Variables|/Game/Movement/Sprinting/BPC_Sprint.BPC_Sprint_C|GetCan_Sprint (Actor|GetComponentbyClass (Components|GetOwner) "/Game/Movement/Sprinting/BPC_Sprint.BPC_Sprint_C")) "SPRINT - SHIFT"))
    (:then_9
      (if (Utilities|IsValid _equipped_weapon_2)
        (bind _basics_2 (Class|BPIWeapon|GetBasicInfo(Message) _equipped_weapon_2))
        ;[1 1 1] Melee attack with melee weapon
        (Utilities|AvailableAction (not (.ranged _basics_2)) "LEFT MOUSE - MELEE ATTACK")))))

(event EventBeginPlay
  (bind _returnvalue (UserInterface|CreateWidget "/Game/UI/WBP_HUD.WBP_HUD_C"))
  (UserInterface|Viewport|AddtoViewport _returnvalue 0)
  (Variables|Default|SetHUD_Ref _returnvalue)
  (Utilities|FlowControl|Delay 0.2)
  (Components|Tick|SetComponentTickEnabled true))