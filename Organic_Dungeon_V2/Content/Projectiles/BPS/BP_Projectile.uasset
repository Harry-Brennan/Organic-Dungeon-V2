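; Data-driven projectile actor whose speed, gravity, mesh and on-hit behavior come from ProjectileInfo and DT_Projectiles.
; Construction and BeginPlay configure movement and mesh once the table row is found.
; When movement stops, it branches on hit effect: bullet impact by collision type (decal, particle and sound, or physics push), explosion via BPCExplode, or direct damage.
; DealDamage feeds the target's health and optional blood-effect components, then destroys the projectile.
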(event OnProjectileStop(ProjectileMovement)
  (params (ImpactResult :type Hit%20Result%20Structure%20%28by%20ref%29))
  (bind _returnvalue (Math|Random|RandomFloatinRange 5.0 15.0))
  (bind (_bblockinghit _binitialoverlap _time _distance _location _impactpoint _normal _impactnormal _physmat _hitactor _hitcomponent) (Collision|BreakHitResult ImpactResult))
  (bind _projectile_info (Variables|Default|GetProjectile_Info))
  (bind _projectile_info_2 (Variables|Default|GetProjectile_Info))
  (bind _returnvalue_2 (Math|Conversions|RotationFromXVector _impactnormal))
  (Development|PrintString "projectile stopped")
  (switch Utilities|FlowControl|Switch|SwitchonEnum_On_Hit_Effects (.onhiteffect _projectile_info)
    (:NewEnumerator0
      (switch Utilities|FlowControl|Switch|SwitchonECollisionChannel (Collision|GetCollisionObjectType _hitcomponent)
        (:ECC_WorldStatic
          (Rendering|Decal|SpawnDecalatLocation "/Game/Projectiles/Bullet_Hole/M_Bullet_Hole.M_Bullet_Hole" (Math|Vector|MakeVector _returnvalue _returnvalue _returnvalue) _impactpoint _returnvalue_2 1e+01 :!label _label)
          (Game|SpawnActorfromClass "/Game/VFX_SFX/Realistic_Starter_VFX_Pack_Vol2/Blueprints/Spawn_Particle.Spawn_Particle_C" (Math|Transform|MakeTransform _impactpoint _returnvalue_2 "0.100000,0.100000,0.100000") "AlwaysSpawn" "MultiplyWithRoot" 0 1.0 false "/Game/VFX_SFX/Realistic_Starter_VFX_Pack_Vol2/Particles/Explosion/P_Explosion_Big_A.P_Explosion_Big_A" 0)
          (Audio|PlaySoundatLocation "/Game/VFX_SFX/Sounds/Bullet_Impact/Bullet_Impact_SC.Bullet_Impact_SC" _impactpoint "0, 0, 0" 1.0 1.0 0.0 0 0 0 0)
          (Actor|DestroyActor))
        (:ECC_WorldDynamic
          (goto _label))
        (:ECC_Pawn
          (Actor|DestroyActor))
        (:ECC_PhysicsBody
          (Physics|AddForce _hitcomponent (+ (* (Transformation|GetActorUpVector) (* (.speed _projectile_info_2) 1e+01)) (* (Transformation|GetActorForwardVector) (* (.speed _projectile_info_2) 5e+01))) "None" true)
          (Actor|DestroyActor))))
    (:NewEnumerator1
      (Default|Explode (Variables|Default|GetBPC_Explode) _location (.explosiononhit _projectile_info) true (.speed _projectile_info) (.damage _projectile_info) false))
    (:NewEnumerator2
      (CallFunction|DealDamage (.damage _projectile_info) _hitactor _location _impactnormal))))

(event EventBeginPlay
  (bind _projectile_info (Variables|Default|GetProjectile_Info))
  (bind _projectilemovement (Variables|Default|GetProjectileMovement))
  (Utilities|GetDataTableRow "/Game/Projectiles/Structs_DataTables/DT_Projectiles.DT_Projectiles" (Utilities|String|StringToName (Utilities|String|EnumtoString (.name (Variables|Default|GetProjectile_Info))))
    (:then
      (bind _output_get (Variables|/Script/Engine.ProjectileMovementComponent|SetInitialSpeed _projectilemovement (.speed _projectile_info)))
      (Variables|/Script/Engine.ProjectileMovementComponent|SetMaxSpeed _projectilemovement _output_get)
      (Components|StaticMesh|SetStaticMesh (Variables|Default|GetStaticMesh) (.mesh _projectile_info))
      (bind _output_get_2 (Variables|/Script/Engine.ProjectileMovementComponent|SetProjectileGravityScale (Variables|Default|GetProjectileMovement) (.gravity _projectile_info)))
      (Development|PrintString (Utilities|String|ToString(Float) _output_get_2)))))

(fn ConstructionScript
  (bind _projectilemovement (Variables|Default|GetProjectileMovement))
  (bind _projectile_info (Variables|Default|GetProjectile_Info))
  (bind _returnvalue (Utilities|GetDataTableRow "/Game/Projectiles/Structs_DataTables/DT_Projectiles.DT_Projectiles" (Utilities|String|StringToName (Utilities|String|EnumtoString (.name _projectile_info))))
    (:then
      (bind _output_get (Variables|/Script/Engine.ProjectileMovementComponent|SetInitialSpeed _projectilemovement (.speed _projectile_info)))
      (Variables|/Script/Engine.ProjectileMovementComponent|SetMaxSpeed _projectilemovement _output_get)
      (Components|StaticMesh|SetStaticMesh (Variables|Default|GetStaticMesh) (.mesh _returnvalue))
      (Variables|/Script/Engine.ProjectileMovementComponent|SetProjectileGravityScale (Variables|Default|GetProjectileMovement) (.gravity _projectile_info)))))

(fn DealDamage
  (params (Damage :type Float%20%28double-precision%29) (To%20Who :type Actor%20Object%20Reference) (Where :type Vector) (Normal :type Vector))
  (bind _returnvalue (Actor|GetComponentbyClass To%20Who "/Game/VFX_SFX/Blood_Splatter/BPS/BPC_Blood_Effect.BPC_Blood_Effect_C"))
  (Default|TakeDamage (Actor|GetComponentbyClass To%20Who "/Game/Health/BPs/BPC_Health.BPC_Health_C") Damage Where To%20Who)
  (Utilities|IsValid _returnvalue
    (:Is%20Valid
      (Default|BloodEffect _returnvalue Where Normal To%20Who Damage))
    (:Is%20Not%20Valid
      _))
  (Actor|DestroyActor))