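; Actor component that plays surface-specific footstep sounds and ground particles for a character's feet.
; Each tick while not falling, it traces from each foot bone along the actor's negative up vector.
; A per-bone map fires effects once per contact, resetting when the trace misses.
; The hit's physical surface picks the sound and Niagara colour, and movement speed feeds a particle parameter.
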(event EventBeginPlay
  (for _array_element (Variables|Bones|GetFeet_Bones)
    (Utilities|Map|Add (Variables|Bones|GetBone%20-%20Played%20Sound) _array_element false))
  (Variables|Default|SetMesh (Actor|GetComponentbyClass (Components|GetOwner) "/Script/Engine.SkeletalMeshComponent")))

(event EventTick
  (params (DeltaSeconds :type Float%20%28single-precision%29))
  (if (not (AI|Components|NavMovement|IsFalling (Actor|GetComponentbyClass (Components|GetOwner) "/Script/Engine.CharacterMovementComponent")))
    (for _array_element (Variables|Bones|GetFeet_Bones)
      (CallFunction|Footstep _array_element))))

(fn Footstep
  (params (Bone :type Name))
  (bind _mesh (Variables|Default|GetMesh))
  (bind _returnvalue (Transformation|GetSocketLocation _mesh Bone))
  (bind (_outhit _returnvalue_2) (Collision|LineTraceByChannel _returnvalue (+ (* (Transformation|GetActorUpVector (Components|GetOwner)) (* (Variables|Trace|GetTrace_Distance) -1.0)) _returnvalue) "TraceTypeQuery1" false (Utilities|Array|MakeArray (Components|GetOwner)) (Variables|Trace|GetTrace)))
  (if _returnvalue_2
    (if (not (.Value (Utilities|Map|Find (Variables|Bones|GetBone%20-%20Played%20Sound) Bone)))
      (Audio|PlaySoundatLocation (Utilities|Select :Index (Variables|/Script/PhysicsCore.PhysicalMaterial|GetSurfaceType (.PhysMat (Collision|BreakHitResult _outhit))) :SurfaceType_Default "/Game/VFX_SFX/Sounds/Footfalls/Tile/Footstep_Tile_SC.Footstep_Tile_SC" :SurfaceType1 "/Game/VFX_SFX/Sounds/Footfalls/Wood/Footstep_Wood_SC.Footstep_Wood_SC" :SurfaceType2 "/Game/VFX_SFX/Sounds/Footfalls/Grass/Footstep_Grass_SC.Footstep_Grass_SC" :SurfaceType3 "/Game/VFX_SFX/Blood_Splatter/Audio/Blood_Audio/Blood_Splatter_SC.Blood_Splatter_SC" :SurfaceType4 "/Game/VFX_SFX/Sounds/Footfalls/Tile/Footstep_Tile_SC.Footstep_Tile_SC") (.Location (Collision|BreakHitResult _outhit)) "0, 0, 0" 1.0 1.0 0.0 "/Game/VFX_SFX/Sounds/Footfalls/SA_Footfall.SA_Footfall" 0 0 0)
      (Utilities|Map|Add (Variables|Bones|GetBone%20-%20Played%20Sound) Bone true)
      (CallFunction|SpawnParticle (.Location (Collision|BreakHitResult _outhit)) (.Normal (Collision|BreakHitResult _outhit)) (Variables|/Script/PhysicsCore.PhysicalMaterial|GetSurfaceType (.PhysMat (Collision|BreakHitResult _outhit))) 5.0))
    (else
      (Utilities|Map|Add (Variables|Bones|GetBone%20-%20Played%20Sound) Bone false))))

(fn SpawnParticle
  (params (Hit_Location :type Vector) (Hit_Normal :type Vector) (Surface_Type :type EPhysicalSurface%20Enum :default "SurfaceType_Default") (Speed_Division_Amount :type Float%20%28double-precision%29))
  (bind _returnvalue (Niagara|SpawnSystematLocation "/Game/VFX_SFX/Niagara/Ground_Particles/NS_Ground_Particles.NS_Ground_Particles" Hit_Location (Math|Rotator|MakeRotfromZX Hit_Normal (Transformation|GetActorForwardVector (Components|GetOwner))) "0.100000,0.100000,0.100000"))
  (Niagara|SetNiagaraVariable(LinearColor) _returnvalue "user.Ground_Colour" (Utilities|Select :Index Surface_Type :SurfaceType_Default (Math|Color|MakeColor 0.0 0.0 0.0) :SurfaceType1 (Math|Color|MakeColor 0.7 0.3 0.0) :SurfaceType2 (Math|Color|MakeColor 0.002 0.8 0.0) :SurfaceType3 (Math|Color|MakeColor 1.0 0.0 0.0) :SurfaceType4 (Math|Color|MakeColor 1e+01 1e+01 1e+01)))
  (Niagara|SetNiagaraVariable(Float) _returnvalue "user.Character_Speed" (/ (Math|Vector|VectorLength (Variables|/Script/Engine.MovementComponent|GetVelocity (Actor|GetComponentbyClass (Components|GetOwner) "/Script/Engine.CharacterMovementComponent"))) Speed_Division_Amount)))