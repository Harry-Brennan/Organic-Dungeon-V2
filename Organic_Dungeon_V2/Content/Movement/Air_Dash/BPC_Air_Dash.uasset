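; Actor component that gives its owning pawn an air dash when the dash input triggers while it is falling and off cooldown.
; The dash briefly switches movement to Flying, applies a velocity-change impulse along the last input direction, then sets Walking after a short delay.
; It also plays a sound, spawns a Niagara effect near the feet, and adds a strength-scaled camera shake for owners implementing BPI_Player.
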(event Custom|Air_Dash
  (bind _returnvalue (Components|GetOwner))
  (bind _returnvalue_2 (Components|GetOwner))
  (bind _returnvalue_3 (Actor|GetComponentbyClass _returnvalue "/Script/Engine.SkeletalMeshComponent"))
  (bind _returnvalue_4 (Actor|GetComponentbyClass _returnvalue_2 "/Script/Engine.CharacterMovementComponent"))
  (bind _returnvalue_5 (Transformation|GetSocketLocation _returnvalue_3 "foot_l"))
  (Audio|PlaySoundatLocation "/Game/VFX_SFX/Air_Dash/Air_Dash_SC.Air_Dash_SC" (Transformation|GetActorLocation (Components|GetOwner)) "0, 0, 0" 1.0 1.0 0.0 0 0 0 0)
  (Development|PrintString "AIR DASH")
  (bind _aspawn (Utilities|Casting|CastToPawn _returnvalue_2))
  (Pawn|Components|CharacterMovement|SetMovementMode _returnvalue_4 "MOVE_Flying" 0)
  (Physics|AddImpulse _returnvalue_4 (* (Class|Pawn|GetLastMovementInputVector _aspawn) (Variables|Strength|GetDash_Strength)) true)
  (CallFunction|AirDashCooldownCE)
  (Niagara|SpawnSystematLocation "/Game/VFX_SFX/Niagara/Double_Jump/NS_Double_Jump.NS_Double_Jump" (+ (* (Class|Pawn|GetLastMovementInputVector _aspawn) 25.0) (+ _returnvalue_5 (/ (- (Transformation|GetSocketLocation _returnvalue_3 "foot_r") _returnvalue_5) 2.0))) (Math|Rotator|FindLookatRotation (+ (* (Class|Pawn|GetLastMovementInputVector _aspawn) 25.0) (+ _returnvalue_5 (/ (- (Transformation|GetSocketLocation _returnvalue_3 "foot_r") _returnvalue_5) 2.0))) (Transformation|GetActorLocation (Components|GetOwner))))
  (Utilities|FlowControl|Sequence
    (:then_0
      (if (Utilities|DoesObjectImplementInterface (Components|GetOwner) "/Game/Characters/Player/BPI_Player.BPI_Player_C")
        (CallFunction|AirDashCameraShake)))
    (:then_1
      (Utilities|FlowControl|Delay 0.2)
      (Pawn|Components|CharacterMovement|SetMovementMode _returnvalue_4 "MOVE_Walking" 0))))

(event Custom|Air_Dash_Cooldown_CE
  (Variables|Cooldown|SetAir_Dash_Cooldown true)
  (Utilities|FlowControl|Delay (Variables|Cooldown|GetAir_Dash_Cooldown_Length))
  (Variables|Cooldown|SetAir_Dash_Cooldown false))

(event Custom|Air_Dash_Camera_Shake
  (Class|LegacyCameraShake|StartLegacyCameraShake (Game|GetPlayerCameraManager 0) "/Game/Movement/BP_Slight_Camera_Shake.BP_Slight_Camera_Shake_C" (+ (/ (Variables|Strength|GetDash_Strength) 7.5e+02) 2.0) "CameraLocal" "0, 0, 0"))

(event Input|EnhancedActionEvents|EnhancedInputActionIA_Air_Dash
  (params (ActionValue :type Boolean) (ElapsedSeconds :type Float%20%28double-precision%29) (TriggeredSeconds :type Float%20%28double-precision%29) (InputAction :type Input%20Action%20Object%20Reference :default "/Game/Characters/Player/Input/Actions/IA_Air_Dash.IA_Air_Dash"))
  (:Triggered
    (if (and (AI|Components|NavMovement|IsFalling (Actor|GetComponentbyClass (Components|GetOwner) "/Script/Engine.CharacterMovementComponent")) (not (Variables|Cooldown|GetAir_Dash_Cooldown)))
      (CallFunction|AirDash))))