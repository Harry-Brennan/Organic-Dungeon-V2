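; Slide component for a character, driven by IA_Slide input and started only above a minimum forward speed.
; Starting ignores move input, cuts friction and notifies BPC_Custom_Movement_Handler, while stopping restores these and runs a cooldown.
; Tick lerps MaxWalkSpeed down, blends capsule height and mesh offset, and requests a stop on low speed, timeout, released input or non-walking movement.
; An upward trace blocks stopping beneath obstacles.
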(event Custom|Start_Sliding
  (bind _returnvalue (Components|GetOwner))
  (bind _returnvalue_2 (Components|GetOwner))
  (bind _returnvalue_3 (Components|GetOwner))
  (bind _returnvalue_4 (Actor|GetComponentbyClass _returnvalue_2 "/Script/Engine.CharacterMovementComponent"))
  (bind _returnvalue_5 (Actor|GetComponentbyClass _returnvalue_3 "/Script/Engine.CharacterMovementComponent"))
  (bind _maxwalkspeed (Variables|/Script/Engine.CharacterMovementComponent|GetMaxWalkSpeed _returnvalue_4))
  (if (and (Variables|Checks&Status|GetCan_Slide) (not (Variables|Checks&Status|GetSliding)))
    (bind _slide_info (Class|BPICanSlide|GetSlidingInfo(Message) (Components|GetOwner)))
    (Variables|Speed|SetMin_Sliding_Speed (.min_slide_speed _slide_info))
    (Variables|Speed|SetBase_Movement_Speed (.base_movement_speed _slide_info))
    (if (>= (.x (Math|Vector|UnrotateVector (Transformation|GetVelocity _returnvalue) (Transformation|GetActorRotation _returnvalue))) (Variables|Speed|GetMin_Sliding_Speed))
      (if (not (Variables|Checks&Status|GetSliding))
        (Variables|Time|SetMax_Slide_Time (Math|Float|Clamp(Float) (- (/ _maxwalkspeed 5e+01) (/ _maxwalkspeed 2e+02)) 3.0 12.0))
        (Variables|Transitioning|SetSliding_Transition_Percentage 0.0)
        (bind _aspawn (Utilities|Casting|CastToPawn (Components|GetOwner)))
        (Input|SetIgnoreMoveInput (Pawn|GetController _aspawn) true)
        (Variables|Speed|SetCurrent_Speed_At_Sliding (Variables|/Script/Engine.CharacterMovementComponent|GetMaxWalkSpeed (Actor|GetComponentbyClass (Components|GetOwner) "/Script/Engine.CharacterMovementComponent")))
        (Components|Tick|SetComponentTickEnabled true)
        (Variables|Checks&Status|SetStarting_Sliding true)
        (Variables|Checks&Status|SetSliding true)
        (Variables|Checks&Status|SetStopping_Sliding false)
        (Variables|/Script/Engine.CharacterMovementComponent|SetBrakingDecelerationWalking _returnvalue_5 2.5e+02)
        (Variables|/Script/Engine.CharacterMovementComponent|SetGroundFriction _returnvalue_5 0.0)
        (Default|UpdateCustomMovementMode (Actor|GetComponentbyClass (Components|GetOwner) "/Game/Movement/BPC_Custom_Movement_Handler.BPC_Custom_Movement_Handler_C") "NewEnumerator0")))))

(event Custom|Stop_Sliding
  (bind _returnvalue (Components|GetOwner))
  (bind _returnvalue_2 (Actor|GetComponentbyClass _returnvalue "/Script/Engine.CharacterMovementComponent"))
  (if (and (Variables|Checks&Status|GetCan_Stop_Sliding) (Variables|Checks&Status|GetSliding))
    (Development|PrintString "STOPPING SLIDING" true true "(R=1.000000,G=0.026684,B=0.000000,A=1.000000)")
    (Variables|Checks&Status|SetStarting_Sliding false)
    (Variables|Transitioning|SetSliding_Transition_Percentage 0.0)
    (Variables|Time|SetSlide_Speed_Percentage 0.0)
    (Variables|Checks&Status|SetStopping_Sliding true)
    (Variables|Checks&Status|SetSliding false)
    (Variables|/Script/Engine.CharacterMovementComponent|SetBrakingDecelerationWalking _returnvalue_2 1.25e+03)
    (Variables|/Script/Engine.CharacterMovementComponent|SetGroundFriction _returnvalue_2 8.0)
    (Variables|Checks&Status|SetSlide_Cooldown true)
    (Default|TransitionfromMode (Actor|GetComponentbyClass (Components|GetOwner) "/Game/Movement/BPC_Custom_Movement_Handler.BPC_Custom_Movement_Handler_C") "NewEnumerator0")
    (bind _aspawn (Utilities|Casting|CastToPawn (Components|GetOwner)))
    (Input|SetIgnoreMoveInput (Pawn|GetController _aspawn) false)
    (Utilities|FlowControl|Delay (Variables|Time|GetSlide_Cooldown_Length))
    (Variables|Checks&Status|SetSlide_Cooldown false)))

(event Custom|Sliding_Hitbox
  (params (Alpha :type Float%20%28double-precision%29))
  ;[1 1 1] Changing the half height of the character's capsule collision, this needs to be made more modular by getting the normal half height and the targeted half height
  (bind _capsule_hitbox (Class|BPICanSlide|GetHitbox(Message) (Components|GetOwner)))
  (Components|Capsule|SetCapsuleHalfHeight _capsule_hitbox (Math|Float|Lerp (Components|Capsule|GetUnscaledCapsuleHalfHeight _capsule_hitbox) 3e+01 Alpha) true)
  (bind _skeletal_mesh (Class|BPICanSlide|GetMesh(Message) (Components|GetOwner)))
  (Transformation|SetRelativeLocation _skeletal_mesh (Math|Vector|Lerp(Vector) (Variables|/Script/Engine.SceneComponent|GetRelativeLocation _skeletal_mesh) "0.000000,0.000000,-40.000000" Alpha) false false))

(event Custom|Revert_Hitbox
  (params (Alpha :type Float%20%28double-precision%29))
  ;[1 1 1] Changing the half height of the character's capsule collision, this needs to be made more modular by getting the normal half height and the targeted half height
  (bind _capsule_hitbox (Class|BPICanSlide|GetHitbox(Message) (Components|GetOwner)))
  (Components|Capsule|SetCapsuleHalfHeight _capsule_hitbox (Math|Float|Lerp (Components|Capsule|GetUnscaledCapsuleHalfHeight _capsule_hitbox) 9e+01 Alpha) true)
  (bind _skeletal_mesh (Class|BPICanSlide|GetMesh(Message) (Components|GetOwner)))
  (Transformation|SetRelativeLocation _skeletal_mesh (Math|Vector|Lerp(Vector) (Variables|/Script/Engine.SceneComponent|GetRelativeLocation _skeletal_mesh) "0.000000,0.000000,-89.000000" Alpha) false false))

(event Input|EnhancedActionEvents|EnhancedInputActionIA_Slide
  (params (ActionValue :type Boolean) (ElapsedSeconds :type Float%20%28double-precision%29) (TriggeredSeconds :type Float%20%28double-precision%29) (InputAction :type Input%20Action%20Object%20Reference :default "/Game/Characters/Player/Input/Actions/IA_Slide.IA_Slide"))
  (:Triggered
    (CallFunction|StartSliding)
    (Variables|Checks&Status|SetAttempting_To_Slide true))
  (:Canceled
    (CallFunction|StopSliding :!label _label)
    (Variables|Checks&Status|SetAttempting_To_Slide false))
  (:Completed
    (goto _label)))

(event EventTick
  (params (DeltaSeconds :type Float%20%28single-precision%29))
  (bind _returnvalue (Components|GetOwner))
  (bind _returnvalue_2 (Components|GetOwner))
  (bind _returnvalue_3 (Transformation|GetActorLocation _returnvalue_2))
  (Utilities|FlowControl|Sequence
    (:then_0
      (if (Variables|Checks&Status|GetSliding)
        (Utilities|FlowControl|Sequence
          (:then_0
            (bind _output_get (Variables|Time|SetSlide_Speed_Percentage (+ (Variables|Time|GetSlide_Speed_Percentage) (/ 1.0 (/ (Variables|Time|GetMax_Slide_Time) (Class|ActorComponent|GetComponentTickInterval))))))
            (bind _output_get_2 (Variables|/Script/Engine.CharacterMovementComponent|SetMaxWalkSpeed (Actor|GetComponentbyClass (Components|GetOwner) "/Script/Engine.CharacterMovementComponent") (Math|Float|Lerp (Variables|Speed|GetCurrent_Speed_At_Sliding) (- (Variables|Speed|GetMin_Sliding_Speed) 5e+01) (Variables|Time|GetSlide_Speed_Percentage))))
            (if (or (>= (Variables|Time|GetSlide_Speed_Percentage) 1.0) (<= (.x (Math|Vector|UnrotateVector (Transformation|GetVelocity _returnvalue) (Transformation|GetActorRotation _returnvalue))) 1e+01))
              (CallFunction|StopSliding)
              (Variables|Time|SetSlide_Cooldown_Length 0.7)))
          (:then_1
            (bind _returnvalue_4 (Collision|LineTraceForObjects _returnvalue_3 (+ _returnvalue_3 (* (Transformation|GetActorUpVector _returnvalue_2) 1.5e+02)) (Utilities|Array|MakeArray "ObjectTypeQuery1" "ObjectTypeQuery2") false (Utilities|Array|MakeArray _returnvalue_2) "ForDuration"))
            (Development|PrintString "HIT A WORLD STATIC OR WORLD DYNAMIC" _returnvalue_4)
            (bind _output_get_3 (Variables|Checks&Status|SetCan_Stop_Sliding (not _returnvalue_4)))
            (if (and _output_get_3 (not (Variables|Checks&Status|GetAttempting_To_Slide)))
              (CallFunction|StopSliding))))))
    (:then_1
      (if (Variables|Checks&Status|GetStarting_Sliding)
        (Variables|Transitioning|SetSliding_Transition_Percentage (+ (Variables|Transitioning|GetSliding_Transition_Percentage) (/ 1.0 (/ 0.6 (Class|ActorComponent|GetComponentTickInterval)))))
        (CallFunction|SlidingHitbox (Variables|Transitioning|GetSliding_Transition_Percentage))
        (if (>= (Variables|Transitioning|GetSliding_Transition_Percentage) 1.0)
          (Variables|Checks&Status|SetStarting_Sliding false))
        (elif (Variables|Checks&Status|GetStopping_Sliding)
          (Variables|Transitioning|SetSliding_Transition_Percentage (+ (Variables|Transitioning|GetSliding_Transition_Percentage) (/ 1.0 (/ 0.2 (Class|ActorComponent|GetComponentTickInterval)))))
          (CallFunction|RevertHitbox (Variables|Transitioning|GetSliding_Transition_Percentage))
          (if (>= (Variables|Transitioning|GetSliding_Transition_Percentage) 1.0)
            (Variables|Checks&Status|SetStopping_Sliding false)
            (Variables|/Script/Engine.CharacterMovementComponent|SetMaxWalkSpeed (Actor|GetComponentbyClass (Components|GetOwner) "/Script/Engine.CharacterMovementComponent") (Variables|Speed|GetBase_Movement_Speed))
            (Components|Tick|SetComponentTickEnabled false))))
      (if (Utilities|Enum|NotEqual(Enum) (Variables|/Script/Engine.CharacterMovementComponent|GetMovementMode (Actor|GetComponentbyClass (Components|GetOwner) "/Script/Engine.CharacterMovementComponent")) "MOVE_Walking")
        (CallFunction|StopSliding)
        (Variables|Time|SetSlide_Cooldown_Length 0.1)))))

(event EventBeginPlay
  (bind _returnvalue (Components|GetOwner))
  (bind _returnvalue_2 (Actor|GetComponentbyClass _returnvalue "/Script/Engine.CharacterMovementComponent"))
  (bind _maxwalkspeed (Variables|/Script/Engine.CharacterMovementComponent|GetMaxWalkSpeed _returnvalue_2))
  (bind _slide_info (Class|BPICanSlide|GetSlidingInfo(Message) (Components|GetOwner)))
  (Variables|Speed|SetMin_Sliding_Speed (.min_slide_speed _slide_info))
  (Variables|Time|SetMax_Slide_Time (Math|Float|Clamp(Float) (- (/ _maxwalkspeed 5e+01) (/ _maxwalkspeed 1e+01)) 3.0 12.0)))