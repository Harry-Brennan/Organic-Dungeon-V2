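; Sprint component that raises and restores its owner's walk speed from Enhanced Input press and release.
; Starting pulls speed and timing settings from the owner through message calls and sets the sprint mode on BPC_Custom_Movement_Handler.
; Tick, enabled only during transitions, lerps CharacterMovement MaxWalkSpeed using startup or stopping time.
; Stopping selects the next movement mode according to whether BPC_Slide is attempting a slide.
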(event Custom|Start_Sprint
  (if (and (not (Variables|Default|GetSprinting)) (Variables|Default|GetCan_Sprint))
    (bind _sprint_info (Class|BPICanSprint|GetSprintInfo(Message) (Components|GetOwner)))
    (Variables|Default|SetNormal_Walking_Speed (.normal_walking_speed _sprint_info))
    (Variables|Default|SetMax_Sprint_Speed (.sprinting_max_speed _sprint_info))
    (Variables|Default|SetSprint_Startup_Speed (.sprint_startup_speed _sprint_info))
    (Variables|Default|SetSprint_Stopping_Speed (.sprint_stopping_speed _sprint_info))
    (Variables|Default|SetStarting/Stopping true)
    (Components|Tick|SetComponentTickEnabled true)
    (Default|UpdateCustomMovementMode (Actor|GetComponentbyClass (Components|GetOwner) "/Game/Movement/BPC_Custom_Movement_Handler.BPC_Custom_Movement_Handler_C") "NewEnumerator1")
    (Variables|Default|SetSprinting true)))

(event Custom|Stop_Sprint
  (bind _returnvalue (Components|GetOwner))
  (bind _returnvalue_2 (Actor|GetComponentbyClass _returnvalue "/Game/Movement/BPC_Custom_Movement_Handler.BPC_Custom_Movement_Handler_C"))
  (Variables|Default|SetStarting/Stopping false)
  (Variables|Default|SetSprint_Percentage 0.0)
  (Components|Tick|SetComponentTickEnabled true)
  (if (Utilities|Enum|Equal(Enum) (Variables|/Game/Movement/BPC_Custom_Movement_Handler.BPC_Custom_Movement_Handler_C|GetCurrent_Movement_Mode _returnvalue_2) "NewEnumerator1")
    (Default|UpdateCustomMovementMode _returnvalue_2 (select (Variables|/Game/Movement/Sliding/BPC_Slide.BPC_Slide_C|GetAttempting_To_Slide (Actor|GetComponentbyClass (Components|GetOwner) "/Game/Movement/Sliding/BPC_Slide.BPC_Slide_C")) "NewEnumerator0" "NewEnumerator3")))
  (Variables|Default|SetSprinting false))

(event Input|EnhancedActionEvents|EnhancedInputActionIA_Sprint
  (params (ActionValue :type Boolean) (ElapsedSeconds :type Float%20%28double-precision%29) (TriggeredSeconds :type Float%20%28double-precision%29) (InputAction :type Input%20Action%20Object%20Reference :default "/Game/Characters/Player/Input/Actions/IA_Sprint.IA_Sprint"))
  (:Triggered
    (CallFunction|StartSprint)
    (Variables|Default|SetAttempting_To_Sprint true))
  (:Canceled
    (CallFunction|StopSprint :!label _label)
    (Variables|Default|SetAttempting_To_Sprint false))
  (:Completed
    (goto _label)))

(event EventTick
  (params (DeltaSeconds :type Float%20%28single-precision%29))
  (bind _returnvalue (Components|GetOwner))
  (bind _returnvalue_2 (Actor|GetComponentbyClass _returnvalue "/Script/Engine.CharacterMovementComponent"))
  (bind _output_get (Variables|Default|SetSprint_Percentage (+ (Variables|Default|GetSprint_Percentage) (/ 1.0 (/ (Math|Float|SelectFloat (Variables|Default|GetSprint_Startup_Speed) (Variables|Default|GetSprint_Stopping_Speed) (Variables|Default|GetStarting/Stopping)) (Class|ActorComponent|GetComponentTickInterval))))))
  ;[1 1 1] Starting is true / stopping is false
  (if (Variables|Default|GetStarting/Stopping)
    (Variables|/Script/Engine.CharacterMovementComponent|SetMaxWalkSpeed _returnvalue_2 (Math|Float|Lerp (Variables|/Script/Engine.CharacterMovementComponent|GetMaxWalkSpeed _returnvalue_2) (Variables|Default|GetMax_Sprint_Speed) (Variables|Default|GetSprint_Percentage)))
    (else
      (Variables|/Script/Engine.CharacterMovementComponent|SetMaxWalkSpeed _returnvalue_2 (Math|Float|Lerp (Math|Float|Lerp (Variables|/Script/Engine.CharacterMovementComponent|GetMaxWalkSpeed _returnvalue_2) (Variables|Default|GetMax_Sprint_Speed) (Variables|Default|GetSprint_Percentage)) (Variables|Default|GetNormal_Walking_Speed) (Variables|Default|GetSprint_Percentage)))))
  (if (>= (Variables|Default|GetSprint_Percentage) 1.0)
    (Components|Tick|SetComponentTickEnabled false)))

(event EventBeginPlay
  (bind _output_get (Variables|Default|SetNormal_Walking_Speed (Variables|/Script/Engine.CharacterMovementComponent|GetMaxWalkSpeed (Actor|GetComponentbyClass (Components|GetOwner) "/Script/Engine.CharacterMovementComponent"))))
  (Class|BPICanSprint|UpdateNormalWalkingSpeed(Message) (Components|GetOwner) _output_get))