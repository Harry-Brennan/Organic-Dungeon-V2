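; Actor component that gives its owner a ground slam: an input pressed while falling fires one downward impulse and activates the owner's air Niagara effect.
; Releasing or canceling the input re-arms the slam and stops the effect.
; A separate knockup event takes a landing location, plays impact sound and a fading decal, then capsule-traces with debug drawing.
; It launches each unique pawn or physics body upward unless already moving vertically, then stops the slam.
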(event Custom|Ground_Slam_Impulse
  (bind _returnvalue (Components|GetOwner))
  (Development|PrintString "GROUND SLAM")
  (Physics|AddImpulse (Actor|GetComponentbyClass _returnvalue "/Script/Engine.CharacterMovementComponent") (Math|Vector|MakeVector 0.0 0.0 (.Z (Math|Vector|BreakVector (* (Transformation|GetActorUpVector _returnvalue) (* (Variables|Force|GetGround_Slam_Force) -1.0))))) true))

(event Custom|Stop_Ground_Slam
  (Variables|Checks|SetGround_Slam_Active false)
  (Components|Activation|Deactivate (Variables|Default|GetGround_Slam_Air_Niagara)))

(event Custom|Ground_Slam_Knockup
  (params (Land%20Location :type Vector))
  (bind _ground_slam_force (Variables|Force|GetGround_Slam_Force))
  (bind _returnvalue (/ _ground_slam_force 2.0))
  (Audio|PlaySoundatLocation "/Game/VFX_SFX/Ground_Slam/Ground_Slam_Impact_SC.Ground_Slam_Impact_SC" Land%20Location "0, 0, 0" 1.0 1.0 0.0 0 0 0 0)
  (bind _returnvalue_2 (Rendering|Decal|SpawnDecalatLocation "/Game/VFX_SFX/Blood_Splatter/Materials/MI_Blood_Decal_Advanced.MI_Blood_Decal_Advanced" "128.000000,256.000000,256.000000" Land%20Location "-90.000000,0.000000,0.000000" 0.0))
  (Rendering|Components|Decal|SetFadeOut _returnvalue_2 2.0 3.0 true)
  (bind _returnvalue_3 (Rendering|Material|CreateDynamicMaterialInstance _returnvalue_2 :!class /Script/Engine.DecalComponent))
  (Rendering|Material|SetScalarParameterValue _returnvalue_3 "Radius" 125.0 :!class /Script/Engine.MaterialInstanceDynamic)
  (Utilities|Array|Clear (Variables|Knockup|GetHit_Actors))
  (bind (_outhits _returnvalue_4) (Class|KismetSystemLibrary|CapsuleTraceMultiforObjects Land%20Location Land%20Location 6e+02 2e+02 (Utilities|Array|MakeArray "ObjectTypeQuery3" "ObjectTypeQuery4") false (Utilities|Array|MakeArray (Components|GetOwner)) "ForDuration" true))
  (if _returnvalue_4
    (for _array_element _outhits
      (if (not (Utilities|Array|ContainsItem (Variables|Knockup|GetHit_Actors) (.HitActor (Collision|BreakHitResult _array_element))))
        (Utilities|Array|Add (Variables|Knockup|GetHit_Actors) (.HitActor (Collision|BreakHitResult _array_element)))
        (Development|PrintString (Utilities|GetDisplayName (.HitActor (Collision|BreakHitResult _array_element))))
        (Utilities|IsValid (Actor|GetComponentbyClass (.HitActor (Collision|BreakHitResult _array_element)) "/Script/Engine.CharacterMovementComponent")
          (:Is%20Valid
            (if (not (AI|Components|NavMovement|IsFalling (Actor|GetComponentbyClass (.HitActor (Collision|BreakHitResult _array_element)) "/Script/Engine.CharacterMovementComponent")))
              (Physics|AddImpulse (Actor|GetComponentbyClass (.HitActor (Collision|BreakHitResult _array_element)) "/Script/Engine.CharacterMovementComponent") (Math|Vector|MakeVector 0.0 0.0 _returnvalue) true)))
          (:Is%20Not%20Valid
            (if (not (!= (.z (Transformation|GetComponentVelocity (.HitComponent (Collision|BreakHitResult _array_element)))) 0.0))
              (Physics|AddImpulse (.HitComponent (Collision|BreakHitResult _array_element)) (Math|Vector|MakeVector 0.0 0.0 _returnvalue) "None" true)))))))
  (CallFunction|StopGroundSlam))

(event Input|EnhancedActionEvents|EnhancedInputActionIA_Ground_Slam
  (params (ActionValue :type Boolean) (ElapsedSeconds :type Float%20%28double-precision%29) (TriggeredSeconds :type Float%20%28double-precision%29) (InputAction :type Input%20Action%20Object%20Reference :default "/Game/Characters/Player/Input/Actions/IA_Ground_Slam.IA_Ground_Slam"))
  (:Triggered
    (if (AI|Components|NavMovement|IsFalling (Actor|GetComponentbyClass (Components|GetOwner) "/Script/Engine.CharacterMovementComponent"))
      (Utilities|FlowControl|DoOnce false :!label _label
        (:Completed
          (CallFunction|GroundSlamImpulse)
          (Variables|Checks|SetGround_Slam_Active true)
          (Components|Activation|Activate (Variables|Default|GetGround_Slam_Air_Niagara) false)))))
  (:Canceled
    (Utilities|FlowControl|Sequence :!label _label_2
      (:then_0
        (goto _label Reset))
      (:then_1
        (Variables|Checks|SetGround_Slam_Active false)
        (Components|Activation|Deactivate (Variables|Default|GetGround_Slam_Air_Niagara)))))
  (:Completed
    (goto _label_2)))

(event EventBeginPlay
  (bind _niagara (Class|BPICanGroundSlam|GetGroundSlamAirNiagara(Message) (Components|GetOwner)))
  (Variables|Default|SetGround_Slam_Air_Niagara _niagara))