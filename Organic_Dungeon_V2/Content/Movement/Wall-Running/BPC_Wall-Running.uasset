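; Actor component that adds wall running and wall jump-off to a falling character.
; Tick traces right, then left, for near-vertical walls and uses LaunchCharacter along the normal-cross-up direction to move the character while easing gravity down.
; Run speed and duration derive from MaxWalkSpeed, with speed decaying until the run times out.
; Ending a run restores gravity, starts a timed cooldown and notifies BPC_Custom_Movement_Handler to transition out.
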(event Custom|Jump_Off_Wall
  (bind _wall_run_normal (Variables|Wall|GetWall_Run_Normal))
  (bind _jump_off_horizontal_force (Variables|JumpForce|GetJump_Off_Horizontal_Force))
  (if (Variables|Status&Checks|GetWall-Running)
    (CallFunction|EndWallRun 0.35)
    (bind _ascharacter (Utilities|Casting|CastToCharacter (Components|GetOwner)))
    (Character|LaunchCharacter _ascharacter (Math|Vector|MakeVector (* (.x _wall_run_normal) _jump_off_horizontal_force) (* (.y _wall_run_normal) _jump_off_horizontal_force) (Variables|JumpForce|GetJump_Off_Vertical_Force)) false true)))

(event Custom|Reset_Wall_Run_Cooldown
  (Utilities|Time|ClearTimerbyFunctionName 0 "Reset_Wall_Run_Cooldown")
  (Variables|Status&Checks|SetWall_Run_Cooldown false))

(event EventTick
  (params (DeltaSeconds :type Float%20%28single-precision%29))
  (bind _returnvalue (Components|GetOwner))
  (bind _returnvalue_2 (Components|GetOwner))
  (bind _returnvalue_3 (Actor|GetComponentbyClass _returnvalue "/Script/Engine.CharacterMovementComponent"))
  (bind _returnvalue_4 (Actor|GetComponentbyClass _returnvalue_2 "/Script/Engine.CharacterMovementComponent"))
  (bind _maxwalkspeed (Variables|/Script/Engine.CharacterMovementComponent|GetMaxWalkSpeed _returnvalue_3))
  (Utilities|FlowControl|Sequence
    (:then_0
      (if (and (AI|Components|NavMovement|IsFalling (Actor|GetComponentbyClass (Components|GetOwner) "/Script/Engine.CharacterMovementComponent")) (not (Variables|Status&Checks|GetWall_Run_Cooldown)))
        (Variables|Status&Checks|SetCan_Wall_Run true)
        (else
          (Variables|Status&Checks|SetCan_Wall_Run false)
          (goto _label Reset))))
    (:then_1
      (if (Variables|Status&Checks|GetCan_Wall_Run)
        (Utilities|FlowControl|Sequence
          (:then_0
            (Utilities|FlowControl|DoOnce false :!label _label
              (:Completed
                (Variables|Timing|SetMax_Wall_Run_Time (Math|Float|Clamp(Float) (- (/ _maxwalkspeed 25.0) (/ _maxwalkspeed 1e+02)) 3.0 5.0))
                (Variables|Speed|SetSpeed_At_Start_Of_Wall_Run (* _maxwalkspeed 1.25)))))
          (:then_1
            (bind _output_get (Variables|Speed|SetWall_Run_Speed_Percentage (+ (Variables|Speed|GetWall_Run_Speed_Percentage) (/ 1.0 (/ (Variables|Timing|GetMax_Wall_Run_Time) (Class|ActorComponent|GetComponentTickInterval))))))
            (CallFunction|LerpWallRunSpeed (Math|Float|Clamp(Float) _output_get))
            (if (== (Math|Float|Clamp(Float) _output_get) 1.0)
              (Utilities|FlowControl|Delay 0.5)
              (CallFunction|EndWallRun 0.7)))
          (:then_2
            (bind _on_wall (CallFunction|WallRunMovement (Transformation|GetActorLocation (Components|GetOwner)) (.Right (Utilities|WallRunEndVectors)) -1.0))
            (if _on_wall
              (Variables|Status&Checks|SetWall-Running true)
              (Variables|Status&Checks|SetWall_Run_Right true)
              (Variables|Status&Checks|SetWall_Run_Left false)
              (Variables|/Script/Engine.CharacterMovementComponent|SetGravityScale _returnvalue_4 (Math|Interpolation|FInterpTo (Variables|/Script/Engine.CharacterMovementComponent|GetGravityScale _returnvalue_4) 0.25 (Utilities|Time|GetWorldDeltaSeconds) 1e+01) :!label _label_2)
              (elif (Variables|Status&Checks|GetWall_Run_Right)
                (CallFunction|EndWallRun 1.0)
                (else
                  (bind _on_wall_2 (CallFunction|WallRunMovement (Transformation|GetActorLocation (Components|GetOwner)) (.Left (Utilities|WallRunEndVectors)) 1.0))
                  (if _on_wall_2
                    (Variables|Status&Checks|SetWall-Running true)
                    (Variables|Status&Checks|SetWall_Run_Right false)
                    (Variables|Status&Checks|SetWall_Run_Left true)
                    (goto _label_2)
                    (else
                      (CallFunction|EndWallRun 1.0))))))))))))

(event EventBeginPlay
  (bind _returnvalue (Components|GetOwner))
  (bind _wall_running_info (Class|BPICanWall-Run|GetWall-RunInfo(Message) (Components|GetOwner)))
  (Variables|Timing|SetMax_Wall_Run_Time (.max_wall_run_time _wall_running_info))
  (bind _capsule (Class|BPICanDash|GetCapsuleCollision(Message) _returnvalue))
  (Variables|Default|SetOwner_Capsule_Collision _capsule)
  (Class|MovementComponent|SetPlaneConstraintEnabled (Actor|GetComponentbyClass _returnvalue "/Script/Engine.CharacterMovementComponent") true))

(fn WallRunMovement
  (params (Start :type Vector) (End :type Vector) (Direction :type Float%20%28double-precision%29))
  (bind _outhit (Collision|LineTraceByChannel Start End "TraceTypeQuery1" false 0 "ForDuration"))
  (if (.bblockinghit _outhit)
    (if (.ReturnValue (Utilities|WallRunVectorValidity (.normal _outhit)))
      (Variables|Wall|SetWall_Run_Normal (.Vector2 (Utilities|WallRunVectorValidity (.normal _outhit))))
      ;[1 1 1] Stick character to wall
      (bind _ascharacter (Utilities|Casting|CastToCharacter (Components|GetOwner)))
      (Character|LaunchCharacter _ascharacter (Utilities|PlayertoWallVector) false false)
      ;[1 1 1] Move character forward
      (Character|LaunchCharacter _ascharacter (* (Math|Vector|CrossProduct (Variables|Wall|GetWall_Run_Normal) "0.000000,0.000000,1.000000") (* (Variables|Speed|GetWall_Run_Speed) Direction)) true (not (Variables|Status&Checks|GetWall_Run_Gravity)))
      (Default|UpdateCustomMovementMode (Actor|GetComponentbyClass (Components|GetOwner) "/Game/Movement/BPC_Custom_Movement_Handler.BPC_Custom_Movement_Handler_C") "NewEnumerator2")
      (return true)
      (else
        (return false)))
    (else
      (return false))))

(fn EndWallRun
  (params (Wall_Run_Cooldown :type Float%20%28double-precision%29))
  (if (Variables|Status&Checks|GetWall-Running)
    (Variables|Status&Checks|SetWall-Running false)
    (Variables|Status&Checks|SetWall_Run_Right false)
    (Variables|Status&Checks|SetWall_Run_Left false)
    (Variables|/Script/Engine.CharacterMovementComponent|SetGravityScale (Actor|GetComponentbyClass (Components|GetOwner) "/Script/Engine.CharacterMovementComponent") 1.75)
    (Variables|Status&Checks|SetWall_Run_Cooldown true)
    (Variables|Speed|SetWall_Run_Speed_Percentage 0.0)
    (Utilities|Time|SetTimerbyFunctionName 0 "Reset_Wall_Run_Cooldown" Wall_Run_Cooldown)
    (Default|TransitionfromMode (Actor|GetComponentbyClass (Components|GetOwner) "/Game/Movement/BPC_Custom_Movement_Handler.BPC_Custom_Movement_Handler_C") "NewEnumerator2")))

(fn LerpWallRunSpeed
  (params (Alpha :type Float%20%28double-precision%29))
  (Variables|Speed|SetWall_Run_Speed (Math|Float|Lerp (Variables|Speed|GetSpeed_At_Start_Of_Wall_Run) 5e+01 Alpha)))