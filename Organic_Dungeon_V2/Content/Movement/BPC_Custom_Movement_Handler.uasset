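; Movement handler component that arbitrates between sprint, slide, double jump and wall-running on its owner.
; Each tick it sets those abilities' permission flags from walking, falling, rolling and current mode, and toggles player speed-line Niagara effects by velocity through DoOnce gates.
; It tracks current and previous modes, and on leaving one chains into an attempted sprint or slide, otherwise returning to Default unless wall-running.
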(event Custom|Update_Custom_Movement_Mode
  (params (New_Movement_Mode :type Enum_Custom_Movement_Modes%20Enum :default "NewEnumerator3"))
  (if (Utilities|Enum|NotEqual(Enum) New_Movement_Mode (Variables|Default|GetCurrent_Movement_Mode))
    (Variables|Default|SetPrevious_Movement_Mode (Variables|Default|GetCurrent_Movement_Mode))
    (Variables|Default|SetCurrent_Movement_Mode New_Movement_Mode)))

(event Custom|Transition_From_Mode
  (params (Transitioning_From :type Enum_Custom_Movement_Modes%20Enum :default "NewEnumerator3"))
  (bind _returnvalue (Components|GetOwner))
  (bind _returnvalue_2 (Actor|GetComponentbyClass _returnvalue "/Game/Movement/Sprinting/BPC_Sprint.BPC_Sprint_C"))
  (bind _returnvalue_3 (Actor|GetComponentbyClass _returnvalue "/Game/Movement/Sliding/BPC_Slide.BPC_Slide_C"))
  (switch Utilities|FlowControl|Switch|SwitchonEnum_Custom_Movement_Modes Transitioning_From
    (:NewEnumerator0
      (if (and (Variables|/Game/Movement/Sprinting/BPC_Sprint.BPC_Sprint_C|GetAttempting_To_Sprint _returnvalue_2) (Variables|/Game/Movement/Sprinting/BPC_Sprint.BPC_Sprint_C|GetCan_Sprint _returnvalue_2)) :!label _label
        (Default|StartSprint _returnvalue_2)
        (else
          (if (not (Variables|/Game/Movement/Wall-Running/BPC_Wall-Running.BPC_Wall-Running_C|GetWall-Running (Actor|GetComponentbyClass _returnvalue "/Game/Movement/Wall-Running/BPC_Wall-Running.BPC_Wall-Running_C"))) :!label _label_2
            (Variables|Default|SetCurrent_Movement_Mode "NewEnumerator3")))))
    (:NewEnumerator1
      (if (and (Variables|/Game/Movement/Sliding/BPC_Slide.BPC_Slide_C|GetAttempting_To_Slide _returnvalue_3) (Variables|/Game/Movement/Sliding/BPC_Slide.BPC_Slide_C|GetCan_Slide _returnvalue_3)) :!label _label_3
        (Default|StartSliding _returnvalue_3)
        (else
          (goto _label_2))))
    (:NewEnumerator2
      (Utilities|FlowControl|Sequence
        (:then_0
          (goto _label))
        (:then_1
          (goto _label_3))))))

(event EventBeginPlay
  (bind _returnvalue (Components|GetOwner))
  (if (Utilities|DoesObjectImplementInterface _returnvalue "/Game/Characters/Player/BPI_Player.BPI_Player_C")
    (bind _speed_lines (Class|BPIPlayer|GetSpeedLinesNiagara(Message) _returnvalue))
    (Variables|Default|SetSpeed_Lines _speed_lines)))

(event EventTick
  (params (DeltaSeconds :type Float%20%28single-precision%29))
  (bind _returnvalue (Components|GetOwner))
  (bind _current_movement_mode (Variables|Default|GetCurrent_Movement_Mode))
  (bind _speed_lines (Variables|Default|GetSpeed_Lines))
  (Variables|/Game/Movement/Sprinting/BPC_Sprint.BPC_Sprint_C|SetCan_Sprint (Actor|GetComponentbyClass (Components|GetOwner) "/Game/Movement/Sprinting/BPC_Sprint.BPC_Sprint_C") (Math|Boolean|ANDBoolean (Utilities|Enum|Equal(Enum) (Variables|/Script/Engine.CharacterMovementComponent|GetMovementMode (Actor|GetComponentbyClass (Components|GetOwner) "/Script/Engine.CharacterMovementComponent")) "MOVE_Walking") (Utilities|Enum|NotEqual(Enum) (Variables|Default|GetCurrent_Movement_Mode) "NewEnumerator0") (not (Variables|Default|GetRolling))))
  (Variables|/Game/Movement/Sliding/BPC_Slide.BPC_Slide_C|SetCan_Slide (Actor|GetComponentbyClass (Components|GetOwner) "/Game/Movement/Sliding/BPC_Slide.BPC_Slide_C") (and (Utilities|Enum|Equal(Enum) (Variables|/Script/Engine.CharacterMovementComponent|GetMovementMode (Actor|GetComponentbyClass (Components|GetOwner) "/Script/Engine.CharacterMovementComponent")) "MOVE_Walking") (not (Variables|Default|GetRolling))))
  (Variables|/Game/Movement/Double_Jump/BPC_Double_Jump.BPC_Double_Jump_C|SetCan_Double_Jump (Actor|GetComponentbyClass (Components|GetOwner) "/Game/Movement/Double_Jump/BPC_Double_Jump.BPC_Double_Jump_C") (Math|Boolean|ANDBoolean (AI|Components|NavMovement|IsFalling (Actor|GetComponentbyClass (Components|GetOwner) "/Script/Engine.CharacterMovementComponent")) (not (Utilities|Enum|Equal(Enum) _current_movement_mode "NewEnumerator2")) (not (Utilities|Enum|Equal(Enum) _current_movement_mode "NewEnumerator0"))))
  (if (Utilities|DoesObjectImplementInterface _returnvalue "/Game/Characters/Player/BPI_Player.BPI_Player_C")
    (if (> (Math|Vector|VectorLength (Variables|/Script/Engine.MovementComponent|GetVelocity (Actor|GetComponentbyClass _returnvalue "/Script/Engine.CharacterMovementComponent"))) 751.0)
      (Utilities|FlowControl|Sequence
        (:then_0
          (Utilities|FlowControl|DoOnce false :!label _label
            (:Completed
              (Components|Activation|Activate _speed_lines false))))
        (:then_1
          (goto _label_2 Reset)))
      (else
        (Utilities|FlowControl|Sequence
          (:then_0
            (Utilities|FlowControl|DoOnce false :!label _label_2
              (:Completed
                (Components|Activation|Deactivate _speed_lines))))
          (:then_1
            (goto _label Reset)))))))