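; Actor component that gives its owning character a limited, upgradeable pool of mid-air jumps.
; Double_Jump launches the character along its up vector, keeping forward-axis speed, and plays sound plus a camera shake for BPI_Player owners.
; It also stops any ground slam and clears the air-dash cooldown through sibling components.
; Cooldown refills jumps immediately, as the JumpCooldown delay is unconnected; max-jump upgrades also refill them.
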(event EventBeginPlay
  (Variables|Jumps|SetAvailable_Jumps (Variables|Jumps|GetMax_Jumps)))

(event Custom|Cooldown
  (Variables|Jumps|SetAvailable_Jumps (Variables|Jumps|GetMax_Jumps)))

(event Custom|Double_Jump
  (bind _returnvalue (Components|GetOwner))
  (bind _returnvalue_2 (Components|GetOwner))
  (bind _returnvalue_3 (Components|GetOwner))
  (bind _returnvalue_4 (Actor|GetComponentbyClass _returnvalue_2 "/Game/Movement/Air_Dash/BPC_Air_Dash.BPC_Air_Dash_C"))
  (bind _returnvalue_5 (Actor|GetComponentbyClass _returnvalue_3 "/Game/Movement/Ground_Slam/BPC_Ground_Slam.BPC_Ground_Slam_C"))
  (if (Math|Boolean|ANDBoolean (> (Variables|Jumps|GetAvailable_Jumps) 0) (Variables|Status|GetCan_Double_Jump) (not (Variables|Status|GetAlready_Jumping)))
    (Utilities|IsValid _returnvalue_5
      (:Is%20Valid
        (Default|StopGroundSlam _returnvalue_5))
      (:Is%20Not%20Valid
        _))
    (bind _ascharacter (Utilities|Casting|CastToCharacter _returnvalue))
    (Character|LaunchCharacter _ascharacter (+ (* (Transformation|GetActorUpVector _returnvalue) (Variables|Force|GetJump_Force)) (* (Transformation|GetActorForwardVector _returnvalue) (.x (Math|Vector|UnrotateVector (Variables|/Script/Engine.MovementComponent|GetVelocity (Actor|GetComponentbyClass _returnvalue "/Script/Engine.CharacterMovementComponent")) (Transformation|GetActorRotation _returnvalue))))) true true)
    (if (Utilities|DoesObjectImplementInterface (Components|GetOwner) "/Game/Characters/Player/BPI_Player.BPI_Player_C")
      (Class|LegacyCameraShake|StartLegacyCameraShake (Game|GetPlayerCameraManager 0) "/Game/Movement/BP_Slight_Camera_Shake.BP_Slight_Camera_Shake_C" 2.0 "CameraLocal" "0, 0, 0"))
    (Math|Integer|DecrementInt (Variables|Jumps|GetAvailable_Jumps)
      (:%20%20
        (Audio|PlaySoundatLocation "/Game/VFX_SFX/Double_Jump/Double_Jump_SC.Double_Jump_SC" (Transformation|GetActorLocation (Components|GetOwner)) "0, 0, 0" 1.0 1.0 0.0 0 0 0 0)
        (Utilities|IsValid _returnvalue_4
          (:Is%20Valid
            (Variables|/Game/Movement/Air_Dash/BPC_Air_Dash.BPC_Air_Dash_C|SetAir_Dash_Cooldown _returnvalue_4 false)))))))

(event Custom|Increase_Max_Jumps
  (params (Amount_To_Increase_By :type Integer))
  (bind _output_get (Variables|Jumps|SetMax_Jumps (+ (Variables|Jumps|GetMax_Jumps) Amount_To_Increase_By)))
  (Variables|Jumps|SetAvailable_Jumps _output_get))