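; Health component that tracks an actor's health, with healing, damage, max health changes, debug keys and a still-empty death switch on DeathType.
; BeginPlay pulls settings from the owner via an interface message and caches the health widget for player owners.
; Tick arms one-shot protection above a health percentage, so TakeDamage clamps at a floor, then spawns floating damage numbers through the hit actor's BPC_Floating_Damage.
; A separate heart-based max health graph uses different variables.
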(event EventTick
  (params (DeltaSeconds :type Float%20%28single-precision%29))
  (Utilities|FlowControl|Sequence
    (:then_0
      ;[1 1 1] One shot protection detection
      (if (and (> (Variables|Health|GetHealth) (* (Variables|Health|GetMaximum_Health) (Variables|OSP|GetHealth%20Percentage%20Activation%20Threshold))) (Variables|OSP|GetOne_Shot_Protection))
        (Variables|OSP|SetOSP_Active true)
        (else
          (Variables|OSP|SetOSP_Active false))))))

(event EventBeginPlay
  (Utilities|FlowControl|Sequence
    (:then_0
      ;[1 1 1] Setup of basic health info
      (bind _health_info (Class|BPIHasHealth|GetHealthInfo(Message) (Components|GetOwner)))
      (Variables|Health|SetHealth (.starting_health _health_info))
      (Variables|Health|SetMaximum_Health (.max_health _health_info))
      (Variables|OSP|SetOne_Shot_Protection (.one_shot_protection _health_info))
      (Variables|OSP|SetHealth%20Percentage%20Stopping%20Threshold (.Health_Percentage_Stopping_Threshold (Utilities|Struct|BreakStruct_One_Shot_Protection_Info (.one_shot_protection_info _health_info))))
      (Variables|OSP|SetHealth%20Percentage%20Activation%20Threshold (.Health_Percentage_Activation_Threshold (Utilities|Struct|BreakStruct_One_Shot_Protection_Info (.one_shot_protection_info _health_info))))
      (Variables|Death|SetDeath_Type (.death_type _health_info)))
    (:then_1
      ;[1 1 1] Getting the health widget for easy access if the player is the owner of this component
      (if (Utilities|DoesObjectImplementInterface (Components|GetOwner) "/Game/Characters/Player/BPI_Player.BPI_Player_C")
        (bind _health_widget (Class|BPIHasHealth|GetHealthWidget(Message) (Components|GetOwner)))
        (Variables|UI|SetHealth%20Widget _health_widget)
        (Variables|/Game/UI/WBP_New_Health.WBP_New_Health_C|SetMaximum_Health (Variables|UI|GetHealth%20Widget) (Variables|Health|GetMaximum_Health))
        (Variables|/Game/UI/WBP_New_Health.WBP_New_Health_C|SetTarget_Health (Variables|UI|GetHealth%20Widget) (Variables|Health|GetHealth))))))

(event Input|KeyboardEvents|DebugKey3
  (params (Key :type Key%20Structure :default "None") (ActionValue :type Input%20Action%20Value%20Structure))
  (:Pressed
    (CallFunction|DecreaseMaxHealth)))

(event Input|KeyboardEvents|DebugKey4
  (params (Key :type Key%20Structure :default "None") (ActionValue :type Input%20Action%20Value%20Structure))
  (:Pressed
    (CallFunction|IncreaseMaxHealth)))

(event Input|KeyboardEvents|DebugKeyB
  (params (Key :type Key%20Structure :default "None") (ActionValue :type Input%20Action%20Value%20Structure))
  (bind _returnvalue (Components|GetOwner))
  (:Pressed
    (CallFunction|TakeDamage 1e+01 (Transformation|GetActorLocation _returnvalue) _returnvalue)))

(event Input|KeyboardEvents|DebugKeyN
  (params (Key :type Key%20Structure :default "None") (ActionValue :type Input%20Action%20Value%20Structure))
  (:Pressed
    (CallFunction|Heal 1e+01)))

(fn TakeDamage
  (params (Damage_To_Take :type Float%20%28double-precision%29) (Damage_Location :type Vector) (Hit_Actor :type Actor%20Object%20Reference))
  (bind (_x _y _z) (Class|KismetMathLibrary|BreakVector3f Damage_Location))
  (bind _returnvalue (Actor|GetComponentbyClass Hit_Actor "/Game/Characters/BPC_Floating_Damage.BPC_Floating_Damage_C"))
  (if (<= (Math|Float|SelectFloat (Math|Float|Clamp(Float) (- (Variables|Health|GetHealth) Damage_To_Take) (Variables|OSP|GetHealth%20Percentage%20Stopping%20Threshold) (Variables|Health|GetHealth)) (- (Variables|Health|GetHealth) Damage_To_Take) (Variables|OSP|GetOSP_Active)) 0.0)
    (Variables|Health|SetHealth 0.0)
    (CallFunction|Death)
    (else
      (Variables|Health|SetHealth (Math|Float|SelectFloat (Math|Float|Clamp(Float) (- (Variables|Health|GetHealth) Damage_To_Take) (Variables|OSP|GetHealth%20Percentage%20Stopping%20Threshold) (Variables|Health|GetHealth)) (- (Variables|Health|GetHealth) Damage_To_Take) (Variables|OSP|GetOSP_Active)))))
  (if (Utilities|DoesObjectImplementInterface (Components|GetOwner) "/Game/Characters/Player/BPI_Player.BPI_Player_C")
    (Variables|/Game/UI/WBP_New_Health.WBP_New_Health_C|SetTarget_Health (Variables|UI|GetHealth%20Widget) (Variables|Health|GetHealth)))
  (bind _damage_is_float (Default|DetermineDamageIsFloat _returnvalue Damage_To_Take))
  (Default|MakeFloatingNumber _returnvalue (Math|Vector|MakeVector (+ _x (Math|Random|RandomFloatinRange -5e+01 5e+01)) (+ _y (Math|Random|RandomFloatinRange -5e+01 5e+01)) (+ _z (Math|Random|RandomFloatinRange -5e+01 5e+01))) Damage_To_Take _damage_is_float))

(fn Death
  (switch Utilities|FlowControl|Switch|SwitchonEnum_Death_Types (Variables|Death|GetDeath_Type)))

(fn Heal
  (params (Amount_To_Heal :type Float%20%28double-precision%29))
  (bind _output_get (Variables|Health|SetHealth (Math|Float|Clamp(Float) (+ (Variables|Health|GetHealth) Amount_To_Heal) 0.0 (Variables|Health|GetMaximum_Health))))
  (if (Utilities|DoesObjectImplementInterface (Components|GetOwner) "/Game/Characters/Player/BPI_Player.BPI_Player_C")
    (Variables|/Game/UI/WBP_New_Health.WBP_New_Health_C|SetTarget_Health (Variables|UI|GetHealth%20Widget) _output_get)))

(fn IncreaseMaxHealth
  (params (Amount_To_Increase_By :type Float%20%28double-precision%29))
  (Variables|Health|SetMaximum_Health (+ (Variables|Health|GetMaximum_Health) Amount_To_Increase_By)))

(fn DecreaseMaxHealth
  (params (Amount_To_Decrease_By :type Float%20%28double-precision%29))
  (Variables|Health|SetMaximum_Health (- (Variables|Health|GetMaximum_Health) Amount_To_Decrease_By)))

(event Custom|Increase_Max_Health
  (bind _health_widget (Variables|Default|GetHealth_Widget))
  (bind _hearts_wrapbox (Variables|/Game/UI/WBP_Health.WBP_Health_C|GetHearts_WrapBox _health_widget))
  (bind _returnvalue (Class|PanelWidget|GetAllChildren _hearts_wrapbox))
  (Math|Integer|IncrementInt (Variables|Default|GetMax_Health)
    (:%20%20
      (Default|AddHeart _health_widget)
      (bind _array_element (Utilities|Array|ForEachLoopwithBreak _returnvalue :!label _label)
        (:LoopBody
          (bind _aswbp_heart (Utilities|Casting|CastToWBP_Heart _array_element))
          (if (not (Variables|/Game/UI/WBP_Heart.WBP_Heart_C|GetFilled? _aswbp_heart))
            (Default|PlayHealAnim _aswbp_heart)
            (Variables|/Game/UI/WBP_Heart.WBP_Heart_C|SetFilled? _aswbp_heart true)
            (bind _aswbp_heart_2 (Utilities|Casting|CastToWBP_Heart (Class|PanelWidget|GetChildat _hearts_wrapbox (Utilities|Array|LastIndex _returnvalue))))
            (Variables|/Script/UMG.Image|SetColorAndOpacity (Variables|/Game/UI/WBP_Heart.WBP_Heart_C|GetHeart_Filled_Img _aswbp_heart_2) (Math|Color|MakeColor 0.0 0.0 0.0))
            (Variables|/Game/UI/WBP_Heart.WBP_Heart_C|SetFilled? _aswbp_heart_2 false)
            (goto _label Break)))
        (:Completed
          (Variables|Default|SetCurrent_Health 0)
          (for _array_element_2 (Class|PanelWidget|GetAllChildren (Variables|/Game/UI/WBP_Health.WBP_Health_C|GetHearts_WrapBox (Variables|Default|GetHealth_Widget)))
            (bind _aswbp_heart_3 (Utilities|Casting|CastToWBP_Heart _array_element_2))
            (if (Variables|/Game/UI/WBP_Heart.WBP_Heart_C|GetFilled? _aswbp_heart_3)
              (Math|Integer|IncrementInt (Variables|Default|GetCurrent_Health)
                (:%20%20
                  (Default|PlayHealAnim _aswbp_heart_3))))))))))

(event Custom|Decrease_Max_Health
  (Math|Integer|DecrementInt (Variables|Default|GetMax_Health)
    (:%20%20
      (if (> (Variables|Default|GetCurrent_Health) (Variables|Default|GetMax_Health))
        (Variables|Default|SetCurrent_Health (Variables|Default|GetMax_Health)))
      (Class|PanelWidget|RemoveChildat (Variables|/Game/UI/WBP_Health.WBP_Health_C|GetHearts_WrapBox (Variables|Default|GetHealth_Widget)) (Utilities|Array|LastIndex (Class|PanelWidget|GetAllChildren (Variables|/Game/UI/WBP_Health.WBP_Health_C|GetHearts_WrapBox (Variables|Default|GetHealth_Widget)))))
      (if (<= (Variables|Default|GetMax_Health) 0)
        (CallFunction|Death)))))