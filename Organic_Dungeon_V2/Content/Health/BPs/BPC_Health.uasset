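; Health component for players and enemies that takes its settings from the owner via interface messages and handles damage, healing and non-player death.
; TakeDamage applies BPC_Blocking reduction, perfect blocks and one-shot protection, then shows floating damage numbers and either shakes the player camera or aggros the enemy controller.
; Tick updates one-shot protection and lerps the player's health bar.
; Death bloodsplodes or explodes non-players, then destroys them and their weapons; N/B keys debug healing and damage.
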(event EventTick
  (params (DeltaSeconds :type Float%20%28single-precision%29))
  (bind _health_widget (Variables|UI|GetHealth%20Widget))
  (bind _healthbar (Variables|/Game/UI/WBP_New_Health.WBP_New_Health_C|GetHealthBar _health_widget))
  (bind _percent (Variables|/Script/UMG.ProgressBar|GetPercent _healthbar))
  (Utilities|FlowControl|Sequence
    (:then_0
      ;[1 1 1] One shot protection detection
      (if (and (> (Variables|Health|GetHealth) (* (Variables|Health|GetMaximum_Health) (Variables|OSP|GetHealth%20Percentage%20Activation%20Threshold))) (Variables|OSP|GetOne_Shot_Protection))
        (Variables|OSP|SetOSP_Active true)
        (else
          (Variables|OSP|SetOSP_Active false))))
    (:then_1
      (if (Utilities|DoesObjectImplementInterface (Components|GetOwner) "/Game/Characters/Player/BPI_Player.BPI_Player_C")
        (if (not (== (* _percent (Variables|Health|GetMaximum_Health)) (Variables|Health|GetHealth)))
          (Variables|UI|SetHealth_Bar_Alpha (Math|Float|Clamp(Float) (+ (Variables|UI|GetHealth_Bar_Alpha) (* DeltaSeconds 2.0))))
          (Progress|SetPercent _healthbar (Math|Float|Lerp _percent (/ (Variables|/Game/UI/WBP_New_Health.WBP_New_Health_C|GetTarget_Health _health_widget) (Variables|Health|GetMaximum_Health)) (Variables|UI|GetHealth_Bar_Alpha))))))))

(event EventBeginPlay
  (Utilities|FlowControl|Sequence
    (:then_0
      ;[1 1 1] Setup of basic health info
      (bind _health_info (Class|BPIHasHealth|GetHealthInfo(Message) (Components|GetOwner)))
      (Variables|Health|SetHealth (.starting_health _health_info))
      (Variables|Health|SetMaximum_Health (.max_health _health_info))
      (Variables|OSP|SetOne_Shot_Protection (.one_shot_protection _health_info))
      (Variables|OSP|SetHealth%20Percentage%20Stopping%20Threshold (.Health_Percentage_Stopping_Threshold (Utilities|Struct|BreakStruct_One_Shot_Protection_Info (.one_shot_protection_info _health_info))))
      (Variables|OSP|SetHealth%20Percentage%20Activation%20Threshold (.Health_Percentage_Activation_Threshold (Utilities|Struct|BreakStruct_One_Shot_Protection_Info (.one_shot_protection_info _health_info))))
      (Variables|Death|SetDeath_Type (.death_type _health_info))
      (Variables|Death|SetExplosion%20Death%20Info (.explodeinfo _health_info)))
    (:then_1
      ;[1 1 1] Getting the health widget for easy access if the player is the owner of this component
      (if (Utilities|DoesObjectImplementInterface (Components|GetOwner) "/Game/Characters/Player/BPI_Player.BPI_Player_C")
        (bind _health_widget (Class|BPIHasHealth|GetHealthWidget(Message) (Components|GetOwner)))
        (Variables|UI|SetHealth%20Widget _health_widget)
        (Variables|/Game/UI/WBP_New_Health.WBP_New_Health_C|SetMaximum_Health (Variables|UI|GetHealth%20Widget) (Variables|Health|GetMaximum_Health))
        (Variables|/Game/UI/WBP_New_Health.WBP_New_Health_C|SetTarget_Health (Variables|UI|GetHealth%20Widget) (Variables|Health|GetHealth))))))

(event Input|KeyboardEvents|DebugKeyB
  (params (Key :type Key%20Structure :default "None") (ActionValue :type Input%20Action%20Value%20Structure))
  (bind _returnvalue (Components|GetOwner))
  (bind _returnvalue_2 (Transformation|GetActorLocation _returnvalue))
  (:Pressed
    (CallFunction|TakeDamage 1e+01 _returnvalue_2 _returnvalue)
    (Audio|PlaySoundatLocation "/Game/VFX_SFX/Blood_Splatter/Audio/Impact_Audio/Body_Impact_SC.Body_Impact_SC" _returnvalue_2 "0, 0, 0" 1.0 1.0 0.0 0 0 0 0)))

(event Input|KeyboardEvents|DebugKeyN
  (params (Key :type Key%20Structure :default "None") (ActionValue :type Input%20Action%20Value%20Structure))
  (:Pressed
    (CallFunction|Heal 1e+01)))

(fn TakeDamage
  (params (Damage_To_Take :type Float%20%28double-precision%29) (Damage_Location :type Vector) (Hit_Actor :type Actor%20Object%20Reference) (Who%20Did%20the%20Damage :type Actor%20Object%20Reference))
  (bind _returnvalue (Components|GetOwner))
  (bind (_x _y _z) (Class|KismetMathLibrary|BreakVector3f Damage_Location))
  (bind _returnvalue_2 (Actor|GetComponentbyClass _returnvalue "/Game/Weapons/Actor_Components/BPC_Blocking.BPC_Blocking_C"))
  (bind _returnvalue_3 (Actor|GetComponentbyClass Hit_Actor "/Game/Characters/BPC_Floating_Damage.BPC_Floating_Damage_C"))
  (bind _blocking_effectiveness (Variables|/Game/Weapons/Actor_Components/BPC_Blocking.BPC_Blocking_C|GetBlocking_Effectiveness _returnvalue_2))
  (Utilities|IsValid Hit_Actor
    (:Is%20Valid
      (Utilities|IsValid _returnvalue_2
        (:Is%20Valid
          (if (Variables|/Game/Weapons/Actor_Components/BPC_Blocking.BPC_Blocking_C|GetBlocking _returnvalue_2)
            (LocalVariables|SetDamage_After_Blocking_Calc (Math|Conversions|ToFloat(Integer) (Math|Float|Floor (* Damage_To_Take (- 1.0 _blocking_effectiveness)))))
            (if (>= _blocking_effectiveness (- 1.0 (Variables|/Game/Weapons/Actor_Components/BPC_Blocking.BPC_Blocking_C|GetPerfect_Block_Threshold _returnvalue_2)))
              (Utilities|FlowControl|DoOnce false :!label _label
                (:Completed
                  (Default|PerfectBlock (Actor|GetComponentbyClass (Components|GetOwner) "/Game/Weapons/Actor_Components/BPC_Blocking.BPC_Blocking_C"))
                  (LocalVariables|SetDamage_After_Blocking_Calc 0.0)))
              (else
                (Audio|PlaySoundatLocation "/Game/VFX_SFX/Blocking/Block_SC.Block_SC" Damage_Location "0, 0, 0" 1.0 1.0 0.0 0 0 0 0)
                (Utilities|FlowControl|Sequence
                  (:then_0
                    (goto _label Reset))
                  (:then_1
                    _))))
            (else
              (LocalVariables|SetDamage_After_Blocking_Calc Damage_To_Take :!label _label_2))))
        (:Is%20Not%20Valid
          (goto _label_2)))
      (if (<= (Math|Float|SelectFloat (Math|Float|Clamp(Float) (- (Variables|Health|GetHealth) (LocalVariables|GetDamage_After_Blocking_Calc)) (Variables|OSP|GetHealth%20Percentage%20Stopping%20Threshold) (Variables|Health|GetHealth)) (- (Variables|Health|GetHealth) (LocalVariables|GetDamage_After_Blocking_Calc)) (Variables|OSP|GetOSP_Active)) 0.0)
        (if (Variables|Health|GetAlive)
          (Variables|Health|SetHealth 0.0)
          (CallFunction|Death)
          (if (Utilities|DoesObjectImplementInterface (Components|GetOwner) "/Game/Characters/Player/BPI_Player.BPI_Player_C") :!label _label_3
            (Utilities|FlowControl|Sequence
              (:then_0
                (Variables|/Game/UI/WBP_New_Health.WBP_New_Health_C|SetTarget_Health (Variables|UI|GetHealth%20Widget) (Variables|Health|GetHealth))
                (Variables|UI|SetHealth_Bar_Alpha 0.0)
                (bind _damage_is_float (Default|DetermineDamageIsFloat _returnvalue_3 (LocalVariables|GetDamage_After_Blocking_Calc) :!label _label_4))
                (Default|MakeFloatingNumber _returnvalue_3 (Math|Vector|MakeVector (+ _x (Math|Random|RandomFloatinRange -5e+01 5e+01)) (+ _y (Math|Random|RandomFloatinRange -5e+01 5e+01)) (+ _z (Math|Random|RandomFloatinRange -5e+01 5e+01))) (LocalVariables|GetDamage_After_Blocking_Calc) _damage_is_float))
              (:then_1
                (goto _label_4))
              (:then_2
                (Class|LegacyCameraShake|StartLegacyCameraShake (Game|GetPlayerCameraManager 0) "/Game/Health/BPs/BP_Damage_Camera_Shake.BP_Damage_Camera_Shake_C" (+ (Math|Float|Clamp(Float) (/ (LocalVariables|GetDamage_After_Blocking_Calc) 1e+01) 0.1 3.0) (* (- 1.0 (/ (Variables|Health|GetHealth) (Variables|Health|GetMaximum_Health))) 2.0)) "CameraLocal" "0, 0, 0")))
            (else
              (bind _ascharacter (Utilities|Casting|CastToCharacter (Components|GetOwner)))
              (if (Utilities|DoesObjectImplementInterface (Pawn|GetController _ascharacter) "/Game/Characters/Enemies/AI/Controllers/BPI_Enemy_Controller.BPI_Enemy_Controller_C")
                (Utilities|IsValid Who%20Did%20the%20Damage
                  (:Is%20Valid
                    (Class|BPIEnemyController|SetChasingCharacterRef(Message) (Pawn|GetController _ascharacter) Who%20Did%20the%20Damage)
                    (Class|BPIEnemyController|SetCanSenseCharacter(Message) (Pawn|GetController _ascharacter) true)
                    (goto _label_4))
                  (:Is%20Not%20Valid
                    (goto _label_4)))))))
        (else
          (Variables|Health|SetHealth (Math|Float|SelectFloat (Math|Float|Clamp(Float) (- (Variables|Health|GetHealth) (LocalVariables|GetDamage_After_Blocking_Calc)) (Variables|OSP|GetHealth%20Percentage%20Stopping%20Threshold) (Variables|Health|GetHealth)) (- (Variables|Health|GetHealth) (LocalVariables|GetDamage_After_Blocking_Calc)) (Variables|OSP|GetOSP_Active)))
          (goto _label_3))))))

(fn Death
  (bind _returnvalue (Components|GetOwner))
  (bind _returnvalue_2 (Components|GetOwner))
  (bind _returnvalue_3 (Components|GetOwner))
  (bind _returnvalue_4 (Components|GetOwner))
  (bind _maximum_health (Variables|Health|GetMaximum_Health))
  (bind _explosion_death_info (Variables|Death|GetExplosion%20Death%20Info))
  (bind _returnvalue_5 (Actor|GetComponentbyClass _returnvalue_3 "/Game/Weapons/Actor_Components/BPC_Explode.BPC_Explode_C"))
  (bind _returnvalue_6 (Transformation|GetActorLocation _returnvalue))
  (bind _returnvalue_7 (* _maximum_health 5.0))
  (if (not (Utilities|DoesObjectImplementInterface (Components|GetOwner) "/Game/Characters/Player/BPI_Player.BPI_Player_C"))
    (Variables|Health|SetAlive false)
    (Development|PrintString (Utilities|String|Append (Utilities|GetDisplayName (Components|GetOwner)) " death") true true "(R=1.000000,G=0.000000,B=0.097792,A=1.000000)" 1e+02)
    (switch Utilities|FlowControl|Switch|SwitchonEnum_Death_Types (Variables|Death|GetDeath_Type)
      (:NewEnumerator0
        (Game|SpawnActorfromClass "/Game/VFX_SFX/Bloodsplosion/BPs/BP_BloodSplosion.BP_BloodSplosion_C" (Math|Transform|MakeTransform (Transformation|GetActorLocation (Components|GetOwner)) "0, 0, 0" "1.000000,1.000000,1.000000") "AlwaysSpawn" "MultiplyWithRoot" 0 (Math|Integer|Clamp(Integer) (* (Variables|Health|GetMaximum_Health) 2) 0 500) 0)
        (Rendering|SetActorHiddenInGame _returnvalue_4 true)
        (for _array_element (Variables|/Game/Weapons/Actor_Components/BPC_Weaponry.BPC_Weaponry_C|GetWeapons (Actor|GetComponentbyClass _returnvalue_4 "/Game/Weapons/Actor_Components/BPC_Weaponry.BPC_Weaponry_C"))
          (Rendering|SetActorHiddenInGame _array_element true))
        (Camera|PlayWorldCameraShake "/Game/VFX_SFX/Bloodsplosion/BPs/BP_Bloodsplosion_Camera_Shake.BP_Bloodsplosion_Camera_Shake_C" (Transformation|GetActorLocation (Components|GetOwner)) _returnvalue_7 (* _returnvalue_7 5.0))
        (Utilities|Time|SetTimerbyFunctionName 0 "Destroy Owning Character And Associated" 0.5))
      (:NewEnumerator1
        (Utilities|IsValid _returnvalue_5
          (:Is%20Valid
            (Default|Explode _returnvalue_5 _returnvalue_6 (Utilities|Struct|MakeStruct_Explosion_On_Hit (.explosionradius _explosion_death_info) (.knockbackradius _explosion_death_info)) false 0.0 (.explosiondamage _explosion_death_info) false))
          (:Is%20Not%20Valid
            (bind _returnvalue_8 (Game|AddComponentbyClass _returnvalue_3 "/Game/Weapons/Actor_Components/BPC_Explode.BPC_Explode_C"))
            (Default|Explode _returnvalue_8 _returnvalue_6 (Utilities|Struct|MakeStruct_Explosion_On_Hit (.explosionradius _explosion_death_info) (.knockbackradius _explosion_death_info)) false 0.0 (.explosiondamage _explosion_death_info) false)))
        (Rendering|SetActorHiddenInGame _returnvalue_2 true)
        (for _array_element_2 (Variables|/Game/Weapons/Actor_Components/BPC_Weaponry.BPC_Weaponry_C|GetWeapons (Actor|GetComponentbyClass _returnvalue_2 "/Game/Weapons/Actor_Components/BPC_Weaponry.BPC_Weaponry_C"))
          (Rendering|SetActorHiddenInGame _array_element_2 true))
        (Utilities|Time|SetTimerbyFunctionName 0 "Destroy Owning Character And Associated" 0.5)))))

(fn Heal
  (params (Amount_To_Heal :type Float%20%28double-precision%29))
  (Development|PrintString (Utilities|String|Append "ATTEMPTING TO HEAL : " (Utilities|GetDisplayName (Components|GetOwner)) (Utilities|String|ToString(Float) Amount_To_Heal) " HEALTH") true true "(R=1.000000,G=0.000000,B=0.099041,A=1.000000)" 2e+02)
  (bind _output_get (Variables|Health|SetHealth (Math|Float|Clamp(Float) (+ (Variables|Health|GetHealth) Amount_To_Heal) 0.0 (Variables|Health|GetMaximum_Health))))
  (if (Utilities|DoesObjectImplementInterface (Components|GetOwner) "/Game/Characters/Player/BPI_Player.BPI_Player_C")
    (Variables|/Game/UI/WBP_New_Health.WBP_New_Health_C|SetTarget_Health (Variables|UI|GetHealth%20Widget) _output_get)
    (Variables|UI|SetHealth_Bar_Alpha 0.0)))

(fn IncreaseMaxHealth
  (params (Amount_To_Increase_By :type Float%20%28double-precision%29))
  (Variables|Health|SetMaximum_Health (+ (Variables|Health|GetMaximum_Health) Amount_To_Increase_By)))

(fn DecreaseMaxHealth
  (params (Amount_To_Decrease_By :type Float%20%28double-precision%29))
  (Variables|Health|SetMaximum_Health (- (Variables|Health|GetMaximum_Health) Amount_To_Decrease_By)))

(fn DestroyOwningCharacterandAssociated
  (for _array_element (Variables|/Game/Weapons/Actor_Components/BPC_Weaponry.BPC_Weaponry_C|GetWeapons (Actor|GetComponentbyClass (Components|GetOwner) "/Game/Weapons/Actor_Components/BPC_Weaponry.BPC_Weaponry_C"))
    (Actor|DestroyActor _array_element))
  (Actor|DestroyActor (Components|GetOwner)))